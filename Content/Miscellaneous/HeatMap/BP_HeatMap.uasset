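; BP_HeatMap is an actor that records where the player moves by painting heat splats into a runtime render target.
; Every tick it multi-traces from the player down past a position-gathering plane, keeping blocking hits on itself.
; Each hit is converted into plane-local coordinates scaled by resolution, then fed with strength and size to a dynamic heat-splat material instance, which is drawn to the render target.
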(event Custom|DrawToRenderTarget
  (params (Location :type Vector) (Strenght :type Float%20%28double-precision%29) (Size :type Float%20%28double-precision%29))
  (bind _mid_heatsplat (Variables|Default|GetMID_HeatSplat))
  (Rendering|Material|SetScalarParameterValue _mid_heatsplat "Strenght" Strenght :!class /Script/Engine.MaterialInstanceDynamic)
  (Rendering|Material|SetScalarParameterValue _mid_heatsplat "Size" Size :!class /Script/Engine.MaterialInstanceDynamic)
  (Rendering|Material|SetVectorParameterValue _mid_heatsplat "Position" (Math|Conversions|ToLinearColor(Vector) (/ (Math|Transform|TransformLocation (Math|Transform|InvertTransform (Transformation|GetWorldTransform (Variables|Default|GetPositionGatheringPlane))) Location) (Variables|Default|GetResolution))) :!class /Script/Engine.MaterialInstanceDynamic)
  (Rendering|DrawMaterialtoRenderTarget (Variables|Default|GetRenderTargetRuntime) _mid_heatsplat))

(event EventBeginPlay
  (Variables|Default|SetTinykinesis%20Player%20Character (CallFunction|GetTinykinesisPlayerCharacter)))

(event EventTick
  (params (DeltaSeconds :type Float%20%28single-precision%29))
  (bind _tinykinesis_player_character (Variables|Default|GetTinykinesis%20Player%20Character))
  (bind _returnvalue (Transformation|GetActorLocation _tinykinesis_player_character))
  (bind (_x _y) (Math|Vector|BreakVector _returnvalue))
  (Utilities|IsValid _tinykinesis_player_character
    (:Is%20Valid
      (bind _outhits (Class|KismetSystemLibrary|LineTraceMultiforObjects _returnvalue (Math|Vector|MakeVector _x _y (- (.Z (Math|Vector|BreakVector (Transformation|GetWorldLocation (Variables|Default|GetPositionGatheringPlane)))) 1.0)) (Utilities|Array|MakeArray "ObjectTypeQuery1" "ObjectTypeQuery2") false 0 "ForOneFrame" false))
      (for _array_element _outhits
        (if (and (.bBlockingHit (Collision|BreakHitResult _array_element)) (== (.HitActor (Collision|BreakHitResult _array_element)) self))
          (CallFunction|DrawtoRenderTarget (.Location (Collision|BreakHitResult _array_element)) 1.0 0.1))))))

(fn ConstructionScript
  (bind _returnvalue (Rendering|Material|CreateDynamicMaterialInstance "/Game/Miscellaneous/HeatMap/M_HeatSplat.M_HeatSplat" "None" "None" :!class /Script/Engine.KismetMaterialLibrary))
  (Variables|Default|SetMID_HeatSplat _returnvalue))