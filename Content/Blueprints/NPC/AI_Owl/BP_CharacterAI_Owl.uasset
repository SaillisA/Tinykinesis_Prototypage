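; Melee enemy Owl NPC character that works with its AI controller, blackboard and Spriggan anim Blueprint, with a random chance of calcined materials at spawn.
; Tick triggers aggro when the player enters detection range, and melee attacks use a forward sphere trace to hit.
; HealthManager events drive death and damage reactions: damage stops movement, applies knockback through blackboard and anim state, then stuns.
; Head collision overlaps get separate handling until death disables them.
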(event OnComponentBeginOverlap(HeadCollide)
  (params (OverlappedComponent :type Primitive%20Component%20Object%20Reference) (OtherActor :type Actor%20Object%20Reference) (OtherComp :type Primitive%20Component%20Object%20Reference) (OtherBodyIndex :type Integer) (bFromSweep :type Boolean) (SweepResult :type Hit%20Result%20Structure%20%28by%20ref%29))
  ;[1 0.8973 0.3638] Détection du joueur sur la tête
  (CallFunction|HeadCollideFunction OtherActor))

(event Custom|DeathDispatcher
  ;[0.3137 0.06274 0.06667] Death Specificity for NpcMelee
  (Collision|SetCollisionEnabled (Variables|Default|GetHeadCollide) "NoCollision")
  (CallFunction|DeathNpc))

(event Custom|DamageDispatcher
  (bind _as_bp_aic_owl (Variables|Cast|GetAs%20BP%20AIC%20Owl))
  (bind _blackboardcomponent (Variables|/Game/Blueprints/NPC/BP_AIControllerBlank.BP_AIControllerBlank_C|GetBlackboardComponent _as_bp_aic_owl))
  ;[0.3137 0.06274 0.06667] Damage specificity for MeleeMobs : knockback & stuns
  (Variables|Default|SetWasKnockbacked true)
  (AI|Navigation|StopMovement _as_bp_aic_owl)
  (AI|Components|Blackboard|SetValueasBool _blackboardcomponent (Utilities|Name|MakeLiteralName "IsKnockbacked") true)
  (CallFunction|Knockback true (Variables|Default|GetVectorHitInfos) (Variables|Default|GetKnockbackForceHitInfos))
  (CallFunction|SetAnimationStateNEW "NewEnumerator1")
  (Utilities|FlowControl|Delay 2.17)
  (AI|Components|Blackboard|SetValueasBool _blackboardcomponent (Utilities|Name|MakeLiteralName "IsKnockbacked") false)
  (CallFunction|SetAnimationStateNEW "NewEnumerator2")
  (Default|EventStun (Variables|Cast|GetAs%20BP%20AIC%20Owl)))

(event EventEventDeath
  (CallFunction|DeathDispatcher))

(event EventBeginPlayNpc
  (bind _as_bp_aic_owl (Variables|Cast|GetAs%20BP%20AIC%20Owl))
  (bind _as_bp_aic_owl_2 (Variables|Cast|GetAs%20BP%20AIC%20Owl))
  (bind _healthmanager (Variables|/Game/Blueprints/NPC/BP_AIControllerBlank.BP_AIControllerBlank_C|GetHealthManager _as_bp_aic_owl_2))
  ;[0.298 1 0.5765] Begin Play
  (CallFunction|AllCast)
  (CallFunction|ChangeSpeedMetrics 0.0 6e+02 0.0)
  (CallFunction|SetDamageValue 1e+01 "NewEnumerator1")
  (if (Math|Random|RandomBool)
    _
    (else
      (CallFunction|MaterialsChangeCalcined)))
  (Default|BeginPlayAICOwl _as_bp_aic_owl)
  (Actor|Tick|SetActorTickEnabled true)
  (Variables|Default|SetBlackboard%20Component (Variables|/Game/Blueprints/NPC/BP_AIControllerBlank.BP_AIControllerBlank_C|GetBlackboardComponent _as_bp_aic_owl))
  (Variables|/Script/Engine.CharacterMovementComponent|SetMaxWalkSpeed (Variables|Character|GetCharacterMovement) (Variables|Default|GetRunSpeed))
  (Variables|Default|SetDamageMeleeAttack 1e+01)
  (Variables|Default|SetKnockbackNormal "15000.000000,15000.000000,15000.000000")
  (EventDispatchers|BindEventtoDeath _healthmanager (EventDispatchers|CreateEvent :!event Custom|DeathDispatcher))
  (EventDispatchers|BindEventtoDamageEffect _healthmanager (EventDispatchers|CreateEvent :!event Custom|DamageDispatcher)))

(event EventEventDamageEffect
  (CallFunction|DamageDispatcher))

(event EventTick
  (params (DeltaSeconds :type Float%20%28single-precision%29))
  ;[0.7412 1 0.3412] Event Tick
  (if (not (Variables|Default|GetIsAggro))
    (if (<= (Transformation|GetDistanceTo (Game|GetPlayerCharacter 0)) (Variables|Metrics|GetRangeDetection))
      (CallFunction|BecameAggro))))

(fn ConstructionScript)

(fn MeleeAttackRaycast
  (bind _returnvalue (Transformation|GetActorRotation))
  (bind _returnvalue_2 (Transformation|GetActorLocation))
  (bind _lenghtrange (LocalVariables|GetLenghtRange))
  (bind _returnvalue_3 (Math|Vector|GetForwardVector _returnvalue))
  (bind _returnvalue_4 (* _returnvalue_3 _lenghtrange))
  (bind _returnvalue_5 (+ _returnvalue_2 _returnvalue_4))
  (bind _outhit (Collision|SphereTraceForObjects _returnvalue_5 _returnvalue_5 6e+01 (LocalVariables|GetObjectsTypes) false 0 "None"))
  (return (.HitActor (Collision|BreakHitResult _outhit)) (.Location (Collision|BreakHitResult _outhit))))

(fn AllCast
  (bind _asabp_spriggan_owl (Utilities|Casting|CastToABP_Spriggan_Owl (Components|SkeletalMesh|GetAnimInstance (Variables|Character|GetMesh))))
  (Variables|Cast|SetAs%20ABP%20Spriggan%20Owl _asabp_spriggan_owl)
  (bind _asbp_aic_owl (Utilities|Casting|CastToBP_AIC_Owl (Components|GetOwner)))
  (Variables|Cast|SetAs%20BP%20AIC%20Owl _asbp_aic_owl)
  (return))

(fn MaterialsChangeCalcined
  (bind _mesh (Variables|Character|GetMesh))
  (Rendering|Material|SetMaterial (Variables|Default|GetEarring_L) 0 "/Game/Characters/NPC/Melee/Materials/Calcined/M_EnemyMelee_Calcined_Earring_Marisa.M_EnemyMelee_Calcined_Earring_Marisa")
  (Rendering|Material|SetMaterial (Variables|Default|GetEarring_R) 0 "/Game/Characters/NPC/Melee/Materials/Calcined/M_EnemyMelee_Calcined_Earring_Marisa.M_EnemyMelee_Calcined_Earring_Marisa")
  (Rendering|Material|SetMaterial _mesh 0 "/Game/Characters/NPC/Melee/Materials/Calcined/M_EnemyMelee_Calcined_Body_Marisa.M_EnemyMelee_Calcined_Body_Marisa")
  (Rendering|Material|SetMaterial _mesh 1 "/Game/Characters/NPC/Melee/Materials/Calcined/M_EnemyMelee_Calcined_Head_Marisa.M_EnemyMelee_Calcined_Head_Marisa")
  (Rendering|Material|SetMaterial _mesh 2 "/Game/Characters/NPC/Melee/Materials/Calcined/M_EnemyMelee_Calcined_Ears_Marisa.M_EnemyMelee_Calcined_Ears_Marisa")
  (Rendering|Material|SetMaterial _mesh 3 "/Game/Characters/NPC/Melee/Materials/Calcined/M_EnemyMelee_Calcined_Antennas_Marisa.M_EnemyMelee_Calcined_Antennas_Marisa")
  (Rendering|Material|SetMaterial _mesh 4 "/Game/Characters/NPC/Melee/Materials/Calcined/M_EnemyMelee_Calcined_Eyes_Marisa.M_EnemyMelee_Calcined_Eyes_Marisa")
  (return))

(fn MeleeAttack
  (if (Variables|MeleeAttack|GetCanAttackMelee)
    (Variables|MeleeAttack|SetCanAttackMelee false)
    (bind (_actorhit _impactlocation) (CallFunction|MeleeAttackRaycast))
    (CallFunction|HitPlayer _actorhit _impactlocation "NewEnumerator1" (Variables|MeleeAttack|GetKnockbackForceMeleeAttack) (Variables|Default|GetDamageMeleeAttack))
    (CallFunction|HitDynamics _actorhit _impactlocation "NewEnumerator1")
    (Variables|MeleeAttack|SetCanAttackMelee true)
    (return)))

(fn SetAnimationStateNEW
  (params (State :type E_Mob_Animation_State%20Enum :default "NewEnumerator0"))
  (Variables|/Game/Characters/NPC/Owl/Animations/ABP_Spriggan_Owl.ABP_Spriggan_Owl_C|SetState (Variables|Cast|GetAs%20ABP%20Spriggan%20Owl) State)
  (return))