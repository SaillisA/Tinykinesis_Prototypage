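; AI controller for BP_AICharacterBlank NPCs that passes aggro and stun states to the Blackboard.
; SeePlayer filters stimuli for sight of the player, then sets IsAggressive and switches a not-yet-aggro pawn to aggro and run speed.
; GiveAggro sets the same key directly without notifying the pawn.
; EventStun halts movement and flags IsStunned; nothing here clears either key.
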(event Custom|EventStun
  (AI|Navigation|StopMovement)
  (CallFunction|StunFunction))

(event EventBeginPlay)

(event EventTick
  (params (DeltaSeconds :type Float%20%28single-precision%29)))

(fn ConstructionScript)

(fn SeePlayer
  (params (Actor :type Actor%20Object%20Reference) (Stimulus :type AI%20Stimulus%20Structure))
  (bind _asbp_aicharacter_blank (Utilities|Casting|CastToBP_AICharacterBlank (Pawn|GetControlledPawn)))
  (if (not (Variables|/Game/Blueprints/NPC/BP_AICharacterBlank.BP_AICharacterBlank_C|GetIsAggro _asbp_aicharacter_blank))
    (bind _returnvalue (Class|AIPerceptionSystem|GetSenseClassforStimulus Stimulus))
    (if (== _returnvalue "/Script/AIModule.AISense_Sight")
      (if (== Actor (Game|GetPlayerCharacter 0))
        (AI|Components|Blackboard|SetValueasBool (Variables|Default|GetBlackboardComponent) (Utilities|Name|MakeLiteralName "IsAggressive") true)
        (bind _asbp_aicharacter_blank_2 (Utilities|Casting|CastToBP_AICharacterBlank (Pawn|GetControlledPawn)))
        (Default|BecameAggro _asbp_aicharacter_blank_2)
        (Default|SetRunSpeed _asbp_aicharacter_blank_2)
        (return)
        (else
          (return)))
      (else
        (return)))))

(fn StunFunction
  (AI|Components|Blackboard|SetValueasBool (Variables|Default|GetBlackboardComponent) (Utilities|Name|MakeLiteralName "IsStunned") true)
  (return))

(fn GiveAggro
  (AI|Components|Blackboard|SetValueasBool (Variables|Default|GetBlackboardComponent) (Utilities|Name|MakeLiteralName "IsAggressive") true)
  (return))