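; Deer enemy NPC character that aggros when the player comes within detection range and performs an area smash melee attack.
; BeginPlay sets speed, damage and scale, starts its BP_AIC_Deer controller and binds to that HealthManager's death and damage events; the damage handler is empty.
; MeleeAttack spawns a short-lived overlap actor, splitting victims into dead-zone and outer hits for players, mobs and dynamic objects.
; Outer-zone mobs take knockback without damage.
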(event Custom|DeathDispatcher
  ;[0.3137 0.06274 0.06667] Death Specificity for NpcMelee
  (CallFunction|DeathNpc))

(event Custom|DamageDispatcher
  ;[0.3137 0.06274 0.06667] Damage specificity for MeleeMobs : knockback & stuns
)

(event EventEventDeath
  (CallFunction|DeathDispatcher))

(event EventBeginPlayNpc
  (bind _as_bp_aic_deer (Variables|Cast|GetAs%20BP%20AIC%20Deer))
  (bind _as_bp_aic_deer_2 (Variables|Cast|GetAs%20BP%20AIC%20Deer))
  (bind _healthmanager (Variables|/Game/Blueprints/NPC/BP_AIControllerBlank.BP_AIControllerBlank_C|GetHealthManager _as_bp_aic_deer_2))
  ;[0.298 1 0.5765] Begin Play
  (CallFunction|AllCast)
  (CallFunction|ChangeSpeedMetrics 0.0 4e+02 0.0)
  (CallFunction|SetDamageValue 2e+01 "NewEnumerator1")
  (Default|BeginPlayAICDeer _as_bp_aic_deer)
  (Actor|Tick|SetActorTickEnabled true)
  (Variables|Default|SetBlackboard%20Component (Variables|/Game/Blueprints/NPC/BP_AIControllerBlank.BP_AIControllerBlank_C|GetBlackboardComponent _as_bp_aic_deer))
  (Variables|/Script/Engine.CharacterMovementComponent|SetMaxWalkSpeed (Variables|Character|GetCharacterMovement) (Variables|Default|GetRunSpeed))
  (Variables|Default|SetKnockbackNormal "40000.000000,40000.000000,40000.000000")
  (EventDispatchers|BindEventtoDeath _healthmanager (EventDispatchers|CreateEvent :!event Custom|DeathDispatcher))
  (EventDispatchers|BindEventtoDamageEffect _healthmanager (EventDispatchers|CreateEvent :!event Custom|DamageDispatcher))
  (Transformation|SetRelativeScale3D (Variables|Default|GetCapsuleComponent) "2.000000,2.000000,2.000000"))

(event EventEventDamageEffect
  (CallFunction|DamageDispatcher))

(event EventTick
  (params (DeltaSeconds :type Float%20%28single-precision%29))
  ;[0.7412 1 0.3412] Event Tick
  (if (not (Variables|Default|GetIsAggro))
    (if (<= (Transformation|GetDistanceTo (Game|GetPlayerCharacter 0)) (Variables|Metrics|GetRangeDetection))
      (CallFunction|BecameAggro))))

(fn ConstructionScript)

(fn AllCast
  (bind _asabp_spriggan_blank (Utilities|Casting|CastToABP_Spriggan_Blank (Components|SkeletalMesh|GetAnimInstance (Variables|Character|GetMesh))))
  (Variables|Cast|SetAs%20ABP%20Spriggan _asabp_spriggan_blank)
  (bind _asbp_aic_deer (Utilities|Casting|CastToBP_AIC_Deer (Components|GetOwner)))
  (Variables|Cast|SetAs%20BP%20AIC%20Deer _asbp_aic_deer)
  (return))

(fn MaterialsChangeCalcined
  (bind _mesh (Variables|Character|GetMesh))
  (Rendering|Material|SetMaterial (Variables|Default|GetEarring_L) 0 "/Game/Characters/NPC/Melee/Materials/Calcined/M_EnemyMelee_Calcined_Earring_Marisa.M_EnemyMelee_Calcined_Earring_Marisa")
  (Rendering|Material|SetMaterial (Variables|Default|GetEarring_R) 0 "/Game/Characters/NPC/Melee/Materials/Calcined/M_EnemyMelee_Calcined_Earring_Marisa.M_EnemyMelee_Calcined_Earring_Marisa")
  (Rendering|Material|SetMaterial _mesh 0 "/Game/Characters/NPC/Melee/Materials/Calcined/M_EnemyMelee_Calcined_Body_Marisa.M_EnemyMelee_Calcined_Body_Marisa")
  (Rendering|Material|SetMaterial _mesh 1 "/Game/Characters/NPC/Melee/Materials/Calcined/M_EnemyMelee_Calcined_Head_Marisa.M_EnemyMelee_Calcined_Head_Marisa")
  (Rendering|Material|SetMaterial _mesh 2 "/Game/Characters/NPC/Melee/Materials/Calcined/M_EnemyMelee_Calcined_Ears_Marisa.M_EnemyMelee_Calcined_Ears_Marisa")
  (Rendering|Material|SetMaterial _mesh 3 "/Game/Characters/NPC/Melee/Materials/Calcined/M_EnemyMelee_Calcined_Antennas_Marisa.M_EnemyMelee_Calcined_Antennas_Marisa")
  (Rendering|Material|SetMaterial _mesh 4 "/Game/Characters/NPC/Melee/Materials/Calcined/M_EnemyMelee_Calcined_Eyes_Marisa.M_EnemyMelee_Calcined_Eyes_Marisa")
  (return))

(fn MeleeAttack
  (bind _returnvalue (Transformation|GetActorRotation))
  (bind _lenghtrange (LocalVariables|GetLenghtRange))
  (bind _mesh (Variables|Character|GetMesh))
  (bind _returnvalue_2 (Transformation|GetWorldLocation _mesh))
  (bind _returnvalue_3 (Math|Vector|GetForwardVector _returnvalue))
  (bind _returnvalue_4 (* _returnvalue_3 _lenghtrange))
  (bind _returnvalue_5 (+ _returnvalue_2 _returnvalue_4))
  (if (Variables|MeleeAttack|GetCanAttackMelee)
    (Variables|MeleeAttack|SetCanAttackMelee false)
    (Utilities|Array|Clear (LocalVariables|GetActorsHit))
    (Utilities|Array|Clear (LocalVariables|GetVectorHit))
    (bind _returnvalue_6 (Game|SpawnActorfromClass "/Game/Blueprints/NPC/Blueprints_AI/BP_RangeMeleeAttack.BP_RangeMeleeAttack_C" (Math|Transform|MakeTransform _returnvalue_5 "0, 0, 0" "1.000000,1.000000,1.000000") "Undefined" "MultiplyWithRoot" 0 0))
    (LocalVariables|SetActorsHit (Variables|/Game/Blueprints/NPC/Blueprints_AI/BP_RangeMeleeAttack.BP_RangeMeleeAttack_C|GetActorsOverlap _returnvalue_6))
    (LocalVariables|SetVectorHit (Variables|/Game/Blueprints/NPC/Blueprints_AI/BP_RangeMeleeAttack.BP_RangeMeleeAttack_C|GetVectorOverlapLocation _returnvalue_6))
    (LocalVariables|SetDeadZoneActorsHit (Variables|/Game/Blueprints/NPC/Blueprints_AI/BP_RangeMeleeAttack.BP_RangeMeleeAttack_C|GetActorsOverlapDeadZone _returnvalue_6))
    (if (Utilities|Array|ContainsItem (LocalVariables|GetDeadZoneActorsHit) self)
      (Utilities|Array|RemoveItem (LocalVariables|GetDeadZoneActorsHit) self)
      (Utilities|Array|RemoveIndex (LocalVariables|GetActorsHit) (Utilities|Array|FindItem (LocalVariables|GetActorsHit) self) :!label _label)
      (Utilities|Array|RemoveIndex (LocalVariables|GetVectorHit) (Utilities|Array|FindItem (LocalVariables|GetActorsHit) self))
      (elif (Utilities|Array|ContainsItem (LocalVariables|GetActorsHit) self)
        (goto _label)
        (else
          _)))
    (for _array_element (LocalVariables|GetDeadZoneActorsHit)
      (if (Utilities|Array|ContainsItem (LocalVariables|GetActorsHit) _array_element)
        (Utilities|Array|RemoveIndex (LocalVariables|GetActorsHit) (Utilities|Array|FindItem (LocalVariables|GetActorsHit) _array_element))))
    (Niagara|SpawnSystematLocation "/Game/VFX/Mobs/NS_SmashMobDeer.NS_SmashMobDeer" _returnvalue_5)
    (Actor|DestroyActor _returnvalue_6)
    (for (_array_element_2 _array_index) (LocalVariables|GetDeadZoneActorsHit)
      (if (Utilities|IsValid _array_element_2)
        (bind _isplayercollidetrue (CallFunction|HitPlayer _array_element_2 (Utilities|Array|Get(acopy) (LocalVariables|GetVectorHit) _array_index) "NewEnumerator1" (Variables|MeleeAttack|GetKnockbackForceMeleeAttack) (Variables|Default|GetDamageMeleeAttack)))
        (if (not _isplayercollidetrue)
          (bind _iscollidemobtrue (CallFunction|HitOtherMob _array_element_2 "0.500000,0.500000,0.500000" 3e+01))
          (if (not _iscollidemobtrue)
            (CallFunction|HitDynamics _array_element_2 (Utilities|Array|Get(acopy) (LocalVariables|GetVectorHit) _array_index) "NewEnumerator1")))))
    (for (_array_element_3 _array_index_2) (LocalVariables|GetActorsHit)
      (if (Utilities|IsValid _array_element_3)
        (bind _isplayercollidetrue_2 (CallFunction|HitPlayer _array_element_3 (Utilities|Array|Get(acopy) (LocalVariables|GetVectorHit) _array_index_2) "NewEnumerator1" (Variables|MeleeAttack|GetKnockbackForceMeleeAttack) (Variables|Default|GetDamageMeleeAttack)))
        (if (not _isplayercollidetrue_2)
          (bind _iscollidemobtrue_2 (CallFunction|HitOtherMob _array_element_3 "0.500000,0.500000,500.000000" 0.0))
          (if (not _iscollidemobtrue_2)
            (CallFunction|HitDynamics _array_element_3 (Utilities|Array|Get(acopy) (LocalVariables|GetVectorHit) _array_index_2) "NewEnumerator1")))))
    (Variables|MeleeAttack|SetCanAttackMelee true)
    (return)))