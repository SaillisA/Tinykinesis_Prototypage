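; AI controller for the Ram enemy NPC, running BT_Ram on BB_Ram.
; A custom init event randomizes long or short nav filters and seeds the blackboard with player, raycast target, start location and charge time.
; Charge wind-up also reaches ABP_Spriggan, but is rolled separately from the blackboard value, as are the two filter picks.
; Short delays stagger target setup; Tick does nothing.
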(event Custom|BeginPlay_AIC_Ram
  (bind _returnvalue (Math|Random|RandomFloatinRange 0.0 0.5))
  (bind _tinykinesisplayercharacter (CallFunction|GetTinykinesisPlayerCharacter))
  (bind _array (Utilities|Array|MakeArray "/Game/Blueprints/NPC/NavigationPath/QuerySystem/NavQueryFilter_BaseLong.NavQueryFilter_BaseLong_C" "/Game/Blueprints/NPC/NavigationPath/QuerySystem/NavQueryFilter_BaseShort.NavQueryFilter_BaseShort_C"))
  (bind _outitem (Utilities|Array|Random _array))
  (bind _returnvalue_2 (+ 0.8 _returnvalue))
  ;[0.298 1 0.5765] BeginPlay
  (Variables|Default|SetCanRunTick true)
  (bind _asbp_character_ai_ram (Utilities|Casting|CastToBP_CharacterAI_Ram (Pawn|GetControlledPawn)))
  (Variables|Default|SetAs%20BP%20Character%20AI%20Ram _asbp_character_ai_ram)
  (AI|RunBehaviorTree "/Game/Blueprints/NPC/AIRam/BT_Ram.BT_Ram")
  (bind _blackboardcomponent (Class|AIController|UseBlackboard "/Game/Blueprints/NPC/AIRam/BB_Ram.BB_Ram"))
  (bind _output_get (Variables|Default|SetBlackboardComponent _blackboardcomponent))
  (AI|Components|Blackboard|SetValueasObject _output_get (Utilities|Name|MakeLiteralName "PlayerActor") (CallFunction|GetTinykinesisPlayerCharacter))
  (Variables|Default|SetDefaultNavigationFilterClass _outitem)
  (Variables|Default|SetNavFilterClass _outitem)
  (AI|Components|Blackboard|SetValueasFloat (Variables|Default|GetBlackboardComponent) (Utilities|Name|MakeLiteralName "TimeChargeLoad") _returnvalue_2)
  (Variables|Default|SetLoadChargeTime _returnvalue_2)
  (Utilities|FlowControl|Delay 0.2)
  (if (Utilities|IsValid _tinykinesisplayercharacter)
    (AI|Components|Blackboard|SetValueasObject (Variables|Default|GetBlackboardComponent) (Utilities|Name|MakeLiteralName "TargetPointPlayer") (Variables|/Game/Blueprints/ActorComponents/BP_AC_PlayerRaycastFly.BP_AC_PlayerRaycastFly_C|GetTargetPointRaycast (Variables|/Game/Blueprints/Player/BP_TinykinesisPlayerCharacter.BP_TinykinesisPlayerCharacter_C|GetBP_AC_PlayerRaycastFly _tinykinesisplayercharacter)))
    (AI|Components|Blackboard|SetValueasVector (Variables|Default|GetBlackboardComponent) (Utilities|Name|MakeLiteralName "AILocationAtStart") (Transformation|GetActorLocation (Pawn|GetControlledPawn)))
    (bind _asabp_spriggan (Utilities|Casting|CastToABP_Spriggan (Components|SkeletalMesh|GetAnimInstance (Variables|/Script/Engine.Character|GetMesh (Variables|Default|GetAs%20BP%20Character%20AI%20Ram)))))
    (Variables|/Game/Characters/NPC/Melee/Animations/ABP_Spriggan.ABP_Spriggan_C|SetLoadCharge _asabp_spriggan (Variables|Default|GetLoadChargeTime))
    (Utilities|FlowControl|Delay 0.2)
    (AI|Components|Blackboard|SetValueasObject (Variables|Default|GetBlackboardComponent) (Utilities|Name|MakeLiteralName "TargetActor") (CallFunction|GetTinykinesisPlayerCharacter))))

(event EventBeginPlay
  ;[0.298 1 0.5765] BeginPlay
)

(event EventTick
  (params (DeltaSeconds :type Float%20%28single-precision%29))
  ;[1 1 1] EventTick
  (if (Variables|Default|GetCanRunTick)
    _))

(fn ConstructionScript)