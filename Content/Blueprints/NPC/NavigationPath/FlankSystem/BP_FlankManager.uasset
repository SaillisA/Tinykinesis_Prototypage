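; BP_FlankManager hands out flank targets to AI controllers so enemies spread out around the player.
; On BeginPlay it caches the left and right flank child actors attached to the player character.
; Each DistributionTarget call advances a cycling index, setting the controller's TargetFlankActor to the left flank, the right flank, or the player itself in turn.
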(event Custom|DistributionTarget
  (params (AIController :type BP%20AIC%20Npc%20Melee%20Object%20Reference))
  (switch int (Variables|Default|GetIndex)
    (:0
      (Variables|Default|SetIndex (+ 1 (Variables|Default|GetIndex)))
      (CallFunction|SetActor AIController (Variables|Default|GetFlank%20L)))
    (:1
      (Variables|Default|SetIndex (+ 1 (Variables|Default|GetIndex)))
      (CallFunction|SetActor AIController (Variables|Default|GetFlank%20R)))
    (:2
      (Variables|Default|SetIndex 0)
      (CallFunction|SetActor AIController (CallFunction|GetTinykinesisPlayerCharacter)))))

(event EventBeginPlay
  (bind _tinykinesisplayercharacter (CallFunction|GetTinykinesisPlayerCharacter))
  (Variables|Default|SetFlank%20R (Variables|/Script/Engine.ChildActorComponent|GetChildActor (Variables|/Game/Blueprints/Player/BP_TinykinesisPlayerCharacter.BP_TinykinesisPlayerCharacter_C|GetBP_FlankActor_Right _tinykinesisplayercharacter)))
  (Variables|Default|SetFlank%20L (Variables|/Script/Engine.ChildActorComponent|GetChildActor (Variables|/Game/Blueprints/Player/BP_TinykinesisPlayerCharacter.BP_TinykinesisPlayerCharacter_C|GetBP_FlankActor_Left _tinykinesisplayercharacter))))

(fn ConstructionScript)

(fn SetActor
  (params (Controller :type BP%20AIC%20Npc%20Melee%20Object%20Reference) (FlankActor :type Actor%20Object%20Reference))
  (Variables|/Game/Blueprints/NPC/AIMelee/BP_AIC_NpcMelee.BP_AIC_NpcMelee_C|SetTargetFlankActor Controller FlankActor)
  (return))