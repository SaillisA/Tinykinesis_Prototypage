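; BP_FlankManager spreads melee AI controllers across three targets: the player's left flank, right flank and the player character.
; Controllers register through IExist and are removed through ImDead.
; GiveTargetFlank assigns one controller in round-robin order and increments per-target counters, while DistributionTarget reassigns the whole list using the same shared index.
; Both write the controller's TargetFlankActor; removal leaves counters and other assignments untouched.
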(event Custom|DistributionTarget
  (for _array_element (Variables|Default|GetAiMeleeController)
    (switch int (Variables|Default|GetIndex)
      (:0
        (Variables|Default|SetIndex (+ 1 (Variables|Default|GetIndex)))
        (CallFunction|SetActor _array_element (Variables|Default|GetFlank%20L)))
      (:1
        (Variables|Default|SetIndex (+ 1 (Variables|Default|GetIndex)))
        (CallFunction|SetActor _array_element (Variables|Default|GetFlank%20R)))
      (:2
        (Variables|Default|SetIndex 0)
        (CallFunction|SetActor _array_element (CallFunction|GetTinykinesisPlayerCharacter))))))

(event EventBeginPlay
  (bind _tinykinesisplayercharacter (CallFunction|GetTinykinesisPlayerCharacter))
  (Variables|Default|SetFlank%20L (Variables|/Game/Blueprints/Player/BP_TinykinesisPlayerCharacter.BP_TinykinesisPlayerCharacter_C|GetFlankL _tinykinesisplayercharacter))
  (Variables|Default|SetFlank%20R (Variables|/Game/Blueprints/Player/BP_TinykinesisPlayerCharacter.BP_TinykinesisPlayerCharacter_C|GetFlankR _tinykinesisplayercharacter)))

(event EventTick
  (params (DeltaSeconds :type Float%20%28single-precision%29)))

(fn ConstructionScript)

(fn ImDead
  (params (Controller :type BP%20AIC%20Npc%20Melee%20Object%20Reference) (TargetFlank :type Object%20Object%20Reference))
  (bind _returnvalue (Utilities|Array|RemoveItem (Variables|Default|GetAiMeleeController) Controller))
  (Development|PrintString (Utilities|String|ToString(Boolean) _returnvalue))
  (return))

(fn IExist
  (params (Controller :type BP%20AIC%20Npc%20Melee%20Object%20Reference))
  (Utilities|Array|Add (Variables|Default|GetAiMeleeController) Controller))

(fn SetActor
  (params (Controller :type BP%20AIC%20Npc%20Melee%20Object%20Reference) (FlankActor :type Object%20Object%20Reference))
  (Variables|/Game/Blueprints/NPC/AIMelee/BP_AIC_NpcMelee.BP_AIC_NpcMelee_C|SetTargetFlankActor Controller FlankActor)
  (return))

(fn GiveTargetFlank
  (params (ControllerInput :type BP%20AIC%20Npc%20Melee%20Object%20Reference))
  (switch int (Variables|Default|GetIndex)
    (:0
      (Variables|Default|SetIndex (+ 1 (Variables|Default|GetIndex)))
      (CallFunction|SetActor ControllerInput (Variables|Default|GetFlank%20L))
      (Variables|Default|SetNbrFlankL (+ 1 (Variables|Default|GetNbrFlankL))))
    (:1
      (Variables|Default|SetIndex (+ 1 (Variables|Default|GetIndex)))
      (CallFunction|SetActor ControllerInput (Variables|Default|GetFlank%20R))
      (Variables|Default|SetNbrFlankR (+ 1 (Variables|Default|GetNbrFlankR))))
    (:2
      (Variables|Default|SetIndex 0)
      (CallFunction|SetActor ControllerInput (CallFunction|GetTinykinesisPlayerCharacter))
      (Variables|Default|SetNbrFlankPlayer (+ 1 (Variables|Default|GetNbrFlankPlayer)))))
  (return))