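; AI controller for turret NPCs that runs their behavior tree and blackboard.
; Its custom begin-play event caches the controlled turret character and seeds the blackboard with the player target and a zeroed ball spawn vector.
; Tick mirrors the blackboard's reloading flag onto the turret's post-hit damage immunity.
; Perception updates feed SeePlayer, and FunctionReload restarts the brain logic.
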(event OnTargetPerceptionUpdated(AIPerception)
  (params (Actor :type Actor%20Object%20Reference) (Stimulus :type AI%20Stimulus%20Structure))
  (CallFunction|SeePlayer Actor Stimulus))

(event Custom|BeginPlay_AICNpcDistance
  ;[0.298 1 0.5765] BeginPlay
  (Variables|Default|SetCanRunTick true)
  (AI|RunBehaviorTree "/Game/Blueprints/NPC/AI_Turrets/BT_Turrets.BT_Turrets")
  (bind _blackboardcomponent (Class|AIController|UseBlackboard "/Game/Blueprints/NPC/AI_Turrets/BB_Turrets.BB_Turrets"))
  (bind _output_get (Variables|Default|SetBlackboardComponent _blackboardcomponent))
  (bind _asbp_character_ai_turrets (Utilities|Casting|CastToBP_CharacterAI_Turrets (Pawn|GetControlledPawn)))
  (Variables|Default|SetAs%20BP%20Character%20Npc%20Distance _asbp_character_ai_turrets)
  (AI|Components|Blackboard|SetValueasObject _output_get (Utilities|Name|MakeLiteralName "TargetPlayer") (CallFunction|GetTinykinesisPlayerCharacter))
  (AI|Components|Blackboard|SetValueasVector _output_get (Utilities|Name|MakeLiteralName "VectorSpawnBalls") "0, 0, 0"))

(event EventTick
  (params (DeltaSeconds :type Float%20%28single-precision%29))
  (if (Variables|Default|GetCanRunTick)
    (Variables|/Game/Blueprints/NPC/BP_AICharacterBlank.BP_AICharacterBlank_C|SetImmunityAfterDamageHit (Variables|Default|GetAs%20BP%20Character%20Npc%20Distance) (ScalableFloat|GetValueasBool (Variables|Default|GetBlackboardComponent) (Utilities|Name|MakeLiteralName "IsReloading")))))

(fn ConstructionScript)

(fn FunctionReload
  (Class|BrainComponent|RestartLogic (Variables|Default|GetBrainComponent))
  (return))