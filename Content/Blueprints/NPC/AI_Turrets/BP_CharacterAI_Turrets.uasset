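; Turret NPC character that becomes aggro when the player enters detection range and can swivel its cannon to face them.
; At begin play it hooks its AI controller's health manager for death and damage, the latter having a scale-pulse timeline.
; A shield event slides the cannon and mask components between two poses.
; Death stops AI logic, drops cannon and mask as physics objects, swaps the mesh for a fracture actor and increments the player's combo.
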(event Custom|EventShieldSetActive
  (params (IsOn :type Boolean))
  (bind _canon (Variables|Default|GetCanon))
  (bind _mask (Variables|Default|GetMask))
  (bind _mask_2 (Variables|Default|GetMask))
  (bind _canon_2 (Variables|Default|GetCanon))
  (if IsOn
    (Components|MoveComponentTo _canon "-0.500000,-17.000000,106.000000" (.rotation (Transformation|GetRelativeTransform _canon)) false false 0.2 false)
    (Components|MoveComponentTo _mask_2 "-4.000000,42.000000,140.000000" (.rotation (Transformation|GetRelativeTransform _mask_2)) false false 0.2 false)
    (else
      (Components|MoveComponentTo _mask "-4.000000,42.000000,182.000000" (.rotation (Transformation|GetRelativeTransform _mask)) false false 0.2 false)
      (Components|MoveComponentTo _canon_2 "-0.500000,30.000000,106.000000" (.rotation (Transformation|GetRelativeTransform _canon_2)) false false 0.2 false))))

(event Custom|Death_Turrets
  ;[0.3137 0.06274 0.06667] Death Specificity for Npc Distance
  (CallFunction|DeathNpc))

(event Custom|DamageEffect_Turrets
  ;[0.3137 0.06274 0.06667] Damage specificity for Npc Distance
  (bind _curvescale (Timeline|TimelineScaleUpAndDown PlayFromStart)
    (:Update
      (Transformation|SetRelativeScale3D (Variables|Default|GetCapsuleComponent) (Math|Conversions|ToVector(Float) _curvescale)))))

(event EventBeginPlayNpc
  ;[0.298 1 0.5765] BeginPlay
  (bind _asbp_aic_turrets (Utilities|Casting|CastToBP_AIC_Turrets (Components|GetOwner)))
  (Default|BeginPlayAICNpcDistance _asbp_aic_turrets)
  (CallFunction|EventShieldSetActive false)
  (EventDispatchers|BindEventtoDeath (Variables|/Game/Blueprints/NPC/BP_AIControllerBlank.BP_AIControllerBlank_C|GetHealthManager _asbp_aic_turrets) (EventDispatchers|CreateEvent :!event Custom|Death_Turrets))
  (EventDispatchers|BindEventtoDamageEffect (Variables|/Game/Blueprints/NPC/BP_AIControllerBlank.BP_AIControllerBlank_C|GetHealthManager _asbp_aic_turrets) (EventDispatchers|CreateEvent :!event Custom|DamageEffect_Turrets))
  (Variables|/Game/Blueprints/ActorComponents/BP_AC_DestructionElement.BP_AC_DestructionElement_C|SetFracturedElement (Variables|Default|GetBP_AC_DestructionElement) "/Game/Blueprints/Actors/FracturedActors/Mobs/BP_ChildFracture_Turrets.BP_ChildFracture_Turrets_C"))

(event EventTick
  (params (DeltaSeconds :type Float%20%28single-precision%29))
  ;[0.7412 1 0.3412] EventTick
  (if (Variables|Default|GetLookPlayer)
    (CallFunction|RotationLauncherBullets))
  (if (not (Variables|Default|GetIsAggro))
    (if (<= (Transformation|GetDistanceTo (Game|GetPlayerCharacter 0)) (Variables|Default|GetRangeDetection))
      (CallFunction|BecameAggro))))

(event EventEventDeath
  (CallFunction|DeathNpc))

(event EventEventDamageEffect
  (CallFunction|DamageEffectTurrets))

(fn ConstructionScript)

(fn RotationLauncherBullets
  (bind _returnvalue (Game|GetPlayerCharacter 0))
  (bind _returnvalue_2 (Transformation|GetActorLocation))
  (bind _returnvalue_3 (Transformation|GetActorLocation _returnvalue))
  (bind _returnvalue_4 (Math|Rotator|FindLookatRotation _returnvalue_2 _returnvalue_3))
  (Transformation|SetWorldRotation (Variables|Default|GetCanon) (Math|Rotator|MakeRotator (.roll _returnvalue_4) 0.0 (+ (.yaw _returnvalue_4) -9e+01)) false false)
  (return))

(fn DeathNpc
  (Variables|Default|SetIsDead true)
  (Collision|SetCollisionEnabled (Variables|Default|GetCapsuleComponent) "NoCollision")
  (Collision|SetCollisionEnabled (Variables|Default|GetCanon) "PhysicsOnly")
  (Physics|SetSimulatePhysics (Variables|Default|GetMask) true)
  (Class|FMODBlueprintStatics|PlayEventatLocation "/Game/Fmod/Events/Mobs/SprigganDeath.SprigganDeath" (Transformation|GetActorTransform))
  (AI|Logic|StopLogic (Variables|/Script/AIModule.AIController|GetBrainComponent (AI|GetAIController (Components|GetOwner (Variables|Transformation|GetRootComponent)))) "ded")
  (bind _returnvalue (Game|SpawnActorfromClass "/Game/Blueprints/Actors/FracturedActors/Mobs/BP_ChildFracture_Turrets.BP_ChildFracture_Turrets_C" (Math|Transform|MakeTransform (Transformation|GetActorLocation) "0, 0, 0" "1.000000,1.000000,1.000000") "Undefined" "MultiplyWithRoot" 0 0))
  (Components|DestroyComponent (Variables|Character|GetMesh))
  (Default|BeginPlayManual _returnvalue)
  (CallFunction|EventDestroy)
  (Default|DisableinSave (Variables|Default|GetBP_AC_StateGameplayElement))
  (Default|CallOnDeathDispatcher)
  (Default|IncrementComboCount (Variables|/Game/Blueprints/WidgetBlueprints/HUD/WBP_PlayerHUD.WBP_PlayerHUD_C|GetWBP_ComboSystem (Variables|/Game/Blueprints/Player/BP_TinykinesisPlayerController.BP_TinykinesisPlayerController_C|GetWBPPlayerHUD (CallFunction|GetTinykinesisPlayerController))))
  (return))