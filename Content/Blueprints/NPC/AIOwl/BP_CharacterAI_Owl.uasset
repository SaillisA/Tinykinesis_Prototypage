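; Owl enemy NPC character that aggros when the player comes within range and attacks in melee, reusing Spriggan animation.
; On begin play it links to its Owl AI controller, registers with the flank manager and randomly applies calcined materials.
; A forward sphere trace feeds melee damage to the player, telekinesis elements and destructibles.
; Hit helpers also handle charge impacts with self-knockback, but the death and knockback-stun chains here are unwired.
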(event OnComponentBeginOverlap(HeadCollide)
  (params (OverlappedComponent :type Primitive%20Component%20Object%20Reference) (OtherActor :type Actor%20Object%20Reference) (OtherComp :type Primitive%20Component%20Object%20Reference) (OtherBodyIndex :type Integer) (bFromSweep :type Boolean) (SweepResult :type Hit%20Result%20Structure%20%28by%20ref%29))
  ;[1 0.8973 0.3638] Détection du joueur sur la tête
  (CallFunction|HeadCollideFunction OtherActor))

(event Custom|EventMeleeAttack
  ;[1 0.3804 0.2078] MeleeAttack
  (if (Variables|MeleeAttack|GetCanAttackMelee)
    (Variables|MeleeAttack|SetCanAttackMelee false)
    (bind (_actorhit _impactlocation) (CallFunction|MeleeAttackRaycast))
    (FunctionsCollide|HitPlayer _actorhit _impactlocation "NewEnumerator1" (Variables|MeleeAttack|GetKnockbackForceMeleeAttack) (Variables|MeleeAttack|GetDamageMeleeAttack))
    (FunctionsCollide|HitDynamicActors _actorhit _impactlocation "NewEnumerator1")
    (Variables|MeleeAttack|SetCanAttackMelee true)))

(event EventBeginPlayNpc
  (bind _as_bp_aic_owl (Variables|Cast|GetAs%20BP%20AIC%20Owl))
  (bind _as_bp_aic_owl_2 (Variables|Cast|GetAs%20BP%20AIC%20Owl))
  (bind _healthmanager (Variables|/Game/Blueprints/NPC/BP_AIC_Blank.BP_AIC_Blank_C|GetHealthManager _as_bp_aic_owl_2))
  ;[0.298 1 0.5765] Begin Play
  (CallFunction|AllCast)
  (if (Math|Random|RandomBool)
    _
    (else
      (CallFunction|MaterialsChangeCalcined)))
  (Default|BeginPlayAICOwl _as_bp_aic_owl)
  (Actor|Tick|SetActorTickEnabled true)
  (Variables|Default|SetBlackboard%20Component (Variables|/Game/Blueprints/NPC/BP_AIC_Blank.BP_AIC_Blank_C|GetBlackboardComponent _as_bp_aic_owl))
  (Variables|/Script/Engine.CharacterMovementComponent|SetMaxWalkSpeed (Variables|Character|GetCharacterMovement) (Variables|Default|GetRunSpeed))
  (EventDispatchers|BindEventtoDeath _healthmanager (EventDispatchers|CreateEvent :!event DamageEffectDispatcher))
  (EventDispatchers|BindEventtoDamageEffect _healthmanager (EventDispatchers|CreateEvent :!event DamageEffectDispatcher))
  (bind _returnvalue (Actor|GetActorOfClass "/Game/Blueprints/NPC/NavigationPath/FlankSystem/BP_FlankManager.BP_FlankManager_C"))
  (bind _output_get (Variables|Cast|SetFlankManager _returnvalue))
  (Default|DistributionTarget _output_get (Variables|Cast|GetAs%20BP%20AIC%20Owl)))

(event EventTick
  (params (DeltaSeconds :type Float%20%28single-precision%29))
  ;[0.7412 1 0.3412] Event Tick
  (if (not (Variables|Default|GetIsAggro))
    (if (<= (Transformation|GetDistanceTo (Game|GetPlayerCharacter 0)) (Variables|Metrics|GetRangeDetection))
      (CallFunction|BecameAggro))))

(fn ConstructionScript)

(fn HitPlayer
  (params (Actor%20hit :type Actor%20Object%20Reference) (ImpactHit :type Vector) (TypeAttack :type E_MobAttackType%20Enum :default "EAttackType_MAX") (KnockbackForce :type Vector) (Dammage :type Float%20%28double-precision%29))
  (bind _tinykinesisplayercharacter (CallFunction|GetTinykinesisPlayerCharacter))
  (if (== Actor%20hit _tinykinesisplayercharacter)
    (switch Utilities|FlowControl|Switch|SwitchonE_MobAttackType TypeAttack
      (:NewEnumerator0
        (LocalVariables|SetImpactLocationHit ImpactHit))
      (:NewEnumerator1
        (LocalVariables|SetImpactLocationHit (Transformation|GetActorLocation))))
    (Default|EventGetHit _tinykinesisplayercharacter (LocalVariables|GetImpactLocationHit) KnockbackForce Dammage)
    (switch Utilities|FlowControl|Switch|SwitchonE_MobAttackType TypeAttack
      (:NewEnumerator0
        ;[1 1 1] Knockback & Stun on self if charge
        (Variables|Default|SetVectorHit (Transformation|GetActorLocation (CallFunction|GetTinykinesisPlayerCharacter)))
        (CallFunction|DamageEffectDispatcher))
      (:NewEnumerator1
        _))
    (return true)
    (else
      (return false))))

(fn HitOtherNpc
  (params (ActorHit :type Actor%20Object%20Reference))
  (bind _asbp_character_npc_melee (Utilities|Casting|CastToBP_CharacterNpcMelee ActorHit)
    (:then
      ;[1 1 1] Knockback + stun on self
      (Variables|Default|SetVectorHit (Transformation|GetActorLocation _asbp_character_npc_melee))
      (CallFunction|DamageEffectDispatcher)
      ;[1 1 1] Stun on other npc
      (bind _asbp_aic_npc_melee (Utilities|Casting|CastToBP_AIC_NpcMelee (Components|GetOwner _asbp_character_npc_melee)))
      (Default|EventStun _asbp_aic_npc_melee)
      (return true))
    (:CastFailed
      (return false))))

(fn HitEnvironment
  (params (ActorHit :type Actor%20Object%20Reference) (LocationHit :type Vector))
  (if (not (Actor|ActorHasTag ActorHit "Ground"))
    (Variables|Default|SetVector%20Hit LocationHit)
    (CallFunction|DamageEffectDispatcher)))

(fn HitDynamicActors
  (params (ActorHit :type Actor%20Object%20Reference) (VectorHit :type Vector) (TypeAttack :type E_MobAttackType%20Enum :default "NewEnumerator0"))
  (Variables|Default|SetVectorHit VectorHit)
  (if (Utilities|DoesObjectImplementInterface ActorHit "/Game/Blueprints/Interfaces/BPI_TelekinesisObject.BPI_TelekinesisObject_C")
    (Utilities|Casting|CastToBP_AbstractPickUpObject ActorHit
      (:then
        (return false))
      (:CastFailed
        (bind _asbp_abstract_telekinesis_element (Utilities|Casting|CastToBP_AbstractTelekinesisElement ActorHit)
          (:then
            (if (not (or (Variables|/Game/Blueprints/Actors/TelekinesisElements/BP_AbstractTelekinesisElement.BP_AbstractTelekinesisElement_C|GetIsBeingReleased _asbp_abstract_telekinesis_element) (Variables|/Game/Blueprints/Actors/TelekinesisElements/BP_AbstractTelekinesisElement.BP_AbstractTelekinesisElement_C|GetIsBeingGrabbed _asbp_abstract_telekinesis_element)))
              (switch Utilities|FlowControl|Switch|SwitchonE_MobAttackType TypeAttack
                (:NewEnumerator0
                  (Default|LooseHP (Variables|/Game/Blueprints/Actors/TelekinesisElements/BP_AbstractTelekinesisElement.BP_AbstractTelekinesisElement_C|GetBP_AC_Health _asbp_abstract_telekinesis_element) (Variables|ChargeAttack|GetDamageChargeAttack)))
                (:NewEnumerator1
                  (Default|LooseHP (Variables|/Game/Blueprints/Actors/TelekinesisElements/BP_AbstractTelekinesisElement.BP_AbstractTelekinesisElement_C|GetBP_AC_Health _asbp_abstract_telekinesis_element) (Variables|MeleeAttack|GetDamageMeleeAttack))))
              (switch Utilities|FlowControl|Switch|SwitchonE_MobAttackType TypeAttack :!label _label
                (:NewEnumerator0
                  (CallFunction|DamageEffectDispatcher)
                  (return true)))))
          (:CastFailed
            (return false)))))
    (else
      (bind _asbp_destructible_object (Utilities|Casting|CastToBP_DestructibleObject ActorHit)
        (:then
          (switch Utilities|FlowControl|Switch|SwitchonE_MobAttackType TypeAttack
            (:NewEnumerator0
              (Default|LooseHP (Variables|/Game/Blueprints/Actors/Traps/DestructibleObject/BP_DestructibleObject.BP_DestructibleObject_C|GetBP_AC_Health _asbp_destructible_object) (Variables|ChargeAttack|GetDamageChargeAttack))
              (goto _label))
            (:NewEnumerator1
              (Default|LooseHP (Variables|/Game/Blueprints/Actors/Traps/DestructibleObject/BP_DestructibleObject.BP_DestructibleObject_C|GetBP_AC_Health _asbp_destructible_object) (Variables|MeleeAttack|GetDamageMeleeAttack))
              (goto _label))))
        (:CastFailed
          (return false))))))

(fn MeleeAttackRaycast
  (bind _returnvalue (Transformation|GetActorRotation))
  (bind _returnvalue_2 (Transformation|GetActorLocation))
  (bind _lenghtrange (LocalVariables|GetLenghtRange))
  (bind _returnvalue_3 (Math|Vector|GetForwardVector _returnvalue))
  (bind _returnvalue_4 (* _returnvalue_3 _lenghtrange))
  (bind _returnvalue_5 (+ _returnvalue_2 _returnvalue_4))
  (bind _outhit (Collision|SphereTraceForObjects _returnvalue_5 _returnvalue_5 6e+01 (LocalVariables|GetObjectsTypes) false 0 "None"))
  (return (.HitActor (Collision|BreakHitResult _outhit)) (.Location (Collision|BreakHitResult _outhit))))

(fn GetImpulseVector0
  (params (VectorImpact :type Vector) (ForceKnockbackHit :type Vector))
  (bind _returnvalue (Transformation|GetActorLocation))
  (bind _returnvalue_2 (- _returnvalue VectorImpact))
  (bind _returnvalue_3 (Math|Vector|Normalize _returnvalue_2))
  (bind _returnvalue_4 (* _returnvalue_3 (.x ForceKnockbackHit)))
  (return (Math|Vector|MakeVector (.x _returnvalue_4) (.y _returnvalue_4) (.z ForceKnockbackHit))))

(fn SetStateAnimation
  (params (InputState :type E_MobStateMelee%20Enum :default "NewEnumerator0"))
  (Variables|/Game/Characters/NPC/Melee/Animations/ABP_Spriggan.ABP_Spriggan_C|SetStateVariable (Variables|Cast|GetAs%20ABP%20Spriggan) InputState)
  (return))

(fn AllCast
  (bind _asabp_spriggan (Utilities|Casting|CastToABP_Spriggan (Components|SkeletalMesh|GetAnimInstance (Variables|Character|GetMesh))))
  (Variables|Cast|SetAs%20ABP%20Spriggan _asabp_spriggan)
  (bind _asbp_aic_owl (Utilities|Casting|CastToBP_AIC_Owl (Components|GetOwner)))
  (Variables|Cast|SetAs%20BP%20AIC%20Owl _asbp_aic_owl)
  (return))

(fn MaterialsChangeCalcined
  (bind _mesh (Variables|Character|GetMesh))
  (Rendering|Material|SetMaterial (Variables|Default|GetEarring_L) 0 "/Game/Characters/NPC/Melee/Materials/Calcined/M_EnemyMelee_Calcined_Earring_Marisa.M_EnemyMelee_Calcined_Earring_Marisa")
  (Rendering|Material|SetMaterial (Variables|Default|GetEarring_R) 0 "/Game/Characters/NPC/Melee/Materials/Calcined/M_EnemyMelee_Calcined_Earring_Marisa.M_EnemyMelee_Calcined_Earring_Marisa")
  (Rendering|Material|SetMaterial _mesh 0 "/Game/Characters/NPC/Melee/Materials/Calcined/M_EnemyMelee_Calcined_Body_Marisa.M_EnemyMelee_Calcined_Body_Marisa")
  (Rendering|Material|SetMaterial _mesh 1 "/Game/Characters/NPC/Melee/Materials/Calcined/M_EnemyMelee_Calcined_Head_Marisa.M_EnemyMelee_Calcined_Head_Marisa")
  (Rendering|Material|SetMaterial _mesh 2 "/Game/Characters/NPC/Melee/Materials/Calcined/M_EnemyMelee_Calcined_Ears_Marisa.M_EnemyMelee_Calcined_Ears_Marisa")
  (Rendering|Material|SetMaterial _mesh 3 "/Game/Characters/NPC/Melee/Materials/Calcined/M_EnemyMelee_Calcined_Antennas_Marisa.M_EnemyMelee_Calcined_Antennas_Marisa")
  (Rendering|Material|SetMaterial _mesh 4 "/Game/Characters/NPC/Melee/Materials/Calcined/M_EnemyMelee_Calcined_Eyes_Marisa.M_EnemyMelee_Calcined_Eyes_Marisa")
  (return))