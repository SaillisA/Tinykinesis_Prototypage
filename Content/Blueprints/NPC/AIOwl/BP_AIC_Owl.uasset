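; AI controller for the Owl NPC that runs BT_Owl and drives its melee attack decisions against the player.
; A custom init event seeds the blackboard with player, target point and start location, randomizes navigation filters and melee windup, and passes the windup to the Spriggan anim Blueprint.
; Tick compares horizontal distance to TargetActor to update the InRangeAttackMelee key.
; Perception updates are forwarded to SeePlayer.
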(event OnTargetPerceptionUpdated(AIPerception)
  (params (Actor :type Actor%20Object%20Reference) (Stimulus :type AI%20Stimulus%20Structure))
  (CallFunction|SeePlayer Actor Stimulus))

(event Custom|Event%20Melee%20Attack
  (params (BoolValue :type Boolean))
  ;[1 1 1] Event pour appeler le melee attack
  (CallFunction|MeleeAttackFunction BoolValue))

(event Custom|BeginPlay_AIC_Owl
  (bind _returnvalue (Math|Random|RandomFloatinRange 0.0 0.3))
  (bind _array (Utilities|Array|MakeArray "/Game/Blueprints/NPC/NavigationPath/QuerySystem/NavQueryFilter_BaseLong.NavQueryFilter_BaseLong_C" "/Game/Blueprints/NPC/NavigationPath/QuerySystem/NavQueryFilter_BaseShort.NavQueryFilter_BaseShort_C"))
  (bind _outitem (Utilities|Array|Random _array))
  (bind _returnvalue_2 (+ 0.4 _returnvalue))
  ;[0.298 1 0.5765] BeginPlay
  (Variables|Default|SetCanRunTick true)
  (bind _asbp_character_ai_owl (Utilities|Casting|CastToBP_CharacterAI_Owl (Pawn|GetControlledPawn)))
  (Variables|Default|SetAs%20BP%20Character%20AI%20Owl _asbp_character_ai_owl)
  (AI|RunBehaviorTree "/Game/Blueprints/NPC/AIOwl/BT_Owl.BT_Owl")
  (bind _blackboardcomponent (Class|AIController|UseBlackboard "/Game/Blueprints/NPC/AIOwl/BB_Owl.BB_Owl"))
  (bind _output_get (Variables|Default|SetBlackboardComponent _blackboardcomponent))
  (AI|Components|Blackboard|SetValueasObject _output_get (Utilities|Name|MakeLiteralName "PlayerActor") (CallFunction|GetTinykinesisPlayerCharacter))
  (Variables|Default|SetDefaultNavigationFilterClass _outitem)
  (Variables|Default|SetNavFilterClass _outitem)
  (AI|Components|Blackboard|SetValueasFloat (Variables|Default|GetBlackboardComponent) (Utilities|Name|MakeLiteralName "TimeMeleeLoad") _returnvalue_2)
  (Variables|Float|SetLoadMeleeAttackTime _returnvalue_2)
  (Utilities|FlowControl|Delay 0.2)
  (bind _asbp_tinykinesis_player_character (Utilities|Casting|CastToBP_TinykinesisPlayerCharacter (Game|GetPlayerCharacter 0)))
  (if (Utilities|IsValid (Variables|/Game/Blueprints/ActorComponents/BP_AC_PlayerRaycastFly.BP_AC_PlayerRaycastFly_C|GetTargetPointRaycast (Variables|/Game/Blueprints/Player/BP_TinykinesisPlayerCharacter.BP_TinykinesisPlayerCharacter_C|GetBP_AC_PlayerRaycastFly _asbp_tinykinesis_player_character)))
    (AI|Components|Blackboard|SetValueasObject (Variables|Default|GetBlackboardComponent) (Utilities|Name|MakeLiteralName "TargetPointPlayer") (Variables|/Game/Blueprints/ActorComponents/BP_AC_PlayerRaycastFly.BP_AC_PlayerRaycastFly_C|GetTargetPointRaycast (Variables|/Game/Blueprints/Player/BP_TinykinesisPlayerCharacter.BP_TinykinesisPlayerCharacter_C|GetBP_AC_PlayerRaycastFly _asbp_tinykinesis_player_character)))
    (AI|Components|Blackboard|SetValueasVector (Variables|Default|GetBlackboardComponent) (Utilities|Name|MakeLiteralName "AILocationAtStart") (Transformation|GetActorLocation (Pawn|GetControlledPawn)))
    (bind _asabp_spriggan (Utilities|Casting|CastToABP_Spriggan (Components|SkeletalMesh|GetAnimInstance (Variables|/Script/Engine.Character|GetMesh (Variables|Default|GetAs%20BP%20Character%20AI%20Owl)))))
    (Variables|/Game/Characters/NPC/Melee/Animations/ABP_Spriggan.ABP_Spriggan_C|SetLoadMeleeAttack _asabp_spriggan (Variables|Float|GetLoadMeleeAttackTime))
    (Utilities|FlowControl|Delay 0.2)
    (AI|Components|Blackboard|SetValueasObject (Variables|Default|GetBlackboardComponent) (Utilities|Name|MakeLiteralName "TargetActor") (CallFunction|GetTinykinesisPlayerCharacter))))

(event EventBeginPlay
  ;[0.298 1 0.5765] BeginPlay
)

(event EventTick
  (params (DeltaSeconds :type Float%20%28single-precision%29))
  ;[1 1 1] EventTick
  (if (Variables|Default|GetCanRunTick)
    (bind _asactor (Utilities|Casting|CastToActor (AI|Components|Blackboard|GetValueasObject (Variables|Default|GetBlackboardComponent) (Utilities|Name|MakeLiteralName "TargetActor"))))
    (if (<= (Transformation|GetHorizontalDistanceTo (Pawn|GetControlledPawn) _asactor) (Variables|Float|GetRangeAttackMelee))
      (CallFunction|EventMeleeAttack true)
      (else
        (CallFunction|EventMeleeAttack false)))))

(fn ConstructionScript)

(fn MeleeAttackFunction
  (params (BoolValue :type Boolean))
  (AI|Components|Blackboard|SetValueasBool (Variables|Default|GetBlackboardComponent) (Utilities|Name|MakeLiteralName "InRangeAttackMelee") BoolValue)
  (return))