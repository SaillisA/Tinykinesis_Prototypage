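; Bee enemy NPC character that aggroes when the player comes within detection range.
; On begin play it sets speeds and damage, caches its AI controller and anim blueprint, and binds the controller's HealthManager death and damage events.
; Damage triggers knockback, a blackboard flag, animation changes and a delayed stun; death disables head collision.
; It also handles head overlaps and defines a gravity-free, impulse-driven projectile throw toward the player.
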(event OnComponentBeginOverlap(HeadCollide)
  (params (OverlappedComponent :type Primitive%20Component%20Object%20Reference) (OtherActor :type Actor%20Object%20Reference) (OtherComp :type Primitive%20Component%20Object%20Reference) (OtherBodyIndex :type Integer) (bFromSweep :type Boolean) (SweepResult :type Hit%20Result%20Structure%20%28by%20ref%29))
  ;[1 0.8973 0.3638] Détection du joueur sur la tête
  (CallFunction|HeadCollideFunction OtherActor))

(event Custom|DeathDispatcher
  ;[0.3137 0.06274 0.06667] Death Specificity for NpcMelee
  (Collision|SetCollisionEnabled (Variables|Default|GetHeadCollide) "NoCollision")
  (CallFunction|DeathNpc))

(event Custom|DamageDispatcher
  (bind _as_bp_aic_bee (Variables|Cast|GetAs%20BP%20AIC%20Bee))
  (bind _blackboardcomponent (Variables|/Game/Blueprints/NPC/BP_AIControllerBlank.BP_AIControllerBlank_C|GetBlackboardComponent _as_bp_aic_bee))
  ;[0.3137 0.06274 0.06667] Damage specificity for MeleeMobs : knockback & stuns
  (Variables|Default|SetWasKnockbacked true)
  (AI|Navigation|StopMovement _as_bp_aic_bee)
  (AI|Components|Blackboard|SetValueasBool _blackboardcomponent (Utilities|Name|MakeLiteralName "IsKnockbacked") true)
  (CallFunction|Knockback true (Variables|Default|GetVectorHitInfos) (Variables|Default|GetKnockbackForceHitInfos))
  (CallFunction|SetAnimationStateNEW "NewEnumerator1")
  (Utilities|FlowControl|Delay 2.17)
  (AI|Components|Blackboard|SetValueasBool _blackboardcomponent (Utilities|Name|MakeLiteralName "IsKnockbacked") false)
  (CallFunction|SetAnimationStateNEW "NewEnumerator2")
  (Default|EventStun (Variables|Cast|GetAs%20BP%20AIC%20Bee)))

(event EventEventDeath
  (CallFunction|DeathDispatcher))

(event EventBeginPlayNpc
  (bind _as_bp_aic_bee (Variables|Cast|GetAs%20BP%20AIC%20Bee))
  (bind _as_bp_aic_bee_2 (Variables|Cast|GetAs%20BP%20AIC%20Bee))
  (bind _healthmanager (Variables|/Game/Blueprints/NPC/BP_AIControllerBlank.BP_AIControllerBlank_C|GetHealthManager _as_bp_aic_bee_2))
  ;[0.298 1 0.5765] Begin Play
  (CallFunction|AllCast)
  (CallFunction|ChangeSpeedMetrics 2.5e+02 5e+02 1.2e+03)
  (CallFunction|SetDamageValue 1e+01 "NewEnumerator1")
  (Default|BeginPlayAICBee _as_bp_aic_bee)
  (Actor|Tick|SetActorTickEnabled true)
  (Variables|Default|SetBlackboard%20Component (Variables|/Game/Blueprints/NPC/BP_AIControllerBlank.BP_AIControllerBlank_C|GetBlackboardComponent _as_bp_aic_bee))
  (Variables|/Script/Engine.CharacterMovementComponent|SetMaxWalkSpeed (Variables|Character|GetCharacterMovement) (Variables|Default|GetRunSpeed))
  (Variables|Default|SetDamageMeleeAttack 1e+01)
  (Variables|Default|SetKnockbackNormal "15000.000000,15000.000000,15000.000000")
  (EventDispatchers|BindEventtoDeath _healthmanager (EventDispatchers|CreateEvent :!event Custom|DeathDispatcher))
  (EventDispatchers|BindEventtoDamageEffect _healthmanager (EventDispatchers|CreateEvent :!event Custom|DamageDispatcher)))

(event EventEventDamageEffect
  (CallFunction|DamageDispatcher))

(event EventTick
  (params (DeltaSeconds :type Float%20%28single-precision%29))
  ;[0.7412 1 0.3412] Event Tick
  (if (not (Variables|Default|GetIsAggro))
    (if (<= (Transformation|GetDistanceTo (Game|GetPlayerCharacter 0)) (Variables|Metrics|GetRangeDetection))
      (CallFunction|BecameAggro))))

(fn ConstructionScript)

(fn AllCast
  (bind _asabp_spriggan_bee (Utilities|Casting|CastToABP_Spriggan_Bee (Components|SkeletalMesh|GetAnimInstance (Variables|Character|GetMesh))))
  (Variables|Cast|SetAs%20ABP%20Spriggan%20Bee _asabp_spriggan_bee)
  (bind _asbp_aic_bee (Utilities|Casting|CastToBP_AIC_Bee (Components|GetOwner)))
  (Variables|Cast|SetAs%20BP%20AIC%20Bee _asbp_aic_bee)
  (return))

(fn ThrowBullet
  (params (ThrowPower :type Float%20%28double-precision%29))
  (bind _returnvalue (Game|SpawnActorfromClass "/Game/Blueprints/Actors/TelekinesisElements/AttractiveObject_Children/TinyObject_Children/BP_BulletsAIDistance.BP_BulletsAIDistance_C" (Math|Transform|MakeTransform (Transformation|GetWorldLocation (Variables|Default|GetSpawnBullets)) "0, 0, 0" "1.000000,1.000000,1.000000") "Undefined" "MultiplyWithRoot" 0 0))
  (Variables|/Game/Blueprints/Actors/TelekinesisElements/BP_AbstractTelekinesisElement.BP_AbstractTelekinesisElement_C|SetCurrentForceKnockback _returnvalue "500.000000,500.000000,500.000000")
  (Physics|SetSimulatePhysics (Variables|/Game/Blueprints/Actors/TelekinesisElements/BP_AbstractTelekinesisElement.BP_AbstractTelekinesisElement_C|GetMesh _returnvalue) true)
  (Physics|AddImpulse (Variables|/Game/Blueprints/Actors/TelekinesisElements/BP_AbstractTelekinesisElement.BP_AbstractTelekinesisElement_C|GetMesh _returnvalue) (* (Math|Vector|Normalize (- (Transformation|GetActorLocation (Game|GetPlayerCharacter 0)) (Transformation|GetActorLocation _returnvalue))) ThrowPower) "None" false)
  (Physics|SetEnableGravity (Variables|/Game/Blueprints/Actors/TelekinesisElements/BP_AbstractTelekinesisElement.BP_AbstractTelekinesisElement_C|GetMesh _returnvalue) false)
  (return))

(fn SetAnimationStateNEW
  (params (State :type E_Mob_Animation_State%20Enum :default "NewEnumerator0"))
  (Development|PrintString (Utilities|String|EnumtoString State))
  (Variables|/Game/Characters/NPC/Bee/Animations/ABP_Spriggan_Bee.ABP_Spriggan_Bee_C|SetState (Variables|Cast|GetAs%20ABP%20Spriggan%20Bee) State)
  (return))