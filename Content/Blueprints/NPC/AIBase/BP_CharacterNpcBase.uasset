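; Base NPC character Blueprint with walk and sprint speeds, player contact checks and targeting-system outline highlighting.
; A player overlap on the head collider triggers a stun on the owning AI controller, launches the player upward and briefly disables player killing.
; Capsule hits on the player currently only print a death message.
; GetHit ragdolls the mesh with an impulse, stops AI logic and destroys the actor after a delay.
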(event OnComponentHit(CapsuleComponent)
  (params (HitComponent :type Primitive%20Component%20Object%20Reference) (OtherActor :type Actor%20Object%20Reference) (OtherComp :type Primitive%20Component%20Object%20Reference) (NormalImpulse :type Vector :default "0, 0, 0") (Hit :type Hit%20Result%20Structure%20%28by%20ref%29))
  (CallFunction|HitPlayer OtherActor))

(event OnComponentBeginOverlap(HeadCollide)
  (params (OverlappedComponent :type Primitive%20Component%20Object%20Reference) (OtherActor :type Actor%20Object%20Reference) (OtherComp :type Primitive%20Component%20Object%20Reference) (OtherBodyIndex :type Integer) (bFromSweep :type Boolean) (SweepResult :type Hit%20Result%20Structure%20%28by%20ref%29))
  (bind _asbp_first_person_character (Utilities|Casting|CastToBP_FirstPersonCharacter OtherActor))
  (Development|PrintString "AIE MA TETE")
  (bind _asaic_npc_base (Utilities|Casting|CastToAIC_NpcBase (Components|GetOwner))
    (:then
      (Default|EventStun _asaic_npc_base)
      (Variables|Default|SetCanKillPlayer false)
      (Character|LaunchCharacter _asbp_first_person_character (Math|Vector|MakeVector (.x (Math|Vector|GetForwardVector (Variables|/Script/Engine.Actor|GetRootComponent _asbp_first_person_character))) (.y (Math|Vector|GetForwardVector (Variables|/Script/Engine.Actor|GetRootComponent _asbp_first_person_character))) 8e+02) false false)
      (Utilities|FlowControl|Delay 2.0)
      (Variables|Default|SetCanKillPlayer true))
    (:CastFailed
      (Development|PrintString "Probleme de cast vers call"))))

(event Custom|Despawn
  (Utilities|FlowControl|Delay 1e+01)
  (Development|PrintString "Je disparut")
  (Actor|DestroyActor))

(event EventBeginPlay
  (Variables|/Script/Engine.CharacterMovementComponent|SetMaxWalkSpeed (Variables|Character|GetCharacterMovement) (Variables|Default|GetWalkSpeed)))

(event EventDeleteOutline
  (params (IsTargeted :type Boolean))
  ;[1 1 1] Intégration dans le système de ciblage
  (Rendering|Material|SetOverlayMaterial (Variables|Character|GetMesh) 0 :!class /Script/Engine.MeshComponent))

(event EventDetectTarget
  (params (TargetLocation :type Vector :default "0, 0, 0") (IsTargeted :type Boolean))
  ;[1 1 1] Intégration dans le système de ciblage
  (CallFunction|GiveTargetLocation (Transformation|GetWorldLocation (Variables|Character|GetMesh)))
  (Rendering|Material|SetOverlayMaterial (Variables|Character|GetMesh) "/Game/Materials/M_OutlineTarget.M_OutlineTarget" :!class /Script/Engine.MeshComponent))

(fn ConstructionScript)

(fn Sprint
  (Variables|/Script/Engine.CharacterMovementComponent|SetMaxWalkSpeed (Variables|Character|GetCharacterMovement) (Variables|Default|GetSprintSpeed))
  (return))

(fn Walk
  (Variables|/Script/Engine.CharacterMovementComponent|SetMaxWalkSpeed (Variables|Character|GetCharacterMovement) (Variables|Default|GetWalkSpeed))
  (return))

(fn HitPlayer
  (params (Actor%20hit :type Actor%20Object%20Reference))
  (if (Variables|Default|GetCanKillPlayer)
    (Variables|Default|SetCanKillPlayer false)
    (Utilities|Casting|CastToBP_FirstPersonCharacter Actor%20hit)
    (Development|PrintString "TU ES DEAAAAAAAAAD")
    (Variables|Default|SetCanKillPlayer true)
    (return)))

(fn GetHit
  (params (NPC :type Actor%20Object%20Reference) (ResultHit :type Hit%20Result%20Structure) (VectorObject :type Vector))
  (Collision|SetCollisionEnabled (Variables|Collision|GetCapsuleComponent) "NoCollision")
  (Collision|SetCollisionEnabled (Variables|Default|GetHeadCollide) "NoCollision")
  (Physics|SetSimulatePhysics (Variables|Character|GetMesh) true)
  (Physics|AddImpulse (Variables|Character|GetMesh) (* VectorObject 5e+02) "None" true)
  (AI|Logic|StopLogic (Variables|/Script/AIModule.AIController|GetBrainComponent (AI|GetAIController (Components|GetOwner (Variables|/Script/Engine.Actor|GetRootComponent NPC)))) "ded")
  (CallFunction|Despawn)
  (return))

(fn GiveTargetLocation
  (params (TargetLocationInput :type Vector :default "0, 0, 0"))
  (return (Transformation|GetWorldLocation (Variables|Character|GetMesh))))