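; Base AI controller for NPCs that runs the base behavior tree and feeds its blackboard with the player as target.
; On start it randomly picks a short- or long-path navigation filter and stores the player's raycast target point.
; Each tick it updates player location and melee-range state.
; Sight of the player by a non-aggro NPC triggers aggression, while stun stops movement, shows the effect and sets a blackboard flag.
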(event OnTargetPerceptionUpdated(AIPerception)
  (params (Actor :type Actor%20Object%20Reference) (Stimulus :type AI%20Stimulus%20Structure))
  (CallFunction|SeePlayer Actor Stimulus))

(event Custom|Event%20Stun
  ;[1 1 1] Event pour appeler le stun
  (bind _asbp_character_npc_base (Utilities|Casting|CastToBP_CharacterNpcBase (Pawn|GetControlledPawn)))
  (Default|HideShowStunEffect _asbp_character_npc_base true)
  (AI|Navigation|StopMovement)
  (CallFunction|StunFunction))

(event Custom|Event%20Melee%20Attack
  (params (BoolValue :type Boolean))
  ;[1 1 1] Event pour appeler le melee attack
  (CallFunction|MeleeAttackFunction BoolValue))

(event EventBeginPlay
  (AI|RunBehaviorTree "/Game/Blueprints/NPC/AIBase/BT_NpcBase.BT_NpcBase")
  (bind _blackboardcomponent (Class|AIController|UseBlackboard "/Game/Blueprints/NPC/AIBase/BB_NpcBase.BB_NpcBase"))
  (bind _output_get (Variables|Default|SetBlackboard%20Component _blackboardcomponent))
  (AI|Components|Blackboard|SetValueasObject _output_get (Utilities|Name|MakeLiteralName "TargetActor") (Game|GetPlayerCharacter 0))
  (bind _output_get_2 (Variables|Default|SetDefaultNavigationFilterClass (Utilities|Select :Index (Math|Random|RandomIntegerinRange 0 1) :Option%200 "/Game/Blueprints/NPC/NavigationPath/NavQueryFilter_ShortPath.NavQueryFilter_ShortPath_C" :Option%201 "/Game/Blueprints/NPC/NavigationPath/NavQueryFilter_LongPath.NavQueryFilter_LongPath_C")))
  (Variables|Default|SetNavFilterClass _output_get_2)
  (Utilities|FlowControl|Delay 0.2)
  (bind _asbp_tinykinesis_player_character (Utilities|Casting|CastToBP_TinykinesisPlayerCharacter (Game|GetPlayerCharacter 0)))
  (if (Utilities|IsValid (Variables|/Game/Blueprints/ActorComponents/BP_AC_PlayerRaycastFly.BP_AC_PlayerRaycastFly_C|GetTargetPointRaycast (Variables|/Game/Blueprints/Player/BP_TinykinesisPlayerCharacter.BP_TinykinesisPlayerCharacter_C|GetBP_AC_PlayerRaycastFly _asbp_tinykinesis_player_character)))
    (AI|Components|Blackboard|SetValueasObject (Variables|Default|GetBlackboard%20Component) (Utilities|Name|MakeLiteralName "TargetPointPlayer") (Variables|/Game/Blueprints/ActorComponents/BP_AC_PlayerRaycastFly.BP_AC_PlayerRaycastFly_C|GetTargetPointRaycast (Variables|/Game/Blueprints/Player/BP_TinykinesisPlayerCharacter.BP_TinykinesisPlayerCharacter_C|GetBP_AC_PlayerRaycastFly _asbp_tinykinesis_player_character)))))

(event EventTick
  (params (DeltaSeconds :type Float%20%28single-precision%29))
  ;[1 1 1] Comment
  (AI|Components|Blackboard|SetValueasVector (Variables|Default|GetBlackboard%20Component) (Utilities|Name|MakeLiteralName "PlayerLocation") (Transformation|GetActorLocation (Game|GetPlayerCharacter 0)))
  (bind _asactor (Utilities|Casting|CastToActor (AI|Components|Blackboard|GetValueasObject (Variables|Default|GetBlackboard%20Component) (Utilities|Name|MakeLiteralName "TargetActor"))))
  (if (<= (Transformation|GetHorizontalDistanceTo (Pawn|GetControlledPawn) _asactor) (Variables|Default|GetRangeAttackMelee))
    (CallFunction|EventMeleeAttack true)
    (else
      (CallFunction|EventMeleeAttack false))))

(fn ConstructionScript)

(fn StunFunction
  (AI|Components|Blackboard|SetValueasBool (Variables|Default|GetBlackboard%20Component) (Utilities|Name|MakeLiteralName "IsStunned") true)
  (return))

(fn SeePlayer
  (params (Actor :type Actor%20Object%20Reference) (Stimuls :type AI%20Stimulus%20Structure))
  (bind _asbp_aicharacter_blank (Utilities|Casting|CastToBP_AICharacterBlank (Pawn|GetControlledPawn)))
  (if (not (Variables|/Game/Blueprints/NPC/BP_AICharacterBlank.BP_AICharacterBlank_C|GetIsAggro _asbp_aicharacter_blank))
    (bind _returnvalue (Class|AIPerceptionSystem|GetSenseClassforStimulus Stimuls))
    (if (== _returnvalue "/Script/AIModule.AISense_Sight")
      (if (== Actor (Game|GetPlayerCharacter 0))
        (AI|Components|Blackboard|SetValueasBool (Variables|Default|GetBlackboard%20Component) (Utilities|Name|MakeLiteralName "IsAggresive") true)
        (bind _asbp_character_npc_base (Utilities|Casting|CastToBP_CharacterNpcBase (Pawn|GetControlledPawn)))
        (Default|BecameAggro _asbp_character_npc_base)
        (return)
        (else
          (return)))
      (else
        (return)))))

(fn GiveAggro
  (AI|Components|Blackboard|SetValueasBool (Variables|Default|GetBlackboard%20Component) (Utilities|Name|MakeLiteralName "IsAggresive") true)
  (return))

(fn MeleeAttackFunction
  (params (BoolValue :type Boolean))
  (AI|Components|Blackboard|SetValueasBool (Variables|Default|GetBlackboard%20Component) (Utilities|Name|MakeLiteralName "InRangeAttackMelee") BoolValue)
  (return))