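; Base AI character for NPCs, providing shared hit, aggro, death and combat behavior, with empty hooks such as MeleeAttack and EventDeath.
; Incoming hits and poison drain the controller's HealthManager; damaging hits trigger aggro, which spreads via sphere trace.
; Repulse, bait and time-dilation freeze serve as crowd control, while attack helpers damage players, mobs and props.
; Death ragdolls with an impulse, updates the save through BPACStateGameplayElement and despawns after a delay.
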(event Custom|BeginPlay_Npc
  ;[0.298 1 0.5765] Begin Play
)

(event Custom|EventDestroy
  (Utilities|FlowControl|Delay 1e+01)
  (DeathFunctions|Despawn))

(event Custom|EventDeath)

(event Custom|EventDamageEffect)

(event Custom|LoadNpc
  (bind _bp_ac_stategameplayelement (Variables|Default|GetBP_AC_StateGameplayElement))
  ;[0.298 1 0.5765] Begin Play
  (Default|LoadElement _bp_ac_stategameplayelement (Variables|/Game/Blueprints/ActorComponents/BP_AC_StateGameplayElement.BP_AC_StateGameplayElement_C|GetIsActivated _bp_ac_stategameplayelement) self))

(event Custom|ImmunityHitEvent
  (Variables|Bools|SetImmunityAfterDamageHit true)
  (Utilities|FlowControl|Delay 0.5)
  (Variables|Bools|SetImmunityAfterDamageHit false))

(event Custom|ImmunityPoisonEvent
  (Variables|Bools|SetImmunityAfterDamageHit true)
  (Utilities|FlowControl|Delay 1.0)
  (Variables|Bools|SetImmunityAfterDamageHit false))

(event Custom|GetPoison_1
  (params (Damage :type Float%20%28double-precision%29))
  (if (not (Variables|Bools|GetImmunityAfterDamagePoison))
    (CallFunction|ImmunityPoisonEvent)
    (Default|LooseHP (Variables|/Game/Blueprints/NPC/BP_AIControllerBlank.BP_AIControllerBlank_C|GetHealthManager (Variables|Default|GetAs%20BP%20AIController%20Blank)) Damage)))

(event EventBeginPlay
  (bind _bp_ac_stategameplayelement (Variables|Default|GetBP_AC_StateGameplayElement))
  ;[0.298 1 0.5765] Begin Play
  (EventDispatchers|BindEventtoBeginPlayActiveElement _bp_ac_stategameplayelement (EventDispatchers|CreateEvent :!event Custom|BeginPlay_Npc))
  (bind _asbp_aicontroller_blank (Utilities|Casting|CastToBP_AIControllerBlank (Components|GetOwner)))
  (Variables|Default|SetAs%20BP%20AIController%20Blank _asbp_aicontroller_blank)
  (Default|LaunchBeginPlay _bp_ac_stategameplayelement))

(event EventFeedbacksDetectTarget
  ;[1 0.851 0] Feedback for Target (en soit, ce code s'applique aussi pour tout ce qui est piège, boutons, éléments qu'on peut cibler)
  (Rendering|Material|SetOverlayMaterial (Variables|Character|GetMesh) "/Game/Materials/MI_OutlineTarget_01.MI_OutlineTarget_01" :!class /Script/Engine.MeshComponent)
  (Default|CallFeedbacksTargetEventDispatcher))

(event EventDeleteFeedbacksDetectTarget
  ;[1 0.851 0] Feedback for Target (en soit, ce code s'applique aussi pour tout ce qui est piège, boutons, éléments qu'on peut cibler)
  (Rendering|Material|SetOverlayMaterial (Variables|Character|GetMesh) 0 :!class /Script/Engine.MeshComponent)
  (Default|CallDeleteFeedbacksTargetEventDispatcher))

(event EventGetRepulsedWave
  (params (ForceRepulse :type Float%20%28double-precision%29) (HitLocation :type Vector :default "0, 0, 0"))
  ;[0 0.175 1] Repulse Function
  (AI|Navigation|StopMovement (Variables|Default|GetAs%20BP%20AIController%20Blank))
  (if (== ForceRepulse 1e+04)
    (Variables|Default|SetFloatPowerRepulse 5e+02)
    (Character|LaunchCharacter (Math|Vector|MakeVector (.x (* (Math|Vector|Normalize (- (Transformation|GetWorldLocation (Variables|Collision|GetCapsuleComponent)) (Transformation|GetActorLocation (Game|GetPlayerCharacter 0)))) (Variables|Default|GetFloatPowerRepulse))) (.y (* (Math|Vector|Normalize (- (Transformation|GetWorldLocation (Variables|Collision|GetCapsuleComponent)) (Transformation|GetActorLocation (Game|GetPlayerCharacter 0)))) (Variables|Default|GetFloatPowerRepulse))) 3e+02) true true :!label _label)
    (elif (== ForceRepulse 2e+04)
      (Variables|Default|SetFloatPowerRepulse 1e+03)
      (goto _label))))

(event EventSetActive
  (params (IsActive :type Boolean))
  (bind _bp_ac_stategameplayelement (Variables|Default|GetBP_AC_StateGameplayElement))
  ;[0.298 1 0.5765] Begin Play
  (EventDispatchers|BindEventtoSetActiveElementEventDispatcher _bp_ac_stategameplayelement (EventDispatchers|CreateEvent :!event Custom|LoadNpc))
  (EventDispatchers|BindEventtoBeginPlayActiveElement _bp_ac_stategameplayelement (EventDispatchers|CreateEvent :!event Custom|BeginPlay_Npc))
  (Default|SetActiveElement _bp_ac_stategameplayelement IsActive))

(event EventGetHit
  (params (TelekinesisElement :type BP%20Abstract%20Telekinesis%20Element%20Object%20Reference) (CanDamage :type Boolean) (DamageObject :type Float%20%28double-precision%29) (VectorHit :type Vector :default "0, 0, 0") (ForceKnockback :type Vector :default "0, 0, 0"))
  (Utility|SetImpactParameters TelekinesisElement VectorHit ForceKnockback)
  (if CanDamage
    (if (not (Variables|Bools|GetImmunityAfterDamageHit))
      ;[1 1 1] Pour déclencher l'aggro du mob
      (if (Variables|Bools|GetIsAggro)
        _
        (else
          (AggroManager|BecameAggro)))
      (CallFunction|ImmunityHitEvent)
      (if (not (== DamageObject 0.0))
        (Default|LooseHP (Variables|/Game/Blueprints/NPC/BP_AIControllerBlank.BP_AIControllerBlank_C|GetHealthManager (Variables|Default|GetAs%20BP%20AIController%20Blank)) DamageObject)
        (Niagara|SpawnSystematLocation "/Game/VFX/Mobs/NS_MobDamage.NS_MobDamage" (Transformation|GetActorLocation))))))

(event EventGetBaited
  (params (VectorPositionBait :type Vector :default "0, 0, 0"))
  (bind _as_bp_aicontroller_blank (Variables|Default|GetAs%20BP%20AIController%20Blank))
  (bind _blackboard (Variables|/Script/AIModule.AIController|GetBlackboard _as_bp_aicontroller_blank))
  (AI|Navigation|StopMovement _as_bp_aicontroller_blank)
  (AI|Components|Blackboard|SetValueasBool _blackboard (Utilities|Name|MakeLiteralName "IsBaited") true)
  (AI|Components|Blackboard|SetValueasVector _blackboard (Utilities|Name|MakeLiteralName "VectorBait") (.ProjectedLocation (AI|Navigation|ProjectPointtoNavigation VectorPositionBait 0 0 "0, 0, 0"))))

(event EventGetFreezed
  (CallFunction|FreezeFunction true)
  (Variables|Default|SetCustomTimeDilation 0.0)
  (Utilities|FlowControl|Delay 3.0)
  (Variables|Default|SetCustomTimeDilation 1.0)
  (CallFunction|FreezeFunction false))

(fn ConstructionScript)

(fn DeathNpc
  (Variables|Bools|SetIsDead true)
  (Collision|SetCollisionEnabled (Variables|Collision|GetCapsuleComponent) "NoCollision")
  (Collision|SetCollisionEnabled (Variables|Character|GetMesh) "PhysicsOnly")
  (Physics|SetSimulatePhysics (Variables|Character|GetMesh) true)
  (bind _impulsevector (Utility|GetImpulseVector (Variables|ActorHitInfos|GetVectorHitInfos) (Variables|ActorHitInfos|GetKnockbackForceHitInfos) (Variables|Default|GetKnockbackNormal)))
  (Physics|AddImpulse (Variables|Character|GetMesh) _impulsevector "None" false)
  (Class|FMODBlueprintStatics|PlayEventatLocation "/Game/Fmod/Events/Mobs/SprigganDeath.SprigganDeath" (Transformation|GetActorTransform))
  (AI|Logic|StopLogic (Variables|/Script/AIModule.AIController|GetBrainComponent (AI|GetAIController (Components|GetOwner (Variables|Transformation|GetRootComponent)))) "ded")
  (CallFunction|EventDestroy)
  (Default|DisableinSave (Variables|Default|GetBP_AC_StateGameplayElement))
  (Default|CallOnDeathDispatcher)
  (return))

(fn BecameAggro
  (Default|GiveAggro (Variables|Default|GetAs%20BP%20AIController%20Blank))
  (Utility|SetRunSpeed)
  (Default|CallOnBecameAggro)
  (Variables|Bools|SetIsAggro true)
  (AggroManager|MakeAggroArround)
  (return))

(fn MakeAggroArround
  (bind _returnvalue (Transformation|GetActorLocation))
  (bind _outhits (Collision|MultiSphereTraceForObjects _returnvalue _returnvalue (Variables|Default|GetRadiusAggroAround) (LocalVariables|GetNewLocalVar) false (Utilities|Array|MakeArray (Game|GetPlayerCharacter 0)) "None" true "(R=0.456733,G=1.000000,B=0.960172,A=1.000000)" "(R=0.942750,G=1.000000,B=0.000000,A=1.000000)"))
  (for _array_element _outhits
    (bind _asbp_aicharacter_blank (Utilities|Casting|CastToBP_AICharacterBlank (.HitActor (Collision|BreakHitResult _array_element))))
    (if (Variables|BP_AICharacterBlank_C|GetIsAggro _asbp_aicharacter_blank)
      (return)
      (else
        (AggroManager|BecameAggro _asbp_aicharacter_blank)
        (return)))))

(fn Despawn
  (Actor|DestroyActor)
  (return))

(fn SetImpactParameters
  (params (NewActorHit :type Actor%20Object%20Reference) (NewVectorHit :type Vector) (NewKnockbackForceHit :type Vector))
  (Variables|ActorHitInfos|SetActorHitInfos NewActorHit)
  (Variables|ActorHitInfos|SetVectorHitInfos NewVectorHit)
  (Variables|ActorHitInfos|SetKnockbackForceHitInfos NewKnockbackForceHit))

(fn SetStrollSpeed
  (Variables|/Script/Engine.CharacterMovementComponent|SetMaxWalkSpeed (Variables|Character|GetCharacterMovement) (Variables|Speeds|GetStrollSpeed))
  (return))

(fn SetRunSpeed
  (Variables|/Script/Engine.CharacterMovementComponent|SetMaxWalkSpeed (Variables|Character|GetCharacterMovement) (Variables|Speeds|GetRunSpeed))
  (return))

(fn SetChargeSpeed
  (Variables|/Script/Engine.CharacterMovementComponent|SetMaxWalkSpeed (Variables|Character|GetCharacterMovement) (Variables|Speeds|GetChargeSpeed))
  (return))

(fn ChangeSpeedMetrics
  (params (NewStrollSpeed :type Float%20%28double-precision%29) (NewRunSpeed :type Float%20%28double-precision%29) (NewChargeSpeed :type Float%20%28double-precision%29))
  (if (== NewStrollSpeed 0.0)
    _
    (else
      (Variables|Speeds|SetStrollSpeed NewStrollSpeed)))
  (if (== NewRunSpeed 0.0)
    _
    (else
      (Variables|Speeds|SetRunSpeed NewRunSpeed)))
  (if (== NewChargeSpeed 0.0)
    _
    (else
      (Variables|Speeds|SetChargeSpeed NewChargeSpeed)))
  (return))

(fn HeadCollideFunction
  (params (ActorHit :type Actor%20Object%20Reference))
  (bind _as_bp_aicontroller_blank (Variables|Default|GetAs%20BP%20AIController%20Blank))
  (bind _asbp_tinykinesis_player_character (Utilities|Casting|CastToBP_TinykinesisPlayerCharacter ActorHit))
  (Default|EventStun _as_bp_aicontroller_blank)
  (Class|BrainComponent|RestartLogic (Variables|/Script/AIModule.AIController|GetBrainComponent _as_bp_aicontroller_blank))
  (Character|LaunchCharacter _asbp_tinykinesis_player_character (Math|Vector|MakeVector (.x (Math|Vector|GetForwardVector (Variables|/Script/Engine.Actor|GetRootComponent _asbp_tinykinesis_player_character))) (.y (Math|Vector|GetForwardVector (Variables|/Script/Engine.Actor|GetRootComponent _asbp_tinykinesis_player_character))) 2.5e+02) false true))

(fn Knockback
  (params (FirstTime :type Boolean) (VectorImpact :type Vector) (ForceKnockback :type Vector))
  (bind _returnvalue (Transformation|GetActorLocation))
  (bind _returnvalue_2 (- _returnvalue VectorImpact))
  (bind _returnvalue_3 (Math|Vector|Normalize _returnvalue_2))
  (bind _returnvalue_4 (* _returnvalue_3 (.x ForceKnockback)))
  (Character|LaunchCharacter (Math|Vector|MakeVector (.x _returnvalue_4) (.y _returnvalue_4) (.z ForceKnockback)) false false))

(fn GetImpulseVector
  (params (VectorImpact :type Vector) (ForceKnockbackHit :type Vector) (KnockBackNormal :type Vector))
  (bind _returnvalue (Transformation|GetActorLocation))
  (bind _returnvalue_2 (- _returnvalue VectorImpact))
  (bind _returnvalue_3 (Math|Vector|Normalize _returnvalue_2))
  (bind _returnvalue_4 (* _returnvalue_3 (.x KnockBackNormal)))
  (return (* (Math|Vector|MakeVector (.x _returnvalue_4) (.y _returnvalue_4) (.z KnockBackNormal)) ForceKnockbackHit)))

(fn MeleeAttack
  (return))

(fn HitPlayer
  (params (ActorHit :type Actor%20Object%20Reference) (ImpactHit :type Vector) (TypeAttack :type E_MobAttackType%20Enum :default "NewEnumerator0") (KnockbackForce :type Vector) (Dammage :type Float%20%28double-precision%29))
  (bind _tinykinesisplayercharacter (CallFunction|GetTinykinesisPlayerCharacter))
  (if (== ActorHit _tinykinesisplayercharacter)
    (switch Utilities|FlowControl|Switch|SwitchonE_MobAttackType TypeAttack
      (:NewEnumerator0
        (LocalVariables|SetImpactLocationHit ImpactHit :!label _label))
      (:NewEnumerator1
        (LocalVariables|SetImpactLocationHit (Transformation|GetActorLocation)))
      (:NewEnumerator3
        (goto _label)))
    (Default|EventGetHit _tinykinesisplayercharacter (LocalVariables|GetImpactLocationHit) KnockbackForce Dammage)
    (switch Utilities|FlowControl|Switch|SwitchonE_MobAttackType TypeAttack
      (:NewEnumerator0
        ;[1 1 1] Knockback & Stun on self if charge
        (Variables|ActorHitInfos|SetVectorHitInfos (Transformation|GetActorLocation (CallFunction|GetTinykinesisPlayerCharacter)))
        (CallFunction|EventDamageEffect))
      (:NewEnumerator1
        _)
      (:NewEnumerator3
        _)
      (:NewEnumerator2
        _)
      (:NewEnumerator4
        _))
    (return true)
    (else
      (return false))))

(fn HitEnvironment
  (params (ActorHit :type Actor%20Object%20Reference) (LocationHit :type Vector))
  (if (not (Actor|ActorHasTag ActorHit "Ground"))
    (Variables|ActorHitInfos|SetVectorHitInfos LocationHit)
    (CallFunction|EventDamageEffect)
    (return)))

(fn HitOtherMob
  (params (ActorHit :type Actor%20Object%20Reference) (KnockbackForceHit :type Vector) (Damage :type Float%20%28double-precision%29))
  (bind _asbp_aicharacter_blank (Utilities|Casting|CastToBP_AICharacterBlank ActorHit)
    (:then
      (bind _asbp_aicontroller_blank (Utilities|Casting|CastToBP_AIControllerBlank (Components|GetOwner _asbp_aicharacter_blank)))
      (Variables|BP_AICharacterBlank_C|SetKnockbackForceHitInfos _asbp_aicharacter_blank KnockbackForceHit)
      (Default|LooseHP (Variables|/Game/Blueprints/NPC/BP_AIControllerBlank.BP_AIControllerBlank_C|GetHealthManager _asbp_aicontroller_blank) Damage)
      (return true))
    (:CastFailed
      (return false))))

(fn HitDynamics
  (params (InputActorHit :type Actor%20Object%20Reference) (VectorHitInput :type Vector) (InputTypeAttack :type E_MobAttackType%20Enum :default "NewEnumerator0"))
  (Variables|ActorHitInfos|SetVectorHitInfos VectorHitInput)
  (if (Utilities|DoesObjectImplementInterface InputActorHit "/Game/Blueprints/Interfaces/BPI_TelekinesisObject.BPI_TelekinesisObject_C")
    (Utilities|Casting|CastToBP_AbstractPickUpObject InputActorHit
      (:then
        (return false))
      (:CastFailed
        (bind _asbp_abstract_telekinesis_element (Utilities|Casting|CastToBP_AbstractTelekinesisElement InputActorHit)
          (:then
            (if (not (or (Variables|/Game/Blueprints/Actors/TelekinesisElements/BP_AbstractTelekinesisElement.BP_AbstractTelekinesisElement_C|GetIsBeingReleased _asbp_abstract_telekinesis_element) (Variables|/Game/Blueprints/Actors/TelekinesisElements/BP_AbstractTelekinesisElement.BP_AbstractTelekinesisElement_C|GetIsBeingGrabbed _asbp_abstract_telekinesis_element)))
              (switch Utilities|FlowControl|Switch|SwitchonE_MobAttackType InputTypeAttack
                (:NewEnumerator0
                  (Default|LooseHP (Variables|/Game/Blueprints/Actors/TelekinesisElements/BP_AbstractTelekinesisElement.BP_AbstractTelekinesisElement_C|GetBP_AC_Health _asbp_abstract_telekinesis_element) (Variables|Default|GetDamageChargeAttack))
                  (CallFunction|EventDamageEffect))
                (:NewEnumerator1
                  (Default|LooseHP (Variables|/Game/Blueprints/Actors/TelekinesisElements/BP_AbstractTelekinesisElement.BP_AbstractTelekinesisElement_C|GetBP_AC_Health _asbp_abstract_telekinesis_element) (Variables|Default|GetDamageMeleeAttack) :!label _label))
                (:NewEnumerator3
                  (goto _label)))
              (return true)))
          (:CastFailed
            (return false)))))
    (else
      (bind _asbp_destructible_object (Utilities|Casting|CastToBP_DestructibleObject InputActorHit)
        (:then
          (switch Utilities|FlowControl|Switch|SwitchonE_MobAttackType InputTypeAttack
            (:NewEnumerator0
              (Default|LooseHP (Variables|/Game/Blueprints/Actors/Traps/DestructibleObject/BP_DestructibleObject.BP_DestructibleObject_C|GetBP_AC_Health _asbp_destructible_object) (Variables|Default|GetDamageChargeAttack))
              (CallFunction|EventDamageEffect))
            (:NewEnumerator1
              (Default|LooseHP (Variables|/Game/Blueprints/Actors/Traps/DestructibleObject/BP_DestructibleObject.BP_DestructibleObject_C|GetBP_AC_Health _asbp_destructible_object) (Variables|Default|GetDamageMeleeAttack))))
          (return true))
        (:CastFailed
          (return false))))))

(fn SetDamageValue
  (params (NewValueDamage :type Float%20%28double-precision%29) (Attack :type E_MobAttackType%20Enum :default "NewEnumerator0"))
  (switch Utilities|FlowControl|Switch|SwitchonE_MobAttackType Attack
    (:NewEnumerator0
      (Variables|Default|SetDamageChargeAttack NewValueDamage))
    (:NewEnumerator1
      (Variables|Default|SetDamageMeleeAttack NewValueDamage)))
  (return))

(fn SetAnimationStateNEW
  (params (State :type E_Mob_Animation_State%20Enum :default "NewEnumerator0")))

(fn SpawningVFX
  (Niagara|SpawnSystematLocation "/Game/VFX/Mobs/PoofEffect/NS_PoofExplosion.NS_PoofExplosion" (Transformation|GetActorLocation))
  (return))

(fn ChangeMaterialWeapon
  (params (Change :type Boolean))
  (return))

(fn FreezeFunction
  (params (IsFreezing :type Boolean))
  (bind _mesh (Variables|Character|GetMesh))
  (if IsFreezing
    (Variables|/Script/Engine.SkeletalMeshComponent|SetbPauseAnims _mesh true)
    (else
      (Variables|/Script/Engine.SkeletalMeshComponent|SetbPauseAnims _mesh false))))

(fn FocusPlayer
  (AI|SetFocus (Variables|Default|GetAs%20BP%20AIController%20Blank) (Game|GetPlayerCharacter 0))
  (return))

(fn ResetFocus
  (AI|ClearFocus (Variables|Default|GetAs%20BP%20AIController%20Blank))
  (return))

(fn GetCanTakeDamage
  (return true))