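; BP_RangeMeleeAttack is an NPC melee attack range Blueprint that records which actors enter its collision volumes.
; RangeMelee overlaps add each new actor and its sweep location to paired arrays, both cleared on BeginPlay.
; RangeUnderWeapon overlaps fill a separate dead-zone actor list, which is not cleared here.
; It only collects this data, with no end-overlap removal or damage logic.
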(event OnComponentBeginOverlap(RangeMelee)
  (params (OverlappedComponent :type Primitive%20Component%20Object%20Reference) (OtherActor :type Actor%20Object%20Reference) (OtherComp :type Primitive%20Component%20Object%20Reference) (OtherBodyIndex :type Integer) (bFromSweep :type Boolean) (SweepResult :type Hit%20Result%20Structure%20%28by%20ref%29))
  (if (not (Utilities|Array|ContainsItem (Variables|Default|GetActorsOverlap) OtherActor))
    (Utilities|Array|Add (Variables|Default|GetActorsOverlap) OtherActor)
    (Utilities|Array|Add (Variables|Default|GetVectorOverlapLocation) (.Location (Collision|BreakHitResult SweepResult)))))

(event OnComponentBeginOverlap(RangeUnderWeapon)
  (params (OverlappedComponent :type Primitive%20Component%20Object%20Reference) (OtherActor :type Actor%20Object%20Reference) (OtherComp :type Primitive%20Component%20Object%20Reference) (OtherBodyIndex :type Integer) (bFromSweep :type Boolean) (SweepResult :type Hit%20Result%20Structure%20%28by%20ref%29))
  (bind _actorsoverlapdeadzone (Variables|Default|GetActorsOverlapDeadZone))
  (if (not (Utilities|Array|ContainsItem _actorsoverlapdeadzone OtherActor))
    (Utilities|Array|Add _actorsoverlapdeadzone OtherActor)))

(event EventBeginPlay
  (Utilities|Array|Clear (Variables|Default|GetActorsOverlap))
  (Utilities|Array|Clear (Variables|Default|GetVectorOverlapLocation)))

(fn ConstructionScript)