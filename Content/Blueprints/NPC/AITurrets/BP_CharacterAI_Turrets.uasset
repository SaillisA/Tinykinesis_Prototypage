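; Turret NPC character that detects the player by distance, turns its cannon toward them and breaks apart on death.
; Tick triggers aggro within detection range and, while LookPlayer is set, rotates the cannon from a look-at rotation with zero pitch.
; A shield event slides Cannon and Mask between two poses, starting with the shield off.
; The owning BP_AIC_Turrets' HealthManager drives death destruction and a timeline-driven mesh shake on damage, both through BPACDestructionElement.
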(event Custom|EventShieldSetActive
  (params (IsOn :type Boolean))
  (bind _cannon (Variables|Default|GetCannon))
  (bind _cannon_2 (Variables|Default|GetCannon))
  (bind _mask (Variables|Default|GetMask))
  (bind _mask_2 (Variables|Default|GetMask))
  (if IsOn
    (Components|MoveComponentTo _cannon "0.000000,-20.000000,88.000000" (.rotation (Transformation|GetRelativeTransform _cannon)) false false 0.2 false)
    (Components|MoveComponentTo _mask_2 "1.000000,39.000000,73.000000" (.rotation (Transformation|GetRelativeTransform _mask_2)) false false 0.2 false)
    (else
      (Components|MoveComponentTo _mask "1.000000,39.000000,110.000000" (.rotation (Transformation|GetRelativeTransform _mask)) false false 0.2 false)
      (Components|MoveComponentTo _cannon_2 "0.000000,30.000000,88.000000" (.rotation (Transformation|GetRelativeTransform _cannon_2)) false false 0.2 false))))

(event Custom|Death_Turrets
  ;[0.3137 0.06274 0.06667] Death Specificity for Npc Distance
  (CallFunction|DeathNpc)
  (Default|LaunchDestruction (Variables|Default|GetBP_AC_DestructionElement) (Transformation|GetRelativeTransform (Variables|Character|GetMesh)) self))

(event Custom|DamageEffect_Turrets
  ;[0.3137 0.06274 0.06667] Damage specificity for Npc Distance
  (bind _newlocation (Timeline|ShakeDamage PlayFromStart)
    (:Update
      (Default|ShakeSkeletalMesh (Variables|Default|GetBP_AC_DestructionElement) (Variables|Character|GetMesh) _newlocation))))

(event EventBeginPlayNpc
  ;[0.298 1 0.5765] BeginPlay
  (bind _asbp_aic_turrets (Utilities|Casting|CastToBP_AIC_Turrets (Components|GetOwner)))
  (Default|BeginPlayAICNpcDistance _asbp_aic_turrets)
  (CallFunction|EventShieldSetActive false)
  (EventDispatchers|BindEventtoDeath (Variables|/Game/Blueprints/NPC/BP_AIC_Blank.BP_AIC_Blank_C|GetHealthManager _asbp_aic_turrets) (EventDispatchers|CreateEvent :!event Custom|Death_Turrets))
  (EventDispatchers|BindEventtoDamageEffect (Variables|/Game/Blueprints/NPC/BP_AIC_Blank.BP_AIC_Blank_C|GetHealthManager _asbp_aic_turrets) (EventDispatchers|CreateEvent :!event Custom|DamageEffect_Turrets)))

(event EventTick
  (params (DeltaSeconds :type Float%20%28single-precision%29))
  ;[0.7412 1 0.3412] EventTick
  (if (Variables|Default|GetLookPlayer)
    (CallFunction|RotationLauncherBullets))
  (if (not (Variables|Default|GetIsAggro))
    (if (<= (Transformation|GetDistanceTo (Game|GetPlayerCharacter 0)) (Variables|Default|GetRangeDetection))
      (CallFunction|BecameAggro))))

(fn ConstructionScript)

(fn RotationLauncherBullets
  (bind _returnvalue (Game|GetPlayerCharacter 0))
  (bind _returnvalue_2 (Transformation|GetActorLocation))
  (bind _returnvalue_3 (Transformation|GetActorLocation _returnvalue))
  (bind _returnvalue_4 (Math|Rotator|FindLookatRotation _returnvalue_2 _returnvalue_3))
  (Transformation|SetWorldRotation (Variables|Default|GetCannon) (Math|Rotator|MakeRotator (.roll _returnvalue_4) 0.0 (+ (.yaw _returnvalue_4) -9e+01)) false false)
  (return))