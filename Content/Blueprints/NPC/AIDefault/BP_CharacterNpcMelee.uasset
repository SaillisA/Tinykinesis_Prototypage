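; Melee enemy NPC character that aggros when the player comes within range, then attacks by sphere-traced strike or charge, with a random calcined skin variant.
; Its AI controller handles aggro, stuns and blackboard flags, while health-manager events trigger knockback-then-stun or ragdoll death.
; Charging into the player or another melee NPC knocks it back, also stunning the NPC it hit.
; Landing on its head stuns it and bounces the player.
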(event OnComponentBeginOverlap(HeadCollide_0)
  (params (OverlappedComponent :type Primitive%20Component%20Object%20Reference) (OtherActor :type Actor%20Object%20Reference) (OtherComp :type Primitive%20Component%20Object%20Reference) (OtherBodyIndex :type Integer) (bFromSweep :type Boolean) (SweepResult :type Hit%20Result%20Structure%20%28by%20ref%29))
  (bind _as_bp_aic_npc_melee (Variables|Cast|GetAs%20BP%20AIC%20Npc%20Melee))
  ;[1 0.8973 0.3638] Détection du joueur sur la tête
  (bind _asbp_tinykinesis_player_character (Utilities|Casting|CastToBP_TinykinesisPlayerCharacter OtherActor))
  (Default|EventStun _as_bp_aic_npc_melee)
  (Class|BrainComponent|RestartLogic (Variables|/Script/AIModule.AIController|GetBrainComponent _as_bp_aic_npc_melee))
  ;[1 1 1] Faire rebondir le joueur
  (Character|LaunchCharacter _asbp_tinykinesis_player_character (Math|Vector|MakeVector (.x (Math|Vector|GetForwardVector (Variables|/Script/Engine.Actor|GetRootComponent _asbp_tinykinesis_player_character))) (.y (Math|Vector|GetForwardVector (Variables|/Script/Engine.Actor|GetRootComponent _asbp_tinykinesis_player_character))) 2.5e+02) false true)
  (Variables|Default|SetCanBeStunned true))

(event OnComponentHit(CapsuleComponent)
  (params (HitComponent :type Primitive%20Component%20Object%20Reference) (OtherActor :type Actor%20Object%20Reference) (OtherComp :type Primitive%20Component%20Object%20Reference) (NormalImpulse :type Vector :default "0, 0, 0") (Hit :type Hit%20Result%20Structure%20%28by%20ref%29))
  ;[1 0.2627 0.05882] Event Charge : Player, other Npc and Objects
  (if (ScalableFloat|GetValueasBool (Variables|Default|GetBlackboard%20Component) (Utilities|Name|MakeLiteralName "IsCharging"))
    (bind _iscollideplayertrue (FunctionsCollide|HitPlayer OtherActor (.ImpactPoint (Collision|BreakHitResult Hit)) "NewEnumerator0" (Variables|MeleeAttack|GetKnockbackForceMeleeAttack) (Variables|ChargeAttack|GetDamageChargeAttack_0)))
    (if (not _iscollideplayertrue)
      (bind _iscollidenpctrue (FunctionsCollide|HitOtherNpc OtherActor))
      (if _iscollidenpctrue
        _))))

(event Custom|EventMeleeAttack
  ;[1 0.3804 0.2078] MeleeAttack
  (if (Variables|MeleeAttack|GetCanAttackMelee)
    (Variables|MeleeAttack|SetCanAttackMelee false)
    (bind (_actorhit _impactlocation) (CallFunction|MeleeAttackRaycast))
    (FunctionsCollide|HitPlayer _actorhit _impactlocation "NewEnumerator1" (Variables|MeleeAttack|GetKnockbackForceMeleeAttack) (Variables|MeleeAttack|GetDamageMeleeAttack_0))))

(event Custom|Death_NpcMelee
  ;[0.3137 0.06274 0.06667] Death Specificity for NpcMelee
  (Collision|SetCollisionEnabled (Variables|Default|GetHeadCollide_0) "NoCollision")
  (Physics|SetSimulatePhysics (Variables|Character|GetMesh) true)
  (bind _impulsevector (CallFunction|GetImpulseVector0 (Variables|Default|GetVectorHitInfos) (Variables|Default|GetKnockbackForceHitInfos)))
  (Physics|AddImpulse (Variables|Character|GetMesh) _impulsevector "None" false)
  (Class|FMODBlueprintStatics|PlayEventatLocation "/Game/Fmod/Events/Mobs/SprigganDeath.SprigganDeath" (Transformation|GetActorTransform))
  (CallFunction|DeathNpc))

(event Custom|DamageEffect_NpcMelee
  (bind _as_bp_aic_npc_melee (Variables|Cast|GetAs%20BP%20AIC%20Npc%20Melee))
  (bind _blackboard_component (Variables|/Game/Blueprints/NPC/AIDefault/BP_AIC_NpcMelee.BP_AIC_NpcMelee_C|GetBlackboard%20Component _as_bp_aic_npc_melee))
  ;[0.3137 0.06274 0.06667] Damage specificity for MeleeMobs : knockback & stuns
  (Variables|Default|SetWasKnockbacked true)
  (AI|Navigation|StopMovement _as_bp_aic_npc_melee)
  (AI|Components|Blackboard|SetValueasBool _blackboard_component (Utilities|Name|MakeLiteralName "IsKnockbacked") true)
  (CallFunction|Knockback0 (Variables|Default|GetVectorHitInfos))
  (CallFunction|SetStateAnimation "NewEnumerator13")
  (Utilities|FlowControl|Delay 2.17)
  (AI|Components|Blackboard|SetValueasBool _blackboard_component (Utilities|Name|MakeLiteralName "IsKnockbacked") false)
  (CallFunction|SetStateAnimation "NewEnumerator6")
  (Default|EventStun (Variables|Cast|GetAs%20BP%20AIC%20Npc%20Melee)))

(event EventBeginPlayNpc
  (bind _as_bp_aic_npc_melee (Variables|Cast|GetAs%20BP%20AIC%20Npc%20Melee))
  (bind _as_bp_aic_npc_melee_2 (Variables|Cast|GetAs%20BP%20AIC%20Npc%20Melee))
  (bind _healthmanager (Variables|/Game/Blueprints/NPC/AIDefault/BP_AIC_NpcMelee.BP_AIC_NpcMelee_C|GetHealthManager _as_bp_aic_npc_melee_2))
  ;[0.298 1 0.5765] Begin Play
  (CallFunction|AllCast)
  (if (Math|Random|RandomBool)
    _
    (else
      (CallFunction|MaterialsChangeCalcined)))
  (Default|BeginPlayAICNpcMelee _as_bp_aic_npc_melee)
  (Actor|Tick|SetActorTickEnabled true)
  (Variables|Default|SetBlackboard%20Component (Variables|/Game/Blueprints/NPC/AIDefault/BP_AIC_NpcMelee.BP_AIC_NpcMelee_C|GetBlackboard%20Component _as_bp_aic_npc_melee))
  (Variables|/Script/Engine.CharacterMovementComponent|SetMaxWalkSpeed (Variables|Character|GetCharacterMovement) (Variables|Movements|GetRunSpeed_0))
  (EventDispatchers|BindEventtoDeath _healthmanager (EventDispatchers|CreateEvent :!event Custom|Death_NpcMelee))
  (EventDispatchers|BindEventtoDamageEffect _healthmanager (EventDispatchers|CreateEvent :!event Custom|DamageEffect_NpcMelee))
  (bind _returnvalue (Actor|GetActorOfClass "/Game/Blueprints/NPC/NavigationPath/FlankSystem/BP_FlankManager.BP_FlankManager_C"))
  (Variables|Cast|SetFlankManager _returnvalue))

(event EventTick
  (params (DeltaSeconds :type Float%20%28single-precision%29))
  ;[0.7412 1 0.3412] Event Tick
  (if (not (Variables|Default|GetIsAggro))
    (if (<= (Transformation|GetDistanceTo (Game|GetPlayerCharacter 0)) (Variables|Metrics|GetRangeDetection))
      (CallFunction|BecameAggro))))

(fn ConstructionScript)

(fn SetStrollSpeed00
  (Variables|/Script/Engine.CharacterMovementComponent|SetMaxWalkSpeed (Variables|Character|GetCharacterMovement) (Variables|Movements|GetStrollSpeed_0))
  (return))

(fn SetRunSpeed00
  (Variables|/Script/Engine.CharacterMovementComponent|SetMaxWalkSpeed (Variables|Character|GetCharacterMovement) (Variables|Movements|GetRunSpeed_0))
  (return))

(fn HitPlayer
  (params (Actor%20hit :type Actor%20Object%20Reference) (ImpactHit :type Vector) (TypeAttack :type E_MobAttackType%20Enum :default "EAttackType_MAX") (KnockbackForce :type Vector) (Dammage :type Float%20%28double-precision%29))
  (bind _tinykinesisplayercharacter (CallFunction|GetTinykinesisPlayerCharacter))
  (if (== Actor%20hit _tinykinesisplayercharacter)
    (switch Utilities|FlowControl|Switch|SwitchonE_MobAttackType TypeAttack
      (:NewEnumerator0
        (LocalVariables|SetImpactLocationHit ImpactHit))
      (:NewEnumerator1
        (LocalVariables|SetImpactLocationHit (Transformation|GetActorLocation))))
    (Default|EventGetHit _tinykinesisplayercharacter (LocalVariables|GetImpactLocationHit) KnockbackForce Dammage)
    (switch Utilities|FlowControl|Switch|SwitchonE_MobAttackType TypeAttack
      (:NewEnumerator0
        ;[1 1 1] Knockback & Stun on self if charge
        (Variables|Default|SetVectorHitInfos (Transformation|GetActorLocation (CallFunction|GetTinykinesisPlayerCharacter)))
        (CallFunction|DamageEffectNpcMelee))
      (:NewEnumerator1
        _))
    (return true)
    (else
      (return false))))

(fn Knockback0
  (params (VectorImpact :type Vector))
  (bind _impulsevector (CallFunction|GetImpulseVector0 VectorImpact (Variables|Default|GetKnockbackForceHitInfos)))
  (Character|LaunchCharacter _impulsevector false false)
  (return))

(fn HitOtherNpc
  (params (ActorHit :type Actor%20Object%20Reference))
  (bind _asbp_character_npc_melee (Utilities|Casting|CastToBP_CharacterNpcMelee ActorHit)
    (:then
      ;[1 1 1] Knockback + stun on self
      (Variables|Default|SetVectorHitInfos (Transformation|GetActorLocation _asbp_character_npc_melee))
      (CallFunction|DamageEffectNpcMelee)
      ;[1 1 1] Stun on other npc
      (bind _asbp_aic_npc_melee (Utilities|Casting|CastToBP_AIC_NpcMelee (Components|GetOwner _asbp_character_npc_melee)))
      (Default|EventStun _asbp_aic_npc_melee)
      (return true))
    (:CastFailed
      (return false))))

(fn SetChargeSpeed0
  (Variables|/Script/Engine.CharacterMovementComponent|SetMaxWalkSpeed (Variables|Character|GetCharacterMovement) (Variables|Movements|GetChargeSpeed_0))
  (return))

(fn BecameAggro
  (Default|GiveAggro (Variables|Cast|GetAs%20BP%20AIC%20Npc%20Melee))
  (CallFunction|SetRunSpeed)
  (|CallParentFunction)
  (return))

(fn HitEnvironment0
  (params (ActorHit :type Actor%20Object%20Reference) (LocationHit :type Vector))
  (if (not (Actor|ActorHasTag ActorHit "Ground"))
    (Variables|Default|SetVector%20Hit_0 LocationHit)
    (CallFunction|DamageEffectNpcMelee)))

(fn OnOffColisionStick
  (params (OnOff :type Boolean)))

(fn CheckFloor
  (params (HitActor :type Actor%20Object%20Reference))
  (Variables|Default|SetHitFloorPlatform (Actor|ActorHasTag HitActor "Platform"))
  (return))

(fn MeleeAttackRaycast
  (bind _returnvalue (Transformation|GetActorRotation))
  (bind _returnvalue_2 (Transformation|GetActorLocation))
  (bind _lenghtrange (LocalVariables|GetLenghtRange))
  (bind _returnvalue_3 (Math|Vector|GetForwardVector _returnvalue))
  (bind _returnvalue_4 (* _returnvalue_3 _lenghtrange))
  (bind _returnvalue_5 (+ _returnvalue_2 _returnvalue_4))
  (bind _outhit (Collision|SphereTraceForObjects _returnvalue_5 _returnvalue_5 6e+01 (LocalVariables|GetObjectsTypes) false 0 "None"))
  (return (.HitActor (Collision|BreakHitResult _outhit)) (.Location (Collision|BreakHitResult _outhit))))

(fn GetImpulseVector0
  (params (VectorImpact :type Vector) (ForceKnockbackHit :type Vector))
  (bind _returnvalue (Transformation|GetActorLocation))
  (bind _returnvalue_2 (- _returnvalue VectorImpact))
  (bind _returnvalue_3 (Math|Vector|Normalize _returnvalue_2))
  (bind _returnvalue_4 (* _returnvalue_3 (.x ForceKnockbackHit)))
  (return (Math|Vector|MakeVector (.x _returnvalue_4) (.y _returnvalue_4) (.z ForceKnockbackHit))))

(fn SetStateAnimation
  (params (InputState :type E_MobStateMelee%20Enum :default "NewEnumerator0")))

(fn AllCast
  (bind _asbp_aic_npc_melee (Utilities|Casting|CastToBP_AIC_NpcMelee (Components|GetOwner)))
  (Variables|Cast|SetAs%20BP%20AIC%20Npc%20Melee _asbp_aic_npc_melee)
  (return))

(fn MaterialsChangeCalcined
  (bind _mesh (Variables|Character|GetMesh))
  (Rendering|Material|SetMaterial (Variables|Default|GetEarring_L) 0 "/Game/Characters/NPC/Melee/Materials/Calcined/M_EnemyMelee_Calcined_Earring_Marisa.M_EnemyMelee_Calcined_Earring_Marisa")
  (Rendering|Material|SetMaterial (Variables|Default|GetEarring_R) 0 "/Game/Characters/NPC/Melee/Materials/Calcined/M_EnemyMelee_Calcined_Earring_Marisa.M_EnemyMelee_Calcined_Earring_Marisa")
  (Rendering|Material|SetMaterial _mesh 0 "/Game/Characters/NPC/Melee/Materials/Calcined/M_EnemyMelee_Calcined_Body_Marisa.M_EnemyMelee_Calcined_Body_Marisa")
  (Rendering|Material|SetMaterial _mesh 1 "/Game/Characters/NPC/Melee/Materials/Calcined/M_EnemyMelee_Calcined_Head_Marisa.M_EnemyMelee_Calcined_Head_Marisa")
  (Rendering|Material|SetMaterial _mesh 2 "/Game/Characters/NPC/Melee/Materials/Calcined/M_EnemyMelee_Calcined_Ears_Marisa.M_EnemyMelee_Calcined_Ears_Marisa")
  (Rendering|Material|SetMaterial _mesh 3 "/Game/Characters/NPC/Melee/Materials/Calcined/M_EnemyMelee_Calcined_Antennas_Marisa.M_EnemyMelee_Calcined_Antennas_Marisa")
  (Rendering|Material|SetMaterial _mesh 4 "/Game/Characters/NPC/Melee/Materials/Calcined/M_EnemyMelee_Calcined_Eyes_Marisa.M_EnemyMelee_Calcined_Eyes_Marisa")
  (return))