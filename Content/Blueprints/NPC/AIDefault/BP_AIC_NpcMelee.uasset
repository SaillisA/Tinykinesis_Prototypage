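; AI controller for melee NPCs, running BT_NpcMelee and feeding its blackboard.
; A custom init event seeds player, target and start location, randomizes navigation filter and attack wind-up times, and passes timings to ABP_Spriggan.
; Tick flags melee range from horizontal distance to TargetActor; sighting the player triggers aggro and run speed, and Stun halts movement.
; GiveAggro writes a misspelled "IsAggresive" key, unlike the sight path's "IsAggressive".
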(event OnTargetPerceptionUpdated(AIPerception)
  (params (Actor :type Actor%20Object%20Reference) (Stimulus :type AI%20Stimulus%20Structure))
  (CallFunction|SeePlayer Actor Stimulus))

(event Custom|Event%20Stun
  ;[1 1 1] Event pour appeler le stun
  (AI|Navigation|StopMovement)
  (CallFunction|StunFunction))

(event Custom|Event%20Melee%20Attack
  (params (BoolValue :type Boolean))
  ;[1 1 1] Event pour appeler le melee attack
  (CallFunction|MeleeAttackFunction BoolValue))

(event Custom|BeginPlay_AICNpcMelee
  (bind _returnvalue (Math|Random|RandomFloatinRange 0.0 0.3))
  (bind _returnvalue_2 (Math|Random|RandomFloatinRange 0.0 0.5))
  (bind _arrayfilterclass (Variables|Default|GetArrayFilterClass))
  (bind _outitem (Utilities|Array|Random _arrayfilterclass))
  (bind _returnvalue_3 (+ 0.4 _returnvalue))
  (bind _returnvalue_4 (+ 0.8 _returnvalue_2))
  ;[0.298 1 0.5765] BeginPlay
  (Variables|Default|SetCanRunTick true)
  (bind _asbp_character_npc_melee (Utilities|Casting|CastToBP_CharacterNpcMelee (Pawn|GetControlledPawn)))
  (Variables|Default|SetAs%20BP%20Character%20Npc%20Melee _asbp_character_npc_melee)
  (AI|RunBehaviorTree "/Game/Blueprints/NPC/AIDefault/BT_NpcMelee.BT_NpcMelee")
  (bind _blackboardcomponent (Class|AIController|UseBlackboard "/Game/Blueprints/NPC/AIDefault/BB_NpcMelee.BB_NpcMelee"))
  (Variables|Default|SetBlackboard%20Component _blackboardcomponent)
  (AI|Components|Blackboard|SetValueasObject (Variables|Default|GetBlackboard%20Component) (Utilities|Name|MakeLiteralName "PlayerActor") (CallFunction|GetTinykinesisPlayerCharacter))
  (Variables|Default|SetDefaultNavigationFilterClass _outitem)
  (Variables|Default|SetNavFilterClass _outitem)
  (AI|Components|Blackboard|SetValueasFloat (Variables|Default|GetBlackboard%20Component) (Utilities|Name|MakeLiteralName "TimeChargeLoad") _returnvalue_4)
  (Variables|Float|SetLoadChargeTime _returnvalue_4)
  (AI|Components|Blackboard|SetValueasFloat (Variables|Default|GetBlackboard%20Component) (Utilities|Name|MakeLiteralName "TimeMeleeLoad") _returnvalue_3)
  (Variables|Float|SetLoadMeleeAttackTime _returnvalue_3)
  (Utilities|FlowControl|Delay 0.2)
  (bind _asbp_tinykinesis_player_character (Utilities|Casting|CastToBP_TinykinesisPlayerCharacter (Game|GetPlayerCharacter 0)))
  (if (Utilities|IsValid (Variables|/Game/Blueprints/ActorComponents/BP_AC_PlayerRaycastFly.BP_AC_PlayerRaycastFly_C|GetTargetPointRaycast (Variables|/Game/Blueprints/Player/BP_TinykinesisPlayerCharacter.BP_TinykinesisPlayerCharacter_C|GetBP_AC_PlayerRaycastFly _asbp_tinykinesis_player_character)))
    (AI|Components|Blackboard|SetValueasObject (Variables|Default|GetBlackboard%20Component) (Utilities|Name|MakeLiteralName "TargetPointPlayer") (Variables|/Game/Blueprints/ActorComponents/BP_AC_PlayerRaycastFly.BP_AC_PlayerRaycastFly_C|GetTargetPointRaycast (Variables|/Game/Blueprints/Player/BP_TinykinesisPlayerCharacter.BP_TinykinesisPlayerCharacter_C|GetBP_AC_PlayerRaycastFly _asbp_tinykinesis_player_character)))
    (AI|Components|Blackboard|SetValueasVector (Variables|Default|GetBlackboard%20Component) (Utilities|Name|MakeLiteralName "AILocationAtStart") (Transformation|GetActorLocation (Pawn|GetControlledPawn)))
    (bind _asabp_spriggan (Utilities|Casting|CastToABP_Spriggan (Components|SkeletalMesh|GetAnimInstance (Variables|/Script/Engine.Character|GetMesh (Variables|Default|GetAs%20BP%20Character%20Npc%20Melee)))))
    (Variables|/Game/Characters/NPC/Melee/Animations/ABP_Spriggan.ABP_Spriggan_C|SetLoadCharge _asabp_spriggan (Variables|Float|GetLoadChargeTime))
    (Variables|/Game/Characters/NPC/Melee/Animations/ABP_Spriggan.ABP_Spriggan_C|SetLoadMeleeAttack _asabp_spriggan (Variables|Float|GetLoadMeleeAttackTime))
    (Utilities|FlowControl|Delay 0.2)
    (AI|Components|Blackboard|SetValueasObject (Variables|Default|GetBlackboard%20Component) (Utilities|Name|MakeLiteralName "TargetActor") (Variables|Default|GetTargetFlankActor))))

(event EventBeginPlay
  ;[0.298 1 0.5765] BeginPlay
)

(event EventTick
  (params (DeltaSeconds :type Float%20%28single-precision%29))
  ;[1 1 1] EventTick
  (if (Variables|Default|GetCanRunTick)
    (bind _asactor (Utilities|Casting|CastToActor (AI|Components|Blackboard|GetValueasObject (Variables|Default|GetBlackboard%20Component) (Utilities|Name|MakeLiteralName "TargetActor"))))
    (if (<= (Transformation|GetHorizontalDistanceTo (Pawn|GetControlledPawn) _asactor) (Variables|Float|GetRangeAttackMelee))
      (CallFunction|EventMeleeAttack true)
      (else
        (CallFunction|EventMeleeAttack false)))))

(fn ConstructionScript)

(fn StunFunction
  (AI|Components|Blackboard|SetValueasBool (Variables|Default|GetBlackboard%20Component) (Utilities|Name|MakeLiteralName "IsStunned") true)
  (return))

(fn SeePlayer
  (params (Actor :type Actor%20Object%20Reference) (Stimuls :type AI%20Stimulus%20Structure))
  (bind _asbp_aicharacter_blank (Utilities|Casting|CastToBP_AICharacterBlank (Pawn|GetControlledPawn)))
  (if (not (Variables|/Game/Blueprints/NPC/BP_AICharacterBlank.BP_AICharacterBlank_C|GetIsAggro _asbp_aicharacter_blank))
    (bind _returnvalue (Class|AIPerceptionSystem|GetSenseClassforStimulus Stimuls))
    (if (== _returnvalue "/Script/AIModule.AISense_Sight")
      (if (== Actor (Game|GetPlayerCharacter 0))
        (AI|Components|Blackboard|SetValueasBool (Variables|Default|GetBlackboard%20Component) (Utilities|Name|MakeLiteralName "IsAggressive") true)
        (bind _asbp_character_npc_melee (Utilities|Casting|CastToBP_CharacterNpcMelee (Pawn|GetControlledPawn)))
        (Default|BecameAggro _asbp_character_npc_melee)
        (Default|SetRunSpeed00 (Variables|Default|GetAs%20BP%20Character%20Npc%20Melee))
        (return)
        (else
          (return)))
      (else
        (return)))))

(fn GiveAggro
  (AI|Components|Blackboard|SetValueasBool (Variables|Default|GetBlackboard%20Component) (Utilities|Name|MakeLiteralName "IsAggresive") true)
  (return))

(fn MeleeAttackFunction
  (params (BoolValue :type Boolean))
  (AI|Components|Blackboard|SetValueasBool (Variables|Default|GetBlackboard%20Component) (Utilities|Name|MakeLiteralName "InRangeAttackMelee") BoolValue)
  (return))