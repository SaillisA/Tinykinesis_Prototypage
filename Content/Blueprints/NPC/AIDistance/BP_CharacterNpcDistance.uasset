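; Ranged NPC character that detects the player, aims at them and works with its AI controller, BP_AIC_NpcDistance.
; On BeginPlay it hides its shield and binds to the controller's health component for death; the damage feedback handler is empty.
; Tick yaws the Lance toward the player when LookPlayer is set and triggers aggro within RangeDetection, notifying controller and parent.
; Tick also clears the overlay material unless it is the telekinesis target's outline.
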(event Custom|Death_NpcDistance
  (CallFunction|DeathNpc))

(event Custom|DamageFeedbacks_NpcDistance)

(event EventBeginPlay
  ;[0.298 1 0.5765] BeginPlay
  (CallFunction|HideShowShield false)
  (bind _asbp_aic_npc_distance (Utilities|Casting|CastToBP_AIC_NpcDistance (Components|GetOwner)))
  (EventDispatchers|BindEventtoDeath (Variables|/Game/Blueprints/NPC/AIDistance/BP_AIC_NpcDistance.BP_AIC_NpcDistance_C|GetBP_AC_HealthAI _asbp_aic_npc_distance) (EventDispatchers|CreateEvent :!event Custom|Death_NpcDistance))
  (EventDispatchers|BindEventtoDamageFeedback (Variables|/Game/Blueprints/NPC/AIDistance/BP_AIC_NpcDistance.BP_AIC_NpcDistance_C|GetBP_AC_HealthAI _asbp_aic_npc_distance) (EventDispatchers|CreateEvent :!event Custom|DamageFeedbacks_NpcDistance)))

(event EventTick
  (params (DeltaSeconds :type Float%20%28single-precision%29))
  ;[0.7412 1 0.3412] EventTick
  (Utilities|FlowControl|Sequence
    (:then_0
      (if (Variables|Default|GetLookPlayer)
        (CallFunction|RotationLauncherBullets))
      (if (not (Variables|Default|GetIsAggro))
        (if (<= (Transformation|GetDistanceTo (Game|GetPlayerCharacter 0)) (Variables|Default|GetRangeDetection))
          (CallFunction|BecameAggro))))
    (:then_1
      (if (not (and (== (Rendering|Material|GetOverlayMaterial (Variables|Character|GetMesh) :!class /Script/Engine.MeshComponent) "/Game/Materials/M_OutlineTarget.M_OutlineTarget") (== (Variables|/Game/Blueprints/ActorComponents/PlayerAbilities/BP_AC_Telekinesis.BP_AC_Telekinesis_C|GetActualTarget (Variables|/Game/Blueprints/Player/BP_TinykinesisPlayerController.BP_TinykinesisPlayerController_C|GetBP_AC_Telekinesis (CallFunction|GetTinykinesisPlayerController))) self)))
        (Rendering|Material|SetOverlayMaterial (Variables|Character|GetMesh) 0 :!class /Script/Engine.MeshComponent)))))

(fn ConstructionScript)

(fn BecameAggro
  (bind _asbp_aic_npc_distance (Utilities|Casting|CastToBP_AIC_NpcDistance (Components|GetOwner)))
  (Default|GiveAggro _asbp_aic_npc_distance)
  (|CallParentFunction)
  (return))

(fn HideShowShield
  (params (Show :type Boolean))
  (Rendering|SetVisibility (Variables|Default|GetShield) Show true)
  (return))

(fn RotationLauncherBullets
  (bind _returnvalue (Game|GetPlayerCharacter 0))
  (bind _returnvalue_2 (Transformation|GetActorLocation))
  (bind _returnvalue_3 (Transformation|GetActorLocation _returnvalue))
  (bind _returnvalue_4 (Math|Rotator|FindLookatRotation _returnvalue_2 _returnvalue_3))
  (Transformation|SetWorldRotation (Variables|Default|GetLance) (Math|Rotator|MakeRotator (.roll _returnvalue_4) 0.0 (+ (.yaw _returnvalue_4) -9e+01)) false false)
  (return))