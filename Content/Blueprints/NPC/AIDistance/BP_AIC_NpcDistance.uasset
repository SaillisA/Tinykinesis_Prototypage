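; AI controller for the ranged (distance) NPC, running BT_NpcDistance with BB_NpcDistance and seeding the player target and ball spawn vector at BeginPlay.
; Sight of the player sets IsAggressive if not already aggroed, then calls BecameAggro through a cast to the melee NPC class.
; Tick copies the blackboard's IsReloading into the pawn's ImmunityAfterDamage.
; Helper functions force aggro or restart behavior tree logic.
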(event OnTargetPerceptionUpdated(AIPerception)
  (params (Actor :type Actor%20Object%20Reference) (Stimulus :type AI%20Stimulus%20Structure))
  (CallFunction|SeePlayer Actor Stimulus))

(event Custom|BeginPlay_AICNpcDistance
  ;[0.298 1 0.5765] BeginPlay
  (Variables|Default|SetCanRunTick true)
  (AI|RunBehaviorTree "/Game/Blueprints/NPC/AIDistance/BT_NpcDistance.BT_NpcDistance")
  (bind _blackboardcomponent (Class|AIController|UseBlackboard "/Game/Blueprints/NPC/AIDistance/BB_NpcDistance.BB_NpcDistance"))
  (bind _output_get (Variables|Default|SetBlackboard%20Component _blackboardcomponent))
  (bind _asbp_character_npc_distance (Utilities|Casting|CastToBP_CharacterNpcDistance (Pawn|GetControlledPawn)))
  (Variables|Default|SetAs%20BP%20Character%20Npc%20Distance _asbp_character_npc_distance)
  (AI|Components|Blackboard|SetValueasObject _output_get (Utilities|Name|MakeLiteralName "TargetPlayer") (CallFunction|GetTinykinesisPlayerCharacter))
  (AI|Components|Blackboard|SetValueasVector (Variables|Default|GetBlackboard%20Component) (Utilities|Name|MakeLiteralName "VectorSpawnBalls") "0, 0, 0"))

(event EventTick
  (params (DeltaSeconds :type Float%20%28single-precision%29))
  (if (Variables|Default|GetCanRunTick)
    (Variables|/Game/Blueprints/NPC/BP_AICharacterBlank.BP_AICharacterBlank_C|SetImmunityAfterDamage (Variables|Default|GetAs%20BP%20Character%20Npc%20Distance) (ScalableFloat|GetValueasBool (Variables|Default|GetBlackboard%20Component) (Utilities|Name|MakeLiteralName "IsReloading")))))

(fn ConstructionScript)

(fn SeePlayer
  (params (Actor :type Actor%20Object%20Reference) (Stimuli :type AI%20Stimulus%20Structure))
  (bind _asbp_aicharacter_blank (Utilities|Casting|CastToBP_AICharacterBlank (Pawn|GetControlledPawn)))
  (if (not (Variables|/Game/Blueprints/NPC/BP_AICharacterBlank.BP_AICharacterBlank_C|GetIsAggro _asbp_aicharacter_blank))
    (bind _returnvalue (Class|AIPerceptionSystem|GetSenseClassforStimulus Stimuli))
    (if (== _returnvalue "/Script/AIModule.AISense_Sight")
      (if (== Actor (Game|GetPlayerCharacter 0))
        (AI|Components|Blackboard|SetValueasBool (Variables|Default|GetBlackboard%20Component) (Utilities|Name|MakeLiteralName "IsAggressive") true)
        (bind _asbp_character_npc_melee (Utilities|Casting|CastToBP_CharacterNpcMelee (Pawn|GetControlledPawn)))
        (Default|BecameAggro _asbp_character_npc_melee)
        (return)
        (else
          (return)))
      (else
        (return)))))

(fn GiveAggro
  (AI|Components|Blackboard|SetValueasBool (Variables|Default|GetBlackboard%20Component) (Utilities|Name|MakeLiteralName "IsAggressive") true)
  (return))

(fn FunctionReload
  (Class|BrainComponent|RestartLogic (Variables|Default|GetBrainComponent))
  (return))