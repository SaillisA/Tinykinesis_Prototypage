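; Actor component that holds an unfinished or disabled player dash, with the IA_Dash input event left unwired.
; Its disconnected logic zeroes ground friction and gravity, then launches the Tinykinesis character horizontally along its normalized velocity.
; After a short delay, it applies a slightly weaker reverse launch as a brake and restores friction and gravity.
; A stray StopMovementImmediately call and a CanDash read are also unconnected, so nothing in the graph runs.
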(event Input|EnhancedActionEvents|EnhancedInputActionIA_Dash
  (params (ActionValue :type Boolean) (ElapsedSeconds :type Float%20%28double-precision%29) (TriggeredSeconds :type Float%20%28double-precision%29) (InputAction :type Input%20Action%20Object%20Reference :default "/Game/Blueprints/Player/Input/Actions/IA_Dash.IA_Dash")))

(event EventBeginPlay)

(event EventTick
  (params (DeltaSeconds :type Float%20%28single-precision%29)))