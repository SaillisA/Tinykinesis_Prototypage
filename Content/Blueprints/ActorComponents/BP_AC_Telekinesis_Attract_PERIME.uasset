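; Actor component for the player's telekinesis grab and attract power, marked PERIME (outdated) in its name.
; Grab input sends a grab message to the controller's LockedItem and briefly flags ActivatePower.
; Releasing the attract input blocks power use for a short cooldown.
; The attract logic itself (animation, AttractMessage toward character grab points, UI prompts, capacity use) is disconnected and never runs.
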(event Input|EnhancedActionEvents|EnhancedInputActionIA_GrabItem
  (params (ActionValue :type Boolean) (ElapsedSeconds :type Float%20%28double-precision%29) (TriggeredSeconds :type Float%20%28double-precision%29) (InputAction :type Input%20Action%20Object%20Reference :default "/Game/Blueprints/Player/Input/Actions/IA_GrabItem.IA_GrabItem"))
  (bind _tinykinesisplayercontroller (CallFunction|GetTinykinesisPlayerController))
  (:Triggered
    (if (Utilities|IsValid (Variables|/Game/Blueprints/Player/BP_TinykinesisPlayerController.BP_TinykinesisPlayerController_C|GetLockedItem _tinykinesisplayercontroller))
      (Class|BPIInteractable|GrabObject(Message) (Variables|/Game/Blueprints/Player/BP_TinykinesisPlayerController.BP_TinykinesisPlayerController_C|GetLockedItem (CallFunction|GetTinykinesisPlayerController)))))
  (:Started
    (Variables|/Game/Blueprints/Player/BP_TinykinesisPlayerController.BP_TinykinesisPlayerController_C|SetActivatePower _tinykinesisplayercontroller true)
    (Utilities|FlowControl|Delay 0.2)
    (Variables|/Game/Blueprints/Player/BP_TinykinesisPlayerController.BP_TinykinesisPlayerController_C|SetActivatePower _tinykinesisplayercontroller false)))

(event Input|EnhancedActionEvents|EnhancedInputActionIA_Attract_PERIME
  (params (ActionValue :type Boolean) (ElapsedSeconds :type Float%20%28double-precision%29) (TriggeredSeconds :type Float%20%28double-precision%29) (InputAction :type Input%20Action%20Object%20Reference :default "/Game/Blueprints/Player/Input/Actions/IA_Attract_PERIME.IA_Attract_PERIME"))
  (:Completed
    (Variables|/Game/Blueprints/Player/BP_TinykinesisPlayerController.BP_TinykinesisPlayerController_C|SetCanUsePower (CallFunction|GetTinykinesisPlayerController) false)
    (Utilities|FlowControl|Delay 1.0)
    (Variables|/Game/Blueprints/Player/BP_TinykinesisPlayerController.BP_TinykinesisPlayerController_C|SetCanUsePower (CallFunction|GetTinykinesisPlayerController) true)))