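; Actor component that makes its owner's static mesh a telekinesis object that can be levitated, attracted, thrown or smashed down.
; Levitate lifts the mesh without gravity, while AttractPERIME disables collision responses and moves it unless levitating.
; PropulsePERIME restores blocking, then moves the mesh to a locked target or launches it by impulse.
; A hit-style handler destroys the owner after a short delay when thrown or flagged as smashed.
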(event Custom|CustomEvent_2
  (params (MyComp :type Primitive%20Component%20Object%20Reference) (Other :type Actor%20Object%20Reference) (OtherComp :type Primitive%20Component%20Object%20Reference) (bSelfMoved :type Boolean) (HitLocation :type Vector) (HitNormal :type Vector) (NormalImpulse :type Vector) (Hit :type Hit%20Result%20Structure%20%28by%20ref%29))
  (Utilities|FlowControl|Sequence
    (:then_0
      (if (Variables|Default|GetGetting%20Smashed)
        (Utilities|FlowControl|Delay 0.2)
        (Actor|DestroyActor (Components|GetOwner))
        (Variables|Default|SetIs%20Levitating false)))
    (:then_1
      (if (Variables|Default|GetIs%20Thrown)
        (Utilities|FlowControl|Delay 0.2)
        (Actor|DestroyActor (Components|GetOwner))
        (else
          (Components|MoveComponentTo (Variables|Default|GetUsableMesh) (stale EventAttractPERIME Player%20Location%20R) "0, 0, 0" false false 0.1 false) ; enters at Stop
        )))))

(event EventSmash
  (Physics|SetEnableGravity (Variables|Default|GetUsableMesh) true)
  (Physics|AddImpulse (Variables|Default|GetUsableMesh) "0.000000,0.000000,-2600.000000" "None" true)
  (Variables|Default|SetGetting%20Smashed false))

(event EventPropulsePERIME
  (params (TargetLocation :type Vector :default "0, 0, 0") (PropulseLocation :type Vector :default "0, 0, 0") (TargetLocked? :type Boolean))
  (bind _usablemesh (Variables|Default|GetUsableMesh))
  (if (Variables|Default|GetCan%20be%20Thrown)
    (if TargetLocked?
      (Collision|SetCollisionResponsetoAllChannels (Variables|Default|GetUsableMesh) "ECR_Block")
      (Variables|Default|SetIs%20Thrown true)
      (Components|MoveComponentTo _usablemesh (+ TargetLocation 5e+01) "0, 0, 0" false false 0.15 false)
      (Physics|SetEnableGravity (Variables|Default|GetUsableMesh) true)
      (else
        (Collision|SetCollisionResponsetoAllChannels (Variables|Default|GetUsableMesh) "ECR_Block")
        (Physics|SetPhysicsLinearVelocity _usablemesh "0, 0, 0" false "None")
        (Physics|AddImpulse (Variables|Default|GetUsableMesh) (* PropulseLocation 5500) "None" true)
        (Physics|SetEnableGravity (Variables|Default|GetUsableMesh) true)
        (Variables|Default|SetIs%20Thrown true)))))

(event EventLevitate
  (bind _returnvalue (Components|GetOwner))
  (bind _returnvalue_2 (Transformation|GetActorLocation _returnvalue))
  (Class|PrimitiveComponent|SetAllPhysicsLinearVelocity (Variables|Default|GetUsableMesh) "0, 0, 0" false)
  (Components|MoveComponentTo (Variables|Default|GetUsableMesh) (Math|Vector|MakeVector (.x _returnvalue_2) (.y _returnvalue_2) (+ (.z _returnvalue_2) 1e+02)) "0, 0, 0" false false 0.2 false)
  (Variables|Default|SetIs%20Levitating true)
  (Physics|SetEnableGravity (Variables|Default|GetUsableMesh) false))

(event EventGrabObject
  (Variables|Default|SetCan%20be%20Thrown true))

(event EventAttractPERIME
  (params (Player%20Location%20R :type Vector :default "0, 0, 0") (Player%20Location%20Front :type Vector :default "0, 0, 0") (PlayerHit :type Boolean))
  (if (not (Variables|Default|GetIs%20Levitating))
    (Variables|Default|SetCan%20be%20Thrown true)
    (Collision|SetCollisionResponsetoAllChannels (Variables|Default|GetUsableMesh) "ECR_Ignore")
    (Components|MoveComponentTo (Variables|Default|GetUsableMesh) Player%20Location%20R "0, 0, 0" false false 0.1 false)))

(event EventBeginPlay
  (bind _returnvalue (Components|GetOwner))
  (bind _returnvalue_2 (Actor|GetComponentbyClass _returnvalue "/Script/Engine.StaticMeshComponent"))
  (Development|PrintString (Utilities|GetDisplayName _returnvalue_2))
  (Variables|Default|SetUsableMesh _returnvalue_2))