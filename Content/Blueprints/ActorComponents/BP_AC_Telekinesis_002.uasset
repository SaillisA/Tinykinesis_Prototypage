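; Player telekinesis component that attracts and propels "Light" objects, and levitates then smashes "Heavy" ones.
; It reads the controller's locked item and target, messages that item, and drives character animations, camera shake and input prompts.
; Hold input acts while triggered and launches or smashes on release; tap input toggles instead, with Tick pulling the grabbed item.
; CanUsePower, short delays and DoOnce gates enforce cooldowns and single levitation triggers.
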(event Input|EnhancedActionEvents|EnhancedInputActionIA_Telekinesis
  (params (ActionValue :type Boolean) (ElapsedSeconds :type Float%20%28double-precision%29) (TriggeredSeconds :type Float%20%28double-precision%29) (InputAction :type Input%20Action%20Object%20Reference :default "/Game/Blueprints/Player/Input/Actions/IA_Telekinesis.IA_Telekinesis"))
  (bind _tinykinesisplayercontroller (CallFunction|GetTinykinesisPlayerController))
  (bind _tinykinesisplayercontroller_2 (CallFunction|GetTinykinesisPlayerController))
  (bind _tinykinesisplayercontroller_3 (CallFunction|GetTinykinesisPlayerController))
  (bind _tinykinesisplayercontroller_4 (CallFunction|GetTinykinesisPlayerController))
  (bind _tinykinesisplayercontroller_5 (CallFunction|GetTinykinesisPlayerController))
  (bind _tinykinesisplayercontroller_6 (CallFunction|GetTinykinesisPlayerController))
  (:Triggered
    (Utilities|IsValid (Variables|/Game/Blueprints/Player/BP_TinykinesisPlayerController.BP_TinykinesisPlayerController_C|GetLockedItem _tinykinesisplayercontroller)
      (:Is%20Valid
        (if (Variables|/Game/Blueprints/Player/BP_TinykinesisPlayerController.BP_TinykinesisPlayerController_C|GetCanUsePower (CallFunction|GetTinykinesisPlayerController))
          (if (Actor|ActorHasTag (Variables|/Game/Blueprints/Player/BP_TinykinesisPlayerController.BP_TinykinesisPlayerController_C|GetLockedItem _tinykinesisplayercontroller) "Light")
            (if (!= (Variables|/Game/Blueprints/Player/BP_TinykinesisPlayerController.BP_TinykinesisPlayerController_C|GetLockedItem _tinykinesisplayercontroller_4) (Variables|/Game/Blueprints/Player/BP_TinykinesisPlayerController.BP_TinykinesisPlayerController_C|GetEmptyItem _tinykinesisplayercontroller_4))
              (Camera|PlayWorldCameraShake "/Game/Blueprints/Actors/BP_PowerCameraShake.BP_PowerCameraShake_C" (Transformation|GetActorLocation (CallFunction|GetTinykinesisPlayerCharacter)) 0.0 5e+02)
              (if (Variables|/Game/Blueprints/Player/BP_TinykinesisPlayerController.BP_TinykinesisPlayerController_C|GetCanUsePower _tinykinesisplayercontroller_4)
                (OldFunctions|AttractObject)
                (Variables|Default|SetIsAttracted true)
                (OldFunctions|SetAttractionUsage))
              (else
                (Variables|/Game/Blueprints/Player/BP_TinykinesisPlayerController.BP_TinykinesisPlayerController_C|SetUsingPower _tinykinesisplayercontroller_4 false)))
            (elif (Actor|ActorHasTag (Variables|/Game/Blueprints/Player/BP_TinykinesisPlayerController.BP_TinykinesisPlayerController_C|GetLockedItem _tinykinesisplayercontroller) "Heavy")
              (OldFunctions|UseLevitate)
              (Camera|PlayWorldCameraShake "/Game/Blueprints/Actors/BP_PowerCameraShake.BP_PowerCameraShake_C" (Transformation|GetActorLocation (CallFunction|GetTinykinesisPlayerCharacter)) 0.0 5e+02)
              (Utilities|FlowControl|DoOnce false :!label _label
                (:Completed
                  (Class|BPISmash|Levitate(Message) (Variables|/Game/Blueprints/Player/BP_TinykinesisPlayerController.BP_TinykinesisPlayerController_C|GetLockedItem _tinykinesisplayercontroller_3))
                  (Variables|Default|SetIsLevitating true)
                  (Variables|/Game/Blueprints/Player/BP_TinykinesisPlayerController.BP_TinykinesisPlayerController_C|SetUsingPower _tinykinesisplayercontroller_3 true)))))))
      (:Is%20Not%20Valid
        (Utilities|IsValid (Variables|Default|GetItemGrabbed)
          (:Is%20Valid
            (Variables|/Game/Blueprints/Player/BP_TinykinesisPlayerController.BP_TinykinesisPlayerController_C|SetLockedItem _tinykinesisplayercontroller_6 (Variables|Default|GetItemGrabbed))
            (Variables|Default|SetItemGrabbed (Variables|/Game/Blueprints/Player/BP_TinykinesisPlayerController.BP_TinykinesisPlayerController_C|GetEmptyItem _tinykinesisplayercontroller_6))
            (Variables|Default|SetAttracting false))))))
  (:Completed
    (Utilities|IsValid (Variables|/Game/Blueprints/Player/BP_TinykinesisPlayerController.BP_TinykinesisPlayerController_C|GetLockedItem (CallFunction|GetTinykinesisPlayerController))
      (:Is%20Valid
        (if (Actor|ActorHasTag (Variables|/Game/Blueprints/Player/BP_TinykinesisPlayerController.BP_TinykinesisPlayerController_C|GetLockedItem (CallFunction|GetTinykinesisPlayerController)) "Heavy")
          (OldFunctions|UseSmash)
          (Utilities|FlowControl|Delay 0.5)
          (Default|Animation (CallFunction|GetTinykinesisPlayerCharacter) "NewEnumerator6")
          (Utilities|FlowControl|Sequence
            (:then_0
              (Utilities|FlowControl|DoOnce false) ; enters at Reset
            )
            (:then_1
              (goto _label Reset))
            (:then_2
              (Variables|/Game/Blueprints/Player/BP_TinykinesisPlayerController.BP_TinykinesisPlayerController_C|SetCanUsePower (CallFunction|GetTinykinesisPlayerController) false)
              (Utilities|FlowControl|Delay 1.0)
              (Variables|/Game/Blueprints/Player/BP_TinykinesisPlayerController.BP_TinykinesisPlayerController_C|SetCanUsePower (CallFunction|GetTinykinesisPlayerController) true)))
          (elif (and (Actor|ActorHasTag (Variables|/Game/Blueprints/Player/BP_TinykinesisPlayerController.BP_TinykinesisPlayerController_C|GetLockedItem _tinykinesisplayercontroller_5) "Light") (Variables|/Game/Blueprints/Player/BP_TinykinesisPlayerController.BP_TinykinesisPlayerController_C|GetCanUsePower _tinykinesisplayercontroller_5))
            (OldFunctions|PropulseObject)
            (OldFunctions|UsedPropulse)
            (Utilities|FlowControl|Delay 0.5)
            (Default|Animation (CallFunction|GetTinykinesisPlayerCharacter) "NewEnumerator6")
            (Variables|/Game/Blueprints/Player/BP_TinykinesisPlayerController.BP_TinykinesisPlayerController_C|SetCanUsePower _tinykinesisplayercontroller_2 false)
            (Utilities|FlowControl|Delay 0.5)
            (Variables|/Game/Blueprints/Player/BP_TinykinesisPlayerController.BP_TinykinesisPlayerController_C|SetCanUsePower _tinykinesisplayercontroller_2 true)))))))

(event Input|EnhancedActionEvents|EnhancedInputActionIA_TelekinesisTap
  (params (ActionValue :type Boolean) (ElapsedSeconds :type Float%20%28double-precision%29) (TriggeredSeconds :type Float%20%28double-precision%29) (InputAction :type Input%20Action%20Object%20Reference :default "/Game/Blueprints/Player/Input/Actions/IA_TelekinesisTap.IA_TelekinesisTap"))
  (bind _tinykinesisplayercontroller (CallFunction|GetTinykinesisPlayerController))
  (bind _tinykinesisplayercharacter (CallFunction|GetTinykinesisPlayerCharacter))
  (bind _tinykinesisplayercontroller_2 (CallFunction|GetTinykinesisPlayerController))
  (bind _tinykinesisplayercontroller_3 (CallFunction|GetTinykinesisPlayerController))
  (bind _tinykinesisplayercontroller_4 (CallFunction|GetTinykinesisPlayerController))
  (bind _lockeditem (Variables|/Game/Blueprints/Player/BP_TinykinesisPlayerController.BP_TinykinesisPlayerController_C|GetLockedItem _tinykinesisplayercontroller_2))
  (bind _lockeditem_2 (Variables|/Game/Blueprints/Player/BP_TinykinesisPlayerController.BP_TinykinesisPlayerController_C|GetLockedItem _tinykinesisplayercontroller_4))
  (Utilities|IsValid (Variables|Default|GetItemGrabbed)
    (:Is%20Valid
      (Development|PrintString "stop")
      (Variables|Default|SetAttracting false)
      (Default|Animation (CallFunction|GetTinykinesisPlayerCharacter) "NewEnumerator2")
      (bind _output_get (Variables|/Game/Blueprints/Player/BP_TinykinesisPlayerController.BP_TinykinesisPlayerController_C|SetTargetLocation _tinykinesisplayercontroller (Math|Vector|MakeVector (.X (Math|Vector|BreakVector (Variables|/Game/Blueprints/Player/BP_TinykinesisPlayerController.BP_TinykinesisPlayerController_C|GetTargetLocation _tinykinesisplayercontroller))) (.Y (Math|Vector|BreakVector (Variables|/Game/Blueprints/Player/BP_TinykinesisPlayerController.BP_TinykinesisPlayerController_C|GetTargetLocation _tinykinesisplayercontroller))) (+ (.Z (Math|Vector|BreakVector (Variables|/Game/Blueprints/Player/BP_TinykinesisPlayerController.BP_TinykinesisPlayerController_C|GetTargetLocation _tinykinesisplayercontroller))) 1e+01))))
      (Class|BPITelekinesisObject|Propulse(Message) (Variables|Default|GetItemGrabbed) _output_get (Math|Vector|GetForwardVector (Variables|/Game/Blueprints/Player/BP_TinykinesisPlayerCharacter.BP_TinykinesisPlayerCharacter_C|GetGrabPointR (CallFunction|GetTinykinesisPlayerCharacter))) (Variables|/Game/Blueprints/Player/BP_TinykinesisPlayerController.BP_TinykinesisPlayerController_C|GetHasTarget (CallFunction|GetTinykinesisPlayerController)))
      (Variables|Default|SetItemGrabbed (Variables|/Game/Blueprints/Player/BP_TinykinesisPlayerController.BP_TinykinesisPlayerController_C|GetEmptyItem (CallFunction|GetTinykinesisPlayerController)))
      (Utilities|FlowControl|Delay 0.5)
      (Default|Animation (CallFunction|GetTinykinesisPlayerCharacter) "NewEnumerator6"))
    (:Is%20Not%20Valid
      (Utilities|IsValid _lockeditem
        (:Is%20Valid
          (if (Variables|/Game/Blueprints/Player/BP_TinykinesisPlayerController.BP_TinykinesisPlayerController_C|GetCanUsePower _tinykinesisplayercontroller_2)
            (if (Actor|ActorHasTag _lockeditem "Light")
              (Development|PrintString "Hello")
              (Variables|Default|SetAttracting true)
              (Variables|Default|SetItemGrabbed _lockeditem)
              (Variables|Default|SetIsAttracted true)
              (OldFunctions|SetAttractionUsage)
              (elif (Actor|ActorHasTag _lockeditem "Heavy")
                (if (Variables|Default|GetIsLevitating)
                  (OldFunctions|UseSmash)
                  (Utilities|FlowControl|Delay 0.5)
                  (Default|Animation (CallFunction|GetTinykinesisPlayerCharacter) "NewEnumerator6")
                  (Utilities|FlowControl|Sequence
                    (:then_0
                      (Variables|/Game/Blueprints/Player/BP_TinykinesisPlayerController.BP_TinykinesisPlayerController_C|SetCanUsePower (CallFunction|GetTinykinesisPlayerController) false)
                      (Utilities|FlowControl|Delay 1.0)
                      (Variables|/Game/Blueprints/Player/BP_TinykinesisPlayerController.BP_TinykinesisPlayerController_C|SetCanUsePower (CallFunction|GetTinykinesisPlayerController) true))
                    (:then_1
                      (goto _label Reset)))
                  (else
                    (Development|PrintString "Levitate")
                    (Default|Animation _tinykinesisplayercharacter "NewEnumerator1")
                    (Default|PlayHoldLevite _tinykinesisplayercharacter)
                    (if (and (Utilities|IsValid _lockeditem_2) (not (Variables|/Game/Blueprints/Player/BP_TinykinesisPlayerController.BP_TinykinesisPlayerController_C|GetGotHit _tinykinesisplayercontroller_4)))
                      (Variables|/Game/Blueprints/Player/BP_TinykinesisPlayerController.BP_TinykinesisPlayerController_C|SetUsingPower _tinykinesisplayercontroller_3 true)
                      (Default|UsedCapacity _tinykinesisplayercontroller_3)
                      (Camera|PlayWorldCameraShake "/Game/Blueprints/Actors/BP_PowerCameraShake.BP_PowerCameraShake_C" (Transformation|GetActorLocation (CallFunction|GetTinykinesisPlayerCharacter)) 0.0 5e+02)
                      (Utilities|FlowControl|DoOnce false :!label _label
                        (:Completed
                          (Class|BPISmash|Levitate(Message) (Variables|/Game/Blueprints/Player/BP_TinykinesisPlayerController.BP_TinykinesisPlayerController_C|GetLockedItem (CallFunction|GetTinykinesisPlayerController)))
                          (Variables|Default|SetIsLevitating true)
                          (Variables|/Game/Blueprints/Player/BP_TinykinesisPlayerController.BP_TinykinesisPlayerController_C|SetUsingPower (CallFunction|GetTinykinesisPlayerController) true)))
                      (else
                        (Class|BPISmash|CancelLevitation(Message) _lockeditem_2)))))))))))))

(event EventTick
  (params (DeltaSeconds :type Float%20%28single-precision%29))
  (bind _tinykinesisplayercharacter (CallFunction|GetTinykinesisPlayerCharacter))
  (Utilities|IsValid (Variables|Default|GetItemGrabbed)
    (:Is%20Valid
      (if (Variables|Default|GetAttracting)
        (Variables|/Game/Blueprints/Player/BP_TinykinesisPlayerController.BP_TinykinesisPlayerController_C|SetUsingPower (CallFunction|GetTinykinesisPlayerController) true)
        (Default|Animation _tinykinesisplayercharacter "NewEnumerator0")
        (Default|PlayHoldAttract _tinykinesisplayercharacter)
        (Class|BPITelekinesisObject|Attract(Message) (Variables|Default|GetItemGrabbed) (Transformation|GetWorldLocation (Variables|/Game/Blueprints/Player/BP_TinykinesisPlayerCharacter.BP_TinykinesisPlayerCharacter_C|GetGrabPointR (CallFunction|GetTinykinesisPlayerCharacter))) "0, 0, 0" false)))))

(fn AttractObject
  (bind _tinykinesisplayercontroller (CallFunction|GetTinykinesisPlayerController))
  (bind _tinykinesisplayercharacter (CallFunction|GetTinykinesisPlayerCharacter))
  (bind _tinykinesisplayercharacter_2 (CallFunction|GetTinykinesisPlayerCharacter))
  (bind _lockeditem (Variables|/Game/Blueprints/Player/BP_TinykinesisPlayerController.BP_TinykinesisPlayerController_C|GetLockedItem _tinykinesisplayercontroller))
  (Variables|/Game/Blueprints/Player/BP_TinykinesisPlayerController.BP_TinykinesisPlayerController_C|SetUsingPower (CallFunction|GetTinykinesisPlayerController) true)
  (Default|Animation _tinykinesisplayercharacter_2 "NewEnumerator0")
  (Default|PlayHoldAttract _tinykinesisplayercharacter_2)
  (if (Utilities|IsValid _lockeditem)
    (Class|BPITelekinesisObject|Attract(Message) _lockeditem (Transformation|GetWorldLocation (Variables|/Game/Blueprints/Player/BP_TinykinesisPlayerCharacter.BP_TinykinesisPlayerCharacter_C|GetGrabPointR _tinykinesisplayercharacter)) (Transformation|GetWorldLocation (Variables|/Game/Blueprints/Player/BP_TinykinesisPlayerCharacter.BP_TinykinesisPlayerCharacter_C|GetGrabPointFront _tinykinesisplayercharacter)) (Variables|/Game/Blueprints/Player/BP_TinykinesisPlayerController.BP_TinykinesisPlayerController_C|GetGotHit _tinykinesisplayercontroller))
    (Variables|/Game/Blueprints/Player/BP_TinykinesisPlayerController.BP_TinykinesisPlayerController_C|SetCharging (CallFunction|GetTinykinesisPlayerController) true)))

(fn SetAttractionUsage
  (bind _tinykinesisplayercontroller (CallFunction|GetTinykinesisPlayerController))
  (bind _tinykinesisplayercontroller_2 (CallFunction|GetTinykinesisPlayerController))
  (Default|ShowInput _tinykinesisplayercontroller)
  (Default|ChangeTextInput _tinykinesisplayercontroller "Release")
  (Default|ShowInputLeft _tinykinesisplayercontroller)
  (Variables|/Game/Blueprints/Player/BP_TinykinesisPlayerController.BP_TinykinesisPlayerController_C|SetUsesTelekinesis (CallFunction|GetTinykinesisPlayerController) true)
  (Variables|/Game/Blueprints/Player/BP_TinykinesisPlayerController.BP_TinykinesisPlayerController_C|SetUsingPower _tinykinesisplayercontroller_2 true)
  (Default|UsedCapacity _tinykinesisplayercontroller_2))

(fn UseLevitate
  (bind _tinykinesisplayercharacter (CallFunction|GetTinykinesisPlayerCharacter))
  (bind _tinykinesisplayercontroller (CallFunction|GetTinykinesisPlayerController))
  (bind _tinykinesisplayercontroller_2 (CallFunction|GetTinykinesisPlayerController))
  (bind _lockeditem (Variables|/Game/Blueprints/Player/BP_TinykinesisPlayerController.BP_TinykinesisPlayerController_C|GetLockedItem _tinykinesisplayercontroller_2))
  (Default|Animation _tinykinesisplayercharacter "NewEnumerator1")
  (Default|PlayHoldLevite _tinykinesisplayercharacter)
  (if (and (Utilities|IsValid _lockeditem) (not (Variables|/Game/Blueprints/Player/BP_TinykinesisPlayerController.BP_TinykinesisPlayerController_C|GetGotHit _tinykinesisplayercontroller_2)))
    (Variables|/Game/Blueprints/Player/BP_TinykinesisPlayerController.BP_TinykinesisPlayerController_C|SetUsingPower _tinykinesisplayercontroller true)
    (Default|UsedCapacity _tinykinesisplayercontroller)
    (else
      (Class|BPISmash|CancelLevitation(Message) _lockeditem))))

(fn PropulseObject
  (bind _tinykinesisplayercontroller (CallFunction|GetTinykinesisPlayerController))
  (bind _tinykinesisplayercontroller_2 (CallFunction|GetTinykinesisPlayerController))
  (if (and (Variables|/Game/Blueprints/Player/BP_TinykinesisPlayerController.BP_TinykinesisPlayerController_C|GetCanUsePower _tinykinesisplayercontroller_2) (Variables|/Game/Blueprints/Player/BP_TinykinesisPlayerController.BP_TinykinesisPlayerController_C|GetUsesTelekinesis _tinykinesisplayercontroller_2))
    (Default|Animation (CallFunction|GetTinykinesisPlayerCharacter) "NewEnumerator2")
    (bind _output_get (Variables|/Game/Blueprints/Player/BP_TinykinesisPlayerController.BP_TinykinesisPlayerController_C|SetTargetLocation (CallFunction|GetTinykinesisPlayerController) (Math|Vector|MakeVector (.X (Math|Vector|BreakVector (Variables|/Game/Blueprints/Player/BP_TinykinesisPlayerController.BP_TinykinesisPlayerController_C|GetTargetLocation (CallFunction|GetTinykinesisPlayerController)))) (.Y (Math|Vector|BreakVector (Variables|/Game/Blueprints/Player/BP_TinykinesisPlayerController.BP_TinykinesisPlayerController_C|GetTargetLocation (CallFunction|GetTinykinesisPlayerController)))) (+ (.Z (Math|Vector|BreakVector (Variables|/Game/Blueprints/Player/BP_TinykinesisPlayerController.BP_TinykinesisPlayerController_C|GetTargetLocation (CallFunction|GetTinykinesisPlayerController)))) 1e+01))))
    (Class|BPITelekinesisObject|Propulse(Message) (Variables|/Game/Blueprints/Player/BP_TinykinesisPlayerController.BP_TinykinesisPlayerController_C|GetLockedItem _tinykinesisplayercontroller) _output_get (Math|Vector|GetForwardVector (Variables|/Game/Blueprints/Player/BP_TinykinesisPlayerCharacter.BP_TinykinesisPlayerCharacter_C|GetGrabPointR (CallFunction|GetTinykinesisPlayerCharacter))) (Variables|/Game/Blueprints/Player/BP_TinykinesisPlayerController.BP_TinykinesisPlayerController_C|GetHasTarget _tinykinesisplayercontroller))
    (Variables|/Game/Blueprints/Player/BP_TinykinesisPlayerController.BP_TinykinesisPlayerController_C|SetCanUsePower (CallFunction|GetTinykinesisPlayerController) false)
    (Variables|Default|SetItemGrabbed (Variables|/Game/Blueprints/Player/BP_TinykinesisPlayerController.BP_TinykinesisPlayerController_C|GetEmptyItem (CallFunction|GetTinykinesisPlayerController)))))

(fn UsedPropulse
  (bind _tinykinesisplayercontroller (CallFunction|GetTinykinesisPlayerController))
  (Default|UsedCapacity _tinykinesisplayercontroller)
  (Variables|/Game/Blueprints/Player/BP_TinykinesisPlayerController.BP_TinykinesisPlayerController_C|SetUsingPower _tinykinesisplayercontroller false)
  (Default|HideInput (CallFunction|GetTinykinesisPlayerController))
  (Variables|/Game/Blueprints/Player/BP_TinykinesisPlayerController.BP_TinykinesisPlayerController_C|SetLockedItem _tinykinesisplayercontroller (Variables|/Game/Blueprints/Player/BP_TinykinesisPlayerController.BP_TinykinesisPlayerController_C|GetEmptyItem _tinykinesisplayercontroller)))

(fn UseSmash
  (bind _tinykinesisplayercontroller (CallFunction|GetTinykinesisPlayerController))
  (Default|Animation (CallFunction|GetTinykinesisPlayerCharacter) "NewEnumerator3")
  (Class|BPISmash|Smash(Message) (Variables|/Game/Blueprints/Player/BP_TinykinesisPlayerController.BP_TinykinesisPlayerController_C|GetLockedItem _tinykinesisplayercontroller))
  (Variables|/Game/Blueprints/Player/BP_TinykinesisPlayerController.BP_TinykinesisPlayerController_C|SetLockedItem _tinykinesisplayercontroller (Variables|/Game/Blueprints/Player/BP_TinykinesisPlayerController.BP_TinykinesisPlayerController_C|GetEmptyItem _tinykinesisplayercontroller))
  (Variables|/Game/Blueprints/Player/BP_TinykinesisPlayerController.BP_TinykinesisPlayerController_C|SetUsingPower _tinykinesisplayercontroller false)
  (Default|HideInput (CallFunction|GetTinykinesisPlayerController))
  (Variables|Default|SetIsLevitating false))

(fn CheckLockedItem
  (Utilities|IsValid (Variables|/Game/Blueprints/Player/BP_TinykinesisPlayerController.BP_TinykinesisPlayerController_C|GetLockedItem (CallFunction|GetTinykinesisPlayerController))))