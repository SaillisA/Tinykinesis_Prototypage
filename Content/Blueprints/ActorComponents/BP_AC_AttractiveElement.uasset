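; Actor component that lets an object be pulled to the player and thrown, for the Tinykinesis player controller's grab-and-throw mechanic.
; AttractObject disables physics and collision and slides the mesh to the player, or restores physics and resets selection if the player was hit.
; PropulseObject re-enables physics and collision, then either moves the mesh quickly to a locked target or launches it with a velocity-change impulse.
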(event Custom|PropulseObject
  (params (TargetLocation :type Vector) (PropulseLocation :type Vector) (TargetLocket? :type Boolean) (UsableMesh :type Primitive%20Component%20Object%20Reference))
  (Variables|Default|SetLocationBeforeThrown PropulseLocation)
  (if (Variables|Default|GetCanBeThrown)
    (Physics|SetSimulatePhysics UsableMesh true)
    (Collision|SetCollisionResponsetoAllChannels UsableMesh "ECR_Block")
    (if TargetLocket?
      (Variables|Default|SetIsThrown true)
      (Components|MoveComponentTo UsableMesh (+ TargetLocation 25.0) "0, 0, 0" false false 0.15 false)
      (else
        (Physics|SetPhysicsLinearVelocity UsableMesh "0, 0, 0" false "None")
        (Physics|AddImpulse UsableMesh (* PropulseLocation 5500) "None" true)
        (Variables|Default|SetIsThrown true)))
    (Physics|SetEnableGravity UsableMesh true)
    (Variables|Default|SetCanBeGrabbed false)
    (Variables|Default|SetCanBeThrown false)))

(event Custom|AttractObject
  (params (PlayerLocationR :type Vector) (PlayerHit :type Boolean) (UsableMesh :type Primitive%20Component%20Object%20Reference) (AimAssistCollision :type Sphere%20Component%20Object%20Reference) (Mesh :type Mesh%20Component%20Object%20Reference) (AttractSpeed :type Float%20%28double-precision%29))
  (Variables|Default|SetCanBeGrabbed true)
  (if (Variables|Default|GetCanBeGrabbed)
    (Variables|Default|SetIsThrown false)
    (Physics|SetSimulatePhysics UsableMesh true)
    (Physics|SetSimulatePhysics UsableMesh false)
    (Collision|SetCollisionResponsetoAllChannels AimAssistCollision "ECR_Ignore")
    (Variables|Default|SetCanBeThrown true)
    (Collision|SetCollisionResponsetoAllChannels UsableMesh "ECR_Ignore")
    (if (Variables|/Game/Blueprints/Player/BP_TinykinesisPlayerController.BP_TinykinesisPlayerController_C|GetGotHit (CallFunction|GetTinykinesisPlayerController))
      (Physics|SetEnableGravity Mesh true)
      (Physics|SetSimulatePhysics Mesh true)
      (Collision|SetCollisionResponsetoAllChannels Mesh "ECR_Block")
      (Default|ResetSelection (CallFunction|GetTinykinesisPlayerController))
      (else
        (Utilities|FlowControl|Sequence
          (:then_0
            (Components|MoveComponentTo UsableMesh PlayerLocationR "0, 0, 0" false false (* AttractSpeed 0.1) false)))))
    (else
      (Collision|SetCollisionResponsetoAllChannels UsableMesh "ECR_Block")
      (Variables|Default|SetCanBeThrown false)
      (Collision|SetCollisionResponsetoAllChannels UsableMesh "ECR_Block"))))