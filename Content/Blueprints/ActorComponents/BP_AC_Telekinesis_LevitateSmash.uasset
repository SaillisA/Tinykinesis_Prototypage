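; Actor component that handles the player's telekinesis Levitate and Smash input on the selected item.
; Levitate requires a valid item and no recent hit, flags power use, consumes capacity and sends a levitate message through a DoOnce, otherwise sending a cancel message.
; Smash works only while no power is in use, messaging the item, clearing the selection and re-arming the DoOnce.
; Selection and power state live on the Tinykinesis player controller.
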(event Input|EnhancedActionEvents|EnhancedInputActionIA_Levitate
  (params (ActionValue :type Boolean) (ElapsedSeconds :type Float%20%28double-precision%29) (TriggeredSeconds :type Float%20%28double-precision%29) (InputAction :type Input%20Action%20Object%20Reference :default "/Game/Blueprints/Player/Input/Actions/IA_Levitate.IA_Levitate"))
  (bind _tinykinesisplayercontroller (CallFunction|GetTinykinesisPlayerController))
  (bind _tinykinesisplayercontroller_2 (CallFunction|GetTinykinesisPlayerController))
  (bind _selecteditem (Variables|/Game/Blueprints/Player/BP_TinykinesisPlayerController.BP_TinykinesisPlayerController_C|GetSelectedItem _tinykinesisplayercontroller))
  (if (and (Utilities|IsValid _selecteditem) (not (Variables|/Game/Blueprints/Player/BP_TinykinesisPlayerController.BP_TinykinesisPlayerController_C|GetGotHit _tinykinesisplayercontroller)))
    (Variables|/Game/Blueprints/Player/BP_TinykinesisPlayerController.BP_TinykinesisPlayerController_C|SetUsingPower _tinykinesisplayercontroller_2 true)
    (Default|UsedCapacity _tinykinesisplayercontroller_2)
    (Utilities|FlowControl|DoOnce false
      (:Completed
        (Class|BPISmash|Levitate(Message) (Variables|/Game/Blueprints/Player/BP_TinykinesisPlayerController.BP_TinykinesisPlayerController_C|GetSelectedItem (CallFunction|GetTinykinesisPlayerController)))))
    (else
      (Class|BPISmash|CancelLevitation(Message) _selecteditem))))

(event Input|EnhancedActionEvents|EnhancedInputActionIA_Smash
  (params (ActionValue :type Boolean) (ElapsedSeconds :type Float%20%28double-precision%29) (TriggeredSeconds :type Float%20%28double-precision%29) (InputAction :type Input%20Action%20Object%20Reference :default "/Game/Blueprints/Player/Input/Actions/IA_Smash.IA_Smash"))
  (bind _tinykinesisplayercontroller (CallFunction|GetTinykinesisPlayerController))
  (if (and (Utilities|IsValid (Variables|/Game/Blueprints/Player/BP_TinykinesisPlayerController.BP_TinykinesisPlayerController_C|GetSelectedItem _tinykinesisplayercontroller)) (not (Variables|/Game/Blueprints/Player/BP_TinykinesisPlayerController.BP_TinykinesisPlayerController_C|GetUsingPower _tinykinesisplayercontroller)))
    (Class|BPISmash|Smash(Message) (Variables|/Game/Blueprints/Player/BP_TinykinesisPlayerController.BP_TinykinesisPlayerController_C|GetSelectedItem _tinykinesisplayercontroller))
    (Variables|/Game/Blueprints/Player/BP_TinykinesisPlayerController.BP_TinykinesisPlayerController_C|SetSelectedItem _tinykinesisplayercontroller (Variables|/Game/Blueprints/Player/BP_TinykinesisPlayerController.BP_TinykinesisPlayerController_C|GetEmptyItem _tinykinesisplayercontroller))
    (Variables|/Game/Blueprints/Player/BP_TinykinesisPlayerController.BP_TinykinesisPlayerController_C|SetUsingPower (CallFunction|GetTinykinesisPlayerController) false)
    (Utilities|FlowControl|DoOnce false) ; enters at Reset
  ))

(event EventBeginPlay)

(event EventTick
  (params (DeltaSeconds :type Float%20%28single-precision%29)))