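; Player telekinesis component that attracts and propels "Light" tagged objects and levitates and smashes "Heavy" ones.
; Hold, tap and unfinished V2 input actions act on the controller's LockedItem, sending interface messages to it and driving character animation, camera shake and cooldowns.
; Tick keeps a grabbed item attracted to the character's grab point.
; Power state lives on the player controller; comments plan to replace tag branching with Event Dispatchers.
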(event Input|EnhancedActionEvents|EnhancedInputActionIA_Telekinesis
  (params (ActionValue :type Boolean) (ElapsedSeconds :type Float%20%28double-precision%29) (TriggeredSeconds :type Float%20%28double-precision%29) (InputAction :type Input%20Action%20Object%20Reference :default "/Game/Blueprints/Player/Input/Actions/IA_Telekinesis.IA_Telekinesis"))
  (bind _tinykinesisplayercontroller (CallFunction|GetTinykinesisPlayerController))
  (bind _tinykinesisplayercontroller_2 (CallFunction|GetTinykinesisPlayerController))
  (bind _tinykinesisplayercontroller_3 (CallFunction|GetTinykinesisPlayerController))
  (bind _tinykinesisplayercontroller_4 (CallFunction|GetTinykinesisPlayerController))
  (bind _tinykinesisplayercontroller_5 (CallFunction|GetTinykinesisPlayerController))
  (bind _tinykinesisplayercontroller_6 (CallFunction|GetTinykinesisPlayerController))
  (bind _tinykinesisplayercontroller_7 (CallFunction|GetTinykinesisPlayerController))
  (:Triggered
    (Utilities|IsValid (Variables|/Game/Blueprints/Player/BP_TinykinesisPlayerController.BP_TinykinesisPlayerController_C|GetLockedItem _tinykinesisplayercontroller_2)
      (:Is%20Valid
        (if (Variables|/Game/Blueprints/Player/BP_TinykinesisPlayerController.BP_TinykinesisPlayerController_C|GetCanUsePower (CallFunction|GetTinykinesisPlayerController))
          ;[1 0.02083 0.02083] Useless avec Event Dispatcher
          (if (Actor|ActorHasTag (Variables|/Game/Blueprints/Player/BP_TinykinesisPlayerController.BP_TinykinesisPlayerController_C|GetLockedItem _tinykinesisplayercontroller_2) "Light")
            (if (!= (Variables|/Game/Blueprints/Player/BP_TinykinesisPlayerController.BP_TinykinesisPlayerController_C|GetLockedItem _tinykinesisplayercontroller_7) (Variables|/Game/Blueprints/Player/BP_TinykinesisPlayerController.BP_TinykinesisPlayerController_C|GetEmptyItem _tinykinesisplayercontroller_7))
              ;[1 0.4323 0.4323] A decaler dans l'Event Dispatcher (Grab Item for Light  Object)
              (Camera|PlayWorldCameraShake "/Game/Blueprints/Actors/BP_PowerCameraShake.BP_PowerCameraShake_C" (Transformation|GetActorLocation (CallFunction|GetTinykinesisPlayerCharacter)) 0.0 5e+02)
              (if (Variables|/Game/Blueprints/Player/BP_TinykinesisPlayerController.BP_TinykinesisPlayerController_C|GetCanUsePower _tinykinesisplayercontroller_7)
                (OldFunctions|AttractObject)
                (OldFunctions|SetAttractionUsage)
                ;[1 0.3582 0.7407] A remplacer par new Variable
                (Variables|Default|SetIsAttracted true)
                (Variables|/Game/Blueprints/Player/BP_TinykinesisPlayerController.BP_TinykinesisPlayerController_C|SetUsesTelekinesis (CallFunction|GetTinykinesisPlayerController) true)
                (Variables|/Game/Blueprints/Player/BP_TinykinesisPlayerController.BP_TinykinesisPlayerController_C|SetUsingPower _tinykinesisplayercontroller_5 true)
                (Default|UsedCapacity _tinykinesisplayercontroller_5))
              (else
                (Variables|/Game/Blueprints/Player/BP_TinykinesisPlayerController.BP_TinykinesisPlayerController_C|SetUsingPower _tinykinesisplayercontroller_7 false)))
            (elif (Actor|ActorHasTag (Variables|/Game/Blueprints/Player/BP_TinykinesisPlayerController.BP_TinykinesisPlayerController_C|GetLockedItem _tinykinesisplayercontroller_2) "Heavy")
              ;[1 0.4323 0.4323] A decaler dans l'Event Dispatcher (Grab Item for Heavy Object)
              (OldFunctions|UseLevitate)
              (Camera|PlayWorldCameraShake "/Game/Blueprints/Actors/BP_PowerCameraShake.BP_PowerCameraShake_C" (Transformation|GetActorLocation (CallFunction|GetTinykinesisPlayerCharacter)) 0.0 5e+02)
              ;[1 0.4323 0.4323] A decaler dans l'Event Dispatcher (Grab Item for Heavy Object)
              (Utilities|FlowControl|DoOnce false :!label _label
                (:Completed
                  (Class|BPISmash|Levitate(Message) (Variables|/Game/Blueprints/Player/BP_TinykinesisPlayerController.BP_TinykinesisPlayerController_C|GetLockedItem _tinykinesisplayercontroller_3))
                  ;[1 0.3582 0.7407] A remplacer par new Variable
                  (Variables|Default|SetIsLevitating true)
                  (Variables|/Game/Blueprints/Player/BP_TinykinesisPlayerController.BP_TinykinesisPlayerController_C|SetUsingPower _tinykinesisplayercontroller_3 true)))))))
      (:Is%20Not%20Valid
        (Utilities|IsValid (Variables|Default|GetItemGrabbed)
          (:Is%20Valid
            (Variables|/Game/Blueprints/Player/BP_TinykinesisPlayerController.BP_TinykinesisPlayerController_C|SetLockedItem _tinykinesisplayercontroller (Variables|Default|GetItemGrabbed))
            (Variables|Default|SetItemGrabbed (Variables|/Game/Blueprints/Player/BP_TinykinesisPlayerController.BP_TinykinesisPlayerController_C|GetEmptyItem _tinykinesisplayercontroller))
            ;[1 0.3582 0.7407] A remplacer par new Variable
            (Variables|Default|SetAttracting false))))))
  (:Completed
    (Utilities|IsValid (Variables|/Game/Blueprints/Player/BP_TinykinesisPlayerController.BP_TinykinesisPlayerController_C|GetLockedItem (CallFunction|GetTinykinesisPlayerController))
      (:Is%20Valid
        ;[1 0.02083 0.02083] Useless avec Event Dispatcher
        (if (Actor|ActorHasTag (Variables|/Game/Blueprints/Player/BP_TinykinesisPlayerController.BP_TinykinesisPlayerController_C|GetLockedItem (CallFunction|GetTinykinesisPlayerController)) "Heavy")
          ;[1 0.4323 0.4323] A decaler dans l'Event Dispatcher (Release Item for Heavy Object)
          (OldFunctions|UseSmash)
          ;[0.115 1 0.3785] Anim stuff
          (Utilities|FlowControl|Delay 0.5)
          (Default|Animation (CallFunction|GetTinykinesisPlayerCharacter) "NewEnumerator6")
          (Utilities|FlowControl|Sequence
            (:then_0
              ;[1 0.4323 0.4323] A decaler dans l'Event Dispatcher (Grab Item for Heavy Object)
              (Utilities|FlowControl|DoOnce false) ; enters at Reset
            )
            (:then_1
              (goto _label Reset))
            (:then_2
              (Variables|/Game/Blueprints/Player/BP_TinykinesisPlayerController.BP_TinykinesisPlayerController_C|SetCanUsePower (CallFunction|GetTinykinesisPlayerController) false)
              (Utilities|FlowControl|Delay 1.0)
              (Variables|/Game/Blueprints/Player/BP_TinykinesisPlayerController.BP_TinykinesisPlayerController_C|SetCanUsePower (CallFunction|GetTinykinesisPlayerController) true)))
          (elif (and (Actor|ActorHasTag (Variables|/Game/Blueprints/Player/BP_TinykinesisPlayerController.BP_TinykinesisPlayerController_C|GetLockedItem _tinykinesisplayercontroller_4) "Light") (Variables|/Game/Blueprints/Player/BP_TinykinesisPlayerController.BP_TinykinesisPlayerController_C|GetCanUsePower _tinykinesisplayercontroller_4))
            ;[1 0.4323 0.4323] A decaler dans l'Event Dispatcher (Release Item for Light  Object)
            (OldFunctions|PropulseObject)
            (OldFunctions|UsedPropulse)
            ;[0.115 1 0.3785] Anim stuff
            (Utilities|FlowControl|Delay 0.5)
            (Default|Animation (CallFunction|GetTinykinesisPlayerCharacter) "NewEnumerator6")
            (Variables|/Game/Blueprints/Player/BP_TinykinesisPlayerController.BP_TinykinesisPlayerController_C|SetCanUsePower _tinykinesisplayercontroller_6 false)
            (Utilities|FlowControl|Delay 0.5)
            (Variables|/Game/Blueprints/Player/BP_TinykinesisPlayerController.BP_TinykinesisPlayerController_C|SetCanUsePower _tinykinesisplayercontroller_6 true)))))))

(event Input|EnhancedActionEvents|EnhancedInputActionIA_TelekinesisTap
  (params (ActionValue :type Boolean) (ElapsedSeconds :type Float%20%28double-precision%29) (TriggeredSeconds :type Float%20%28double-precision%29) (InputAction :type Input%20Action%20Object%20Reference :default "/Game/Blueprints/Player/Input/Actions/IA_TelekinesisTap.IA_TelekinesisTap"))
  (bind _tinykinesisplayercontroller (CallFunction|GetTinykinesisPlayerController))
  (bind _tinykinesisplayercharacter (CallFunction|GetTinykinesisPlayerCharacter))
  (bind _tinykinesisplayercontroller_2 (CallFunction|GetTinykinesisPlayerController))
  (bind _tinykinesisplayercontroller_3 (CallFunction|GetTinykinesisPlayerController))
  (bind _tinykinesisplayercontroller_4 (CallFunction|GetTinykinesisPlayerController))
  (bind _lockeditem (Variables|/Game/Blueprints/Player/BP_TinykinesisPlayerController.BP_TinykinesisPlayerController_C|GetLockedItem _tinykinesisplayercontroller_2))
  (bind _lockeditem_2 (Variables|/Game/Blueprints/Player/BP_TinykinesisPlayerController.BP_TinykinesisPlayerController_C|GetLockedItem _tinykinesisplayercontroller_4))
  (Utilities|IsValid (Variables|Default|GetItemGrabbed)
    (:Is%20Valid
      ;[1 0.3582 0.7407] A remplacer par new Variable
      (Development|PrintString "stop")
      (Variables|Default|SetAttracting false)
      ;[0.115 1 0.3785] Anim stuff
      (Default|Animation (CallFunction|GetTinykinesisPlayerCharacter) "NewEnumerator2")
      ;[1 0.4323 0.4323] A decaler dans l'Event Dispatcher (Release item for Light Object)
      (bind _output_get (Variables|/Game/Blueprints/Player/BP_TinykinesisPlayerController.BP_TinykinesisPlayerController_C|SetTargetLocation _tinykinesisplayercontroller (Math|Vector|MakeVector (.X (Math|Vector|BreakVector (Variables|/Game/Blueprints/Player/BP_TinykinesisPlayerController.BP_TinykinesisPlayerController_C|GetTargetLocation _tinykinesisplayercontroller))) (.Y (Math|Vector|BreakVector (Variables|/Game/Blueprints/Player/BP_TinykinesisPlayerController.BP_TinykinesisPlayerController_C|GetTargetLocation _tinykinesisplayercontroller))) (+ (.Z (Math|Vector|BreakVector (Variables|/Game/Blueprints/Player/BP_TinykinesisPlayerController.BP_TinykinesisPlayerController_C|GetTargetLocation _tinykinesisplayercontroller))) 1e+01))))
      (Class|BPITelekinesisObject|Propulse(Message) (Variables|Default|GetItemGrabbed) _output_get (Math|Vector|GetForwardVector (Variables|/Game/Blueprints/Player/BP_TinykinesisPlayerCharacter.BP_TinykinesisPlayerCharacter_C|GetGrabPointR (CallFunction|GetTinykinesisPlayerCharacter))) (Variables|/Game/Blueprints/Player/BP_TinykinesisPlayerController.BP_TinykinesisPlayerController_C|GetHasTarget (CallFunction|GetTinykinesisPlayerController)))
      (Variables|Default|SetItemGrabbed (Variables|/Game/Blueprints/Player/BP_TinykinesisPlayerController.BP_TinykinesisPlayerController_C|GetEmptyItem (CallFunction|GetTinykinesisPlayerController)))
      ;[0.115 1 0.3785] Anim stuff
      (Utilities|FlowControl|Delay 0.5)
      (Default|Animation (CallFunction|GetTinykinesisPlayerCharacter) "NewEnumerator6"))
    (:Is%20Not%20Valid
      (Utilities|IsValid _lockeditem
        (:Is%20Valid
          (if (Variables|/Game/Blueprints/Player/BP_TinykinesisPlayerController.BP_TinykinesisPlayerController_C|GetCanUsePower _tinykinesisplayercontroller_2)
            ;[1 0.02083 0.02083] Useless avec Event Dispatcher
            (if (Actor|ActorHasTag _lockeditem "Light")
              ;[1 0.3582 0.7407] A remplacer par new Variable
              (Development|PrintString "Hello")
              (Variables|Default|SetAttracting true)
              (Variables|Default|SetIsAttracted true)
              (Variables|Default|SetItemGrabbed _lockeditem)
              ;[1 0.4323 0.4323] A decaler dans l'Event Dispatcher (Grab Item for Light  Object)
              (OldFunctions|SetAttractionUsage)
              (else
                ;[1 0.02083 0.02083] Useless avec Event Dispatcher
                (if (Actor|ActorHasTag _lockeditem "Heavy")
                  (if (Variables|Default|GetIsLevitating)
                    ;[1 0.4323 0.4323] A decaler dans l'Event Dispatcher (Release Item for Heavy Object)
                    (OldFunctions|UseSmash)
                    (Utilities|FlowControl|Delay 0.5)
                    ;[0.115 1 0.3785] Anim stuff
                    (Default|Animation (CallFunction|GetTinykinesisPlayerCharacter) "NewEnumerator6")
                    (Utilities|FlowControl|Sequence
                      (:then_0
                        (Variables|/Game/Blueprints/Player/BP_TinykinesisPlayerController.BP_TinykinesisPlayerController_C|SetCanUsePower (CallFunction|GetTinykinesisPlayerController) false)
                        (Utilities|FlowControl|Delay 1.0)
                        (Variables|/Game/Blueprints/Player/BP_TinykinesisPlayerController.BP_TinykinesisPlayerController_C|SetCanUsePower (CallFunction|GetTinykinesisPlayerController) true))
                      (:then_1
                        (goto _label Reset)))
                    (else
                      (Development|PrintString "Levitate")
                      ;[0.115 1 0.3785] Anim stuff
                      (Default|Animation _tinykinesisplayercharacter "NewEnumerator1")
                      (Default|PlayHoldLevite _tinykinesisplayercharacter)
                      ;[1 0.2863 0.06522] Mystery
                      (if (and (Utilities|IsValid _lockeditem_2) (not (Variables|/Game/Blueprints/Player/BP_TinykinesisPlayerController.BP_TinykinesisPlayerController_C|GetGotHit _tinykinesisplayercontroller_4)))
                        (Variables|/Game/Blueprints/Player/BP_TinykinesisPlayerController.BP_TinykinesisPlayerController_C|SetUsingPower _tinykinesisplayercontroller_3 true)
                        (Default|UsedCapacity _tinykinesisplayercontroller_3)
                        ;[1 0.4323 0.4323] A decaler dans l'Event Dispatcher (Grab Item for Heavy Object)
                        (Camera|PlayWorldCameraShake "/Game/Blueprints/Actors/BP_PowerCameraShake.BP_PowerCameraShake_C" (Transformation|GetActorLocation (CallFunction|GetTinykinesisPlayerCharacter)) 0.0 5e+02)
                        (Utilities|FlowControl|DoOnce false :!label _label
                          (:Completed
                            (Class|BPISmash|Levitate(Message) (Variables|/Game/Blueprints/Player/BP_TinykinesisPlayerController.BP_TinykinesisPlayerController_C|GetLockedItem (CallFunction|GetTinykinesisPlayerController)))
                            (Variables|Default|SetIsLevitating true)
                            (Variables|/Game/Blueprints/Player/BP_TinykinesisPlayerController.BP_TinykinesisPlayerController_C|SetUsingPower (CallFunction|GetTinykinesisPlayerController) true)))
                        (else
                          ;[1 0.2863 0.06522] Mystery
                          (Class|BPISmash|CancelLevitation(Message) _lockeditem_2))))))))))))))

(event Input|EnhancedActionEvents|EnhancedInputActionIA_TelekinesisV2
  (params (ActionValue :type Boolean) (ElapsedSeconds :type Float%20%28double-precision%29) (TriggeredSeconds :type Float%20%28double-precision%29) (InputAction :type Input%20Action%20Object%20Reference :default "/Game/Blueprints/Player/Input/Actions/IA_TelekinesisV2.IA_TelekinesisV2"))
  (bind _tinykinesisplayercontroller (CallFunction|GetTinykinesisPlayerController))
  (bind _tinykinesisplayercontroller_2 (CallFunction|GetTinykinesisPlayerController))
  (:Triggered
    ;[1 1 1] Ici, on charge l'objet avant l'attaque, via un Event Dispatcher
    (Development|PrintString "Triggered"))
  (:Started
    ;[1 1 1] Ici, interaction dès le clic : on check si le joueur possède ou non un objet dans sa main. Si non, et qu'un objet est visé, on le fait récuperer (Event Dispatcher). Si oui, on le fait projeter.
    (Development|PrintString "Started")
    (Utilities|IsValid (Variables|Default|GetItemGrabbed)
      (:Is%20Valid
        ;;[1 0.3582 0.7407] A remplacer par new Variable
        (Variables|Default|SetAttracting false)
        ;;[1 1 1] Release item (event dispatcher)
        (Development|PrintString "Realease item")
        (Variables|/Game/Blueprints/Player/BP_TinykinesisPlayerController.BP_TinykinesisPlayerController_C|SetLockedItem (CallFunction|GetTinykinesisPlayerController) (Variables|Default|GetItemGrabbed))
        (Variables|Default|SetItemGrabbed (Variables|/Game/Blueprints/Player/BP_TinykinesisPlayerController.BP_TinykinesisPlayerController_C|GetEmptyItem (CallFunction|GetTinykinesisPlayerController)))
        (Variables|/Game/Blueprints/Player/BP_TinykinesisPlayerController.BP_TinykinesisPlayerController_C|SetCanUsePower (CallFunction|GetTinykinesisPlayerController) false)
        (Utilities|FlowControl|Delay 0.5)
        (Variables|/Game/Blueprints/Player/BP_TinykinesisPlayerController.BP_TinykinesisPlayerController_C|SetCanUsePower (CallFunction|GetTinykinesisPlayerController) true)
        (Default|UsedCapacity (CallFunction|GetTinykinesisPlayerController)))
      (:Is%20Not%20Valid
        (Utilities|IsValid (Variables|/Game/Blueprints/Player/BP_TinykinesisPlayerController.BP_TinykinesisPlayerController_C|GetLockedItem (CallFunction|GetTinykinesisPlayerController))
          (:Is%20Valid
            (if (Variables|/Game/Blueprints/Player/BP_TinykinesisPlayerController.BP_TinykinesisPlayerController_C|GetCanUsePower _tinykinesisplayercontroller_2)
              (Variables|/Game/Blueprints/Player/BP_TinykinesisPlayerController.BP_TinykinesisPlayerController_C|SetUsingPower _tinykinesisplayercontroller_2 true)
              ;;[1 0.3582 0.7407] A remplacer par new Variable
              (Variables|Default|SetAttracting true)
              (Variables|Default|SetIsAttracted true)
              (Variables|Default|SetItemGrabbed (Variables|/Game/Blueprints/Player/BP_TinykinesisPlayerController.BP_TinykinesisPlayerController_C|GetLockedItem (CallFunction|GetTinykinesisPlayerController)))
              (if (!= (Variables|/Game/Blueprints/Player/BP_TinykinesisPlayerController.BP_TinykinesisPlayerController_C|GetLockedItem _tinykinesisplayercontroller) (Variables|/Game/Blueprints/Player/BP_TinykinesisPlayerController.BP_TinykinesisPlayerController_C|GetEmptyItem _tinykinesisplayercontroller))
                ;;[1 1 1] Grab item (event dispatcher)
                (Class|BPITelekinesisObject|GrabObject(Message) (Variables|Default|GetItemGrabbed) "0, 0, 0" false)
                (Default|UsedCapacity (CallFunction|GetTinykinesisPlayerController))
                (else
                  (Variables|/Game/Blueprints/Player/BP_TinykinesisPlayerController.BP_TinykinesisPlayerController_C|SetUsingPower _tinykinesisplayercontroller false)))))))))
  (:Ongoing
    ;[1 1 1] Ici, on autorise la saisie d'un objet (marge d'erreur). Revient à peu près au même que pour le Started, à la seule différence qu'on ne permet pas la projection d'un élément.
    (Development|PrintString "OnGoing"))
  (:Canceled
    ;[1 1 1] Ici, on autorise la projection d'un élément, à condition qu'on en possède un. Revient à peu près au même que pour le Completed.
    (Development|PrintString "Canceled"))
  (:Completed
    ;[1 1 1] Ici, interaction dès le realease : on projette l'élément grabbed vers la cible, ou vers le vide, via un event dispatcher associé à l'objet.
    (Development|PrintString "Completed")))

(event EventTick
  (params (DeltaSeconds :type Float%20%28single-precision%29))
  (bind _tinykinesisplayercharacter (CallFunction|GetTinykinesisPlayerCharacter))
  (Utilities|IsValid (Variables|Default|GetItemGrabbed)
    (:Is%20Valid
      (if (Variables|Default|GetAttracting)
        (Variables|/Game/Blueprints/Player/BP_TinykinesisPlayerController.BP_TinykinesisPlayerController_C|SetUsingPower (CallFunction|GetTinykinesisPlayerController) true)
        ;[0.115 1 0.3785] Anim stuff
        (Default|Animation _tinykinesisplayercharacter "NewEnumerator0")
        (Default|PlayHoldAttract _tinykinesisplayercharacter)
        (Class|BPITelekinesisObject|Attract(Message) (Variables|Default|GetItemGrabbed) (Transformation|GetWorldLocation (Variables|/Game/Blueprints/Player/BP_TinykinesisPlayerCharacter.BP_TinykinesisPlayerCharacter_C|GetGrabPointR (CallFunction|GetTinykinesisPlayerCharacter))) "0, 0, 0" false)))))

(fn AttractObject
  (bind _tinykinesisplayercontroller (CallFunction|GetTinykinesisPlayerController))
  (bind _tinykinesisplayercharacter (CallFunction|GetTinykinesisPlayerCharacter))
  (bind _tinykinesisplayercharacter_2 (CallFunction|GetTinykinesisPlayerCharacter))
  (bind _lockeditem (Variables|/Game/Blueprints/Player/BP_TinykinesisPlayerController.BP_TinykinesisPlayerController_C|GetLockedItem _tinykinesisplayercontroller))
  (Variables|/Game/Blueprints/Player/BP_TinykinesisPlayerController.BP_TinykinesisPlayerController_C|SetUsingPower (CallFunction|GetTinykinesisPlayerController) true)
  (Default|Animation _tinykinesisplayercharacter_2 "NewEnumerator0")
  (Default|PlayHoldAttract _tinykinesisplayercharacter_2)
  (if (Utilities|IsValid _lockeditem)
    (Class|BPITelekinesisObject|Attract(Message) _lockeditem (Transformation|GetWorldLocation (Variables|/Game/Blueprints/Player/BP_TinykinesisPlayerCharacter.BP_TinykinesisPlayerCharacter_C|GetGrabPointR _tinykinesisplayercharacter)) (Transformation|GetWorldLocation (Variables|/Game/Blueprints/Player/BP_TinykinesisPlayerCharacter.BP_TinykinesisPlayerCharacter_C|GetGrabPointFront _tinykinesisplayercharacter)) (Variables|/Game/Blueprints/Player/BP_TinykinesisPlayerController.BP_TinykinesisPlayerController_C|GetGotHit _tinykinesisplayercontroller))
    (Variables|/Game/Blueprints/Player/BP_TinykinesisPlayerController.BP_TinykinesisPlayerController_C|SetCharging (CallFunction|GetTinykinesisPlayerController) true)))

(fn SetAttractionUsage
  (bind _tinykinesisplayercontroller (CallFunction|GetTinykinesisPlayerController))
  (Default|ShowInput _tinykinesisplayercontroller)
  (Default|ChangeTextInput _tinykinesisplayercontroller "Release")
  (Default|ShowInputLeft _tinykinesisplayercontroller))

(fn UseLevitate
  (bind _tinykinesisplayercharacter (CallFunction|GetTinykinesisPlayerCharacter))
  (bind _tinykinesisplayercontroller (CallFunction|GetTinykinesisPlayerController))
  (bind _tinykinesisplayercontroller_2 (CallFunction|GetTinykinesisPlayerController))
  (bind _lockeditem (Variables|/Game/Blueprints/Player/BP_TinykinesisPlayerController.BP_TinykinesisPlayerController_C|GetLockedItem _tinykinesisplayercontroller_2))
  (Default|Animation _tinykinesisplayercharacter "NewEnumerator1")
  (Default|PlayHoldLevite _tinykinesisplayercharacter)
  (if (and (Utilities|IsValid _lockeditem) (not (Variables|/Game/Blueprints/Player/BP_TinykinesisPlayerController.BP_TinykinesisPlayerController_C|GetGotHit _tinykinesisplayercontroller_2)))
    (Variables|/Game/Blueprints/Player/BP_TinykinesisPlayerController.BP_TinykinesisPlayerController_C|SetUsingPower _tinykinesisplayercontroller true)
    (Default|UsedCapacity _tinykinesisplayercontroller)
    (else
      (Class|BPISmash|CancelLevitation(Message) _lockeditem))))

(fn PropulseObject
  (bind _tinykinesisplayercontroller (CallFunction|GetTinykinesisPlayerController))
  (bind _tinykinesisplayercontroller_2 (CallFunction|GetTinykinesisPlayerController))
  (if (and (Variables|/Game/Blueprints/Player/BP_TinykinesisPlayerController.BP_TinykinesisPlayerController_C|GetCanUsePower _tinykinesisplayercontroller_2) (Variables|/Game/Blueprints/Player/BP_TinykinesisPlayerController.BP_TinykinesisPlayerController_C|GetUsesTelekinesis _tinykinesisplayercontroller_2))
    (Default|Animation (CallFunction|GetTinykinesisPlayerCharacter) "NewEnumerator2")
    (bind _output_get (Variables|/Game/Blueprints/Player/BP_TinykinesisPlayerController.BP_TinykinesisPlayerController_C|SetTargetLocation (CallFunction|GetTinykinesisPlayerController) (Math|Vector|MakeVector (.X (Math|Vector|BreakVector (Variables|/Game/Blueprints/Player/BP_TinykinesisPlayerController.BP_TinykinesisPlayerController_C|GetTargetLocation (CallFunction|GetTinykinesisPlayerController)))) (.Y (Math|Vector|BreakVector (Variables|/Game/Blueprints/Player/BP_TinykinesisPlayerController.BP_TinykinesisPlayerController_C|GetTargetLocation (CallFunction|GetTinykinesisPlayerController)))) (+ (.Z (Math|Vector|BreakVector (Variables|/Game/Blueprints/Player/BP_TinykinesisPlayerController.BP_TinykinesisPlayerController_C|GetTargetLocation (CallFunction|GetTinykinesisPlayerController)))) 1e+01))))
    (Class|BPITelekinesisObject|Propulse(Message) (Variables|/Game/Blueprints/Player/BP_TinykinesisPlayerController.BP_TinykinesisPlayerController_C|GetLockedItem _tinykinesisplayercontroller) _output_get (Math|Vector|GetForwardVector (Variables|/Game/Blueprints/Player/BP_TinykinesisPlayerCharacter.BP_TinykinesisPlayerCharacter_C|GetGrabPointR (CallFunction|GetTinykinesisPlayerCharacter))) (Variables|/Game/Blueprints/Player/BP_TinykinesisPlayerController.BP_TinykinesisPlayerController_C|GetHasTarget _tinykinesisplayercontroller))
    (Variables|/Game/Blueprints/Player/BP_TinykinesisPlayerController.BP_TinykinesisPlayerController_C|SetCanUsePower (CallFunction|GetTinykinesisPlayerController) false)
    (Variables|Default|SetItemGrabbed (Variables|/Game/Blueprints/Player/BP_TinykinesisPlayerController.BP_TinykinesisPlayerController_C|GetEmptyItem (CallFunction|GetTinykinesisPlayerController)))))

(fn UsedPropulse
  (bind _tinykinesisplayercontroller (CallFunction|GetTinykinesisPlayerController))
  (Default|UsedCapacity _tinykinesisplayercontroller)
  (Variables|/Game/Blueprints/Player/BP_TinykinesisPlayerController.BP_TinykinesisPlayerController_C|SetUsingPower _tinykinesisplayercontroller false)
  (Default|HideInput (CallFunction|GetTinykinesisPlayerController))
  (Variables|/Game/Blueprints/Player/BP_TinykinesisPlayerController.BP_TinykinesisPlayerController_C|SetLockedItem _tinykinesisplayercontroller (Variables|/Game/Blueprints/Player/BP_TinykinesisPlayerController.BP_TinykinesisPlayerController_C|GetEmptyItem _tinykinesisplayercontroller)))

(fn UseSmash
  (bind _tinykinesisplayercontroller (CallFunction|GetTinykinesisPlayerController))
  (Default|Animation (CallFunction|GetTinykinesisPlayerCharacter) "NewEnumerator3")
  (Class|BPISmash|Smash(Message) (Variables|/Game/Blueprints/Player/BP_TinykinesisPlayerController.BP_TinykinesisPlayerController_C|GetLockedItem _tinykinesisplayercontroller))
  (Variables|/Game/Blueprints/Player/BP_TinykinesisPlayerController.BP_TinykinesisPlayerController_C|SetLockedItem _tinykinesisplayercontroller (Variables|/Game/Blueprints/Player/BP_TinykinesisPlayerController.BP_TinykinesisPlayerController_C|GetEmptyItem _tinykinesisplayercontroller))
  (Variables|/Game/Blueprints/Player/BP_TinykinesisPlayerController.BP_TinykinesisPlayerController_C|SetUsingPower _tinykinesisplayercontroller false)
  (Default|HideInput (CallFunction|GetTinykinesisPlayerController))
  (Variables|Default|SetIsLevitating false))

(fn CheckItem
  (bind _tinykinesisplayercontroller (CallFunction|GetTinykinesisPlayerController))
  (Utilities|IsValid (Variables|Default|GetItemGrabbed)
    (:Is%20Valid
      ;[1 1 1] Release item (event dispatcher)
      (Development|PrintString "Grab item"))
    (:Is%20Not%20Valid
      (Utilities|IsValid (Variables|/Game/Blueprints/Player/BP_TinykinesisPlayerController.BP_TinykinesisPlayerController_C|GetLockedItem (CallFunction|GetTinykinesisPlayerController))
        (:Is%20Valid
          (if (Variables|/Game/Blueprints/Player/BP_TinykinesisPlayerController.BP_TinykinesisPlayerController_C|GetCanUsePower _tinykinesisplayercontroller)
            (Variables|/Game/Blueprints/Player/BP_TinykinesisPlayerController.BP_TinykinesisPlayerController_C|SetUsingPower _tinykinesisplayercontroller true)
            (Variables|Default|SetItemGrabbed (CallFunction|GetTinykinesisPlayerController))))))))