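; Actor component that tracks the spot beneath the Tinykinesis player character while it is not moving on the ground.
; At BeginPlay it caches the character and spawns a TargetPoint.
; Each airborne tick, it line-traces 1500 units straight down and moves the TargetPoint to the hit location, without checking whether the trace hit anything.
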(event EventBeginPlay
  (bind _asbp_tinykinesis_player_character (Utilities|Casting|CastToBP_TinykinesisPlayerCharacter (Game|GetPlayerCharacter 0)))
  (Variables|Default|SetAs%20BP%20First%20Person%20Character _asbp_tinykinesis_player_character)
  (bind _returnvalue (Game|SpawnActorfromClass "/Script/Engine.TargetPoint" (Math|Transform|MakeTransform "0, 0, 0" "0, 0, 0" "1.000000,1.000000,1.000000") "AlwaysSpawn" "MultiplyWithRoot" 0 0))
  (Variables|Default|SetTargetPointRaycast _returnvalue))

(event EventTick
  (params (DeltaSeconds :type Float%20%28single-precision%29))
  (bind _as_bp_first_person_character (Variables|Default|GetAs%20BP%20First%20Person%20Character))
  (bind _returnvalue (Transformation|GetActorLocation _as_bp_first_person_character))
  (bind (_x _y _z) (Math|Vector|BreakVector _returnvalue))
  (if (not (AI|Components|NavMovement|IsMovingonGround (Variables|/Script/Engine.Character|GetCharacterMovement (Variables|Default|GetAs%20BP%20First%20Person%20Character))))
    (bind _outhit (Collision|LineTraceByChannel _returnvalue (Math|Vector|MakeVector _x _y (- _z 1.5e+03)) "TraceTypeQuery3" false 0 "None"))
    (if true
      (Transformation|SetActorLocation (Variables|Default|GetTargetPointRaycast) (.Location (Collision|BreakHitResult _outhit)) false false))))