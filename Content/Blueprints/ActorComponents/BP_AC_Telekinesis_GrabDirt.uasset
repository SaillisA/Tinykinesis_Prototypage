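; Actor component for the telekinesis grab-dirt power, driven by the IA_GrabDirt input action.
; On start, it sets the player controller's UsingPower lock, unless already set, and line-traces from the first-person camera out to CastRange.
; A hit on a Dirt physical surface fires the controller's grab-dirt timeline event at the impact point.
; Cancelling the input clears the lock and calls the controller's canceled event.
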(event Input|EnhancedActionEvents|EnhancedInputActionIA_GrabDirt
  (params (ActionValue :type Boolean) (ElapsedSeconds :type Float%20%28double-precision%29) (TriggeredSeconds :type Float%20%28double-precision%29) (InputAction :type Input%20Action%20Object%20Reference :default "/Game/Blueprints/Player/Input/Actions/IA_GrabDirt.IA_GrabDirt"))
  (bind _tinykinesisplayercontroller (CallFunction|GetTinykinesisPlayerController))
  (bind _tinykinesisplayercharacter (CallFunction|GetTinykinesisPlayerCharacter))
  (bind _tinykinesisplayercontroller_2 (CallFunction|GetTinykinesisPlayerController))
  (bind _firstpersoncameracomponent (Variables|/Script/Tinykinesis_Proto.Tinykinesis_ProtoCharacter|GetFirstPersonCameraComponent _tinykinesisplayercharacter))
  (bind _returnvalue (Transformation|GetWorldLocation _firstpersoncameracomponent))
  (:Started
    (if (Variables|/Game/Blueprints/Player/BP_TinykinesisPlayerController.BP_TinykinesisPlayerController_C|GetUsingPower _tinykinesisplayercontroller)
      (Development|PrintString "can't use power")
      (else
        (Variables|/Game/Blueprints/Player/BP_TinykinesisPlayerController.BP_TinykinesisPlayerController_C|SetUsingPower _tinykinesisplayercontroller true)
        (bind _outhit (Collision|LineTraceByChannel _returnvalue (+ _returnvalue (* (Math|Vector|GetForwardVector (Transformation|GetWorldRotation _firstpersoncameracomponent)) (Variables|/Game/Blueprints/Player/BP_TinykinesisPlayerController.BP_TinykinesisPlayerController_C|GetCastRange _tinykinesisplayercontroller_2))) "TraceTypeQuery1" false 0 "None"))
        (Utilities|IsValid (.HitComponent (Collision|BreakHitResult _outhit))
          (:Is%20Valid
            (if (Utilities|Select :Index (Collision|GetSurfaceType _outhit) :SurfaceType_Default false :SurfaceType1 true)
              (Default|EventTimelineGrabDirt (CallFunction|GetTinykinesisPlayerController) (.ImpactPoint (Collision|BreakHitResult _outhit)))))))))
  (:Canceled
    (Variables|/Game/Blueprints/Player/BP_TinykinesisPlayerController.BP_TinykinesisPlayerController_C|SetUsingPower _tinykinesisplayercontroller false)
    (Default|EventTimelineGrabDirtCanceled _tinykinesisplayercontroller_2 (.ImpactPoint (Collision|BreakHitResult _outhit)))))