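; Actor component that tracks player health and death state.
; On BeginPlay it sets max HP and fills current HP to match.
; TakeDamage records the incoming amount, subtracts it from current HP without clamping, then sets the Dead flag according to whether HP has reached zero or below.
; The component only updates these variables and triggers no death response itself.
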(event Custom|TakeDamage
  (params (DamageAmount :type Float%20%28double-precision%29))
  (Variables|Default|SetDamageTaken DamageAmount)
  (Variables|Default|SetCurrentHP (- (Variables|Default|GetCurrentHP) (Variables|Default|GetDamageTaken)))
  (if (<= (Variables|Default|GetCurrentHP) 0.0)
    (Variables|Default|SetDead true)
    (else
      (Variables|Default|SetDead false))))

(event EventBeginPlay
  (bind _output_get (Variables|Default|SetMaxHP 1e+02))
  (Variables|Default|SetCurrentHP _output_get))