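; BP_AC_Telekinesis_Propulse_PERIME is an apparently deprecated component for the telekinesis propulse power, which launches the player's locked item.
; Its IA_Propulse_PERIME input event is empty, leaving all the logic disconnected so it never runs.
; That orphaned chain checks the controller's power flags, sends PropulseMessage to the locked item with target and grab-point direction, then clears the lock.
; It also switches character animations and applies a short delay-based cooldown.
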(event Input|EnhancedActionEvents|EnhancedInputActionIA_Propulse_PERIME
  (params (ActionValue :type Boolean) (ElapsedSeconds :type Float%20%28double-precision%29) (TriggeredSeconds :type Float%20%28double-precision%29) (InputAction :type Input%20Action%20Object%20Reference :default "/Game/Blueprints/Player/Input/Actions/IA_Propulse_PERIME.IA_Propulse_PERIME")))