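; Actor component that manages the active state of a gameplay element and its persistence through the level manager.
; DisableInSave reports the owner to BP_AbstractLevelManager, while SetActiveElement stores the flag and fires a dispatcher.
; LoadElement applies a given state to an actor's visibility, tick and collision, firing an active BeginPlay dispatcher when active.
; LaunchBeginPlay fires that dispatcher only if the level has launched or no manager exists.
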(event EventBeginPlay)

(event EventTick
  (params (DeltaSeconds :type Float%20%28single-precision%29)))

(fn DisableinSave
  (bind _returnvalue (Actor|GetActorOfClass "/Game/Blueprints/SaveSystem/BP_AbstractLevelManager.BP_AbstractLevelManager_C"))
  (Utilities|IsValid _returnvalue
    (:Is%20Valid
      (bind _output_get (Variables|Default|SetLevelManager _returnvalue))
      (Default|SetBoolActive _output_get (Components|GetOwner)))))

(fn SetActiveElement
  (params (IsActive :type Boolean))
  (Variables|Default|SetIsActivated IsActive)
  (Default|CallSetActiveElementEventDispatcher))

(fn LoadElement
  (params (IsActive :type Boolean) (Actor :type Actor%20Object%20Reference))
  (Rendering|SetActorHiddenInGame Actor (not IsActive))
  (Actor|Tick|SetActorTickEnabled Actor IsActive)
  (Collision|SetActorEnableCollision Actor IsActive)
  (if IsActive
    (Default|CallBeginPlayActiveElement)))

(fn LaunchBeginPlay
  (bind _returnvalue (Actor|GetActorOfClass "/Game/Blueprints/SaveSystem/BP_AbstractLevelManager.BP_AbstractLevelManager_C"))
  (Utilities|IsValid _returnvalue
    (:Is%20Valid
      (if (Variables|/Game/Blueprints/SaveSystem/BP_AbstractLevelManager.BP_AbstractLevelManager_C|GetHasLaunchedLevel _returnvalue)
        (Default|CallBeginPlayActiveElement :!label _label)))
    (:Is%20Not%20Valid
      (goto _label))))