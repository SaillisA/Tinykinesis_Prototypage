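; Actor component that supplies shake and destruction functions for breakable elements.
; LaunchDestruction spawns the FracturedElement actor, sizes its explosion force and radial impulse, starts it through BeginPlayManual, then destroys the target actor to swap in the fractured version.
; The shake helpers add an offset to a static or skeletal mesh's relative XY location while keeping Z; only the skeletal version sweeps.
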(fn ShakeStaticMesh
  (params (StaticMesh :type Static%20Mesh%20Component%20Object%20Reference) (PositionParameter :type Float%20%28double-precision%29))
  (bind _relativelocation (Variables|/Script/Engine.SceneComponent|GetRelativeLocation StaticMesh))
  (bind _returnvalue (+ (Math|Vector|MakeVector (.x _relativelocation) (.y _relativelocation) 0.0) PositionParameter))
  (Transformation|SetRelativeLocation StaticMesh (Math|Vector|MakeVector (.x _returnvalue) (.y _returnvalue) (.z _relativelocation)) false false))

(fn LaunchDestruction
  (params (SpawnTransform :type Transform) (ScaleExplosionFracture :type Float%20%28double-precision%29) (RadiusSphereImpulse :type Float%20%28double-precision%29) (Target :type Actor%20Object%20Reference))
  (bind _returnvalue (Game|SpawnActorfromClass (Variables|Default|GetFracturedElement) SpawnTransform "Undefined" "MultiplyWithRoot" 0 0))
  (Transformation|SetRelativeScale3D (Variables|/Game/Blueprints/Actors/FracturedActors/BP_FracturedMesh.BP_FracturedMesh_C|GetExplosionForce _returnvalue) (Math|Conversions|ToVector(Float) ScaleExplosionFracture))
  (Variables|/Script/Engine.RadialForceComponent|SetRadius (Variables|/Game/Blueprints/Actors/FracturedActors/BP_FracturedMesh.BP_FracturedMesh_C|GetRadialForce _returnvalue) RadiusSphereImpulse)
  (Default|BeginPlayManual _returnvalue)
  (Actor|DestroyActor Target))

(fn ShakeSkeletalMesh
  (params (SkeletalMesh :type Skeletal%20Mesh%20Component%20Object%20Reference) (InputPin :type Float%20%28double-precision%29))
  (bind _relativelocation (Variables|/Script/Engine.SceneComponent|GetRelativeLocation SkeletalMesh))
  (bind _returnvalue (+ (Math|Vector|MakeVector (.x _relativelocation) (.y _relativelocation) 0.0) InputPin))
  (Transformation|SetRelativeLocation SkeletalMesh (Math|Vector|MakeVector (.x _returnvalue) (.y _returnvalue) (.z _relativelocation)) true false))