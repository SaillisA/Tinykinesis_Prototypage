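; Actor component that handles jump input for the Tinykinesis player's double jump.
; Press starts a timeline on the player controller, which holds the state flags; once triggering is allowed, it tunes character movement and jumps.
; Grounded jumps immediately start cooldown and reset jump settings; otherwise a pending press does so after a short delay.
; Cancelled or disallowed input stops the timeline and resets; an older double-jump version remains unconnected.
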(event Input|EnhancedActionEvents|EnhancedInputActionIA_Jump
  (params (ActionValue :type Boolean) (ElapsedSeconds :type Float%20%28double-precision%29) (TriggeredSeconds :type Float%20%28double-precision%29) (InputAction :type Input%20Action%20Object%20Reference :default "/Game/Blueprints/Player/Input/Actions/IA_Jump.IA_Jump"))
  (bind _tinykinesisplayercontroller (CallFunction|GetTinykinesisPlayerController))
  (bind _tinykinesisplayercharacter (CallFunction|GetTinykinesisPlayerCharacter))
  (bind _tinykinesisplayercontroller_2 (CallFunction|GetTinykinesisPlayerController))
  (bind _tinykinesisplayercontroller_3 (CallFunction|GetTinykinesisPlayerController))
  (bind _tinykinesisplayercharacter_2 (CallFunction|GetTinykinesisPlayerCharacter))
  (bind _tinykinesisplayercontroller_4 (CallFunction|GetTinykinesisPlayerController))
  (bind _charactermovement (Variables|/Script/Engine.Character|GetCharacterMovement _tinykinesisplayercharacter_2))
  (bind _charactermovement_2 (Variables|/Script/Engine.Character|GetCharacterMovement _tinykinesisplayercharacter))
  (:Triggered
    (if (and (Variables|/Game/Blueprints/Player/BP_TinykinesisPlayerController.BP_TinykinesisPlayerController_C|GetCanDoubleJump _tinykinesisplayercontroller_2) (Variables|/Game/Blueprints/Player/BP_TinykinesisPlayerController.BP_TinykinesisPlayerController_C|GetCanTriggerDoubleJump _tinykinesisplayercontroller_2))
      (Variables|/Script/Engine.Character|SetJumpMaxHoldTime _tinykinesisplayercharacter 0.1)
      (Variables|/Script/Engine.CharacterMovementComponent|SetJumpZVelocity _charactermovement_2 5.2e+02)
      (Variables|/Script/Engine.Character|SetJumpMaxCount _tinykinesisplayercharacter 2)
      (Variables|/Script/Engine.CharacterMovementComponent|SetMaxWalkSpeed _charactermovement_2 2.8e+02)
      (Character|Jump _tinykinesisplayercharacter)
      (Utilities|FlowControl|Sequence
        (:then_0
          (if (AI|Components|NavMovement|IsMovingonGround (Variables|/Script/Engine.Character|GetCharacterMovement (CallFunction|GetTinykinesisPlayerCharacter)))
            (Default|LaunchJumpCooldown (CallFunction|GetTinykinesisPlayerController) :!label _label)
            (Variables|/Game/Blueprints/Player/BP_TinykinesisPlayerController.BP_TinykinesisPlayerController_C|SetCanDoubleJump _tinykinesisplayercontroller_3 false)
            (Default|StopTimelineDoubleJump _tinykinesisplayercontroller_3 :!label _label_2)
            (Variables|/Game/Blueprints/Player/BP_TinykinesisPlayerController.BP_TinykinesisPlayerController_C|SetCanTriggerDoubleJump _tinykinesisplayercontroller_3 false)
            (Variables|/Game/Blueprints/Player/BP_TinykinesisPlayerController.BP_TinykinesisPlayerController_C|SetInputPressedDoubleJump _tinykinesisplayercontroller_3 false)
            (Variables|/Script/Engine.Character|SetJumpMaxHoldTime _tinykinesisplayercharacter_2 0.0)
            (Variables|/Script/Engine.Character|SetJumpMaxCount _tinykinesisplayercharacter_2 1)
            (Variables|/Script/Engine.CharacterMovementComponent|SetJumpZVelocity _charactermovement 5.2e+02)
            (Variables|/Script/Engine.CharacterMovementComponent|SetGravityScale _charactermovement 1.5)))
        (:then_1
          (if (Variables|/Game/Blueprints/Player/BP_TinykinesisPlayerController.BP_TinykinesisPlayerController_C|GetInputPressedDoubleJump _tinykinesisplayercontroller_4)
            (Variables|/Game/Blueprints/Player/BP_TinykinesisPlayerController.BP_TinykinesisPlayerController_C|SetInputPressedDoubleJump _tinykinesisplayercontroller_4 false)
            (Utilities|FlowControl|Delay 0.1)
            (goto _label))))
      (else
        (goto _label_2))))
  (:Started
    (if (Variables|/Game/Blueprints/Player/BP_TinykinesisPlayerController.BP_TinykinesisPlayerController_C|GetCanDoubleJump _tinykinesisplayercontroller)
      (if (not (Variables|/Game/Blueprints/Player/BP_TinykinesisPlayerController.BP_TinykinesisPlayerController_C|GetInputPressedDoubleJump _tinykinesisplayercontroller))
        (Variables|/Game/Blueprints/Player/BP_TinykinesisPlayerController.BP_TinykinesisPlayerController_C|SetInputPressedDoubleJump _tinykinesisplayercontroller true)
        (Default|LaunchTimelineDoubleJump (CallFunction|GetTinykinesisPlayerController)))))
  (:Canceled
    (goto _label_2)))

(event EventBeginPlay)

(event EventTick
  (params (DeltaSeconds :type Float%20%28single-precision%29)))