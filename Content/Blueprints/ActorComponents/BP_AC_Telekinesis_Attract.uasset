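; Actor component that handles player input for the telekinesis attract and grab power in Tinykinesis.
; Grab sends a grab message to the controller's selected item and briefly pulses an ActivatePower flag.
; While Attract is held, it plays character animation and hold feedback, passes grab-point locations and hit state to the item, and updates power usage and capacity on the controller.
; Releasing Attract starts a short cooldown before power is usable again.
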(event Input|EnhancedActionEvents|EnhancedInputActionIA_GrabItem
  (params (ActionValue :type Boolean) (ElapsedSeconds :type Float%20%28double-precision%29) (TriggeredSeconds :type Float%20%28double-precision%29) (InputAction :type Input%20Action%20Object%20Reference :default "/Game/Blueprints/Player/Input/Actions/IA_GrabItem.IA_GrabItem"))
  (bind _tinykinesisplayercontroller (CallFunction|GetTinykinesisPlayerController))
  (:Triggered
    (if (Utilities|IsValid (Variables|/Game/Blueprints/Player/BP_TinykinesisPlayerController.BP_TinykinesisPlayerController_C|GetSelectedItem _tinykinesisplayercontroller))
      (Class|BPIInteractable|GrabObject(Message) (Variables|/Game/Blueprints/Player/BP_TinykinesisPlayerController.BP_TinykinesisPlayerController_C|GetSelectedItem (CallFunction|GetTinykinesisPlayerController)))))
  (:Started
    (Variables|/Game/Blueprints/Player/BP_TinykinesisPlayerController.BP_TinykinesisPlayerController_C|SetActivatePower _tinykinesisplayercontroller true)
    (Utilities|FlowControl|Delay 0.2)
    (Variables|/Game/Blueprints/Player/BP_TinykinesisPlayerController.BP_TinykinesisPlayerController_C|SetActivatePower _tinykinesisplayercontroller false)))

(event Input|EnhancedActionEvents|EnhancedInputActionIA_Attract
  (params (ActionValue :type Boolean) (ElapsedSeconds :type Float%20%28double-precision%29) (TriggeredSeconds :type Float%20%28double-precision%29) (InputAction :type Input%20Action%20Object%20Reference :default "/Game/Blueprints/Player/Input/Actions/IA_Attract.IA_Attract"))
  (bind _tinykinesisplayercontroller (CallFunction|GetTinykinesisPlayerController))
  (bind _tinykinesisplayercontroller_2 (CallFunction|GetTinykinesisPlayerController))
  (bind _tinykinesisplayercharacter (CallFunction|GetTinykinesisPlayerCharacter))
  (bind _tinykinesisplayercharacter_2 (CallFunction|GetTinykinesisPlayerCharacter))
  (bind _tinykinesisplayercontroller_3 (CallFunction|GetTinykinesisPlayerController))
  (bind _selecteditem (Variables|/Game/Blueprints/Player/BP_TinykinesisPlayerController.BP_TinykinesisPlayerController_C|GetSelectedItem _tinykinesisplayercontroller_2))
  (:Triggered
    (if (!= (Variables|/Game/Blueprints/Player/BP_TinykinesisPlayerController.BP_TinykinesisPlayerController_C|GetSelectedItem _tinykinesisplayercontroller_3) (Variables|/Game/Blueprints/Player/BP_TinykinesisPlayerController.BP_TinykinesisPlayerController_C|GetEmptyItem _tinykinesisplayercontroller_3))
      (if (Variables|/Game/Blueprints/Player/BP_TinykinesisPlayerController.BP_TinykinesisPlayerController_C|GetCanUsePower _tinykinesisplayercontroller_3)
        (Variables|/Game/Blueprints/Player/BP_TinykinesisPlayerController.BP_TinykinesisPlayerController_C|SetUsingPower (CallFunction|GetTinykinesisPlayerController) true)
        (Default|Animation _tinykinesisplayercharacter "NewEnumerator0")
        (Default|PlayHoldAttract _tinykinesisplayercharacter)
        (if (Utilities|IsValid _selecteditem)
          (Class|BPIInteractable|Attract(Message) _selecteditem (Transformation|GetWorldLocation (Variables|/Game/Blueprints/Player/BP_TinykinesisPlayerCharacter.BP_TinykinesisPlayerCharacter_C|GetGrabPointR _tinykinesisplayercharacter_2)) (Transformation|GetWorldLocation (Variables|/Game/Blueprints/Player/BP_TinykinesisPlayerCharacter.BP_TinykinesisPlayerCharacter_C|GetGrabPointFront _tinykinesisplayercharacter_2)) (Variables|/Game/Blueprints/Player/BP_TinykinesisPlayerController.BP_TinykinesisPlayerController_C|GetGotHit _tinykinesisplayercontroller_2))
          (Variables|/Game/Blueprints/Player/BP_TinykinesisPlayerController.BP_TinykinesisPlayerController_C|SetUsesTelekinesis (CallFunction|GetTinykinesisPlayerController) true)
          (Variables|/Game/Blueprints/Player/BP_TinykinesisPlayerController.BP_TinykinesisPlayerController_C|SetUsingPower _tinykinesisplayercontroller true)
          (Default|UsedCapacity _tinykinesisplayercontroller)))
      (else
        (Variables|/Game/Blueprints/Player/BP_TinykinesisPlayerController.BP_TinykinesisPlayerController_C|SetUsingPower _tinykinesisplayercontroller_3 false))))
  (:Completed
    (Variables|/Game/Blueprints/Player/BP_TinykinesisPlayerController.BP_TinykinesisPlayerController_C|SetCanUsePower (CallFunction|GetTinykinesisPlayerController) false)
    (Utilities|FlowControl|Delay 0.5)
    (Variables|/Game/Blueprints/Player/BP_TinykinesisPlayerController.BP_TinykinesisPlayerController_C|SetCanUsePower (CallFunction|GetTinykinesisPlayerController) true)))