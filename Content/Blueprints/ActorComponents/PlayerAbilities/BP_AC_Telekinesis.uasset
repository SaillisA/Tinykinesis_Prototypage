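; Player telekinesis component that grabs the controller's locked item, charges it and launches it.
; IA_TelekinesisV2 phases drive PlayerGrab, PlayerCharge and PlayerRelease, which check CanUseTelekinesis and message the held item.
; Controller state is updated throughout; grab and release trigger aggro, with camera shake on grab and delayed idle animation after release.
; Tick re-sends the grab message for held items tagged AttractiveElement.
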(event Custom|SetIddleAnimation
  ;[1 1 1] La présence d'un délai contraint de le placer ici
  (Utilities|FlowControl|Delay 0.5)
  (Default|Animation (CallFunction|GetTinykinesisPlayerCharacter) "NewEnumerator6"))

(event Input|EnhancedActionEvents|EnhancedInputActionIA_Telekinesis
  (params (ActionValue :type Boolean) (ElapsedSeconds :type Float%20%28double-precision%29) (TriggeredSeconds :type Float%20%28double-precision%29) (InputAction :type Input%20Action%20Object%20Reference :default "/Game/Blueprints/Player/Input/Actions/IA_Telekinesis.IA_Telekinesis")))

(event Input|EnhancedActionEvents|EnhancedInputActionIA_TelekinesisTap
  (params (ActionValue :type Boolean) (ElapsedSeconds :type Float%20%28double-precision%29) (TriggeredSeconds :type Float%20%28double-precision%29) (InputAction :type Input%20Action%20Object%20Reference :default "/Game/Blueprints/Player/Input/Actions/IA_TelekinesisTap.IA_TelekinesisTap")))

(event Input|EnhancedActionEvents|EnhancedInputActionIA_TelekinesisV2
  (params (ActionValue :type Boolean) (ElapsedSeconds :type Float%20%28double-precision%29) (TriggeredSeconds :type Float%20%28double-precision%29) (InputAction :type Input%20Action%20Object%20Reference :default "/Game/Blueprints/Player/Input/Actions/IA_TelekinesisV2.IA_TelekinesisV2"))
  (:Triggered
    ;[1 1 1] Ici, on charge l'objet avant l'attaque, via un Event Dispatcher
    (Utilities|IsValid (Variables|Default|GetItemGrabbed)
      (:Is%20Valid
        (CallFunction|PlayerCharge))))
  (:Started
    ;[1 1 1] Ici, interaction dès le clic : on check si le joueur possède ou non un objet dans sa main. Si non, et qu'un objet est visé, on le fait récuperer (Event Dispatcher). Si oui, on le fait projeter.
    (Utilities|IsValid (Variables|Default|GetItemGrabbed)
      (:Is%20Valid
        (CallFunction|PlayerCharge))
      (:Is%20Not%20Valid
        (CallFunction|PlayerGrab))))
  (:Ongoing
    ;[1 1 1] Ici, on autorise la saisie d'un objet (marge d'erreur). Revient à peu près au même que pour le Started, à la seule différence qu'on ne permet pas la projection d'un élément.
    (Utilities|IsValid (Variables|Default|GetItemGrabbed)
      (:Is%20Not%20Valid
        (CallFunction|PlayerGrab))))
  (:Canceled
    ;[1 0.2083 0.2083] Ici, on autorise la projection d'un élément, à condition qu'on en possède un. Revient à peu près au même que pour le Completed (sans doute foireux, car logiquement, ça devrait projeter qq chose direct après un tap)
    (Utilities|IsValid (Variables|Default|GetItemGrabbed)
      (:Is%20Valid
        (if (Variables|Default|GetHasBeenGrabbedCompletely)
          (CallFunction|PlayerRelease)
          (else
            (Variables|Default|SetHasBeenGrabbedCompletely true))))))
  (:Completed
    ;[1 1 1] Ici, interaction dès le realease : on projette l'élément grabbed vers la cible, ou vers le vide, via un event dispatcher associé à l'objet.
    (Utilities|IsValid (Variables|Default|GetItemGrabbed)
      (:Is%20Valid
        (CallFunction|PlayerRelease)))))

(event EventTick
  (params (DeltaSeconds :type Float%20%28single-precision%29))
  (bind _itemgrabbed (Variables|Default|GetItemGrabbed))
  (Utilities|IsValid _itemgrabbed
    (:Is%20Valid
      (if (Actor|ActorHasTag _itemgrabbed "AttractiveElement")
        (Variables|/Game/Blueprints/Player/BP_TinykinesisPlayerController.BP_TinykinesisPlayerController_C|SetIsUsingTelekinesis (CallFunction|GetTinykinesisPlayerController) true)
        (Class|BPITelekinesisObject|GrabObject(Message) (Variables|Default|GetItemGrabbed))))))

(fn ClearParameters
  (bind _tinykinesisplayercontroller (CallFunction|GetTinykinesisPlayerController))
  (bind _emptyitem (Variables|/Game/Blueprints/Player/BP_TinykinesisPlayerController.BP_TinykinesisPlayerController_C|GetEmptyItem _tinykinesisplayercontroller))
  (Variables|/Game/Blueprints/Player/BP_TinykinesisPlayerController.BP_TinykinesisPlayerController_C|SetLockedItem _tinykinesisplayercontroller _emptyitem)
  (Variables|Default|SetItemGrabbed _emptyitem)
  (Variables|/Game/Blueprints/Player/BP_TinykinesisPlayerController.BP_TinykinesisPlayerController_C|SetIsUsingTelekinesis _tinykinesisplayercontroller false)
  (Variables|Default|SetHasBeenGrabbedCompletely false)
  (Variables|/Game/Blueprints/Player/BP_TinykinesisPlayerController.BP_TinykinesisPlayerController_C|SetIsCharging (CallFunction|GetTinykinesisPlayerController) false))

(fn ChangeParameters
  (Variables|/Game/Blueprints/Player/BP_TinykinesisPlayerController.BP_TinykinesisPlayerController_C|SetIsUsingTelekinesis (CallFunction|GetTinykinesisPlayerController) true)
  (Variables|Default|SetItemGrabbed (Variables|/Game/Blueprints/Player/BP_TinykinesisPlayerController.BP_TinykinesisPlayerController_C|GetLockedItem (CallFunction|GetTinykinesisPlayerController))))

(fn PlayerGrab
  (bind _tinykinesisplayercontroller (CallFunction|GetTinykinesisPlayerController))
  (Utilities|IsValid (Variables|/Game/Blueprints/Player/BP_TinykinesisPlayerController.BP_TinykinesisPlayerController_C|GetLockedItem (CallFunction|GetTinykinesisPlayerController))
    (:Is%20Valid
      (if (Variables|/Game/Blueprints/Player/BP_TinykinesisPlayerController.BP_TinykinesisPlayerController_C|GetCanUseTelekinesis (CallFunction|GetTinykinesisPlayerController))
        (if (!= (Variables|/Game/Blueprints/Player/BP_TinykinesisPlayerController.BP_TinykinesisPlayerController_C|GetLockedItem _tinykinesisplayercontroller) (Variables|/Game/Blueprints/Player/BP_TinykinesisPlayerController.BP_TinykinesisPlayerController_C|GetEmptyItem _tinykinesisplayercontroller))
          (Camera|PlayWorldCameraShake "/Game/Blueprints/Actors/BP_PowerCameraShake.BP_PowerCameraShake_C" (Transformation|GetActorLocation (CallFunction|GetTinykinesisPlayerCharacter)) 0.0 5e+02)
          (CallFunction|ChangeParameters)
          (Class|BPITelekinesisObject|GrabObject(Message) (Variables|Default|GetItemGrabbed))
          (Default|TriggerAggroUsingAbility (CallFunction|GetTinykinesisPlayerController))
          (else
            (Variables|/Game/Blueprints/Player/BP_TinykinesisPlayerController.BP_TinykinesisPlayerController_C|SetIsUsingTelekinesis _tinykinesisplayercontroller false)))))))

(fn PlayerRelease
  ;[0.5331 0.6992 1] Pas sûr de l'utilité de ça
  (if (Variables|/Game/Blueprints/Player/BP_TinykinesisPlayerController.BP_TinykinesisPlayerController_C|GetCanUseTelekinesis (CallFunction|GetTinykinesisPlayerController))
    (Variables|/Game/Blueprints/Player/BP_TinykinesisPlayerController.BP_TinykinesisPlayerController_C|SetTargetLocation (CallFunction|GetTinykinesisPlayerController) (Math|Vector|MakeVector (.X (Math|Vector|BreakVector (Variables|/Game/Blueprints/Player/BP_TinykinesisPlayerController.BP_TinykinesisPlayerController_C|GetTargetLocation (CallFunction|GetTinykinesisPlayerController)))) (.Y (Math|Vector|BreakVector (Variables|/Game/Blueprints/Player/BP_TinykinesisPlayerController.BP_TinykinesisPlayerController_C|GetTargetLocation (CallFunction|GetTinykinesisPlayerController)))) (+ (.Z (Math|Vector|BreakVector (Variables|/Game/Blueprints/Player/BP_TinykinesisPlayerController.BP_TinykinesisPlayerController_C|GetTargetLocation (CallFunction|GetTinykinesisPlayerController)))) 1e+01)))
    (Class|BPITelekinesisObject|ReleaseObject(Message) (Variables|Default|GetItemGrabbed))
    (CallFunction|ClearParameters)
    (Default|TriggerAggroUsingAbility (CallFunction|GetTinykinesisPlayerController))
    (CallFunction|SetIddleAnimation)))

(fn PlayerCharge
  (if (Variables|/Game/Blueprints/Player/BP_TinykinesisPlayerController.BP_TinykinesisPlayerController_C|GetCanUseTelekinesis (CallFunction|GetTinykinesisPlayerController))
    (if (not (Variables|/Game/Blueprints/Player/BP_TinykinesisPlayerController.BP_TinykinesisPlayerController_C|GetIsCharging (CallFunction|GetTinykinesisPlayerController)))
      (Class|BPITelekinesisObject|ChargeObject(Message) (Variables|Default|GetItemGrabbed))
      (Variables|/Game/Blueprints/Player/BP_TinykinesisPlayerController.BP_TinykinesisPlayerController_C|SetIsCharging (CallFunction|GetTinykinesisPlayerController) true))))