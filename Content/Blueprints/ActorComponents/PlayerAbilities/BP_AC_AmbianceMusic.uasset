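; Actor component that plays the exploration ambience music as an FMOD event at its owner's location and controls its muting.
; On BeginPlay it stores the event instance and scales the play rate of the player controller's ExplorationSound timeline to a set length.
; UpdateTimeline feeds that timeline through a linear ramp-down curve into the event's "Mute" parameter, while FinishedTimeline is an empty stub.
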(event Custom|UpdateTimeline
  (Class|FMODBlueprintStatics|EventInstanceSetParameter (Variables|Default|GetExplorationAudioInst) "Mute" (CallFunction|TLCurve "/Niagara/DefaultAssets/Curves/Templates/LinearRampDown.LinearRampDown" (Variables|/Game/Blueprints/Player/BP_TinykinesisPlayerController.BP_TinykinesisPlayerController_C|GetExplorationSound (CallFunction|GetTinykinesisPlayerController)))))

(event Custom|Finished%20Timeline)

(event EventBeginPlay
  (bind _returnvalue (Class|FMODBlueprintStatics|PlayEventatLocation (Variables|Default|GetExplorationAudio) (Transformation|GetActorTransform (Components|GetOwner))))
  (Variables|Default|SetExplorationAudioInst _returnvalue)
  (Components|Timeline|SetPlayRate (Variables|/Game/Blueprints/Player/BP_TinykinesisPlayerController.BP_TinykinesisPlayerController_C|GetExplorationSound (CallFunction|GetTinykinesisPlayerController)) (/ 1.0 (Variables|Default|GetTimelineLenght))))