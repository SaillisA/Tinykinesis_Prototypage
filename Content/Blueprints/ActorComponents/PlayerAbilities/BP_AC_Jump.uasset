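; Player ability component for Tinykinesis that handles the double jump on the IA_Jump input.
; Pressing starts a load on the player controller; on trigger, an externally enabled flag allows the jump by retuning the character's jump limits.
; Ending the jump hides the wings icon and launches a controller-run cooldown, while trigger or cancel stops loading and restores single-jump settings.
; An older gravity-scale version remains unconnected in the event graph.
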(event Custom|DelayBeforeEndDoubleJump
  ;[1 1 1] La présence d'un délai contraint de le placer ici
  (Utilities|FlowControl|Delay 0.1)
  (CallFunction|EndDoubleJump))

(event Input|EnhancedActionEvents|EnhancedInputActionIA_Jump
  (params (ActionValue :type Boolean) (ElapsedSeconds :type Float%20%28double-precision%29) (TriggeredSeconds :type Float%20%28double-precision%29) (InputAction :type Input%20Action%20Object%20Reference :default "/Game/Blueprints/Player/Input/Actions/IA_Jump.IA_Jump"))
  (:Triggered
    (if (and (Variables|Default|GetCanDoubleJump) (Variables|Default|GetCanTriggerDoubleJump))
      (CallFunction|DoubleJump))
    (Default|StopLoadDoubleJump (CallFunction|GetTinykinesisPlayerController) :!label _label)
    (CallFunction|ResetJumpVariables))
  (:Started
    (CallFunction|ShortJump))
  (:Canceled
    (goto _label)))

(fn ChangeJumpConstraints
  (params (JumpMaxCount :type Integer) (JumpMaxHoldTime :type Float%20%28double-precision%29) (JumpZVelocity :type Float%20%28double-precision%29) (MaxWalkSpeed :type Float%20%28double-precision%29))
  (bind _tinykinesisplayercharacter (CallFunction|GetTinykinesisPlayerCharacter))
  (bind _charactermovement (Variables|/Script/Engine.Character|GetCharacterMovement _tinykinesisplayercharacter))
  (Variables|/Script/Engine.Character|SetJumpMaxCount _tinykinesisplayercharacter JumpMaxCount)
  (Variables|/Script/Engine.Character|SetJumpMaxHoldTime _tinykinesisplayercharacter JumpMaxHoldTime)
  (Variables|/Script/Engine.CharacterMovementComponent|SetJumpZVelocity _charactermovement JumpZVelocity)
  (Variables|/Script/Engine.CharacterMovementComponent|SetMaxWalkSpeed _charactermovement MaxWalkSpeed))

(fn ShortJump
  (if (Variables|Default|GetCanDoubleJump)
    (if (not (Variables|Default|GetInputPressedDoubleJump))
      (Variables|Default|SetInputPressedDoubleJump true)
      (Default|StartLoadDoubleJump (CallFunction|GetTinykinesisPlayerController)))))

(fn DoubleJump
  (CallFunction|ChangeJumpConstraints 2 0.1 5.2e+02 2.5e+02)
  (Character|Jump (CallFunction|GetTinykinesisPlayerCharacter))
  (Utilities|FlowControl|Sequence
    (:then_0
      ;[1 1 1] The Player is on ground
      (if (AI|Components|NavMovement|IsMovingonGround (Variables|/Script/Engine.Character|GetCharacterMovement (CallFunction|GetTinykinesisPlayerCharacter)))
        (CallFunction|EndDoubleJump)))
    (:then_1
      ;[1 1 1] The Input has been pressed one time
      (if (Variables|Default|GetInputPressedDoubleJump)
        (Variables|Default|SetInputPressedDoubleJump false)
        (CallFunction|DelayBeforeEndDoubleJump)))))

(fn EndDoubleJump
  (bind _tinykinesisplayercontroller (CallFunction|GetTinykinesisPlayerController))
  (bind _wbplifebar (Variables|/Game/Blueprints/Player/BP_TinykinesisPlayerController.BP_TinykinesisPlayerController_C|GetWBPLifeBar _tinykinesisplayercontroller))
  (bind _wingsfull (Variables|/Game/Blueprints/WidgetBlueprints/HUD/WBP_LifeBar.WBP_LifeBar_C|GetWingsFull _wbplifebar))
  ;[1 1 1] Disable the Double Jump for now
  (Variables|Default|SetCanDoubleJump false)
  (Widget|SetVisibility _wingsfull "Hidden")
  ;[1 1 1] Launch the cooldown for enabling access to jump later
  (Default|LaunchCooldown _tinykinesisplayercontroller "NewEnumerator0" (Variables|Default|GetDoubleJumpCooldown) _wingsfull))

(fn ResetJumpVariables
  (Variables|Default|SetCanTriggerDoubleJump false)
  (Variables|Default|SetInputPressedDoubleJump false)
  (CallFunction|ChangeJumpConstraints 1 0.0 5.2e+02 2.5e+02))