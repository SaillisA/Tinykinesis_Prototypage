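; Player ability component for Freeze Time, an unlockable ultimate that spends a full charge to slow the world while the player keeps normal speed.
; A timeline on the player controller and a curve blend global time dilation and a freeze post-process effect.
; The inverse dilation is applied to character, controller, telekinesis, jump and dash components, and any grabbed item.
; Finishing resets time dilation to normal.
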(event Custom|UpdateFreezeTime
  (bind _tinykinesisplayercontroller (CallFunction|GetTinykinesisPlayerController))
  (bind _freezetimetimer (Variables|/Game/Blueprints/Player/BP_TinykinesisPlayerController.BP_TinykinesisPlayerController_C|GetFreezeTimeTimer _tinykinesisplayercontroller))
  (bind _returnvalue (CallFunction|TLCurve "/Game/Miscellaneous/Curves/C_FreezeTime.C_FreezeTime" _freezetimetimer))
  (bind _output_get (Variables|TimeDilationMetrics|SetCurrentSlowTimeDilation (Math|Float|Lerp 1.0 (Variables|TimeDilationMetrics|GetMaxSlowTimeDilation) _returnvalue)))
  (bind _output_get_2 (Variables|TimeDilationMetrics|SetMyCustomTimeDilation (/ 1.0 (Variables|TimeDilationMetrics|GetCurrentSlowTimeDilation))))
  (CallFunction|SetTimeDilation _output_get true _output_get_2)
  (Variables|/Script/Engine.PostProcessComponent|SetBlendWeight (Variables|/Game/Blueprints/Player/BP_TinykinesisPlayerCharacter.BP_TinykinesisPlayerCharacter_C|GetPostProcessFreeze (Variables|Default|GetPlayerCharacter)) _returnvalue))

(event Custom|FinishedFreezeTime
  (Variables|TimeDilationMetrics|SetCurrentSlowTimeDilation 1.0)
  (Variables|TimeDilationMetrics|SetMyCustomTimeDilation 1.0)
  (CallFunction|SetTimeDilation 1.0 false 1.0))

(event Input|EnhancedActionEvents|EnhancedInputActionIA_FreezeTime
  (params (ActionValue :type Boolean) (ElapsedSeconds :type Float%20%28double-precision%29) (TriggeredSeconds :type Float%20%28double-precision%29) (InputAction :type Input%20Action%20Object%20Reference :default "/Game/Blueprints/Player/Input/Actions/IA_FreezeTime.IA_FreezeTime"))
  (bind _tinykinesisplayercontroller (CallFunction|GetTinykinesisPlayerController))
  (bind _freezetimetimer (Variables|/Game/Blueprints/Player/BP_TinykinesisPlayerController.BP_TinykinesisPlayerController_C|GetFreezeTimeTimer _tinykinesisplayercontroller))
  (:Started
    (if (and (Variables|BoolsVariables|GetFreezeTimeUnlocked) (== (Variables|ChargePoints|GetCurrentUltimateChargePoint) (Variables|ChargePoints|GetMaxUltimateChargePoint)))
      (Variables|ChargePoints|SetCurrentUltimateChargePoint (- (Variables|ChargePoints|GetCurrentUltimateChargePoint) (Variables|ChargePoints|GetMaxUltimateChargePoint)))
      (Components|Timeline|SetTimelineLength _freezetimetimer (Variables|DurationAbility|GetMaxTimer))
      (Components|Timeline|PlayfromStart _freezetimetimer)
      (Variables|Default|SetPlayerCharacter (CallFunction|GetTinykinesisPlayerCharacter)))))

(event EventBeginPlay)

(event EventTick
  (params (DeltaSeconds :type Float%20%28single-precision%29)))

(fn SetTimeDilation
  (params (Global%20Time%20Dilation :type Float%20%28double-precision%29) (IsFreezingTime :type Boolean) (Custom%20Time%20Dilation :type Float%20%28double-precision%29))
  (bind _tinykinesisplayercontroller (CallFunction|GetTinykinesisPlayerController))
  (bind _bp_ac_telekinesis (Variables|/Game/Blueprints/Player/BP_TinykinesisPlayerController.BP_TinykinesisPlayerController_C|GetBP_AC_Telekinesis _tinykinesisplayercontroller))
  (bind _itemgrabbed (Variables|/Game/Blueprints/ActorComponents/PlayerAbilities/BP_AC_Telekinesis.BP_AC_Telekinesis_C|GetItemGrabbed _bp_ac_telekinesis))
  (Utilities|Time|SetGlobalTimeDilation Global%20Time%20Dilation)
  (Utilities|FlowControl|Sequence
    (:then_0
      (bind _output_get (Variables|/Script/Engine.Actor|SetCustomTimeDilation (CallFunction|GetTinykinesisPlayerCharacter) Custom%20Time%20Dilation))
      (bind _output_get_2 (Variables|/Script/Engine.Actor|SetCustomTimeDilation _tinykinesisplayercontroller _output_get))
      (bind _output_get_3 (Variables|/Game/Blueprints/ActorComponents/PlayerAbilities/BP_AC_Telekinesis.BP_AC_Telekinesis_C|SetCurrentTimeDilation _bp_ac_telekinesis _output_get_2))
      (bind _output_get_4 (Variables|/Game/Blueprints/ActorComponents/PlayerAbilities/BP_AC_Jump.BP_AC_Jump_C|SetCurrentTimeDilation (Variables|/Game/Blueprints/Player/BP_TinykinesisPlayerController.BP_TinykinesisPlayerController_C|GetBP_AC_Jump _tinykinesisplayercontroller) _output_get_3))
      (Variables|/Game/Blueprints/ActorComponents/PlayerAbilities/BP_AC_Dash.BP_AC_Dash_C|SetCurrentTimeDilation (Variables|/Game/Blueprints/Player/BP_TinykinesisPlayerController.BP_TinykinesisPlayerController_C|GetBP_AC_Dash _tinykinesisplayercontroller) _output_get_4)
      (Variables|BoolsVariables|SetIsUsingFreezeTime IsFreezingTime))
    (:then_1
      (Utilities|IsValid _itemgrabbed
        (:Is%20Valid
          (Class|BPITelekinesisObject|SetCustomTimeDilation(Message) _itemgrabbed IsFreezingTime Custom%20Time%20Dilation))))))