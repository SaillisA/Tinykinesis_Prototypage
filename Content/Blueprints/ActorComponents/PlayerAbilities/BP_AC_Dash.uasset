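; Player ability component that gives the Tinykinesis character a short horizontal dash on the IA_Dash input when the controller's CanDash is set.
; It zeroes ground friction and gravity, then launches the character along its current velocity direction.
; After a brief delay, an opposite, slightly weaker launch brakes the dash and friction and gravity are restored.
; EndDash runs right after the first launch, clearing CanDash, hiding the life bar's dash indicator and starting the controller's cooldown.
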(event Input|EnhancedActionEvents|EnhancedInputActionIA_Dash
  (params (ActionValue :type Boolean) (ElapsedSeconds :type Float%20%28double-precision%29) (TriggeredSeconds :type Float%20%28double-precision%29) (InputAction :type Input%20Action%20Object%20Reference :default "/Game/Blueprints/Player/Input/Actions/IA_Dash.IA_Dash"))
  (bind _tinykinesisplayercharacter (CallFunction|GetTinykinesisPlayerCharacter))
  (bind _returnvalue (Transformation|GetVelocity _tinykinesisplayercharacter))
  (bind _returnvalue_2 (Math|Vector|Normalize _returnvalue))
  (bind _returnvalue_3 (* _returnvalue_2 2e+03))
  (bind _returnvalue_4 (* (Math|Vector|MakeVector (.x _returnvalue_3) (.y _returnvalue_3) 0.0) -0.95))
  (:Started
    (if (Variables|/Game/Blueprints/Player/BP_TinykinesisPlayerController.BP_TinykinesisPlayerController_C|GetCanDash (CallFunction|GetTinykinesisPlayerController))
      (CallFunction|ChangeDashConstraints 0.0 0.0)
      (Character|LaunchCharacter _tinykinesisplayercharacter (Math|Vector|MakeVector (.x _returnvalue_3) (.y _returnvalue_3) 0.0) false true)
      (CallFunction|EndDash)
      (Utilities|FlowControl|Delay 0.15)
      (Character|LaunchCharacter (CallFunction|GetTinykinesisPlayerCharacter) (Math|Vector|MakeVector (.x _returnvalue_4) (.y _returnvalue_4) 0.0) false true)
      (CallFunction|ChangeDashConstraints 8.0 1.0))))

(fn ChangeDashConstraints
  (params (NewGroundFriction :type Float%20%28double-precision%29) (NewGravity :type Float%20%28double-precision%29))
  (bind _tinykinesisplayercharacter (CallFunction|GetTinykinesisPlayerCharacter))
  (bind _charactermovement (Variables|/Script/Engine.Character|GetCharacterMovement _tinykinesisplayercharacter))
  (Variables|/Script/Engine.CharacterMovementComponent|SetGroundFriction _charactermovement NewGroundFriction)
  (Variables|/Script/Engine.CharacterMovementComponent|SetGravityScale _charactermovement NewGravity))

(fn EndDash
  (bind _tinykinesisplayercontroller (CallFunction|GetTinykinesisPlayerController))
  (bind _wbplifebar (Variables|/Game/Blueprints/Player/BP_TinykinesisPlayerController.BP_TinykinesisPlayerController_C|GetWBPLifeBar _tinykinesisplayercontroller))
  (bind _dashfull (Variables|/Game/Blueprints/WidgetBlueprints/HUD/WBP_LifeBar.WBP_LifeBar_C|GetDashFull _wbplifebar))
  (Variables|/Game/Blueprints/Player/BP_TinykinesisPlayerController.BP_TinykinesisPlayerController_C|SetCanDash _tinykinesisplayercontroller false)
  (Widget|SetVisibility _dashfull "Hidden")
  (Default|LaunchCooldown _tinykinesisplayercontroller "NewEnumerator1" (Variables|/Game/Blueprints/Player/BP_TinykinesisPlayerController.BP_TinykinesisPlayerController_C|GetDashCooldownDuration _tinykinesisplayercontroller) _dashfull))