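; Player ability component for Repulse ("Faery Wave"), a camera-aimed shockwave that costs power, which regenerates on Tick.
; Releasing input early casts the level 1 wave, while completing the charge casts level 2 with different range, impulse and VFX.
; Three yaw-fanned box traces collect targets, notifying BPI_RepulseSensitive actors and activating traps.
; PowerUpRepulse raises max power by one cast's cost, driving HUD unlocks and the first-use tutorial.
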(event Custom|Launch_VFXRepulse
  (params (Niagara%20System :type Niagara%20Component%20Object%20Reference))
  (bind _tinykinesisplayercharacter (CallFunction|GetTinykinesisPlayerCharacter))
  (bind _baserepulsemesh (Variables|/Game/Blueprints/Player/BP_TinykinesisPlayerCharacter.BP_TinykinesisPlayerCharacter_C|GetBaseRepulseMesh _tinykinesisplayercharacter))
  (Components|Activation|Activate Niagara%20System false)
  (Niagara|SetNiagaraVariable(Float) _baserepulsemesh "LifetimeTorus" (/ 0.3 (Variables|Default|GetCurrentTimeDilation)))
  (Components|Activation|Activate _baserepulsemesh true)
  (Utilities|FlowControl|Delay 0.1)
  (Components|Activation|Deactivate Niagara%20System))

(event Custom|Recovery_Repulse
  (Utilities|FlowControl|Delay 0.05)
  (Default|SetPlayerAnimRepulseState (CallFunction|GetTinykinesisPlayerCharacter) "NewEnumerator6"))

(event Input|EnhancedActionEvents|EnhancedInputActionIA_Repulse
  (params (ActionValue :type Boolean) (ElapsedSeconds :type Float%20%28double-precision%29) (TriggeredSeconds :type Float%20%28double-precision%29) (InputAction :type Input%20Action%20Object%20Reference :default "/Game/Blueprints/Player/Input/Actions/IA_Repulse.IA_Repulse"))
  (bind _tinykinesisplayercontroller (CallFunction|GetTinykinesisPlayerController))
  (bind _chargerepulsetimeline (Variables|/Game/Blueprints/Player/BP_TinykinesisPlayerController.BP_TinykinesisPlayerController_C|GetChargeRepulseTimeline _tinykinesisplayercontroller))
  (:Started
    (if (>= (Variables|PowerAmount|GetCurrentPower) (Variables|PowerAmount|GetCostPower))
      (Variables|Default|SetCanRepulse true)
      (Default|SetPlayerAnimRepulseState (CallFunction|GetTinykinesisPlayerCharacter) "NewEnumerator9")
      (Components|Timeline|SetTimelineLength _chargerepulsetimeline 1.0)
      (Components|Timeline|PlayfromStart _chargerepulsetimeline)
      (if (not (Variables|Default|GetTutorialRepulseDone))
        (Default|LaunchFadeOut (Variables|/Game/Blueprints/WidgetBlueprints/HUD/WBP_PlayerHUD.WBP_PlayerHUD_C|GetWBP_PopUpTuto (Variables|/Game/Blueprints/Player/BP_TinykinesisPlayerController.BP_TinykinesisPlayerController_C|GetWBPPlayerHUD _tinykinesisplayercontroller)) 1.0)
        (Variables|Default|SetTutorialRepulseDone true))
      (else
        (Variables|Default|SetCanRepulse false))))
  (:Canceled
    (CallFunction|CastRepulse (Variables|MetricsRepulse|GetRangeRepulseLevel1) (Variables|MetricsRepulse|GetPowerImpulseLevel1) (Variables|/Game/Blueprints/Player/BP_TinykinesisPlayerCharacter.BP_TinykinesisPlayerCharacter_C|GetBaseRepulse (CallFunction|GetTinykinesisPlayerCharacter))))
  (:Completed
    (CallFunction|CastRepulse (Variables|MetricsRepulse|GetRangeRepulseLevel2) (Variables|MetricsRepulse|GetPowerImpulseLevel2) (Variables|/Game/Blueprints/Player/BP_TinykinesisPlayerCharacter.BP_TinykinesisPlayerCharacter_C|GetChargedRepulse (CallFunction|GetTinykinesisPlayerCharacter)))))

(event EventBeginPlay
  (Utilities|FlowControl|Delay 0.1)
  (Variables|PowerAmount|SetCurrentPower (Variables|PowerAmount|GetMaxPower))
  (CallFunction|SetRepulseWidgetVisibility))

(event EventTick
  (params (DeltaSeconds :type Float%20%28single-precision%29))
  (if (< (Variables|PowerAmount|GetCurrentPower) (Variables|PowerAmount|GetMaxPower))
    (Variables|PowerAmount|SetCurrentPower (+ (Variables|PowerAmount|GetCurrentPower) (* DeltaSeconds (Variables|PowerAmount|GetRegenPowerMultiplier))))
    (else
      (Variables|PowerAmount|SetCurrentPower (Variables|PowerAmount|GetMaxPower)))))

(fn GetAllHitTargets
  (params (RangeRepulse :type Float%20%28double-precision%29))
  (bind _tinykinesisplayercharacter (CallFunction|GetTinykinesisPlayerCharacter))
  (bind _firstpersoncameracomponent (Variables|/Script/Tinykinesis_Proto.Tinykinesis_ProtoCharacter|GetFirstPersonCameraComponent _tinykinesisplayercharacter))
  (bind _returnvalue (Transformation|GetWorldLocation _firstpersoncameracomponent))
  (bind _returnvalue_2 (Transformation|GetWorldRotation _firstpersoncameracomponent))
  (Variables|Default|SetWorldLocation _returnvalue)
  (Variables|Default|SetWorldRotation _returnvalue_2)
  (Variables|Default|SetStartLocation (+ _returnvalue (* (Math|Vector|GetForwardVector _returnvalue_2) 1e+01)))
  (Utilities|FlowControl|Sequence
    (:then_0
      (CallFunction|RaycastRepulse RangeRepulse (Variables|Default|GetWorldRotation)))
    (:then_1
      (CallFunction|RaycastRepulse RangeRepulse (Math|Rotator|MakeRotator (.Roll (Math|Rotator|BreakRotator (Variables|Default|GetWorldRotation))) (.Pitch (Math|Rotator|BreakRotator (Variables|Default|GetWorldRotation))) (+ (.Yaw (Math|Rotator|BreakRotator (Variables|Default|GetWorldRotation))) 2e+01))))
    (:then_2
      (bind _endvector (CallFunction|GetEndVector (Variables|Default|GetWorldLocation) (Math|Rotator|MakeRotator (.Roll (Math|Rotator|BreakRotator (Variables|Default|GetWorldRotation))) (.Pitch (Math|Rotator|BreakRotator (Variables|Default|GetWorldRotation))) (- (.Yaw (Math|Rotator|BreakRotator (Variables|Default|GetWorldRotation))) 2e+01)) RangeRepulse))
      (bind _outhits (Class|KismetSystemLibrary|BoxTraceMulti (Variables|Default|GetStartLocation) _endvector (Math|Vector|MakeVector 0.0 (/ RangeRepulse 5.0) 1e+02) (Math|Rotator|MakeRotator (.Roll (Math|Rotator|BreakRotator (Variables|Default|GetWorldRotation))) (.Pitch (Math|Rotator|BreakRotator (Variables|Default|GetWorldRotation))) (- (.Yaw (Math|Rotator|BreakRotator (Variables|Default|GetWorldRotation))) 2e+01)) "TraceTypeQuery7" false 0 "None" true))
      (for _array_element _outhits
        (Utilities|Array|AddUnique (Variables|Default|GetArrayActors) (.HitActor (Collision|BreakHitResult _array_element)))
        (Utilities|Array|AddUnique (Variables|Default|GetArrayLocations) (.Location (Collision|BreakHitResult _array_element))))
      (return (Variables|Default|GetArrayActors) (Variables|Default|GetArrayLocations)))))

(fn GetEndVector
  (params (Location :type Vector) (Rotation :type Rotator) (RangeRepulse :type Float%20%28double-precision%29))
  (return (+ Location (* (Math|Vector|GetForwardVector Rotation) RangeRepulse))))

(fn EffectonHitElements
  (params (ArrayActors :type Array%20of%20Actor%20Object%20References) (LocationsHits :type Array%20of%20Vectors) (PowerImpulse :type Float%20%28double-precision%29))
  (for (_array_element _array_index) ArrayActors
    (Utilities|FlowControl|Sequence
      (:then_0
        (if (Utilities|DoesObjectImplementInterface _array_element "/Game/Blueprints/Interfaces/BPI_RepulseSensitive.BPI_RepulseSensitive_C")
          (Class|BPIRepulseSensitive|GetRepulsedWave(Message) _array_element PowerImpulse (Utilities|Array|Get(acopy) LocationsHits _array_index))))
      (:then_1
        (bind _asbp_abstract_activation_trap (Utilities|Casting|CastToBP_AbstractActivationTrap _array_element))
        (Default|ActivationEffect _asbp_abstract_activation_trap))))
  (Utilities|Array|Clear (Variables|Default|GetArrayActors))
  (Utilities|Array|Clear (Variables|Default|GetArrayLocations)))

(fn CastRepulse
  (params (RangeRepulse :type Float%20%28double-precision%29) (PowerImpulse :type Float%20%28double-precision%29) (Niagara%20System :type Niagara%20Component%20Object%20Reference) (Niagara%20System%20Mesh :type Niagara%20Component%20Object%20Reference))
  (if (Variables|Default|GetCanRepulse)
    (bind (_actorhit _locationhit) (CallFunction|GetAllHitTargets RangeRepulse))
    (CallFunction|EffectonHitElements _actorhit _locationhit PowerImpulse)
    (Variables|Default|SetCanRepulse false)
    (Variables|PowerAmount|SetCurrentPower (- (Variables|PowerAmount|GetCurrentPower) (Variables|PowerAmount|GetCostPower)))
    (CallFunction|LaunchVFXRepulse Niagara%20System)
    (Default|SetPlayerAnimRepulseState (CallFunction|GetTinykinesisPlayerCharacter) "NewEnumerator10")
    (CallFunction|RecoveryRepulse)
    (Default|CallOnRepulseEvent)))

(fn RaycastRepulse
  (params (RangeRepulse :type Float%20%28double-precision%29) (Orientation :type Rotator))
  (bind _endvector (CallFunction|GetEndVector (Variables|Default|GetWorldLocation) Orientation RangeRepulse))
  (bind _outhits (Class|KismetSystemLibrary|BoxTraceMulti (Variables|Default|GetStartLocation) _endvector (Math|Vector|MakeVector 0.0 (/ RangeRepulse 5.0) 1e+02) Orientation "TraceTypeQuery7" false 0 "None" true))
  (for _array_element _outhits
    (Utilities|Array|AddUnique (Variables|Default|GetArrayActors) (.HitActor (Collision|BreakHitResult _array_element)))
    (Utilities|Array|AddUnique (Variables|Default|GetArrayLocations) (.Location (Collision|BreakHitResult _array_element)))))

(fn PowerUpRepulse
  (bind _tinykinesisplayercontroller (CallFunction|GetTinykinesisPlayerController))
  (bind _tinykinesisplayercontroller_2 (CallFunction|GetTinykinesisPlayerController))
  (bind _wbpplayerhud (Variables|/Game/Blueprints/Player/BP_TinykinesisPlayerController.BP_TinykinesisPlayerController_C|GetWBPPlayerHUD _tinykinesisplayercontroller_2))
  (bind _wbpplayerhud_2 (Variables|/Game/Blueprints/Player/BP_TinykinesisPlayerController.BP_TinykinesisPlayerController_C|GetWBPPlayerHUD _tinykinesisplayercontroller))
  (bind _wbp_popuptuto (Variables|/Game/Blueprints/WidgetBlueprints/HUD/WBP_PlayerHUD.WBP_PlayerHUD_C|GetWBP_PopUpTuto _wbpplayerhud))
  (bind _wbp_cdability_repulse (Variables|/Game/Blueprints/WidgetBlueprints/HUD/WBP_PlayerHUD.WBP_PlayerHUD_C|GetWBP_CDAbility_Repulse _wbpplayerhud_2))
  (bind _output_get (Variables|PowerAmount|SetMaxPower (+ (Variables|PowerAmount|GetMaxPower) (Variables|PowerAmount|GetCostPower))))
  (Variables|PowerAmount|SetCurrentPower _output_get)
  (if (Variables|Default|GetRepulseUnlocked)
    (CallFunction|SetRepulseWidgetVisibility)
    (Default|LaunchAbilityAnimationUnlockLevel2 _wbp_cdability_repulse)
    (Variables|/Game/Blueprints/WidgetBlueprints/HUD/WBP_CooldownAbility.WBP_CooldownAbility_C|SetUnlockedLevel2 _wbp_cdability_repulse true)
    (else
      (Variables|Default|SetRepulseUnlocked true)
      (Default|SetValue _wbp_popuptuto "Cast Faery Wave" (Utilities|Struct|MakeSlateColor "(R=1.000000,G=0.768151,B=0.078187,A=1.000000)") "/Game/UI/Sprites/InputsPlayer/T_IconInputRightClick_Sprite.T_IconInputRightClick_Sprite" "/Game/UI/Sprites/InputsPlayer/T_IconInputLT_Sprite.T_IconInputLT_Sprite")
      (Default|LaunchFadein _wbp_popuptuto 1.0)
      (CallFunction|SetRepulseWidgetVisibility)
      (Default|LaunchAbilityAnimationUnlockLevel1 (Variables|/Game/Blueprints/WidgetBlueprints/HUD/WBP_PlayerHUD.WBP_PlayerHUD_C|GetWBP_CDAbility_Repulse _wbpplayerhud)))))

(fn SetRepulseWidgetVisibility
  (bind _tinykinesisplayercontroller (CallFunction|GetTinykinesisPlayerController))
  (bind _wbpplayerhud (Variables|/Game/Blueprints/Player/BP_TinykinesisPlayerController.BP_TinykinesisPlayerController_C|GetWBPPlayerHUD _tinykinesisplayercontroller))
  (bind _wbp_cdability_repulse (Variables|/Game/Blueprints/WidgetBlueprints/HUD/WBP_PlayerHUD.WBP_PlayerHUD_C|GetWBP_CDAbility_Repulse _wbpplayerhud))
  (bind _wbp_roundprogressbar_slot2 (Variables|/Game/Blueprints/WidgetBlueprints/HUD/WBP_CooldownAbility.WBP_CooldownAbility_C|GetWBP_RoundProgressBar_Slot2 _wbp_cdability_repulse))
  (bind _holderright_sprite (Variables|/Game/Blueprints/WidgetBlueprints/HUD/WBP_CooldownAbility.WBP_CooldownAbility_C|GetHolderRight_Sprite _wbp_cdability_repulse))
  (bind _backgroundright_sprite (Variables|/Game/Blueprints/WidgetBlueprints/HUD/WBP_CooldownAbility.WBP_CooldownAbility_C|GetBackgroundRight_Sprite _wbp_cdability_repulse))
  (Default|SetWidgetsVisibility _tinykinesisplayercontroller (Variables|Default|GetRepulseUnlocked) _wbp_cdability_repulse)
  (Default|LinkPlayerAbility _wbp_cdability_repulse (Variables|Default|GetTutorialRepulseDone))
  (if (and (Variables|Default|GetTutorialRepulseDone) (== (Variables|PowerAmount|GetMaxPower) 1e+02))
    (Default|SetWidgetsVisibility _tinykinesisplayercontroller true _wbp_roundprogressbar_slot2)
    (Default|SetWidgetsVisibility _tinykinesisplayercontroller true _holderright_sprite)
    (Default|SetWidgetsVisibility _tinykinesisplayercontroller true _backgroundright_sprite)
    (else
      (Default|SetWidgetsVisibility _tinykinesisplayercontroller false _wbp_roundprogressbar_slot2)
      (Default|SetWidgetsVisibility _tinykinesisplayercontroller false _holderright_sprite)
      (Default|SetWidgetsVisibility _tinykinesisplayercontroller false _backgroundright_sprite))))

(fn GetCurrentTimerRepulse)