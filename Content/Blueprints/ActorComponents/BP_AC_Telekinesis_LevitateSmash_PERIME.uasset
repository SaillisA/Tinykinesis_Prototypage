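; Deprecated (PERIME) telekinesis component for levitating and smashing the player's locked item, with all of its logic now disconnected.
; Both input events are empty, so none of the remaining chains run.
; The orphaned levitate chain messages the item and updates animation, input prompts and power state on the player controller.
; The orphaned smash chain releases the item, clears the lock and resets the DoOnce after a short delay.
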(event Input|EnhancedActionEvents|EnhancedInputActionIA_Levitate_PERIME
  (params (ActionValue :type Boolean) (ElapsedSeconds :type Float%20%28double-precision%29) (TriggeredSeconds :type Float%20%28double-precision%29) (InputAction :type Input%20Action%20Object%20Reference :default "/Game/Blueprints/Player/Input/Actions/IA_Levitate_PERIME.IA_Levitate_PERIME")))

(event Input|EnhancedActionEvents|EnhancedInputActionIA_Smash_PERIME
  (params (ActionValue :type Boolean) (ElapsedSeconds :type Float%20%28double-precision%29) (TriggeredSeconds :type Float%20%28double-precision%29) (InputAction :type Input%20Action%20Object%20Reference :default "/Game/Blueprints/Player/Input/Actions/IA_Smash_PERIME.IA_Smash_PERIME")))