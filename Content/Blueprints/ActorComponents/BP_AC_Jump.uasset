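; Actor component that handles jump input for the Tinykinesis player, including a cooldown-gated double jump.
; Press starts a double-jump load on the player controller; a trigger with the load ready raises the jump count and calls Jump.
; EndDoubleJump then disables the ability, hides the life bar wings and launches the cooldown.
; Trigger and cancel reset load state and single-jump constraints; an older V1 graph remains unconnected.
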(event Input|EnhancedActionEvents|EnhancedInputActionIA_Jump
  (params (ActionValue :type Boolean) (ElapsedSeconds :type Float%20%28double-precision%29) (TriggeredSeconds :type Float%20%28double-precision%29) (InputAction :type Input%20Action%20Object%20Reference :default "/Game/Blueprints/Player/Input/Actions/IA_Jump.IA_Jump"))
  (bind _tinykinesisplayercontroller (CallFunction|GetTinykinesisPlayerController))
  (bind _tinykinesisplayercontroller_2 (CallFunction|GetTinykinesisPlayerController))
  (bind _tinykinesisplayercontroller_3 (CallFunction|GetTinykinesisPlayerController))
  (:Triggered
    (if (and (Variables|/Game/Blueprints/Player/BP_TinykinesisPlayerController.BP_TinykinesisPlayerController_C|GetCanDoubleJump _tinykinesisplayercontroller_2) (Variables|/Game/Blueprints/Player/BP_TinykinesisPlayerController.BP_TinykinesisPlayerController_C|GetCanTriggerDoubleJump _tinykinesisplayercontroller_2))
      (Development|PrintString "Double jump")
      (CallFunction|ChangeJumpConstraints 2 0.1 5.2e+02 2.5e+02)
      (Character|Jump (CallFunction|GetTinykinesisPlayerCharacter))
      (CallFunction|EndDoubleJump))
    (Default|StopLoadDoubleJump _tinykinesisplayercontroller_3 :!label _label)
    (Variables|/Game/Blueprints/Player/BP_TinykinesisPlayerController.BP_TinykinesisPlayerController_C|SetCanTriggerDoubleJump _tinykinesisplayercontroller_3 false)
    (Variables|/Game/Blueprints/Player/BP_TinykinesisPlayerController.BP_TinykinesisPlayerController_C|SetInputPressedDoubleJump _tinykinesisplayercontroller_3 false)
    (CallFunction|ChangeJumpConstraints 1 0.0 5.2e+02 2.5e+02))
  (:Started
    (Development|PrintString "Short jump")
    (if (Variables|/Game/Blueprints/Player/BP_TinykinesisPlayerController.BP_TinykinesisPlayerController_C|GetCanDoubleJump _tinykinesisplayercontroller)
      (if (not (Variables|/Game/Blueprints/Player/BP_TinykinesisPlayerController.BP_TinykinesisPlayerController_C|GetInputPressedDoubleJump _tinykinesisplayercontroller))
        (Variables|/Game/Blueprints/Player/BP_TinykinesisPlayerController.BP_TinykinesisPlayerController_C|SetInputPressedDoubleJump _tinykinesisplayercontroller true)
        (Default|StartLoadDoubleJump (CallFunction|GetTinykinesisPlayerController)))))
  (:Canceled
    (goto _label)))

(fn ChangeJumpConstraints
  (params (JumpMaxCount :type Integer) (JumpMaxHoldTime :type Float%20%28double-precision%29) (JumpZVelocity :type Float%20%28double-precision%29) (MaxWalkSpeed :type Float%20%28double-precision%29))
  (bind _tinykinesisplayercharacter (CallFunction|GetTinykinesisPlayerCharacter))
  (bind _charactermovement (Variables|/Script/Engine.Character|GetCharacterMovement _tinykinesisplayercharacter))
  (Variables|/Script/Engine.Character|SetJumpMaxCount _tinykinesisplayercharacter JumpMaxCount)
  (Variables|/Script/Engine.Character|SetJumpMaxHoldTime _tinykinesisplayercharacter JumpMaxHoldTime)
  (Variables|/Script/Engine.CharacterMovementComponent|SetJumpZVelocity _charactermovement JumpZVelocity)
  (Variables|/Script/Engine.CharacterMovementComponent|SetMaxWalkSpeed _charactermovement MaxWalkSpeed))

(fn EndDoubleJump
  (bind _tinykinesisplayercontroller (CallFunction|GetTinykinesisPlayerController))
  (bind _tinykinesisplayercontroller_2 (CallFunction|GetTinykinesisPlayerController))
  (bind _wbplifebar (Variables|/Game/Blueprints/Player/BP_TinykinesisPlayerController.BP_TinykinesisPlayerController_C|GetWBPLifeBar _tinykinesisplayercontroller))
  (bind _wingsfull (Variables|/Game/Blueprints/WidgetBlueprints/HUD/WBP_LifeBar.WBP_LifeBar_C|GetWingsFull _wbplifebar))
  (Utilities|FlowControl|Sequence
    (:then_0
      ;[1 1 1] The Player is on ground
      (if (AI|Components|NavMovement|IsMovingonGround (Variables|/Script/Engine.Character|GetCharacterMovement (CallFunction|GetTinykinesisPlayerCharacter)))
        ;[1 1 1] Disable the Double Jump for now
        (Variables|/Game/Blueprints/Player/BP_TinykinesisPlayerController.BP_TinykinesisPlayerController_C|SetCanDoubleJump _tinykinesisplayercontroller false :!label _label)
        (Widget|SetVisibility _wingsfull "Hidden")
        ;[1 1 1] Launch the cooldown for enabling access to jump later
        (Default|LaunchCooldown _tinykinesisplayercontroller "NewEnumerator0" (Variables|/Game/Blueprints/Player/BP_TinykinesisPlayerController.BP_TinykinesisPlayerController_C|GetDoubleJumpCooldownDuration _tinykinesisplayercontroller) _wingsfull)))
    (:then_1
      ;[1 1 1] The Input has been pressed one time
      (if (Variables|/Game/Blueprints/Player/BP_TinykinesisPlayerController.BP_TinykinesisPlayerController_C|GetInputPressedDoubleJump _tinykinesisplayercontroller_2)
        (Variables|/Game/Blueprints/Player/BP_TinykinesisPlayerController.BP_TinykinesisPlayerController_C|SetInputPressedDoubleJump _tinykinesisplayercontroller_2 false)
        (goto _label)))))