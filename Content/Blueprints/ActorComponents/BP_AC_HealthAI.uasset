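; Actor component that tracks an AI character's health.
; On BeginPlay it sets HP to MaxHP.
; ManageHP subtracts incoming damage, prints the new HP and returns whether it has reached zero or below, leaving death handling to the caller.
; Getters expose current and maximum HP.
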(event EventBeginPlay
  (Variables|Default|SetHP (Variables|Default|GetmaxHP)))

(event EventTick
  (params (DeltaSeconds :type Float%20%28single-precision%29)))

(fn ManageHP
  (params (Dammage :type Float%20%28double-precision%29))
  (bind _output_get (Variables|Default|SetHP (- (Variables|Default|GetHP) Dammage)))
  (Development|PrintString (Utilities|String|ToString(Float) _output_get) true true "(R=0.434064,G=1.000000,B=0.271652,A=1.000000)")
  (if (<= _output_get 0.0)
    (return true)
    (else
      (return false))))

(fn GetActualHP
  (return (Variables|Default|GetHP)))

(fn GetMaxHP
  (return (Variables|Default|GetmaxHP)))