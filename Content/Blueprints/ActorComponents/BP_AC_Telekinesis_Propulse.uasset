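; Actor component that handles the telekinesis propulse input, launching the item the player currently holds.
; When telekinesis is active and powers are usable, it nudges the controller's target location upward and sends the item a Propulse message with that location, the right grab point's forward vector and target-lock state.
; It then consumes capacity, clears the selection, switches animations and, after a delay, briefly blocks power use.
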(event Input|EnhancedActionEvents|EnhancedInputActionIA_Propulse
  (params (ActionValue :type Boolean) (ElapsedSeconds :type Float%20%28double-precision%29) (TriggeredSeconds :type Float%20%28double-precision%29) (InputAction :type Input%20Action%20Object%20Reference :default "/Game/Blueprints/Player/Input/Actions/IA_Propulse.IA_Propulse"))
  (bind _tinykinesisplayercontroller (CallFunction|GetTinykinesisPlayerController))
  (bind _tinykinesisplayercontroller_2 (CallFunction|GetTinykinesisPlayerController))
  (bind _tinykinesisplayercontroller_3 (CallFunction|GetTinykinesisPlayerController))
  (bind _tinykinesisplayercontroller_4 (CallFunction|GetTinykinesisPlayerController))
  (bind _tinykinesisplayercontroller_5 (CallFunction|GetTinykinesisPlayerController))
  (if (and (Variables|/Game/Blueprints/Player/BP_TinykinesisPlayerController.BP_TinykinesisPlayerController_C|GetCanUsePower _tinykinesisplayercontroller_5) (Variables|/Game/Blueprints/Player/BP_TinykinesisPlayerController.BP_TinykinesisPlayerController_C|GetUsesTelekinesis _tinykinesisplayercontroller_5))
    (Default|Animation (CallFunction|GetTinykinesisPlayerCharacter) "NewEnumerator2")
    (bind _output_get (Variables|/Game/Blueprints/Player/BP_TinykinesisPlayerController.BP_TinykinesisPlayerController_C|SetTargetLocation _tinykinesisplayercontroller_2 (Math|Vector|MakeVector (.X (Math|Vector|BreakVector (Variables|/Game/Blueprints/Player/BP_TinykinesisPlayerController.BP_TinykinesisPlayerController_C|GetTargetLocation _tinykinesisplayercontroller_2))) (.Y (Math|Vector|BreakVector (Variables|/Game/Blueprints/Player/BP_TinykinesisPlayerController.BP_TinykinesisPlayerController_C|GetTargetLocation _tinykinesisplayercontroller_2))) (+ (.Z (Math|Vector|BreakVector (Variables|/Game/Blueprints/Player/BP_TinykinesisPlayerController.BP_TinykinesisPlayerController_C|GetTargetLocation _tinykinesisplayercontroller_2))) 1e+01))))
    (Class|BPIInteractable|Propulse(Message) (Variables|/Game/Blueprints/Player/BP_TinykinesisPlayerController.BP_TinykinesisPlayerController_C|GetSelectedItem _tinykinesisplayercontroller_3) _output_get (Math|Vector|GetForwardVector (Variables|/Game/Blueprints/Player/BP_TinykinesisPlayerCharacter.BP_TinykinesisPlayerCharacter_C|GetGrabPointR (CallFunction|GetTinykinesisPlayerCharacter))) (Variables|/Game/Blueprints/Player/BP_TinykinesisPlayerController.BP_TinykinesisPlayerController_C|GetHasTarget _tinykinesisplayercontroller_3))
    (Default|UsedCapacity _tinykinesisplayercontroller)
    (Variables|/Game/Blueprints/Player/BP_TinykinesisPlayerController.BP_TinykinesisPlayerController_C|SetUsingPower _tinykinesisplayercontroller false)
    (Variables|/Game/Blueprints/Player/BP_TinykinesisPlayerController.BP_TinykinesisPlayerController_C|SetSelectedItem _tinykinesisplayercontroller (Variables|/Game/Blueprints/Player/BP_TinykinesisPlayerController.BP_TinykinesisPlayerController_C|GetEmptyItem _tinykinesisplayercontroller))
    (Utilities|FlowControl|Delay 0.5)
    (Default|Animation (CallFunction|GetTinykinesisPlayerCharacter) "NewEnumerator6")
    (Variables|/Game/Blueprints/Player/BP_TinykinesisPlayerController.BP_TinykinesisPlayerController_C|SetCanUsePower _tinykinesisplayercontroller_4 false)
    (Utilities|FlowControl|Delay 0.5)
    (Variables|/Game/Blueprints/Player/BP_TinykinesisPlayerController.BP_TinykinesisPlayerController_C|SetCanUsePower _tinykinesisplayercontroller_4 true)))