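; Actor component that pulls telekinesis objects to the player's grab point and launches them on release.
; An externally fed tick event drives both: grabbing moves the mesh in, then lerp-follows the hand while rotating it.
; Release re-issues MoveComponentTo toward a live target, raised if floor-bound, or moves once toward the camera aim point.
; Travel time is distance over speed, also timing the owner's emissive tattoo fades alongside audio and animations.
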(event Custom|AttractObject
  (params (Mesh :type Mesh%20Component%20Object%20Reference) (SpeedGrab :type Float%20%28double-precision%29))
  ;[0.1041 0.6523 1] Attract
  (Utilities|FlowControl|Sequence
    (:then_0
      ;;[1 1 1] Do Once
      (Utilities|FlowControl|DoOnce false
        (:Completed
          (CallFunction|DoOnceAttract SpeedGrab Mesh)
          (Components|MoveComponentTo Mesh (Transformation|GetWorldLocation (Variables|/Game/Blueprints/Player/BP_TinykinesisPlayerCharacter.BP_TinykinesisPlayerCharacter_C|GetGrabPointR (CallFunction|GetTinykinesisPlayerCharacter))) (Transformation|GetWorldRotation (Variables|/Script/Tinykinesis_Proto.Tinykinesis_ProtoCharacter|GetFirstPersonCameraComponent (CallFunction|GetTinykinesisPlayerCharacter))) false false (Variables|Default|GetDurationAbitility) false)
          (Variables|Default|SetReachedPlayer true)
          (bind _returnvalue (Class|FMODBlueprintStatics|PlayEventatLocation (Variables|Default|GetAudioEvent) (Transformation|GetActorTransform (CallFunction|GetTinykinesisPlayerCharacter))))
          (Variables|Default|SetAudioInstance _returnvalue)
          (bind _asbp_abstract_telekinesis_element (Utilities|Casting|CastToBP_AbstractTelekinesisElement (Components|GetOwner)))
          (Default|RotationEvent _asbp_abstract_telekinesis_element))))
    (:then_1
      (Variables|Default|SetTargetLocation (Transformation|GetWorldLocation (Variables|/Game/Blueprints/Player/BP_TinykinesisPlayerCharacter.BP_TinykinesisPlayerCharacter_C|GetGrabPointR (CallFunction|GetTinykinesisPlayerCharacter))))
      (if (Variables|Default|GetReachedPlayer)
        (Transformation|SetWorldLocation Mesh (Math|Vector|Lerp(Vector) (Transformation|GetWorldLocation Mesh) (Variables|Default|GetTargetLocation) (* (Utilities|Time|GetWorldDeltaSeconds) 8.0)) true false)))))

(event Custom|DropObject
  (params (Mesh :type Mesh%20Component%20Object%20Reference))
  ;[0.5208 0.814 1] Drop
  (Utilities|FlowControl|Sequence
    (:then_0
      ;[0.1041 0.6523 1] Attract
      ;;[1 1 1] Do Once
      (Utilities|FlowControl|DoOnce false) ; enters at Reset
    )
    (:then_1
      (Variables|Default|SetReachedPlayer false)
      (Class|FMODBlueprintStatics|EventInstanceStop (Variables|Default|GetAudioInstance) false))))

(event Custom|ResetEmissiveStandard
  (params (DelayDuration :type Float%20%28double-precision%29))
  (Development|PrintString (Utilities|String|ToString(Float) DelayDuration))
  (Utilities|FlowControl|Delay DelayDuration)
  (Development|PrintString "Hello")
  (bind _asbp_abstract_telekinesis_element (Utilities|Casting|CastToBP_AbstractTelekinesisElement (Components|GetOwner)))
  (Default|EmissiveTatoosChanges _asbp_abstract_telekinesis_element 0.2 0.2))

(event Custom|PropulseObject
  (params (Mesh :type Mesh%20Component%20Object%20Reference) (SpeedRelease :type Float%20%28double-precision%29))
  (Class|FMODBlueprintStatics|EventInstanceStop (Variables|Default|GetAudioInstance) false)
  ;[1 0.1667 0.6787] Release
  (Rendering|SetVisibility (Variables|/Game/Blueprints/Player/BP_TinykinesisPlayerCharacter.BP_TinykinesisPlayerCharacter_C|GetSparksHand (CallFunction|GetTinykinesisPlayerCharacter)) false false)
  (Utilities|FlowControl|Sequence
    (:then_0
      ;;[1 1 1] Do Once
      (Utilities|FlowControl|DoOnce false
        (:Completed
          (CallFunction|DoOncePropulse Mesh SpeedRelease)
          (Utilities|IsValid (Variables|Default|GetTargetRelease)
            (:Is%20Not%20Valid
              (Development|PrintString "NO TARGET")
              ;;;[1 1 1] If No Target : Launch in front of player
              (Components|MoveComponentTo Mesh (Variables|Default|GetTargetLocation) (Variables|/Script/Engine.SceneComponent|GetRelativeRotation Mesh) false false (Variables|Default|GetDurationAbitility) false))))))
    (:then_1
      ;;[1 1 1] If Target : Launch to Target in real time
      (Utilities|IsValid (Variables|Default|GetTargetRelease)
        (:Is%20Valid
          (Development|PrintString "MOVE TO TARGET")
          (Utilities|FlowControl|Sequence
            (:then_0
              (Components|MoveComponentTo Mesh (CallFunction|GetTargetRelativeRotation) (Variables|/Script/Engine.SceneComponent|GetRelativeRotation Mesh) false false (Variables|Default|GetDurationAbitility) false))
            (:then_1
              (Variables|Default|SetDurationAbitility (- (Variables|Default|GetDurationAbitility) (Utilities|Time|GetWorldDeltaSeconds))))))))))

(event Custom|Tick_AttractiveElement
  (params (Mesh :type Mesh%20Component%20Object%20Reference) (SpeedGrab :type Float%20%28double-precision%29) (SpeedRelease :type Float%20%28double-precision%29) (IsBeingGrabbed :type Boolean) (IsBeingReleased :type Boolean) (CurrentRotation :type Rotator))
  (bind _returnvalue (Utilities|Time|GetWorldDeltaSeconds))
  (bind _relativerotation (Variables|/Script/Engine.SceneComponent|GetRelativeRotation Mesh))
  (bind _returnvalue_2 (Math|Rotator|Lerp(Rotator) _relativerotation CurrentRotation _returnvalue true))
  ;[0.7412 1 0.3412] TICK
  (Utilities|FlowControl|Sequence
    (:then_0
      ;;[1 1 1] Attract and Propulse in real time
      (if IsBeingGrabbed
        (CallFunction|AttractObject Mesh SpeedGrab)
        (elif IsBeingReleased
          (CallFunction|PropulseObject Mesh SpeedRelease))))
    (:then_1
      ;;[1 1 1] Rotate the projectile for flavor purpose
      (if IsBeingGrabbed
        (Transformation|SetRelativeRotation Mesh (Math|Rotator|MakeRotator (.roll _returnvalue_2) (.pitch _returnvalue_2) (.yaw (Transformation|GetWorldRotation (Variables|/Script/Tinykinesis_Proto.Tinykinesis_ProtoCharacter|GetFirstPersonCameraComponent (CallFunction|GetTinykinesisPlayerCharacter))))) false false)))))

(fn DoOnceAttract
  (params (SpeedAttract :type Float%20%28double-precision%29) (Mesh :type Primitive%20Component%20Object%20Reference))
  (CallFunction|SetDurationAbility SpeedAttract (Math|Vector|Distance(Vector) (Transformation|GetWorldLocation Mesh) (Transformation|GetWorldLocation (Variables|/Script/Tinykinesis_Proto.Tinykinesis_ProtoCharacter|GetFirstPersonCameraComponent (CallFunction|GetTinykinesisPlayerCharacter)))))
  (bind _asbp_abstract_telekinesis_element (Utilities|Casting|CastToBP_AbstractTelekinesisElement (Components|GetOwner)))
  (Default|EmissiveTatoosChanges _asbp_abstract_telekinesis_element 1e+01 (Variables|Default|GetDurationAbitility)))

(fn DoOncePropulse
  (params (Mesh :type Primitive%20Component%20Object%20Reference) (Speed :type Float%20%28double-precision%29))
  (bind _tinykinesisplayercharacter (CallFunction|GetTinykinesisPlayerCharacter))
  (bind _tinykinesisplayercharacter_2 (CallFunction|GetTinykinesisPlayerCharacter))
  (bind _firstpersoncameracomponent (Variables|/Script/Tinykinesis_Proto.Tinykinesis_ProtoCharacter|GetFirstPersonCameraComponent _tinykinesisplayercharacter_2))
  (Default|ObjectAnimation _tinykinesisplayercharacter "NewEnumerator0")
  (Default|Animation _tinykinesisplayercharacter "NewEnumerator2")
  (if (Variables|/Game/Blueprints/ActorComponents/PlayerAbilities/BP_AC_Telekinesis.BP_AC_Telekinesis_C|GetHasTarget (Variables|/Game/Blueprints/Player/BP_TinykinesisPlayerController.BP_TinykinesisPlayerController_C|GetBP_AC_Telekinesis (CallFunction|GetTinykinesisPlayerController)))
    ;[1 1 1] If Target : SetParameters to MoveTo
    (Variables|Default|SetTargetRelease (Variables|/Game/Blueprints/ActorComponents/PlayerAbilities/BP_AC_Telekinesis.BP_AC_Telekinesis_C|GetActualTarget (Variables|/Game/Blueprints/Player/BP_TinykinesisPlayerController.BP_TinykinesisPlayerController_C|GetBP_AC_Telekinesis (CallFunction|GetTinykinesisPlayerController))))
    (CallFunction|SetDurationAbility Speed (Math|Vector|Distance(Vector) (Transformation|GetWorldLocation (Actor|GetComponentbyClass (Variables|Default|GetTargetRelease) "/Script/Engine.MeshComponent")) (Transformation|GetWorldLocation (Variables|/Script/Tinykinesis_Proto.Tinykinesis_ProtoCharacter|GetFirstPersonCameraComponent (CallFunction|GetTinykinesisPlayerCharacter)))))
    (Utilities|FlowControl|Sequence
      (:then_0
        (bind _returnvalue (Collision|SphereTraceByChannel (Transformation|GetActorLocation (Variables|Default|GetTargetRelease)) (Math|Vector|MakeVector (.X (Math|Vector|BreakVector (Transformation|GetActorLocation (Variables|Default|GetTargetRelease)))) (.Y (Math|Vector|BreakVector (Transformation|GetActorLocation (Variables|Default|GetTargetRelease)))) (+ (.Z (Math|Vector|BreakVector (Transformation|GetActorLocation (Variables|Default|GetTargetRelease)))) -1e+02)) 5e+01 "TraceTypeQuery5" false 0 "Persistent"))
        (if _returnvalue
          (Variables|Default|SetTargetIsOnFloor true)
          (Development|PrintString "On Floor")
          (else
            (Variables|Default|SetTargetIsOnFloor false)
            (Development|PrintString "NOT On Floor"))))
      (:then_1
        (CallFunction|ReleaseChangeEmissive)))
    (else
      ;[1 1 1] If NO Target : SetParameters to MoveTo
      (Utilities|FlowControl|Sequence
        (:then_0
          (Physics|SetPhysicsLinearVelocity Mesh "0, 0, 0" false "None")
          (bind _outactors (Actor|GetAllActorswithInterface "/Game/Blueprints/Interfaces/BPI_TelekinesisObject.BPI_TelekinesisObject_C"))
          (bind (_start _end) (Default|GetAimCastDistance (Variables|/Game/Blueprints/Player/BP_TinykinesisPlayerController.BP_TinykinesisPlayerController_C|GetBP_AC_Telekinesis (CallFunction|GetTinykinesisPlayerController)) 1e+05))
          (bind (_outhit _returnvalue_2) (Collision|LineTraceByChannel _start _end "TraceTypeQuery1" false _outactors "None"))
          (if _returnvalue_2
            (Variables|Default|SetTargetLocation (.location _outhit))
            (Variables|Default|SetOut%20Hit%20Distance (.distance _outhit))
            (Variables|Default|SetRaycastHit true)
            (else
              (Variables|Default|SetTargetLocation (+ (Transformation|GetWorldLocation _firstpersoncameracomponent) (* (Math|Vector|GetForwardVector (Transformation|GetWorldRotation _firstpersoncameracomponent)) 1e+05)))
              (Variables|Default|SetOut%20Hit%20Distance 1e+05))))
        (:then_1
          (CallFunction|SetDurationAbility Speed (Variables|Default|GetOut%20Hit%20Distance))
          (CallFunction|ReleaseChangeEmissive))))))

(fn SetDurationAbility
  (params (Speed :type Float%20%28double-precision%29) (DistancePlayerTarget :type Float%20%28double-precision%29))
  (Variables|Default|SetDurationAbitility (/ DistancePlayerTarget Speed)))

(fn GetTargetRelativeRotation
  (bind _targetrelease (Variables|Default|GetTargetRelease))
  (bind _targetrelease_2 (Variables|Default|GetTargetRelease))
  (bind _returnvalue (Actor|GetComponentbyClass _targetrelease_2 "/Script/Engine.MeshComponent"))
  (bind _returnvalue_2 (Actor|GetComponentbyClass _targetrelease "/Script/Engine.MeshComponent"))
  (bind _returnvalue_3 (Transformation|GetWorldLocation _returnvalue))
  (bind _returnvalue_4 (Transformation|GetWorldLocation _returnvalue_2))
  (if (Variables|Default|GetTargetIsOnFloor)
    (LocalVariables|SetZTargetLocation (+ (.z _returnvalue_4) 5e+01))
    (else
      (LocalVariables|SetZTargetLocation (.z _returnvalue_4))))
  (return (Math|Vector|MakeVector (.x _returnvalue_3) (.y _returnvalue_3) (LocalVariables|GetZTargetLocation))))

(fn ReleaseChangeEmissive
  (bind _asbp_abstract_telekinesis_element (Utilities|Casting|CastToBP_AbstractTelekinesisElement (Components|GetOwner)))
  (Default|EmissiveTatoosChanges _asbp_abstract_telekinesis_element 0.2 1.0))