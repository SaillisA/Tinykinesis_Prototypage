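; Actor component that links an AI mob to the arena manager that tracks it in the current wave.
; On BeginPlay it binds delegates to the death event of the health component on the mob's AI controller and to the character's became-aggro event.
; SetArenaManager stores the manager reference, and RemoveFromCurrentWave takes the owning mob out of that manager's CurrentWave.
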(event EventBeginPlay
  (bind _asbp_aicharacter_blank (Utilities|Casting|CastToBP_AICharacterBlank (Components|GetOwner)))
  (EventDispatchers|BindEventtoDeath (Actor|GetComponentbyClass (AI|GetAIController _asbp_aicharacter_blank) "/Game/Blueprints/ActorComponents/BP_AC_Health.BP_AC_Health_C") (EventDispatchers|CreateEvent :!event RemovefromCurrentWave))
  (EventDispatchers|BindEventtoOnBecameAggro _asbp_aicharacter_blank (EventDispatchers|CreateEvent (Variables|Default|GetArenaManager) :!event TriggerCombat)))

(fn SetArenaManager
  (params (ArenaManager :type BP%20Abstract%20Arena%20Manager%20Object%20Reference))
  (Variables|Default|SetArenaManager ArenaManager))

(fn RemovefromCurrentWave
  (bind _asbp_aicharacter_blank (Utilities|Casting|CastToBP_AICharacterBlank (Components|GetOwner)))
  (Utilities|Array|RemoveItem (Variables|/Game/Blueprints/Actors/ArenaManagement/BP_AbstractArenaManager.BP_AbstractArenaManager_C|GetCurrentWave (Variables|Default|GetArenaManager)) _asbp_aicharacter_blank))