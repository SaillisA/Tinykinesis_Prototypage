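; Health component that tracks an actor's current HP against a maximum, starting full at BeginPlay.
; LooseHP subtracts damage, broadcasts the HP change, then fires either the death or damage-effect event and returns whether the owner died plus the HP left.
; HealHP adds HP capped at the maximum and broadcasts the change, while damage has no lower clamp, so HP can drop below zero.
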(event EventBeginPlay
  (Variables|Default|SetcurrentHP (Variables|Default|GetmaxHP)))

(fn LooseHP
  (params (Dammage :type Float%20%28double-precision%29))
  (bind _output_get (Variables|Default|SetcurrentHP (- (Variables|Default|GetcurrentHP) Dammage)))
  (Default|CallOnHPChanged _output_get)
  (if (<= _output_get 0.0)
    (Default|CallDeath)
    (return true (Variables|Default|GetcurrentHP))
    (else
      (Default|CallDamageEffect)
      (return false (Variables|Default|GetcurrentHP)))))

(fn HealHP
  (params (HPValueHealed :type Float%20%28double-precision%29))
  (bind _output_get (Variables|Default|SetcurrentHP (+ (Variables|Default|GetcurrentHP) HPValueHealed)))
  (if (> _output_get (Variables|Default|GetmaxHP))
    (Variables|Default|SetcurrentHP (Variables|Default|GetmaxHP)))
  (Default|CallOnHPChanged (Variables|Default|GetcurrentHP))
  (return (Variables|Default|GetcurrentHP)))