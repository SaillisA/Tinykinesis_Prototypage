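; First-person player character for Tinykinesis, handling hit reactions, death, fall respawn, movement sounds and right-hand animation state.
; Hits go through the controller's health component, whose bound events drive knockback, camera shake, a directional damage indicator and timed invincibility, or reload the level on death.
; A timeline fades the invulnerability post-process, and tags on the telekinesis-held item select the hand's animation object type.
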(event Custom|FallRespawn
  (bind _tinykinesisplayercontroller (CallFunction|GetTinykinesisPlayerController))
  (bind _tinykinesisplayercontroller_2 (CallFunction|GetTinykinesisPlayerController))
  (bind _bp_ac_health (Variables|/Game/Blueprints/Player/BP_TinykinesisPlayerController.BP_TinykinesisPlayerController_C|GetBP_AC_Health _tinykinesisplayercontroller))
  (Default|FallDamageWhiteScreen (Variables|Default|GetFallDamageIndicator))
  (Input|DisableInput (CallFunction|GetTinykinesisPlayerController))
  (Utilities|FlowControl|Delay 0.5)
  (Default|FallRespawnWhiteScreen (Variables|Default|GetFallDamageIndicator))
  (Transformation|SetActorTransform (Variables|/Game/Blueprints/Player/BP_TinykinesisPlayerController.BP_TinykinesisPlayerController_C|GetFall_RespawnTransform _tinykinesisplayercontroller_2) false true)
  (Input|EnableInput _tinykinesisplayercontroller_2)
  (EventDispatchers|UnbindallEventsfromDamageEffect _bp_ac_health)
  (EventDispatchers|BindEventtoDamageEffect _bp_ac_health (EventDispatchers|CreateEvent :!event Custom|DamageFeedback_Player)))

(event Custom|MoveSound
  ;[1 1 1] Sound
  (if (and (AI|Components|NavMovement|IsMovingonGround (Variables|Character|GetCharacterMovement)) (> (Math|Vector|VectorLengthXY (Transformation|GetVelocity self)) 1e+01))
    (Utilities|FlowControl|Delay 0.3)
    (bind _returnvalue (Class|FMODBlueprintStatics|PlayEventatLocation "/Game/Fmod/Events/Footsteps.Footsteps" (Transformation|GetActorTransform)))
    (else
      (Class|FMODBlueprintStatics|EventInstanceStop _returnvalue false))))

(event Custom|EventGetHit
  (params (ImpactLocation :type Vector) (KnockbackForce :type Vector) (Dammage :type Float%20%28double-precision%29))
  (bind _tinykinesisplayercontroller (CallFunction|GetTinykinesisPlayerController))
  (bind _bp_ac_health (Variables|/Game/Blueprints/Player/BP_TinykinesisPlayerController.BP_TinykinesisPlayerController_C|GetBP_AC_Health _tinykinesisplayercontroller))
  ;[1 0.2706 0.3098] Event when hit
  (if (not (Variables|/Game/Blueprints/ActorComponents/BP_AC_Health.BP_AC_Health_C|GetInvicibility _bp_ac_health))
    (Variables|/Game/Blueprints/ActorComponents/BP_AC_Health.BP_AC_Health_C|SetInvicibility _bp_ac_health true)
    (Variables|/Script/Engine.PostProcessComponent|SetBlendWeight (Variables|Default|GetPostProcessInvulnerability) 1.0)
    (CallFunction|SetImpactParameters ImpactLocation KnockbackForce)
    (Utilities|FlowControl|Sequence
      (:then_0
        (bind _fading (Timeline|Invicibility PlayFromStart)
          (:Update
            (Variables|/Script/Engine.PostProcessComponent|SetBlendWeight (Variables|Default|GetPostProcessInvulnerability) _fading))))
      (:then_1
        (Default|LooseHP (Variables|/Game/Blueprints/Player/BP_TinykinesisPlayerController.BP_TinykinesisPlayerController_C|GetBP_AC_Health (CallFunction|GetTinykinesisPlayerController)) Dammage)))))

(event Custom|Death_Player
  (bind _tinykinesisplayercontroller (CallFunction|GetTinykinesisPlayerController))
  ;[0.3137 0.06274 0.06667] Death Specificity for NpcMelee
  (Default|DeathBlackScreen (Variables|/Game/Blueprints/Player/BP_TinykinesisPlayerController.BP_TinykinesisPlayerController_C|GetWBPBlackScreen _tinykinesisplayercontroller))
  (Input|DisableInput _tinykinesisplayercontroller)
  (Utilities|FlowControl|Delay 1.5)
  (bind _returnvalue (Game|GetCurrentLevelName true))
  (Game|OpenLevel(byName) (Utilities|String|StringToName _returnvalue) false))

(event Custom|DamageFeedback_Player
  (bind _tinykinesisplayercontroller (CallFunction|GetTinykinesisPlayerController))
  (bind _returnvalue (Transformation|GetActorLocation))
  (bind _impactlocation (Variables|ImpactVars|GetImpactLocation))
  (bind _knockbackforce (Variables|ImpactVars|GetKnockbackForce))
  (bind _firstpersoncameracomponent (Variables|Default|GetFirstPersonCameraComponent))
  (bind _returnvalue_2 (- _returnvalue _impactlocation))
  (bind _returnvalue_3 (Math|Vector|Normalize _returnvalue_2))
  (bind _returnvalue_4 (* _returnvalue_3 (.x _knockbackforce)))
  ;[0.3137 0.06274 0.06667] Damage specificity for MeleeMobs : knockback & stuns
  (Class|Widget|SetRenderTransformAngle (Variables|/Game/Blueprints/WidgetBlueprints/HUD/WBP_DamageIndicator.WBP_DamageIndicator_C|GetHitMarker (Variables|Default|GetFallDamageIndicator)) (- (.yaw (Math|Rotator|FindLookatRotation (Transformation|GetWorldLocation _firstpersoncameracomponent) (Variables|ImpactVars|GetImpactLocation))) (.yaw (Transformation|GetWorldRotation _firstpersoncameracomponent))))
  (Default|HitDamageWhiteScreen (Variables|Default|GetFallDamageIndicator))
  (Camera|PlayWorldCameraShake "/Game/Blueprints/Actors/CameraManager/BP_TakeDamageCameraShake.BP_TakeDamageCameraShake_C" (Transformation|GetActorLocation) 0.0 5e+02)
  (Character|LaunchCharacter (Math|Vector|MakeVector (.x _returnvalue_4) (.y _returnvalue_4) (.z _knockbackforce)) false false)
  (Variables|/Game/Blueprints/Player/BP_TinykinesisPlayerController.BP_TinykinesisPlayerController_C|SetGotHit (CallFunction|GetTinykinesisPlayerController) true)
  (Utilities|FlowControl|Delay (Variables|Default|GetInvulnerabilityFramesDuration))
  (Variables|/Game/Blueprints/Player/BP_TinykinesisPlayerController.BP_TinykinesisPlayerController_C|SetGotHit _tinykinesisplayercontroller false)
  (Variables|/Game/Blueprints/ActorComponents/BP_AC_Health.BP_AC_Health_C|SetInvicibility (Variables|/Game/Blueprints/Player/BP_TinykinesisPlayerController.BP_TinykinesisPlayerController_C|GetBP_AC_Health _tinykinesisplayercontroller) false))

(event EventBeginPlay
  (bind _tinykinesisplayercontroller (CallFunction|GetTinykinesisPlayerController))
  (bind _bp_ac_health (Variables|/Game/Blueprints/Player/BP_TinykinesisPlayerController.BP_TinykinesisPlayerController_C|GetBP_AC_Health _tinykinesisplayercontroller))
  ;[0.298 1 0.5765] BeginPlay
  (Variables|/Script/Engine.PostProcessComponent|SetBlendWeight (Variables|Default|GetPostProcessInvulnerability) 0.0)
  (Variables|/Script/Engine.PostProcessComponent|SetBlendWeight (Variables|Default|GetPostProcessFreeze) 0.0)
  (Variables|/Script/Engine.PostProcessComponent|SetBlendWeight (Variables|Default|GetPostProcessChargeTelekinesis) 0.0)
  (Variables|/Script/Engine.PostProcessComponent|SetBlendWeight (Variables|Default|GetPostProcessDash) 0.0)
  (Variables|/Script/Engine.PostProcessComponent|SetBlendWeight (Variables|Default|GetPostProcessJumpExhausted) 0.0)
  (EventDispatchers|BindEventtoDeath _bp_ac_health (EventDispatchers|CreateEvent :!event Custom|Death_Player))
  (EventDispatchers|BindEventtoDamageEffect _bp_ac_health (EventDispatchers|CreateEvent :!event Custom|DamageFeedback_Player))
  (bind _returnvalue (UserInterface|CreateWidget "/Game/Blueprints/WidgetBlueprints/HUD/WBP_DamageIndicator.WBP_DamageIndicator_C"))
  (bind _output_get (Variables|Default|SetFallDamageIndicator _returnvalue))
  (UserInterface|Viewport|AddtoViewport _output_get 0)
  (Variables|Default|SetValueSensitivity (Variables|/Game/Blueprints/SaveSystem/BP_GameInstanceTinykinesis.BP_GameInstanceTinykinesis_C|GetSensitivityMouse (CallFunction|GetTinykinesisGameInstance)))
  (Rendering|SetVisibility (Variables|Default|GetSparksHand) false false))

(event EventOnLanded
  (params (Hit :type Hit%20Result%20Structure%20%28by%20ref%29))
  ;[1 1 1] Sound
  (Class|FMODBlueprintStatics|PlayEventatLocation "/Game/Fmod/Events/Landed.Landed" (Transformation|GetActorTransform))
  (Variables|/Game/Blueprints/ActorComponents/PlayerAbilities/BP_AC_Jump.BP_AC_Jump_C|SetCanDoubleJump (Variables|/Game/Blueprints/Player/BP_TinykinesisPlayerController.BP_TinykinesisPlayerController_C|GetBP_AC_Jump (CallFunction|GetTinykinesisPlayerController)) true))

(event EventTick
  (params (DeltaSeconds :type Float%20%28single-precision%29))
  (CallFunction|MoveSound))

(fn ConstructionScript
  (bind _returnvalue (Rendering|Material|CreateDynamicMaterialInstance (Variables|Default|GetMesh1P) 0 "/Game/Characters/Player/Materials/M_RightHand_002.M_RightHand_002" "EmissiveParameter" :!class /Script/Engine.PrimitiveComponent))
  (Variables|Default|SetHandMaterialInstance _returnvalue))

(fn ResetVarAnim
  (return))

(fn Animation
  (params (NewParam :type E_PlayerStates%20Enum :default "NewEnumerator6"))
  (bind _asabp_player_character_right_hand_animations (Utilities|Casting|CastToABP_PlayerCharacterRightHandAnimations (Components|SkeletalMesh|GetAnimInstance (Variables|Default|GetMesh1P))))
  (Variables|/Game/Characters/Player/Animations/ABP_PlayerCharacterRightHandAnimations.ABP_PlayerCharacterRightHandAnimations_C|SetPlayerState _asabp_player_character_right_hand_animations NewParam)
  (return))

(fn ObjectAnimation
  (params (ObjectType :type E_TelekinesisElementType%20Enum :default "NewEnumerator0"))
  (bind _asabp_player_character_right_hand_animations (Utilities|Casting|CastToABP_PlayerCharacterRightHandAnimations (Components|SkeletalMesh|GetAnimInstance (Variables|Default|GetMesh1P))))
  (Variables|/Game/Characters/Player/Animations/ABP_PlayerCharacterRightHandAnimations.ABP_PlayerCharacterRightHandAnimations_C|SetObjectType _asabp_player_character_right_hand_animations ObjectType)
  (return))

(fn SetImpactParameters
  (params (VectorHit :type Vector) (KnockbackForce :type Vector))
  (Variables|ImpactVars|SetImpactLocation VectorHit)
  (Variables|ImpactVars|SetKnockbackForce KnockbackForce))

(fn SetPlayerAnimState
  (params (PlayerState :type E_PlayerStates%20Enum :default "NewEnumerator6"))
  (bind _tinykinesisplayercontroller (CallFunction|GetTinykinesisPlayerController))
  (bind _bp_ac_telekinesis (Variables|/Game/Blueprints/Player/BP_TinykinesisPlayerController.BP_TinykinesisPlayerController_C|GetBP_AC_Telekinesis _tinykinesisplayercontroller))
  (bind _itemgrabbed (Variables|/Game/Blueprints/ActorComponents/PlayerAbilities/BP_AC_Telekinesis.BP_AC_Telekinesis_C|GetItemGrabbed _bp_ac_telekinesis))
  (bind _asabp_player_character_right_hand_animations (Utilities|Casting|CastToABP_PlayerCharacterRightHandAnimations (Components|SkeletalMesh|GetAnimInstance (Variables|Default|GetMesh1P))))
  (Variables|/Game/Characters/Player/Animations/ABP_PlayerCharacterRightHandAnimations.ABP_PlayerCharacterRightHandAnimations_C|SetPlayerState _asabp_player_character_right_hand_animations PlayerState)
  (Utilities|IsValid _itemgrabbed
    (:Is%20Valid
      (if (Actor|ActorHasTag _itemgrabbed "AttractiveElement")
        (Variables|/Game/Characters/Player/Animations/ABP_PlayerCharacterRightHandAnimations.ABP_PlayerCharacterRightHandAnimations_C|SetObjectType _asabp_player_character_right_hand_animations "NewEnumerator0")
        (elif (Actor|ActorHasTag _itemgrabbed "Heavy")
          (Variables|/Game/Characters/Player/Animations/ABP_PlayerCharacterRightHandAnimations.ABP_PlayerCharacterRightHandAnimations_C|SetObjectType _asabp_player_character_right_hand_animations "NewEnumerator1")
          (else
            (Variables|/Game/Characters/Player/Animations/ABP_PlayerCharacterRightHandAnimations.ABP_PlayerCharacterRightHandAnimations_C|SetObjectType _asabp_player_character_right_hand_animations "NewEnumerator2" :!label _label)))))
    (:Is%20Not%20Valid
      (goto _label))))