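; Player controller for the Tinykinesis character, handling HUD, pausing debug console, telekinesis targeting and ability timelines.
; Tick adjusts walk speed and runs a camera trace, with a looping MultiGate alternating item selection, clearing and target detection across frames.
; Timeline events serve jump and dirt-grab components: cooldown, plus a cancelable cast that locks the view and spawns a held dirt object.
; UsedCapacity sphere-traces to aggro nearby AI.
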(event Custom|EventTimelineDoubleJump
  ;[1 1 1] Timeline for the actor component Jump
  (bind _cooldown (Timeline|Timeline Play)
    (:Update
      (bind _output_get (Variables|Movements|SetDoubleCooldown _cooldown))
      (Default|CallOnTimeline _output_get))
    (:Finished
      (Variables|Movements|SetCanDoubleJump true)
      (Development|PrintString "canJump"))))

(event Custom|EventTimelineGrabDirt
  (params (Impact :type Vector))
  ;[1 1 1] Timeline for the actor component GrabDirt
  (Variables|Default|SetVectorTimelineGrabDirt Impact)
  (Utilities|FlowControl|DoOnce false :!label _label
    (:Completed
      (Camera|PlayWorldCameraShake "/Game/Blueprints/Actors/BP_CastingCameraShake.BP_CastingCameraShake_C" (Transformation|GetActorLocation (CallFunction|GetTinykinesisPlayerCharacter)) 0.0 5e+02)
      (bind _returnvalue (Niagara|SpawnSystematLocation "/Game/VFX/NS_DirtParticles.NS_DirtParticles" (Variables|Default|GetVectorTimelineGrabDirt) "0, 0, 0" "0.500000,0.500000,0.200000"))
      (Timeline|TimelineCastingTime PlayFromStart
        (:Update
          (Pawn|SetControlRotation (Math|Rotator|FindLookatRotation (Transformation|GetActorLocation (CallFunction|GetTinykinesisPlayerCharacter)) (Variables|Default|GetVectorTimelineGrabDirt))))
        (:Finished
          (Variables|Power|SetUsingPower true)
          (bind _returnvalue_2 (Game|SpawnActorfromClass "/Game/Blueprints/Actors/LightObject/BP_LightObject_Dirt.BP_LightObject_Dirt_C" (Math|Conversions|ToTransform(Vector) (Variables|Default|GetVectorTimelineGrabDirt)) "Undefined" "MultiplyWithRoot" 0 0))
          (Variables|TelekinesisObject|SetSelectedItem _returnvalue_2)
          (goto _label Reset))))))

(event Custom|EventTimelineGrabDirtCanceled
  (params (Impact :type Vector))
  ;[1 1 1] Timeline for the actor component GrabDirt
  (Variables|Default|SetVectorTimelineGrabDirt Impact)
  (Utilities|FlowControl|Sequence
    (:then_0
      (Utilities|FlowControl|DoOnce false) ; enters at Reset
    )
    (:then_1
      (Utilities|IsValid (stale Custom|EventTimelineGrabDirt _returnvalue)
        (:Is%20Valid
          (Components|DestroyComponent (stale Custom|EventTimelineGrabDirt _returnvalue))
          (Timeline|TimelineCastingTime Stop
            (:Update
              (Pawn|SetControlRotation (Math|Rotator|FindLookatRotation (Transformation|GetActorLocation (CallFunction|GetTinykinesisPlayerCharacter)) (Variables|Default|GetVectorTimelineGrabDirt))))
            (:Finished
              (Variables|Power|SetUsingPower true)
              (bind _returnvalue (Game|SpawnActorfromClass "/Game/Blueprints/Actors/LightObject/BP_LightObject_Dirt.BP_LightObject_Dirt_C" (Math|Conversions|ToTransform(Vector) (Variables|Default|GetVectorTimelineGrabDirt)) "Undefined" "MultiplyWithRoot" 0 0))
              (Variables|TelekinesisObject|SetSelectedItem _returnvalue)
              (Utilities|FlowControl|DoOnce false) ; enters at Reset
            )))))))

(event Input|EnhancedActionEvents|EnhancedInputActionIA_OpenConsole
  (params (ActionValue :type Boolean) (ElapsedSeconds :type Float%20%28double-precision%29) (TriggeredSeconds :type Float%20%28double-precision%29) (InputAction :type Input%20Action%20Object%20Reference :default "/Game/Blueprints/Player/Input/Actions/IA_OpenConsole.IA_OpenConsole"))
  (bind _returnvalue (Game|GetPlayerController 0))
  (if (Variables|Default|GetConsole%20Opened)
    (Widget|RemovefromParent (stale _returnvalue_2))
    (Variables|Default|SetConsole%20Opened false)
    (Game|SetGamePaused false)
    (Variables|/Script/Engine.PlayerController|SetbShowMouseCursor _returnvalue false)
    (else
      (bind _returnvalue_2 (UserInterface|CreateWidget "/Game/Blueprints/WidgetBlueprints/DebugConsole/WBP_DebugConsole.WBP_DebugConsole_C"))
      (UserInterface|Viewport|AddtoViewport _returnvalue_2 0)
      (Variables|Default|SetConsole%20Opened true)
      (Game|SetGamePaused true)
      (Variables|/Script/Engine.PlayerController|SetbShowMouseCursor _returnvalue true))))

(event EventBeginPlay
  ;[1 1 1] Begin Play
  (bind _returnvalue (UserInterface|CreateWidget "/Game/Blueprints/WidgetBlueprints/HUD/WBP_LifeBar.WBP_LifeBar_C"))
  (UserInterface|Viewport|AddtoViewport _returnvalue 0)
  (bind _returnvalue_2 (UserInterface|CreateWidget "/Game/Blueprints/WidgetBlueprints/HUD/WBP_Crosshair.WBP_Crosshair_C"))
  (UserInterface|Viewport|AddtoViewport _returnvalue_2 0)
  (Variables|Power|SetCastRange 2e+03)
  (Variables|Movements|SetBaseWalkSpeed (Variables|/Script/Engine.CharacterMovementComponent|GetMaxWalkSpeed (Variables|/Script/Engine.Character|GetCharacterMovement (CallFunction|GetTinykinesisPlayerCharacter))))
  (Variables|Movements|SetStamina 0.0))

(event EventTick
  (params (DeltaSeconds :type Float%20%28single-precision%29))
  (bind _tinykinesisplayercharacter (CallFunction|GetTinykinesisPlayerCharacter))
  (bind _tinykinesisplayercharacter_2 (CallFunction|GetTinykinesisPlayerCharacter))
  (bind _charactermovement (Variables|/Script/Engine.Character|GetCharacterMovement _tinykinesisplayercharacter_2))
  (bind _firstpersoncameracomponent (Variables|/Script/Tinykinesis_Proto.Tinykinesis_ProtoCharacter|GetFirstPersonCameraComponent _tinykinesisplayercharacter))
  (bind _returnvalue (Transformation|GetWorldLocation _firstpersoncameracomponent))
  (if (|CollapseGraph)
    (Variables|/Script/Engine.CharacterMovementComponent|SetMaxWalkSpeed _charactermovement 3.5e+02)
    (else
      (Variables|/Script/Engine.CharacterMovementComponent|SetMaxWalkSpeed _charactermovement (Variables|Movements|GetBaseWalkSpeed))))
  (bind _outhit (Collision|LineTraceByChannel _returnvalue (+ _returnvalue (* (Math|Vector|GetForwardVector (Transformation|GetWorldRotation _firstpersoncameracomponent)) (Variables|Power|GetCastRange))) "TraceTypeQuery1" false 0 "None"))
  (Utilities|FlowControl|MultiGate false true -1
    (:Out%200
      (if (Utilities|DoesObjectImplementInterface (.HitActor (Collision|BreakHitResult _outhit)) "/Game/Blueprints/Interfaces/BPI_Interactable.BPI_Interactable_C")
        (if (not (Variables|Power|GetUsingPower))
          (Variables|TelekinesisObject|SetSelectedItem (.HitActor (Collision|BreakHitResult _outhit))))))
    (:Out%201
      (if (not (or (Utilities|DoesObjectImplementInterface (.HitActor (Collision|BreakHitResult _outhit)) "/Game/Blueprints/Interfaces/BPI_Interactable.BPI_Interactable_C") (Utilities|DoesObjectImplementInterface (.HitActor (Collision|BreakHitResult _outhit)) "/Game/Blueprints/Interfaces/BPI_Target.BPI_Target_C")))
        (Variables|Target|SetHasTarget false)
        (Class|BPITarget|DeleteOutline(Message) (Variables|Target|GetActualTarget) false)
        (Variables|Target|SetActualTarget (Variables|TelekinesisObject|GetEmptyItem))
        (if (not (Variables|Power|GetUsingPower))
          (Variables|TelekinesisObject|SetSelectedItem (Variables|TelekinesisObject|GetEmptyItem)))))
    (:Out%202
      (if (Utilities|DoesObjectImplementInterface (.HitActor (Collision|BreakHitResult _outhit)) "/Game/Blueprints/Interfaces/BPI_Target.BPI_Target_C")
        (if (Variables|Power|GetUsingPower)
          (Variables|Target|SetHasTarget true)
          (Class|BPITarget|DetectTarget(Message) (.HitActor (Collision|BreakHitResult _outhit)) "0, 0, 0" (Variables|Target|GetHasTarget))
          (bind _targetlocation (Class|BPITarget|GiveTargetLocation(Message) (.HitActor (Collision|BreakHitResult _outhit)) "0, 0, 0"))
          (Variables|Target|SetTargetLocation _targetlocation)
          (Variables|Target|SetActualTarget (.HitActor (Collision|BreakHitResult _outhit))))))))

(fn ConstructionScript)

(fn UsedCapacity
  (bind _tinykinesisplayercharacter (CallFunction|GetTinykinesisPlayerCharacter))
  (bind _returnvalue (Transformation|GetActorLocation _tinykinesisplayercharacter))
  (bind _outhits (Collision|MultiSphereTraceForObjects _returnvalue _returnvalue (Variables|Default|GetRadiusSpellDetection) (LocalVariables|GetObjectType) false 0 "None"))
  (for _array_element _outhits
    (bind _asbp_aicharacter_blank (Utilities|Casting|CastToBP_AICharacterBlank (.HitActor (Collision|BreakHitResult _array_element))))
    (if (not (Variables|/Game/Blueprints/NPC/BP_AICharacterBlank.BP_AICharacterBlank_C|GetIsAggro _asbp_aicharacter_blank))
      (Default|BecameAggro _asbp_aicharacter_blank)))
  (return))

(fn DoubleJumpCooldown)

(fn ResetSelection
  (Utilities|IsValid (Variables|TelekinesisObject|GetSelectedItem)
    (:Is%20Valid
      (Variables|TelekinesisObject|SetSelectedItem (Variables|TelekinesisObject|GetEmptyItem))
      (return))))