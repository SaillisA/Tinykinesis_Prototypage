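; BP_HeavyObject is a physics prop that can be levitated, pulled in, thrown or slammed down.
; Levitate raises the mesh on a timeline without gravity, and Smash drives it down, spawning BP_SmashArea.
; Attract disables collision during the pull, while Propulse restores it and moves toward a locked target or applies an impulse.
; Cube hits pass the pre-throw location to GetHit, and Hit destroys smashed or thrown objects after a short delay.
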(event OnComponentHit(Cube)
  (params (HitComponent :type Primitive%20Component%20Object%20Reference) (OtherActor :type Actor%20Object%20Reference) (OtherComp :type Primitive%20Component%20Object%20Reference) (NormalImpulse :type Vector :default "0, 0, 0") (Hit :type Hit%20Result%20Structure%20%28by%20ref%29))
  (bind _asbp_character_npc_base (Utilities|Casting|CastTo OtherActor))
  (Development|PrintString "Hello")
  (CallFunction|GetHit :self _asbp_character_npc_base :NPC _asbp_character_npc_base :VectorObject (Variables|Default|GetLocationBeforeThrown)))

(event EventBeginPlay
  (bind _returnvalue (Actor|GetComponentbyClass "/Script/Engine.StaticMeshComponent"))
  (Development|PrintString (Utilities|GetDisplayName _returnvalue))
  (Variables|Default|SetUsableMesh _returnvalue))

(event EventSmash
  (Physics|SetEnableGravity (Variables|Default|GetUsableMesh) true)
  (Physics|AddImpulse (Variables|Default|GetUsableMesh) "0.000000,0.000000,-2600.000000" "None" true)
  (Game|SpawnActorfromClass "/Game/Blueprints/Actors/BP_SmashArea.BP_SmashArea_C" (Transformation|GetActorTransform) "Undefined" "MultiplyWithRoot" 0 0)
  (Variables|Default|SetGettingSmashed true))

(event Collision|EventHit
  (params (MyComp :type Primitive%20Component%20Object%20Reference) (Other :type Actor%20Object%20Reference) (OtherComp :type Primitive%20Component%20Object%20Reference) (bSelfMoved :type Boolean) (HitLocation :type Vector :default "0, 0, 0") (HitNormal :type Vector :default "0, 0, 0") (NormalImpulse :type Vector :default "0, 0, 0") (Hit :type Hit%20Result%20Structure%20%28by%20ref%29))
  (Utilities|FlowControl|Sequence
    (:then_0
      (if (Variables|Default|GetGettingSmashed)
        (Utilities|FlowControl|Delay 0.2)
        (Actor|DestroyActor)
        (Variables|Default|SetIsLevitating false)))
    (:then_1
      (if (Variables|Default|GetIsThrown)
        (Utilities|FlowControl|Delay 0.2)
        (Actor|DestroyActor)
        (else
          (Components|MoveComponentTo (Variables|Default|GetUsableMesh) (stale EventAttract Player%20Location) "0, 0, 0" false false 0.1 false) ; enters at Stop
        )))))

(event EventAttract
  (params (Player%20Location :type Vector :default "0, 0, 0"))
  (if (not (Variables|Default|GetIsLevitating))
    (Variables|Default|SetCanBeThrown true)
    (Collision|SetCollisionResponsetoAllChannels (Variables|Default|GetUsableMesh) "ECR_Ignore")
    (Components|MoveComponentTo (Variables|Default|GetUsableMesh) Player%20Location "0, 0, 0" false false 0.1 false)))

(event EventPropulse
  (params (TargetLocation :type Vector :default "0, 0, 0") (PropulseLocation :type Vector :default "0, 0, 0") (TargetLocked? :type Boolean))
  (bind _usablemesh (Variables|Default|GetUsableMesh))
  (Variables|Default|SetLocationBeforeThrown (Transformation|GetActorLocation))
  (if (Variables|Default|GetCanBeThrown)
    (if TargetLocked?
      (Collision|SetCollisionResponsetoAllChannels (Variables|Default|GetUsableMesh) "ECR_Block")
      (Variables|Default|SetIsThrown true)
      (Components|MoveComponentTo _usablemesh (+ TargetLocation 5e+01) "0, 0, 0" false false 0.15 false)
      (Physics|SetEnableGravity (Variables|Default|GetUsableMesh) true)
      (else
        (Collision|SetCollisionResponsetoAllChannels (Variables|Default|GetUsableMesh) "ECR_Block")
        (Physics|SetPhysicsLinearVelocity _usablemesh "0, 0, 0" false "None")
        (Physics|AddImpulse (Variables|Default|GetUsableMesh) (* PropulseLocation 5500) "None" true)
        (Physics|SetEnableGravity (Variables|Default|GetUsableMesh) true)
        (Variables|Default|SetIsThrown true)))))

(event EventLevitate
  (bind _usablemesh (Variables|Default|GetUsableMesh))
  (bind _returnvalue (Transformation|GetWorldLocation _usablemesh))
  (bind (_x _y _z) (Math|Vector|BreakVector _returnvalue))
  (Class|PrimitiveComponent|SetAllPhysicsLinearVelocity (Variables|Default|GetUsableMesh) "0, 0, 0" false)
  (bind _levitation (Timeline|Levitation PlayFromStart)
    (:Update
      (Variables|Default|SetIsLevitating true)
      (Transformation|SetWorldLocation (Variables|Default|GetUsableMesh) (Math|Vector|MakeVector _x _y (+ _levitation (+ _z 1e+01))) true false)
      (Physics|SetEnableGravity (Variables|Default|GetUsableMesh) false))))

(event EventGrabObject
  (Variables|Default|SetCanBeThrown true)
  (Development|PrintString "Hello"))

(fn ConstructionScript)