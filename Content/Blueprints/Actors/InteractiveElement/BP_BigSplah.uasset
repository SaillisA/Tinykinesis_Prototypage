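; Interactive actor that triggers a one-time "BigSplash" sequence with the player placed at its Boat component.
; An overlap destroys the trigger and calls LaunchAnimation, which plays the sequence, attaches the player to this actor, disables character movement and moves the pawn to the Boat.
; EndAnimation detaches the player and restores walking, but nothing in this Blueprint calls it.
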(event OnComponentBeginOverlap(TriggerSequence)
  (params (OverlappedComponent :type Primitive%20Component%20Object%20Reference) (OtherActor :type Actor%20Object%20Reference) (OtherComp :type Primitive%20Component%20Object%20Reference) (OtherBodyIndex :type Integer) (bFromSweep :type Boolean) (SweepResult :type Hit%20Result%20Structure%20%28by%20ref%29))
  (Components|DestroyComponent (Variables|Default|GetTriggerSequence))
  (CallFunction|LaunchAnimation))

(event EventBeginPlay)

(event EventTick
  (params (DeltaSeconds :type Float%20%28single-precision%29)))

(fn ConstructionScript)

(fn EndAnimation
  (bind _tinykinesisplayercharacter (CallFunction|GetTinykinesisPlayerCharacter))
  (Transformation|DetachFromActor _tinykinesisplayercharacter "KeepWorld" "KeepWorld" "KeepWorld")
  (Pawn|Components|CharacterMovement|SetMovementMode (Variables|/Script/Engine.Character|GetCharacterMovement _tinykinesisplayercharacter) "MOVE_Walking" 0))

(fn LaunchAnimation
  (Sequencer|Player|Play (Variables|/Script/LevelSequence.LevelSequenceActor|GetSequencePlayer (Variables|Default|GetAnimationSequence)) :!class /Script/MovieScene.MovieSceneSequencePlayer)
  (Transformation|AttachActorToActor (Game|Player|GetPlayerPawn 0) self "None" "KeepWorld" "KeepWorld" "KeepWorld" true)
  (Pawn|Components|CharacterMovement|SetMovementMode (Variables|/Script/Engine.Character|GetCharacterMovement (CallFunction|GetTinykinesisPlayerCharacter)) "MOVE_None" 0)
  (Transformation|SetActorLocation (Game|Player|GetPlayerPawn 0) (Transformation|GetWorldLocation (Variables|Default|GetBoat)) true false))