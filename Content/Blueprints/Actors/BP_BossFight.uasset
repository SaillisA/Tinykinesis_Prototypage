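; Boss fight manager that runs a multi-part boss protected by a force field and crystals, with a health bar fed by combined part health.
; Activation spawns crystals at unobstructed random points, more as parts die.
; Clearing all crystals drops the force field, makes parts projectile-destructible (holding the last back until alone) and starts a respawn countdown on Tick.
; Losing a part respawns crystals; losing all ends the fight and kills the arena's current wave.
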(event EventBeginPlay
  (CallFunction|StartSetup))

(event EventTick
  (params (DeltaSeconds :type Float%20%28single-precision%29))
  (if (not (Variables|BossActor|GetIsBossDead))
    (CallFunction|CrystalSpawnCountdown)))

(fn ConstructionScript)

(fn CalculateCombinedHealth
  (params (CurrentHealth :type Float%20%28double-precision%29))
  (Variables|BossActor|SetCombined%20Health 0.0)
  (for _array_element (Variables|BossActor|GetBoss%20Part)
    (Utilities|IsValid _array_element
      (:Is%20Valid
        (Variables|BossActor|SetCombined%20Health (+ (Variables|BossActor|GetCombined%20Health) (Variables|/Game/Blueprints/ActorComponents/BP_AC_Health.BP_AC_Health_C|GetcurrentHP (Variables|/Game/Blueprints/Actors/Traps/DestructibleObject/BP_DestructibleObject.BP_DestructibleObject_C|GetBP_AC_Health _array_element))))))))

(fn BossFightActivation
  (CallFunction|SpawnCrystal)
  (bind _returnvalue (UserInterface|CreateWidget "/Game/Blueprints/WidgetBlueprints/EndBoss/WBP_BossHealthBar.WBP_BossHealthBar_C"))
  (bind _output_get (Variables|Default|SetWBP%20Boss%20Health _returnvalue))
  (UserInterface|Viewport|AddtoViewport _output_get 0)
  (Variables|/Game/Blueprints/WidgetBlueprints/EndBoss/WBP_BossHealthBar.WBP_BossHealthBar_C|SetBossFightActor (Variables|Default|GetWBP%20Boss%20Health) self))

(fn SetupBossPart
  (for _array_element (Variables|BossActor|GetBoss%20Part)
    (Utilities|IsValid _array_element
      (:Is%20Valid
        (EventDispatchers|BindEventtoOnHPChanged (Variables|/Game/Blueprints/Actors/Traps/DestructibleObject/BP_DestructibleObject.BP_DestructibleObject_C|GetBP_AC_Health _array_element) (EventDispatchers|CreateEvent :!event CalculateCombinedHealth))
        (EventDispatchers|BindEventtoOnDestructionEffect _array_element (EventDispatchers|CreateEvent :!event RemoveBossPart))))))

(fn CalculateCombinedMaxHealth
  (for _array_element (Variables|BossActor|GetBoss%20Part)
    (Utilities|IsValid _array_element
      (:Is%20Valid
        (Variables|BossActor|SetCombinedMaxHealth (+ (Variables|BossActor|GetCombinedMaxHealth) (Variables|/Game/Blueprints/ActorComponents/BP_AC_Health.BP_AC_Health_C|GetcurrentHP (Variables|/Game/Blueprints/Actors/Traps/DestructibleObject/BP_DestructibleObject.BP_DestructibleObject_C|GetBP_AC_Health _array_element))))))))

(fn RemoveBossPart
  (bind _boss_part (Variables|BossActor|GetBoss%20Part))
  (for _array_element (Variables|BossActor|GetBoss%20Part)
    (Utilities|IsValid _array_element
      (:Is%20Valid
        (if (<= (Variables|/Game/Blueprints/ActorComponents/BP_AC_Health.BP_AC_Health_C|GetcurrentHP (Variables|/Game/Blueprints/Actors/Traps/DestructibleObject/BP_DestructibleObject.BP_DestructibleObject_C|GetBP_AC_Health _array_element)) 0.0)
          (Utilities|Array|RemoveItem _boss_part _array_element)
          (if (== (Utilities|Array|Length _boss_part) 0)
            (CallFunction|EndBossFight)
            (else
              (CallFunction|SpawnCrystal))))))))

(fn SpawnCrystal
  (bind _force_field (Variables|BossActor|GetForce%20Field))
  (Variables|Crystal|SetCrystalRespawnCountdown (Variables|Crystal|GetCrystalRespawnCountdown))
  (Variables|Crystal|SetCanSpawnCrystal false)
  (Rendering|SetActorHiddenInGame _force_field false)
  (Collision|SetCollisionEnabled (Variables|/Script/Engine.StaticMeshActor|GetStaticMeshComponent _force_field) "QueryAndPhysics")
  (for _index (range 0 (- (- 4 (Utilities|Array|Length (Variables|BossActor|GetBoss%20Part))) 1))
    (bind _output_get (LocalVariables|SetRandomTargetPoint (.OutItem (Utilities|Array|Random (Variables|Crystal|GetCrystalSpawnPoint))) :!label _label))
    (bind _returnvalue (Collision|SphereTraceByChannel (Transformation|GetActorLocation _output_get) (Transformation|GetActorLocation _output_get) (LocalVariables|GetSphereCastRadius) "TraceTypeQuery1" false 0 "None"))
    (if _returnvalue
      (goto _label)
      (else
        (bind _returnvalue_2 (Game|SpawnActorfromClass "/Game/Blueprints/Actors/ArenaManagement/BP_SpawningCrystal.BP_SpawningCrystal_C" (Transformation|GetActorTransform (LocalVariables|GetRandomTargetPoint)) "Undefined" "MultiplyWithRoot" 0 0))
        (EventDispatchers|BindEventtoOnDeathEvent _returnvalue_2 (EventDispatchers|CreateEvent :!event RemoveCrystal))
        (Utilities|Array|AddUnique (Variables|Crystal|GetCurrentCrystal) _returnvalue_2)))))

(fn RemoveCrystal
  (params (DestroyedCrystal :type BP%20Spawning%20Crystal%20Object%20Reference))
  (bind _currentcrystal (Variables|Crystal|GetCurrentCrystal))
  (bind _boss_part (Variables|BossActor|GetBoss%20Part))
  (bind _force_field (Variables|BossActor|GetForce%20Field))
  (bind _returnvalue (Utilities|Array|Length _boss_part))
  (Utilities|Array|RemoveItem _currentcrystal DestroyedCrystal)
  (if (== (Utilities|Array|Length _currentcrystal) 0)
    (Variables|Crystal|SetCrystalRespawnCountdown 0.0)
    (Rendering|SetActorHiddenInGame _force_field true)
    (Collision|SetCollisionEnabled (Variables|/Script/Engine.StaticMeshActor|GetStaticMeshComponent _force_field) "NoCollision")
    (Variables|Crystal|SetCanSpawnCrystal true)
    (for (_array_element _array_index) _boss_part
      (if (or (!= _array_index (- _returnvalue 1)) (== _returnvalue 1))
        (Variables|/Game/Blueprints/Actors/Traps/DestructibleObject/BP_DestructibleObject.BP_DestructibleObject_C|SetCanBeDestroyByProjectile _array_element true)
        (Development|PrintString "Hello")))))

(fn CrystalSpawnCountdown
  (if (< (Variables|Crystal|GetCrystalRespawnCountdown) (Variables|Crystal|GetCrystalRespawnCooldown))
    (Variables|Crystal|SetCrystalRespawnCountdown (+ (Variables|Crystal|GetCrystalRespawnCountdown) (Utilities|Time|GetWorldDeltaSeconds)))
    (elif (Variables|Crystal|GetCanSpawnCrystal)
      (Variables|Crystal|SetCanSpawnCrystal false)
      (CallFunction|SpawnCrystal))))

(fn StartSetup
  (Variables|Crystal|SetCrystalRespawnCountdown (Variables|Crystal|GetCrystalRespawnCooldown))
  (Variables|Crystal|SetCanSpawnCrystal false)
  (CallFunction|CalculateCombinedHealth 0.0)
  (CallFunction|CalculateCombinedMaxHealth)
  (CallFunction|SetupBossPart)
  (for _array_element (Variables|BossActor|GetBoss%20Part)
    (Variables|/Game/Blueprints/Actors/Traps/DestructibleObject/BP_DestructibleObject.BP_DestructibleObject_C|SetCanBeDestroyByProjectile _array_element false)))

(fn EndBossFight
  (Default|CallOnEndBoss)
  (Default|PlayLifeBarFadeReverse (Variables|Default|GetWBP%20Boss%20Health))
  (bind _arrayelement (Utilities|Array|ReverseforEachLoop (Variables|/Game/Blueprints/Actors/ArenaManagement/BP_AbstractArenaManager.BP_AbstractArenaManager_C|GetCurrentWave (Variables|Default|GetArenaManager)))
    (:LoopBody
      (Utilities|IsValid _arrayelement
        (:Is%20Valid
          (Default|DeathNpc _arrayelement))))
    (:Completed
      (Variables|BossActor|SetIsBossDead true)
      (Development|PrintString "Boss Death"))))