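; BP_FallingObject is a hanging trap that drops when hit, damaging BPI_Target actors on impact.
; A hit detaches the cable, breaks the physics constraint and enables mesh physics.
; Striking a target or Ground-tagged actor shakes the camera, fires a radial impulse, enables a matching-radius damage sphere that spares activation buttons, and launches destruction.
; A state component handles activation, loading and disabling in the save; overlay material outlines it when targeted.
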(event OnComponentBeginOverlap(DamageRangeCollision)
  (params (OverlappedComponent :type Primitive%20Component%20Object%20Reference) (OtherActor :type Actor%20Object%20Reference) (OtherComp :type Primitive%20Component%20Object%20Reference) (OtherBodyIndex :type Integer) (bFromSweep :type Boolean) (SweepResult :type Hit%20Result%20Structure%20%28by%20ref%29))
  (if (Utilities|DoesObjectImplementInterface OtherActor "/Game/Blueprints/Interfaces/BPI_Target.BPI_Target_C")
    (Utilities|Casting|CastToBP_ActivationButton OtherActor
      (:CastFailed
        (Class|BPITarget|GetHit(Message) OtherActor 0 true (Variables|Default|GetDamageTrap) "0, 0, 0" (Variables|Default|GetKnockbackForce))))))

(event OnComponentHit(FallingMesh)
  (params (HitComponent :type Primitive%20Component%20Object%20Reference) (OtherActor :type Actor%20Object%20Reference) (OtherComp :type Primitive%20Component%20Object%20Reference) (NormalImpulse :type Vector :default "0, 0, 0") (Hit :type Hit%20Result%20Structure%20%28by%20ref%29))
  (bind (_bblockinghit _binitialoverlap _time _distance _location _impactpoint _normal _impactnormal _physmat _hitactor) (Collision|BreakHitResult Hit))
  (bind _damagerangecollision (Variables|Default|GetDamageRangeCollision))
  (if (Variables|Default|GetIsFalling)
    (if (Utilities|DoesObjectImplementInterface _hitactor "/Game/Blueprints/Interfaces/BPI_Target.BPI_Target_C")
      (Class|BPITarget|GetHit(Message) OtherActor 0 true (Variables|Default|GetDamageTrap) _location (Variables|Default|GetKnockbackForce))
      (Camera|PlayWorldCameraShake "/Game/Blueprints/Actors/CameraManager/BP_CameraShake.BP_CameraShake_C" (Transformation|GetActorLocation (CallFunction|GetTinykinesisPlayerCharacter)) 0.0 5e+02 :!label _label)
      (Collision|SetCollisionEnabled _damagerangecollision "QueryOnly")
      (Collision|SetCollisionResponsetoAllChannels _damagerangecollision "ECR_Overlap")
      (Class|RadialForceComponent|FireImpulse (Variables|Default|GetRadialForce))
      (Default|DisableinSave (Variables|Default|GetBP_AC_StateGameplayElement))
      (Default|LaunchDestruction (Variables|Default|GetBP_AC_DestructionElement) (Transformation|GetRelativeTransform (Variables|Default|GetFallingMesh)) self)
      (elif (and (not (Variables|Default|GetTouchedGround)) (Actor|ActorHasTag _hitactor "Ground"))
        (Variables|Default|SetTouchedGround true)
        (goto _label)))))

(event Custom|BeginPlay_FallingTrap
  ;[0.298 1 0.5765] BeginPlay
  (Collision|SetCollisionEnabled (Variables|Default|GetDamageRangeCollision) "NoCollision"))

(event Custom|LoadFallingTrap
  (bind _bp_ac_stategameplayelement (Variables|Default|GetBP_AC_StateGameplayElement))
  ;[0.298 1 0.5765] BeginPlay
  (Default|LoadElement _bp_ac_stategameplayelement (Variables|/Game/Blueprints/ActorComponents/BP_AC_StateGameplayElement.BP_AC_StateGameplayElement_C|GetIsActivated _bp_ac_stategameplayelement) self))

(event EventFeedbacksDetectTarget
  ;[1 0.851 0] Feedback for Target
  (Rendering|Material|SetOverlayMaterial (Variables|Default|GetCube) "/Game/Materials/M_OutlineTarget.M_OutlineTarget" :!class /Script/Engine.MeshComponent))

(event EventGetHit
  (params (TelekinesisElement :type BP%20Abstract%20Telekinesis%20Element%20Object%20Reference) (CanDamage :type Boolean) (DamageObject :type Float%20%28double-precision%29) (VectorHit :type Vector :default "0, 0, 0") (ForceKnockback :type Vector :default "0, 0, 0"))
  (if CanDamage
    (Class|CableComponent|SetAttachEndto (Variables|Default|GetCable) 0 "None" "None")
    (Class|PhysicsConstraintComponent|BreakConstraint (Variables|Default|GetPhysicsConstraint))
    (Physics|SetSimulatePhysics (Variables|Default|GetFallingMesh) true)
    (Variables|Default|SetIsFalling true)
    (Collision|SetCollisionResponsetoChannel (Variables|Default|GetFallingMesh) "ECC_Pawn" "ECR_Block")))

(event EventDeleteFeedbacksDetectTarget
  (bind _cube (Variables|Default|GetCube))
  ;[1 0.851 0] Feedback for Target
  (Utilities|IsValid _cube
    (:Is%20Valid
      (Rendering|Material|SetOverlayMaterial _cube 0 :!class /Script/Engine.MeshComponent))))

(event EventBeginPlay
  (bind _bp_ac_stategameplayelement (Variables|Default|GetBP_AC_StateGameplayElement))
  ;[0.298 1 0.5765] BeginPlay
  (EventDispatchers|BindEventtoBeginPlayActiveElement _bp_ac_stategameplayelement (EventDispatchers|CreateEvent :!event Custom|BeginPlay_FallingTrap))
  (Default|LaunchBeginPlayifNoLevelManager _bp_ac_stategameplayelement))

(event EventSetActive
  (params (IsActive :type Boolean))
  (bind _bp_ac_stategameplayelement (Variables|Default|GetBP_AC_StateGameplayElement))
  ;[0.298 1 0.5765] BeginPlay
  (EventDispatchers|BindEventtoSetActiveElementEventDispatcher _bp_ac_stategameplayelement (EventDispatchers|CreateEvent :!event Custom|LoadFallingTrap))
  (EventDispatchers|BindEventtoBeginPlayActiveElement _bp_ac_stategameplayelement (EventDispatchers|CreateEvent :!event Custom|BeginPlay_FallingTrap))
  (Default|SetActiveElement (Variables|Default|GetBP_AC_StateGameplayElement) IsActive))

(fn ConstructionScript
  (Components|Sphere|SetSphereRadius (Variables|Default|GetDamageRangeCollision) (Variables|/Script/Engine.RadialForceComponent|GetRadius (Variables|Default|GetRadialForce)) true))

(fn GetCanTakeDamage
  (return false))