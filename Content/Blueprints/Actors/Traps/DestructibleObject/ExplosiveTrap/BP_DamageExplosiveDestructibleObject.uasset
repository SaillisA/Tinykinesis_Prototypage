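; Explosive destructible trap that damages and knocks back what its explosion hits, built as a child Blueprint that leaves BeginPlay and construction to its parent.
; ExplosionEffect sends a hit message to the struck actor with heavy damage, the hit location and the knockback force.
; ExplosionFeedbacks fires a radial force impulse and plays a world camera shake centered on the Tinykinesis player character rather than on the trap.
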(event EventBeginPlay
  (|CallParentFunction))

(event Collision|EventActorBeginOverlap
  (params (OtherActor :type Actor%20Object%20Reference))
  (|CallParentFunction OtherActor) ; This node is disabled and will not be called.\nDrag off pins to build functionality.
)

(event EventTick
  (params (DeltaSeconds :type Float%20%28single-precision%29))
  (|CallParentFunction DeltaSeconds) ; This node is disabled and will not be called.\nDrag off pins to build functionality.
)

(fn ConstructionScript
  (|CallParentFunction))

(fn ExplosionEffect
  (params (ActorHit :type Actor%20Object%20Reference) (HitLocation :type Vector :default "0, 0, 0"))
  (Class|BPITarget|GetHit(Message) ActorHit 0 true 1e+03 HitLocation (Variables|Default|GetKnockbackForce)))

(fn ExplosionFeedbacks
  (Class|RadialForceComponent|FireImpulse (Variables|Default|GetRadialForce))
  (Camera|PlayWorldCameraShake "/Game/Blueprints/Actors/CameraManager/BP_CameraShake.BP_CameraShake_C" (Transformation|GetActorLocation (CallFunction|GetTinykinesisPlayerCharacter)) 0.0 5e+02))