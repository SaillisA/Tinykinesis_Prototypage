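; Abstract base for explosive destructible trap objects, which apply an area effect when they explode.
; BeginPlay binds to the parent's destruction effect, and the construction script sizes a preview sphere to the explosion radius.
; A one-shot explosion sphere-traces around the mesh, passing BPI_Target actors except activation buttons to ExplosionEffect, then spawns scaled FX.
; ExplosionEffect and ExplosionFeedbacks are empty hooks for child classes.
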(event EventBeginPlay
  (|CallParentFunction)
  (EventDispatchers|BindEventtoOnDestructionEffect (EventDispatchers|CreateEvent :!event CastExplosionEffect)))

(event Collision|EventActorBeginOverlap
  (params (OtherActor :type Actor%20Object%20Reference)))

(event EventTick
  (params (DeltaSeconds :type Float%20%28single-precision%29)))

(fn ConstructionScript
  (|CallParentFunction)
  (Components|Sphere|SetSphereRadius (Variables|Default|GetExplosionRadius_Visual) (Variables|Default|GetExplosionRadius) false))

(fn CastExplosionEffect
  (bind _staticmeshcomponent (Variables|Default|GetStaticMeshComponent))
  (bind _staticmeshcomponent_2 (Variables|Default|GetStaticMeshComponent))
  (bind _returnvalue (Transformation|GetWorldLocation _staticmeshcomponent_2))
  (bind _returnvalue_2 (Transformation|GetWorldTransform _staticmeshcomponent))
  (if (not (Variables|Default|GetIsExploding))
    (Variables|Default|SetIsExploding true)
    (bind _outhits (Collision|MultiSphereTraceForObjects _returnvalue _returnvalue (Variables|Default|GetExplosionRadius) (Variables|Default|GetObject%20Types) false 0 "None"))
    (for _array_element _outhits
      (if (Utilities|DoesObjectImplementInterface (.HitActor (Collision|BreakHitResult _array_element)) "/Game/Blueprints/Interfaces/BPI_Target.BPI_Target_C")
        (Utilities|Casting|CastToBP_ActivationButton (.HitActor (Collision|BreakHitResult _array_element))
          (:CastFailed
            (CallFunction|ExplosionEffect (.HitActor (Collision|BreakHitResult _array_element)) (.Location (Collision|BreakHitResult _array_element)))))))
    (bind _returnvalue_3 (Niagara|SpawnSystematLocation (Variables|Default|GetFXExplosion) (.location _returnvalue_2) (.rotation _returnvalue_2) (.scale _returnvalue_2)))
    (Niagara|SetNiagaraVariable(Float) _returnvalue_3 "ScaleMultiplier" 3.0)
    (CallFunction|ExplosionFeedbacks)))

(fn ExplosionEffect
  (params (ActorHit :type Actor%20Object%20Reference) (HitLocation :type Vector)))

(fn ExplosionFeedbacks)