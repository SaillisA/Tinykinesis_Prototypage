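; Destructible trap object with health that takes damage from BP_LightObject hits when projectile destruction is enabled.
; At zero health it kills the NPCs in MobTurretOn, fires OnDestructionEffect and destroys itself; a separate function spawns a fracture mesh.
; Player entry into its box makes it the blackboard TargetActor for melee AI.
; On exit it attempts to retarget the player, but searches NpcDistance controllers while casting to NpcMelee.
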(event OnComponentHit(StaticMeshComponent)
  (params (HitComponent :type Primitive%20Component%20Object%20Reference) (OtherActor :type Actor%20Object%20Reference) (OtherComp :type Primitive%20Component%20Object%20Reference) (NormalImpulse :type Vector :default "0, 0, 0") (Hit :type Hit%20Result%20Structure%20%28by%20ref%29))
  ;[1 1 1] Get Hit
  (if (Variables|Default|GetCanBeDestroyByProjectile)
    (bind _asbp_light_object (Utilities|Casting|CastToBP_LightObject OtherActor))
    (CallFunction|TakeDamage (Variables|/Game/Blueprints/Actors/BP_LightObject.BP_LightObject_C|GetDammageLightObject _asbp_light_object))))

(event OnComponentEndOverlap(Box)
  (params (OverlappedComponent :type Primitive%20Component%20Object%20Reference) (OtherActor :type Actor%20Object%20Reference) (OtherComp :type Primitive%20Component%20Object%20Reference) (OtherBodyIndex :type Integer))
  (Utilities|Casting|CastToBP_TinykinesisPlayerCharacter OtherActor)
  (bind _outactors (Actor|GetAllActorsOfClass "/Game/Blueprints/NPC/AIDistance/BP_AIC_NpcDistance.BP_AIC_NpcDistance_C"))
  (for _array_element _outactors
    (bind _asbp_aic_npc_melee (Utilities|Casting|CastToBP_AIC_NpcMelee (Components|GetOwner _array_element)))
    (AI|Components|Blackboard|SetValueasObject (Variables|/Game/Blueprints/NPC/AIMelee/BP_AIC_NpcMelee.BP_AIC_NpcMelee_C|GetBlackboard%20Component _asbp_aic_npc_melee) (Utilities|Name|MakeLiteralName "TargetActor") (Game|GetPlayerCharacter 0))))

(event OnComponentBeginOverlap(Box)
  (params (OverlappedComponent :type Primitive%20Component%20Object%20Reference) (OtherActor :type Actor%20Object%20Reference) (OtherComp :type Primitive%20Component%20Object%20Reference) (OtherBodyIndex :type Integer) (bFromSweep :type Boolean) (SweepResult :type Hit%20Result%20Structure%20%28by%20ref%29))
  (Utilities|Casting|CastToBP_TinykinesisPlayerCharacter OtherActor)
  (Actor|GetAllActorsOfClass "/Game/Blueprints/NPC/AIMelee/BP_AIC_NpcMelee.BP_AIC_NpcMelee_C")
  (for _array_element 0
    (bind _asbp_aic_npc_melee (Utilities|Casting|CastToBP_AIC_NpcMelee (Components|GetOwner _array_element)))
    (AI|Components|Blackboard|SetValueasObject (Variables|/Game/Blueprints/NPC/AIMelee/BP_AIC_NpcMelee.BP_AIC_NpcMelee_C|GetBlackboard%20Component _asbp_aic_npc_melee) (Utilities|Name|MakeLiteralName "TargetActor") self)))

(event EventBeginPlay
  (EventDispatchers|BindEventtoOnDestructionEffect (EventDispatchers|CreateEvent :!event FractureMeshSpawn)))

(fn ConstructionScript)

(fn TakeDamage
  (params (Damage :type Float%20%28double-precision%29))
  (bind _output_get (Variables|Default|SetHealth (- (Variables|Default|GetHealth) Damage)))
  (if (<= _output_get 0.0)
    (CallFunction|Destruction)))

(fn Destruction
  (for _array_element (Variables|Default|GetMobTurretOn)
    (Default|DeathNpc _array_element))
  (Default|CallOnDestructionEffect)
  (Actor|DestroyActor))

(fn FractureMeshSpawn
  (Game|SpawnActorfromClass (Variables|Default|GetFractureMesh) (Transformation|GetActorTransform) "Undefined" "MultiplyWithRoot" 0 0))