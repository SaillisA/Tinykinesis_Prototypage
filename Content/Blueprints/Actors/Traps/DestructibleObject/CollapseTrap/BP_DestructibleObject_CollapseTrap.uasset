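; Collapse trap variant of a destructible object that falls under physics and deals max-HP damage to melee NPCs it overlaps while falling.
; Pieces destroyable by projectiles become bearers and bind to their destruction event.
; FallSetup enables physics, switches collision to Pawn and cascades to linked traps, actors and lights, guarded by IsFalling.
; The first hit on a "Ground"-tagged actor while falling triggers Destruction.
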(event OnComponentBeginOverlap(StaticMeshComponent)
  (params (OverlappedComponent :type Primitive%20Component%20Object%20Reference) (OtherActor :type Actor%20Object%20Reference) (OtherComp :type Primitive%20Component%20Object%20Reference) (OtherBodyIndex :type Integer) (bFromSweep :type Boolean) (SweepResult :type Hit%20Result%20Structure%20%28by%20ref%29))
  (if (Variables|Default|GetIsFalling)
    (bind _asbp_character_npc_melee (Utilities|Casting|CastToBP_CharacterNpcMelee OtherActor))
    (CallFunction|InflictDamagetoNpcBase _asbp_character_npc_melee (.Location (Collision|BreakHitResult SweepResult)))))

(event OnComponentHit(StaticMeshComponent)
  (params (HitComponent :type Primitive%20Component%20Object%20Reference) (OtherActor :type Actor%20Object%20Reference) (OtherComp :type Primitive%20Component%20Object%20Reference) (NormalImpulse :type Vector :default "0, 0, 0") (Hit :type Hit%20Result%20Structure%20%28by%20ref%29))
  (if (Math|Boolean|ANDBoolean (Variables|Default|GetIsFalling) (not (Variables|Default|GetHasTouchedGround)) (Actor|ActorHasTag OtherActor "Ground"))
    (Variables|Default|SetHasTouchedGround true)
    (CallFunction|Destruction)))

(event EventBeginPlay
  (|CallParentFunction)
  (if (Variables|Default|GetIsBearer)
    (EventDispatchers|BindEventtoOnDestructionEffect (EventDispatchers|CreateEvent :!event MakeObjectFall))))

(fn ConstructionScript
  (|CallParentFunction)
  (if (Variables|Default|GetCanBeDestroyByProjectile)
    (Variables|Default|SetIsBearer true)
    (else
      (Variables|Default|SetIsBearer false))))

(fn MakeObjectFall
  (for _array_element (Variables|Default|GetRelatedCollapseTrap)
    (Utilities|IsValid _array_element
      (:Is%20Valid
        (CallFunction|FallSetup _array_element))))
  (for _array_element_2 (Variables|Default|GetRelatedActor)
    (Utilities|IsValid _array_element_2
      (:Is%20Valid
        (Physics|SetSimulatePhysics (Variables|/Script/Engine.StaticMeshActor|GetStaticMeshComponent _array_element_2) true)
        (Physics|SetEnableGravity (Variables|/Script/Engine.StaticMeshActor|GetStaticMeshComponent _array_element_2) true))))
  (for _array_element_3 (Variables|Default|GetRelatedLightObject)
    (Utilities|IsValid _array_element_3
      (:Is%20Valid
        (Physics|SetSimulatePhysics (Variables|/Game/Blueprints/Actors/BP_LightObject.BP_LightObject_C|GetMesh _array_element_3) true)
        (Physics|SetEnableGravity (Variables|/Game/Blueprints/Actors/BP_LightObject.BP_LightObject_C|GetMesh _array_element_3) true)))))

(fn FallSetup
  (bind _staticmeshcomponent (Variables|Default|GetStaticMeshComponent))
  (if (not (Variables|Default|GetIsFalling))
    (Default|CallOnFallEvent)
    (Variables|Default|SetIsFalling true)
    (Physics|SetSimulatePhysics _staticmeshcomponent true)
    (Physics|SetEnableGravity _staticmeshcomponent true)
    (Collision|SetCollisionObjectType _staticmeshcomponent "ECC_Pawn")
    (CallFunction|MakeObjectFall)))

(fn InflictDamagetoNpcBase
  (params (NpcBase :type BP%20Character%20Npc%20Melee%20Object%20Reference) (HitLocation :type Vector))
  (bind _asbp_aic_npc_melee (Utilities|Casting|CastToBP_AIC_NpcMelee (Components|GetOwner NpcBase)))
  (bind _isdead (Default|LooseHP (Variables|/Game/Blueprints/NPC/AIMelee/BP_AIC_NpcMelee.BP_AIC_NpcMelee_C|GetHealthManager _asbp_aic_npc_melee) (Variables|/Game/Blueprints/ActorComponents/BP_AC_Health.BP_AC_Health_C|GetmaxHP (Variables|/Game/Blueprints/NPC/AIMelee/BP_AIC_NpcMelee.BP_AIC_NpcMelee_C|GetHealthManager _asbp_aic_npc_melee))))
  (if _isdead
    _))