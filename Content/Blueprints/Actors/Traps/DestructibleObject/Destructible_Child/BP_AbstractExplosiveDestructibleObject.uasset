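; Abstract base for explosive destructible objects, leaving the per-hit effect and extra feedback to child classes.
; CastExplosionEffect runs once, sphere-tracing ExplosionRadius, passing BPI_Target actors except activation buttons to ExplosionEffect, then spawning the explosion FX.
; BeginPlay binds to the destruction-effect event and creates a dynamic overlay material whose color signals spawner detection.
; A timeline drives mesh shaking through BPACDestructionElement, and construction sizes the radius preview sphere.
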(event EventBeginPlay
  (|CallParentFunction)
  (EventDispatchers|BindEventtoOnDestructionEffect (EventDispatchers|CreateEvent :!event CastExplosionEffect))
  (bind _returnvalue (Rendering|Material|CreateDynamicMaterialInstance (Variables|Default|GetStaticMeshComponent) 1 "/Game/Materials/MI_OutlineTarget_BeforeGrab.MI_OutlineTarget_BeforeGrab" "None" :!class /Script/Engine.PrimitiveComponent))
  (bind _output_get (Variables|Default|SetMaterialInstance _returnvalue))
  (Rendering|Material|SetOverlayMaterial (Variables|Default|GetStaticMeshComponent) _output_get :!class /Script/Engine.MeshComponent))

(event Collision|EventActorBeginOverlap
  (params (OtherActor :type Actor%20Object%20Reference)))

(event EventTick
  (params (DeltaSeconds :type Float%20%28single-precision%29)))

(event EventShakeStockage
  (bind _newlocation (Timeline|ShakeStockageTimeline PlayFromStart)
    (:Update
      (Default|ShakeStaticMesh (Variables|Default|GetBP_AC_DestructionElement) (Variables|Default|GetStaticMeshComponent) _newlocation))))

(event EventStopShakeStockage
  (bind _newlocation (Timeline|ShakeStockageTimeline Stop)
    (:Update
      (Default|ShakeStaticMesh (Variables|Default|GetBP_AC_DestructionElement) (Variables|Default|GetStaticMeshComponent) _newlocation))))

(event EventFeedbackDetectSpawner
  ;[1 0.8515 0] Feedback for Target
  (CallFunction|SetTargetMaterial (Variables|Default|GetColorMaterialTarget)))

(event EventDeleteFeedbackDetectSpawner
  ;[1 0.8515 0] Feedback for Target
  (CallFunction|SetTargetMaterial))

(fn ConstructionScript
  (|CallParentFunction)
  (Components|Sphere|SetSphereRadius (Variables|Default|GetExplosionRadius_Visual) (Variables|Default|GetExplosionRadius) false))

(fn CastExplosionEffect
  (bind _staticmeshcomponent (Variables|Default|GetStaticMeshComponent))
  (bind _staticmeshcomponent_2 (Variables|Default|GetStaticMeshComponent))
  (bind _returnvalue (Transformation|GetWorldLocation _staticmeshcomponent_2))
  (bind _returnvalue_2 (Transformation|GetWorldTransform _staticmeshcomponent))
  (if (not (Variables|Default|GetIsExploding))
    (Variables|Default|SetIsExploding true)
    (bind _outhits (Collision|MultiSphereTraceForObjects _returnvalue _returnvalue (Variables|Default|GetExplosionRadius) (Variables|Default|GetObject%20Types) false 0 "None"))
    (for _array_element _outhits
      (if (Utilities|DoesObjectImplementInterface (.HitActor (Collision|BreakHitResult _array_element)) "/Game/Blueprints/Interfaces/BPI_Target.BPI_Target_C")
        (Utilities|Casting|CastToBP_ActivationButton (.HitActor (Collision|BreakHitResult _array_element))
          (:CastFailed
            (CallFunction|ExplosionEffect (.HitActor (Collision|BreakHitResult _array_element)) (.Location (Collision|BreakHitResult _array_element)))))))
    (bind _returnvalue_3 (Niagara|SpawnSystematLocation (Variables|Default|GetFXExplosion) (.location _returnvalue_2) (.rotation _returnvalue_2) (.scale _returnvalue_2)))
    (Niagara|SetNiagaraVariable(Float) _returnvalue_3 "ScaleMultiplier" 3.0)
    (CallFunction|ExplosionFeedbacks)))

(fn ExplosionEffect
  (params (ActorHit :type Actor%20Object%20Reference) (HitLocation :type Vector)))

(fn ExplosionFeedbacks)

(fn SetTargetMaterial
  (params (Value :type Linear%20Color%20Structure))
  (Rendering|Material|SetVectorParameterValue (Variables|Default|GetMaterialInstance) "Color" Value :!class /Script/Engine.MaterialInstanceDynamic))

(fn GetProjectileClass
  (return 0 0))