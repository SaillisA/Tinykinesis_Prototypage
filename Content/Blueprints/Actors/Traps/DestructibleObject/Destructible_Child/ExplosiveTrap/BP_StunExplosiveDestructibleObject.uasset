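; Stun variant of the explosive destructible trap object, whose explosion stuns AI characters.
; It overrides the explosion effect to cast the hit actor's owner to BP_AIControllerBlank and trigger its stun event.
; It also supplies BP_AttractiveObject and the ice cream ball data asset as its projectile class and data.
; The event graph is unused and construction defers to the parent.
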(event EventBeginPlay
  (|CallParentFunction) ; This node is disabled and will not be called.\nDrag off pins to build functionality.
)

(event Collision|EventActorBeginOverlap
  (params (OtherActor :type Actor%20Object%20Reference))
  (|CallParentFunction OtherActor) ; This node is disabled and will not be called.\nDrag off pins to build functionality.
)

(event EventTick
  (params (DeltaSeconds :type Float%20%28single-precision%29))
  (|CallParentFunction DeltaSeconds) ; This node is disabled and will not be called.\nDrag off pins to build functionality.
)

(fn ConstructionScript
  (|CallParentFunction))

(fn ExplosionEffect
  (params (ActorHit :type Actor%20Object%20Reference) (HitLocation :type Vector :default "0, 0, 0"))
  (bind _asbp_aicontroller_blank (Utilities|Casting|CastToBP_AIControllerBlank (Components|GetOwner ActorHit)))
  (Default|EventStun _asbp_aicontroller_blank))

(fn GetProjectileClass
  (return "/Game/Blueprints/Actors/TelekinesisElements/BP_AttractiveObject.BP_AttractiveObject_C" "/Game/Blueprints/Actors/TelekinesisElements/DataAssets/StunObjects/DA_SO_BallIceCream.DA_SO_BallIceCream"))