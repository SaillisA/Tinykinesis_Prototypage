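; BP_ActivationButton is a hittable button that fires an activation event, optionally tied to a linked trap.
; On begin play it links itself to that trap, with startup, active state and saving routed through a gameplay-element state component.
; A damaging hit fires the event once unless the trap is already active, disables it in the save and plays a timeline-driven press.
; Targeting toggles an outline overlay material.
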(event Custom|BeginPlay_Button
  ;[0.298 1 0.5765] BeginPlay
  (Utilities|IsValid (Variables|Default|GetLinkTrap)
    (:Is%20Valid
      (Default|LinktoButton (Variables|Default|GetLinkTrap) self))))

(event Custom|LoadButton
  ;[0.298 1 0.5765] BeginPlay
  (Default|CallBeginPlayActiveElement (Variables|Default|GetBP_AC_StateGameplayElement))
  (if (Variables|/Game/Blueprints/ActorComponents/BP_AC_StateGameplayElement.BP_AC_StateGameplayElement_C|GetIsActivated (Variables|Default|GetBP_AC_StateGameplayElement))
    (Default|CallActivationEvent)))

(event EventBeginPlay
  (bind _bp_ac_stategameplayelement (Variables|Default|GetBP_AC_StateGameplayElement))
  ;[0.298 1 0.5765] BeginPlay
  (EventDispatchers|BindEventtoBeginPlayActiveElement _bp_ac_stategameplayelement (EventDispatchers|CreateEvent :!event Custom|BeginPlay_Button))
  (Default|LaunchBeginPlayifNoLevelManager _bp_ac_stategameplayelement))

(event EventFeedbacksDetectTarget
  (Rendering|Material|SetOverlayMaterial (Variables|Default|GetButton) "/Game/Materials/M_OutlineTarget.M_OutlineTarget" :!class /Script/Engine.MeshComponent))

(event EventDeleteFeedbacksDetectTarget
  (Rendering|Material|SetOverlayMaterial (Variables|Default|GetButton) 0 :!class /Script/Engine.MeshComponent))

(event EventGetHit
  (params (TelekinesisElement :type BP%20Abstract%20Telekinesis%20Element%20Object%20Reference) (CanDamage :type Boolean) (DamageObject :type Float%20%28double-precision%29) (VectorHit :type Vector :default "0, 0, 0") (ForceKnockback :type Vector :default "0, 0, 0"))
  (bind _linktrap (Variables|Default|GetLinkTrap))
  (if CanDamage
    (if (not (Variables|Default|GetIsActivated))
      (Utilities|IsValid _linktrap
        (:Is%20Valid
          (if (not (Variables|/Game/Blueprints/Actors/Traps/ActivationTrap/BP_AbstractActivationTrap.BP_AbstractActivationTrap_C|GetIsActivated _linktrap))
            (Default|CallActivationEvent self :!label _label)
            (Default|DisableinSave (Variables|Default|GetBP_AC_StateGameplayElement))
            (Components|Timeline|PlayfromStart (Variables|Default|GetPressButton))
            (Variables|Default|SetIsActivated true)))
        (:Is%20Not%20Valid
          (goto _label))))))

(event EventSetActive
  (params (IsActive :type Boolean))
  (bind _bp_ac_stategameplayelement (Variables|Default|GetBP_AC_StateGameplayElement))
  ;[0.298 1 0.5765] BeginPlay
  (EventDispatchers|BindEventtoSetActiveElementEventDispatcher _bp_ac_stategameplayelement (EventDispatchers|CreateEvent :!event Custom|LoadButton))
  (EventDispatchers|BindEventtoBeginPlayActiveElement _bp_ac_stategameplayelement (EventDispatchers|CreateEvent :!event Custom|BeginPlay_Button))
  (Default|SetActiveElement (Variables|Default|GetBP_AC_StateGameplayElement) IsActive))

(fn ConstructionScript)

(fn PushAnimation
  (bind _pressbutton (Variables|Default|GetPressButton))
  (if (Variables|Default|GetIsActivated)
    (Components|Timeline|ReversefromEnd _pressbutton)
    (Variables|Default|SetIsActivated false)
    (else
      (Components|Timeline|PlayfromStart _pressbutton)
      (Variables|Default|SetIsActivated true))))

(fn GetCanTakeDamage
  (return false))