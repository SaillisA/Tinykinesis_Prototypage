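; BP_ActivationCristal is a crystal actor, filed with the activation trap, that changes glow, spin speed and height for activation.
; BeginPlay creates a dynamic gemstone material at its off-state emissive and stores a target position above the start.
; Update events lerp emissive and rotation rate from the TurnOnEmissive timeline, and height from DuringActivation through a sinusoidal curve.
; Nothing in this graph starts either timeline.
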(event Custom|Update_Emissive
  (bind _turnonemissive (Variables|Default|GetTurnOnEmissive))
  (bind _value (CallFunction|TLNormalize _turnonemissive))
  (Rendering|Material|SetScalarParameterValue (Variables|Default|GetEmissiveMaterial) "ValueEmissive" (Math|Float|Lerp (Variables|Default|GetOffStateEmissive) (Variables|Default|GetOnStateEmissive) _value) :!class /Script/Engine.MaterialInstanceDynamic)
  (Variables|/Script/Engine.RotatingMovementComponent|SetRotationRate (Variables|Default|GetRotatingMovement) (Math|Rotator|MakeRotator 0.0 0.0 (Math|Float|Lerp 3e+01 9e+01 _value))))

(event Custom|Update_Location
  (Transformation|SetWorldLocation (Variables|Default|GetStaticMesh) (Math|Vector|Lerp(Vector) (Variables|Default|GetInitialPosition) (Variables|Default|GetTargetPosition) (CallFunction|TLCurve "/Game/Miscellaneous/Curves/C_Sinuzoidale.C_Sinuzoidale" (Variables|Default|GetDuringActivation))) false false))

(event EventBeginPlay
  (bind _returnvalue (Rendering|Material|CreateDynamicMaterialInstance (Variables|Default|GetStaticMesh) 0 "/Game/Materials/MI_Gemstone_002.MI_Gemstone_002" "ValueEmissive" :!class /Script/Engine.PrimitiveComponent))
  (bind _output_get (Variables|Default|SetEmissiveMaterial _returnvalue))
  (Rendering|Material|SetScalarParameterValue _output_get "ValueEmissive" (Variables|Default|GetOffStateEmissive) :!class /Script/Engine.MaterialInstanceDynamic)
  (bind _output_get_2 (Variables|Default|SetInitialPosition (Transformation|GetWorldLocation (Variables|Default|GetStaticMesh))))
  (Variables|Default|SetTargetPosition (+ _output_get_2 "0.000000,0.000000,100.000000")))

(event Collision|EventActorBeginOverlap
  (params (OtherActor :type Actor%20Object%20Reference)))

(event EventTick
  (params (DeltaSeconds :type Float%20%28single-precision%29)))

(fn ConstructionScript)