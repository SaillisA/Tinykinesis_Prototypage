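; Fairies wheel activation trap Blueprint, a child trap whose wheel damages actors while active.
; Activation plays a Level Sequence, alternating forward and reverse each time, and switches the wheel to a query-only damage overlap profile.
; Wheel overlaps then inflict damage at the sweep hit location.
; Ending activation calls the parent logic and restores the wheel to blocking, physics-enabled collision.
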(event OnComponentBeginOverlap(Wheel)
  (params (OverlappedComponent :type Primitive%20Component%20Object%20Reference) (OtherActor :type Actor%20Object%20Reference) (OtherComp :type Primitive%20Component%20Object%20Reference) (OtherBodyIndex :type Integer) (bFromSweep :type Boolean) (SweepResult :type Hit%20Result%20Structure%20%28by%20ref%29))
  (CallFunction|InflictDamage OtherActor (.Location (Collision|BreakHitResult SweepResult))))

(event EventBeginPlay
  (|CallParentFunction))

(event Collision|EventActorBeginOverlap
  (params (OtherActor :type Actor%20Object%20Reference))
  (|CallParentFunction OtherActor))

(event EventTick
  (params (DeltaSeconds :type Float%20%28single-precision%29))
  (|CallParentFunction DeltaSeconds))

(fn ConstructionScript
  (|CallParentFunction))

(fn ActivationEffect
  (bind _levelsequence (Variables|Default|GetLevelSequence))
  (bind _wheel (Variables|Default|GetWheel))
  (bind _sequenceplayer (Variables|/Script/LevelSequence.LevelSequenceActor|GetSequencePlayer _levelsequence))
  (if (Variables|Default|GetPlayReverse)
    (Class|MovieSceneSequencePlayer|PlayReverse _sequenceplayer)
    (else
      (Sequencer|Player|Play _sequenceplayer :!class /Script/MovieScene.MovieSceneSequencePlayer)))
  (Variables|Default|SetPlayReverse (not (Variables|Default|GetPlayReverse)))
  (Collision|SetCollisionProfileName _wheel "OverlapDamageElements" true :!class /Script/Engine.PrimitiveComponent)
  (Collision|SetCollisionEnabled _wheel "QueryOnly"))

(fn EndActivation
  (|CallParentFunction)
  (Collision|SetCollisionProfileName (Variables|Default|GetWheel) "BlockAll" true :!class /Script/Engine.PrimitiveComponent)
  (Collision|SetCollisionEnabled (Variables|Default|GetWheel) "QueryAndPhysics"))