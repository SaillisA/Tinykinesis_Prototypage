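; Base trap actor, meant as a parent for traps that a linked button activates.
; LinkToButton binds a delegate to the button's activation event, and ActivationEffect is a placeholder that only prints a debug message.
; InflictDamage applies Damage through the HealthManager on a BP_AICharacterBlank's owner, so only characters owned by BP_AIC_NpcMelee lose HP.
; HitLocation is unused.
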(event Custom|LinkToButton
  (params (ButtonToLink :type BP%20Activation%20Button%20Object%20Reference))
  (EventDispatchers|BindEventtoActivationEvent ButtonToLink (EventDispatchers|CreateEvent :!event ActivationEffect)))

(event EventBeginPlay)

(event Collision|EventActorBeginOverlap
  (params (OtherActor :type Actor%20Object%20Reference)))

(event EventTick
  (params (DeltaSeconds :type Float%20%28single-precision%29)))

(fn ConstructionScript)

(fn ActivationEffect
  (params (ActivatedButton :type BP%20Activation%20Button%20Object%20Reference))
  (Development|PrintString "Hi im the linked Trap"))

(fn InflictDamage
  (params (Actor :type Object%20Object%20Reference) (HitLocation :type Vector))
  (bind _asbp_aicharacter_blank (Utilities|Casting|CastToBP_AICharacterBlank Actor))
  (bind _asbp_aic_npc_melee (Utilities|Casting|CastToBP_AIC_NpcMelee (Components|GetOwner _asbp_aicharacter_blank)))
  (Default|LooseHP (Variables|/Game/Blueprints/NPC/AIMelee/BP_AIC_NpcMelee.BP_AIC_NpcMelee_C|GetHealthManager _asbp_aic_npc_melee) (Variables|Default|GetDamage)))