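; Arena manager child that runs endlessly looping enemy waves until spawning is stopped.
; Once the current wave drops to its switch threshold, it advances through the wave list, wraps to the start and sets up the next wave after a delay.
; Triggering combat optionally spawns a spawning crystal at a preview component's transform, passing it this manager.
; After StopInfiniteSpawn disables spawning, the arena ends when the current wave is empty.
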(event EventBeginPlay
  (|CallParentFunction))

(fn ConstructionScript
  (bind _spawningcrystal_visual (Variables|Default|GetSpawningCrystal_Visual))
  (|CallParentFunction)
  (if (Variables|Default|GetSpawnCrystal)
    (Rendering|SetVisibility _spawningcrystal_visual true true)
    (else
      (Rendering|SetVisibility _spawningcrystal_visual false true))))

(fn CheckEndWave
  (if (and (not (Variables|Default|GetAllowSpawn)) (== (Utilities|Array|Length (Variables|Default|GetCurrentWave)) 0))
    (CallFunction|EndArena)
    (return)
    (elif (Math|Boolean|ANDBoolean (<= (Utilities|Array|Length (Variables|Default|GetCurrentWave)) (.WaveSwitch (Utilities|Struct|BreakS_ArenaManager_Wave (Utilities|Array|Get(acopy) (Variables|Default|GetWaveList) (Variables|Default|GetWaveCount))))) (Variables|Default|GetCanCheckEndWave) (Variables|Default|GetAllowSpawn))
      (if (== (+ (Variables|Default|GetWaveCount) 1) (Utilities|Array|Length (Variables|Default|GetWaveList)))
        (Variables|Default|SetWaveCount 0)
        (else
          (Math|Integer|IncrementInt (Variables|Default|GetWaveCount)
            (:%20%20
              _))))
      (Variables|Default|SetSpawnedWave (.Wave (Utilities|Struct|BreakS_ArenaManager_Wave (Utilities|Array|Get(acopy) (Variables|Default|GetWaveList) (Variables|Default|GetWaveCount)))))
      (CallFunction|SetupWavewithDelay))))

(fn SetupArenaManager
  (|CallParentFunction)
  (Variables|Default|SetAllowSpawn true))

(fn StopInfiniteSpawn
  (Variables|Default|SetAllowSpawn false))

(fn SetupCrystalSpawn
  (if (Variables|Default|GetSpawnCrystal)
    (bind _returnvalue (Game|SpawnActorfromClass "/Game/Blueprints/Actors/ArenaManagement/BP_SpawningCrystal.BP_SpawningCrystal_C" (Transformation|GetWorldTransform (Variables|Default|GetSpawningCrystal_Visual)) "Undefined" "MultiplyWithRoot" 0 0))
    (Default|SetInfiteArenaManager _returnvalue self)))

(fn TriggerCombat
  (|CallParentFunction)
  (CallFunction|SetupCrystalSpawn))