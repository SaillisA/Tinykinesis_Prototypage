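; Destructible spawning crystal that bobs vertically around its start height via a sine-driven lerp on Tick, and stops its linked infinite arena manager's spawning when destroyed.
; Hits that can damage it go through the health component, with a brief immunity window after each non-lethal hit.
; Damage and death effects fire events, using a timeline and destruction component for mesh shake and fracture.
; GetCanTakeDamage always returns false.
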(event EventBeginPlay
  (bind _bp_ac_health (Variables|Components|GetBP_AC_Health))
  (EventDispatchers|BindEventtoDeath _bp_ac_health (EventDispatchers|CreateEvent :!event DeathEffect))
  (EventDispatchers|BindEventtoDamageEffect _bp_ac_health (EventDispatchers|CreateEvent :!event DamageEffect))
  (Utilities|Array|SetArrayElem (Variables|Default|GetSinMovementPos) 0 (Math|Vector|MakeVector 0.0 0.0 (+ (.z (Transformation|GetActorLocation)) 3e+01)))
  (Utilities|Array|SetArrayElem (Variables|Default|GetSinMovementPos) 1 (Math|Vector|MakeVector 0.0 0.0 (+ (.z (Transformation|GetActorLocation)) -3e+01))))

(event EventTick
  (params (DeltaSeconds :type Float%20%28single-precision%29))
  (bind _returnvalue (Transformation|GetActorLocation))
  (bind _returnvalue_2 (Transformation|GetActorLocation))
  (bind _output_get (Variables|Default|SetSinMovementLerp (+ (Variables|Default|GetSinMovementLerp) 0.75)))
  (Transformation|SetActorLocation (Math|Vector|Lerp(Vector) (Math|Vector|MakeVector (.x _returnvalue_2) (.y _returnvalue_2) (.z (Utilities|Array|Get(acopy) (Variables|Default|GetSinMovementPos)))) (Math|Vector|MakeVector (.x _returnvalue) (.y _returnvalue) (.z (Utilities|Array|Get(acopy) (Variables|Default|GetSinMovementPos) 1))) (Math|Trig|Sin(Degrees) _output_get)) false false))

(event EventGetHit
  (params (TelekinesisElement :type BP%20Abstract%20Telekinesis%20Element%20Object%20Reference) (CanDamage :type Boolean) (DamageObject :type Float%20%28double-precision%29) (VectorHit :type Vector :default "0, 0, 0") (ForceKnockback :type Vector :default "0, 0, 0"))
  (if CanDamage
    (if (not (Variables|Default|GetImmunityAfterDamage))
      (Variables|Default|SetImmunityAfterDamage true)
      (bind _isdead (Default|LooseHP (Variables|Components|GetBP_AC_Health) DamageObject))
      (if (not _isdead)
        (Utilities|FlowControl|Delay 0.5)
        (Variables|Default|SetImmunityAfterDamage false)))))

(fn ConstructionScript)

(fn DeathEffect
  (bind _infinitearenamanager (Variables|Default|GetInfiniteArenaManager))
  (Default|CallOnDeathEvent self)
  (Utilities|FlowControl|Sequence
    (:then_0
      (Utilities|IsValid _infinitearenamanager
        (:Is%20Valid
          (Default|StopInfiniteSpawn _infinitearenamanager))))
    (:then_1
      (Default|LaunchDestruction (Variables|Components|GetBP_AC_DestructionElement) (Transformation|GetActorTransform) 1.0 0.0 self))))

(fn DamageEffect
  (Default|CallOnDamageEffect)
  (Components|Timeline|PlayfromStart (Variables|Default|GetTimeline_ShakeOnDamage)))

(fn SetInfiteArenaManager
  (params (InfiniteArenaManager :type BP%20Infinite%20Arena%20Manager%20Object%20Reference))
  (Variables|Default|SetInfiniteArenaManager InfiniteArenaManager))

(fn GetCanTakeDamage
  (return false))