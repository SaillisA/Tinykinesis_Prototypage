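; Base arena manager that runs wave-based combat encounters, locking barriers and switching to battle music when the player triggers it.
; Waves spawn mobs in random order through a self-calling delayed event, each tagged with a component linking it back to the manager.
; CheckEndWave advances waves at a remaining-mob threshold and outlines stragglers when barriers exist.
; The final wave lowers barriers, restores exploration audio, disables the arena in the save and saves the game.
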(event OnComponentBeginOverlap(ArenaTrigger)
  (params (OverlappedComponent :type Primitive%20Component%20Object%20Reference) (OtherActor :type Actor%20Object%20Reference) (OtherComp :type Primitive%20Component%20Object%20Reference) (OtherBodyIndex :type Integer) (bFromSweep :type Boolean) (SweepResult :type Hit%20Result%20Structure%20%28by%20ref%29))
  (if (and (== OtherActor (CallFunction|GetTinykinesisPlayerCharacter)) (not (Variables|EndingArena|GetArenaFinished)))
    (StartingArena|TriggerCombat)))

(event Custom|SetupWaveWithDelay
  (bind _spawnedwave (Variables|Default|GetSpawnedWave))
  (Variables|Spawn|SetCanCheckEndWave false)
  (if (== (Utilities|Array|Length _spawnedwave) 0)
    (Variables|Spawn|SetCanCheckEndWave true)
    (bind _arrayelement (Utilities|Array|ReverseforEachLoop (Variables|Spawn|GetCurrentWave))
      (:LoopBody
        (Rendering|Material|SetOverlayMaterial (Variables|/Script/Engine.Character|GetMesh _arrayelement) 0 :!class /Script/Engine.MeshComponent)))
    (else
      (bind _output_get (Variables|Default|SetRandomMob (.OutItem (Utilities|Array|Random _spawnedwave))))
      (Spawn|SpawnMob (.MobType (Utilities|Struct|BreakS_ArenaManager_MobInfo _output_get)) (.MobSpawnTransform (Utilities|Struct|BreakS_ArenaManager_MobInfo _output_get)))
      (Utilities|Array|RemoveItem _spawnedwave (Variables|Default|GetRandomMob))
      (Utilities|FlowControl|Delay (Variables|Default|GetDelayBetweenSpawn))
      (CallFunction|SetupWavewithDelay))))

(event Custom|BeginPlay_ArenaManager
  ;[0.298 1 0.5765] BeginPlay
  (Variables|Setup|SetCanTick true)
  (Variables|Default|SetPlayerCharacter (CallFunction|GetTinykinesisPlayerCharacter))
  (Setup|SetupArenaManager)
  (Utilities|FlowControl|Delay 0.2)
  (Setup|SetupArenaBarrier))

(event Custom|LoadArenaManager
  (bind _bp_ac_stategameplayelement (Variables|Default|GetBP_AC_StateGameplayElement))
  ;[0.298 1 0.5765] BeginPlay
  (Utilities|FlowControl|Sequence
    (:then_0
      (if (not (Variables|/Game/Blueprints/ActorComponents/BP_AC_StateGameplayElement.BP_AC_StateGameplayElement_C|GetIsActivated (Variables|Default|GetBP_AC_StateGameplayElement)))
        (Variables|EndingArena|SetArenaFinished true)))
    (:then_1
      (Default|LoadElement _bp_ac_stategameplayelement (Variables|/Game/Blueprints/ActorComponents/BP_AC_StateGameplayElement.BP_AC_StateGameplayElement_C|GetIsActivated _bp_ac_stategameplayelement) self))))

(event EventBeginPlay
  (bind _bp_ac_stategameplayelement (Variables|Default|GetBP_AC_StateGameplayElement))
  ;[0.298 1 0.5765] BeginPlay
  (EventDispatchers|BindEventtoBeginPlayActiveElement _bp_ac_stategameplayelement (EventDispatchers|CreateEvent :!event Custom|BeginPlay_ArenaManager))
  (Default|LaunchBeginPlay _bp_ac_stategameplayelement))

(event EventSetActive
  (params (IsActive :type Boolean))
  (bind _bp_ac_stategameplayelement (Variables|Default|GetBP_AC_StateGameplayElement))
  ;[0.298 1 0.5765] BeginPlay
  (EventDispatchers|BindEventtoSetActiveElementEventDispatcher _bp_ac_stategameplayelement (EventDispatchers|CreateEvent :!event Custom|LoadArenaManager))
  (EventDispatchers|BindEventtoBeginPlayActiveElement _bp_ac_stategameplayelement (EventDispatchers|CreateEvent :!event Custom|BeginPlay_ArenaManager))
  (Default|SetActiveElement (Variables|Default|GetBP_AC_StateGameplayElement) IsActive))

(fn ConstructionScript)

(fn SetupArenaBarrier
  (for _array_element (Variables|StartingArena|GetlistArenaBarrier)
    (Utilities|IsValid _array_element
      (:Is%20Valid
        (Variables|/Game/Blueprints/Actors/ArenaManagement/BP_ArenaBarrier.BP_ArenaBarrier_C|SetArenaManager _array_element self)
        (Default|DesactivateBarrier _array_element false)))))

(fn TriggerCombat
  (if (and (or (Variables|StartingArena|GetPlayerInArena) (== (Utilities|Array|Length (Variables|StartingArena|GetlistArenaBarrier)) 0)) (not (Variables|StartingArena|GetIsArenaTrigger)))
    (Variables|/Script/Engine.PrimitiveComponent|SetbGenerateOverlapEvents (Variables|Default|GetArenaTrigger) false)
    (Variables|StartingArena|SetIsArenaTrigger true)
    (Default|CallArenaStartingEvent)
    (Variables|/Game/Blueprints/Player/BP_TinykinesisPlayerController.BP_TinykinesisPlayerController_C|SetIsFightingArena (CallFunction|GetTinykinesisPlayerController) true)
    (Utilities|FlowControl|Sequence
      (:then_0
        (for _array_element (Variables|StartingArena|GetlistArenaBarrier)
          (Utilities|IsValid _array_element
            (:Is%20Valid
              (Default|ActivateBarrier _array_element)))))
      (:then_1
        (for _array_element_2 (Variables|Spawn|GetCurrentWave)
          (Utilities|IsValid _array_element_2
            (:Is%20Valid
              (Default|BecameAggro _array_element_2)))))
      (:then_2
        (if (== (Utilities|Array|Length (Variables|StartingArena|GetlistArenaBarrier)) 0)
          _
          (else
            (Default|LaunchBattleMusic (Variables|/Game/Blueprints/Player/BP_TinykinesisPlayerController.BP_TinykinesisPlayerController_C|GetBP_AC_AmbianceMusic (CallFunction|GetTinykinesisPlayerController)))
            (Components|Timeline|PlayfromStart (Variables|Default|GetSoundVolume))
            (Components|Timeline|ReversefromEnd (Variables|/Game/Blueprints/Player/BP_TinykinesisPlayerController.BP_TinykinesisPlayerController_C|GetExplorationSound (CallFunction|GetTinykinesisPlayerController)))))
        (Variables|Default|SetSpawnedWave (.Wave (Utilities|Struct|BreakS_ArenaManager_Wave (Utilities|Array|Get(acopy) (Variables|Spawn|GetWaveList) (Variables|Spawn|GetWaveCount)))))
        (CallFunction|SetupWavewithDelay)))))

(fn EndArena
  (Development|PrintString "Arena Finished")
  (Variables|EndingArena|SetArenaFinished true)
  (Variables|/Game/Blueprints/Player/BP_TinykinesisPlayerController.BP_TinykinesisPlayerController_C|SetIsFightingArena (CallFunction|GetTinykinesisPlayerController) false)
  (Default|CallArenaEndingEvent)
  (Default|DisableinSave (Variables|Default|GetBP_AC_StateGameplayElement))
  (Components|Timeline|ReversefromEnd (Variables|Default|GetSoundVolume))
  (Components|Timeline|PlayfromStart (Variables|/Game/Blueprints/Player/BP_TinykinesisPlayerController.BP_TinykinesisPlayerController_C|GetExplorationSound (CallFunction|GetTinykinesisPlayerController)))
  (for _array_element (Variables|StartingArena|GetlistArenaBarrier)
    (Utilities|IsValid _array_element
      (:Is%20Valid
        (Default|DesactivateBarrier _array_element false))))
  (bind _returnvalue (Actor|GetActorOfClass "/Game/Blueprints/SaveSystem/BP_AbstractLevelManager.BP_AbstractLevelManager_C"))
  (Utilities|IsValid _returnvalue
    (:Is%20Valid
      (Default|TriggerSaveGame _returnvalue (Transformation|GetActorTransform (CallFunction|GetTinykinesisPlayerCharacter))))))

(fn SetupArenaManager
  (Variables|StartingArena|SetIsArenaTrigger false)
  (Variables|StartingArena|SetPlayerInArena false)
  (for _array_element (Variables|Spawn|GetCurrentWave)
    (Utilities|IsValid _array_element
      (:Is%20Valid
        (bind _returnvalue (AddComponent|AddBPACArenaManagerManageMob _array_element))
        (Default|SetArenaManager _returnvalue self)))))

(fn SetupWave
  (Variables|Spawn|SetCanCheckEndWave false)
  (for _array_element (.Wave (Utilities|Struct|BreakS_ArenaManager_Wave (Utilities|Array|Get(acopy) (Variables|Spawn|GetWaveList) (Variables|Spawn|GetWaveCount))))
    (Spawn|SpawnMob (.MobType (Utilities|Struct|BreakS_ArenaManager_MobInfo _array_element)) (.MobSpawnTransform (Utilities|Struct|BreakS_ArenaManager_MobInfo _array_element))))
  (Variables|Spawn|SetCanCheckEndWave true))

(fn CheckEndWave
  (bind _currentwave (Variables|Spawn|GetCurrentWave))
  (bind (_arrayindex _arrayelement) (Utilities|Array|ReverseforEachLoop _currentwave)
    (:LoopBody
      (Utilities|IsValid _arrayelement
        (:Is%20Not%20Valid
          (Utilities|Array|RemoveIndex _currentwave _arrayindex))))
    (:Completed
      (if (and (<= (Utilities|Array|Length (Variables|Spawn|GetCurrentWave)) (.WaveSwitch (Utilities|Struct|BreakS_ArenaManager_Wave (Utilities|Array|Get(acopy) (Variables|Spawn|GetWaveList) (Variables|Spawn|GetWaveCount))))) (Variables|Spawn|GetCanCheckEndWave))
        (if (== (+ (Variables|Spawn|GetWaveCount) 1) (Utilities|Array|Length (Variables|Spawn|GetWaveList)))
          (EndingArena|EndArena)
          (else
            (Math|Integer|IncrementInt (Variables|Spawn|GetWaveCount)
              (:%20%20
                (Variables|Default|SetSpawnedWave (.Wave (Utilities|Struct|BreakS_ArenaManager_Wave (Utilities|Array|Get(acopy) (Variables|Spawn|GetWaveList) (Variables|Spawn|GetWaveCount)))))
                (CallFunction|SetupWavewithDelay)))))
        (elif (and (<= (Utilities|Array|Length (Variables|Spawn|GetCurrentWave)) (Variables|Default|GetMobOutlineTrigger)) (!= (Utilities|Array|Length (Variables|StartingArena|GetlistArenaBarrier)) 0))
          (bind _arrayelement_2 (Utilities|Array|ReverseforEachLoop (Variables|Spawn|GetCurrentWave))
            (:LoopBody
              (Rendering|Material|SetOverlayMaterial (Variables|/Script/Engine.Character|GetMesh _arrayelement_2) "/Game/Materials/M_OutlineMob.M_OutlineMob" :!class /Script/Engine.MeshComponent))))))))

(fn SpawnMob
  (params (Class :type BP%20AI%20Character%20Blank%20Class%20Reference) (SpawnTransform :type Transform))
  (bind _returnvalue (Game|SpawnActorfromClass Class SpawnTransform "Undefined" "MultiplyWithRoot" 0 0))
  (Default|ImmunityHitEvent _returnvalue)
  (bind _returnvalue_2 (AddComponent|AddBPACArenaManagerManageMob _returnvalue))
  (Default|SetArenaManager _returnvalue_2 self)
  (Default|BecameAggro _returnvalue)
  (Utilities|Array|AddUnique (Variables|Spawn|GetCurrentWave) _returnvalue)
  (return _returnvalue))