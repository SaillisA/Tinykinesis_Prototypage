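; BP_ArenaBarrier is an arena boundary that switches between an invisible pass-through trigger and a visible blocking wall.
; It starts deactivated with query-only Pawn overlap, and each overlap begin by the ArenaManager's player flips that manager's PlayerInArena flag.
; ActivateBarrier enables physics blocking for Pawns, shows the mesh and fires an explosion cloud effect, while DesactivateBarrier restores the hidden trigger state.
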(event OnComponentBeginOverlap(Barrier)
  (params (OverlappedComponent :type Primitive%20Component%20Object%20Reference) (OtherActor :type Actor%20Object%20Reference) (OtherComp :type Primitive%20Component%20Object%20Reference) (OtherBodyIndex :type Integer) (bFromSweep :type Boolean) (SweepResult :type Hit%20Result%20Structure%20%28by%20ref%29))
  (bind _arenamanager (Variables|Default|GetArenaManager))
  (if (== OtherActor (Variables|/Game/Blueprints/Actors/ArenaManagement/BP_AbstractArenaManager.BP_AbstractArenaManager_C|GetPlayerCharacter _arenamanager))
    (Variables|/Game/Blueprints/Actors/ArenaManagement/BP_AbstractArenaManager.BP_AbstractArenaManager_C|SetPlayerInArena (Variables|Default|GetArenaManager) (not (Variables|/Game/Blueprints/Actors/ArenaManagement/BP_AbstractArenaManager.BP_AbstractArenaManager_C|GetPlayerInArena _arenamanager)))))

(event EventBeginPlay
  (CallFunction|DesactivateBarrier))

(fn ConstructionScript)

(fn DesactivateBarrier
  (bind _barrier (Variables|Default|GetBarrier))
  (Collision|SetCollisionEnabled _barrier "QueryOnly")
  (Collision|SetCollisionResponsetoChannel _barrier "ECC_Pawn" "ECR_Overlap")
  (Rendering|SetVisibility _barrier false false))

(fn ActivateBarrier
  (bind _barrier (Variables|Default|GetBarrier))
  (Collision|SetCollisionEnabled _barrier "QueryAndPhysics")
  (Collision|SetCollisionResponsetoChannel _barrier "ECC_Pawn" "ECR_Block")
  (Rendering|SetVisibility _barrier true false)
  (Components|Activation|Activate (Variables|Default|GetNS_ExplosionCloud) false))