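; Base arena manager that locks the player into timed combat behind barriers, started by a trigger overlap or an aggroed mob.
; A timeline is meant to drive mob caps and the timer.
; Tick spawns aggroed melee mobs at random free points within a player-distance range and prunes invalid or ragdolled ones.
; Once the timer has finished and the mob list is empty, it fires the ending event and lowers the barriers.
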(event OnComponentBeginOverlap(ArenaTrigger)
  (params (OverlappedComponent :type Primitive%20Component%20Object%20Reference) (OtherActor :type Actor%20Object%20Reference) (OtherComp :type Primitive%20Component%20Object%20Reference) (OtherBodyIndex :type Integer) (bFromSweep :type Boolean) (SweepResult :type Hit%20Result%20Structure%20%28by%20ref%29))
  (if (== OtherActor (Game|GetPlayerCharacter 0))
    (StartingArena|TriggerCombat)
    (Variables|/Script/Engine.PrimitiveComponent|SetbGenerateOverlapEvents (Variables|Default|GetArenaTrigger) false)))

(event EventBeginPlay
  (Setup|SetupArenaBarrier)
  (bind _asbp_tinykinesis_player_character (Utilities|Casting|CastToBP_TinykinesisPlayerCharacter (Game|GetPlayerCharacter 0)))
  (Variables|Default|SetPlayerCharacter _asbp_tinykinesis_player_character))

(event EventTick
  (params (DeltaSeconds :type Float%20%28single-precision%29))
  (bind _listmob (Variables|MobSpawn|GetlistMob))
  (Utilities|FlowControl|Sequence
    (:then_0
      (if (and (Variables|StartingArena|GetPlayerInArena) (not (Variables|StartingArena|GetIsArenaTrigger))) ; Check if Mob get Aggro
        (bind _array_element (Utilities|Array|ForEachLoopwithBreak (Variables|MobSpawn|GetlistMob) :!label _label)
          (:LoopBody
            (Utilities|IsValid _array_element
              (:Is%20Valid
                (if (Variables|/Game/Blueprints/NPC/BP_AICharacterBlank.BP_AICharacterBlank_C|GetIsAggro _array_element)
                  (StartingArena|TriggerCombat)
                  (goto _label Break))))))))
    (:then_1
      (if (and (Variables|StartingArena|GetIsArenaTrigger) (not (Variables|EndingArena|GetArenaFinished))) ; Check WinCondition
        (EndingArena|CheckingWinCondition)))
    (:then_2
      (if (and (not (Variables|EndingArena|GetisArenaTimerFinished)) (Variables|StartingArena|GetIsArenaTrigger)) ; Spawn de Mob
        (MobSpawn|SpawnBaseMob)))
    (:then_3
      ;[1 1 1] Clear listmob, maybe add component/function on mob for that
      (for (_array_element_2 _array_index) _listmob
        (Utilities|IsValid _array_element_2
          (:Is%20Valid
            (if (Physics|IsSimulatingPhysics (Variables|/Script/Engine.Character|GetMesh _array_element_2) "None")
              (Utilities|Array|RemoveIndex _listmob _array_index)))
          (:Is%20Not%20Valid
            (Utilities|Array|RemoveIndex _listmob _array_index)))))))

(fn ConstructionScript
  (Utilities|FlowControl|Sequence
    (:then_0
      ;[1 1 1] Proctection for enter range value
      (Variables|MobSpawn|SetminDistanceSpawn (Math|Float|Clamp(Float) (Variables|MobSpawn|GetminDistanceSpawn) 0.0 (- (Variables|MobSpawn|GetmaxDistanceSpawn) 0.1))) ; Minimum can't be a negative value and exactly equal to maximum
      (Variables|MobSpawn|SetmaxDistanceSpawn (Math|Float|Clamp(Float) (Variables|MobSpawn|GetmaxDistanceSpawn) (Variables|MobSpawn|GetminDistanceSpawn) (Variables|MobSpawn|GetmaxDistanceSpawn))) ; Maximum can't be smaller than minimum but can be infinite
    )
    (:then_1
      (Components|Sphere|SetSphereRadius (Variables|Tools|GetMinimumSpawnRange) (Variables|MobSpawn|GetminDistanceSpawn) true)
      (Components|Sphere|SetSphereRadius (Variables|Tools|GetMaximumSphereRange) (Variables|MobSpawn|GetmaxDistanceSpawn) true))
    (:then_2
      (Rendering|SetVisibility (Variables|Tools|GetRangeChecker) (Variables|Tools|GetActiveRangeChecker) true))))

(fn SetupArenaBarrier
  (for _array_element (Variables|StartingArena|GetlistArenaBarrier)
    (Utilities|IsValid _array_element
      (:Is%20Valid
        (Variables|/Game/Blueprints/Actors/ArenaManagement/BP_ArenaBarrier.BP_ArenaBarrier_C|SetArenaManager _array_element 0)
        (Default|DesactivateBarrier _array_element)))))

(fn TriggerCombat
  (Variables|StartingArena|SetIsArenaTrigger true)
  (Components|Timeline|PlayfromStart (Variables|Default|GetArenaTimeline))
  (Development|PrintString "Arena Started")
  (Default|CallArenaStartingEvent)
  (for _array_element (Variables|MobSpawn|GetlistMob)
    (Utilities|IsValid _array_element
      (:Is%20Valid
        (Default|BecameAggro _array_element))))
  (for _array_element_2 (Variables|StartingArena|GetlistArenaBarrier)
    (Utilities|IsValid _array_element_2
      (:Is%20Valid
        (Default|ActivateBarrier _array_element_2)))))

(fn SpawnBaseMob
  (bind _output_get (LocalVariables|SetSelectedTargetPoint (.OutItem (Utilities|Array|Random (Variables|MobSpawn|GetlistSpawnPointBaseMob)))))
  (Utilities|IsValid _output_get
    (:Is%20Valid
      (if (Variables|/Game/Blueprints/Actors/ArenaManagement/BP_ArenaSpawnPoint.BP_ArenaSpawnPoint_C|GetCanSpawn (LocalVariables|GetSelectedTargetPoint))
        (Default|UseSpawnPoint (LocalVariables|GetSelectedTargetPoint))
        (bind _returnvalue (Collision|SphereTraceForObjects (Transformation|GetActorLocation (LocalVariables|GetSelectedTargetPoint)) (Transformation|GetActorLocation (LocalVariables|GetSelectedTargetPoint)) (LocalVariables|GetCheckSpawnRadius) (LocalVariables|GetTraceObjectType) false 0 "None"))
        (if (not _returnvalue)
          (if (and (> (Variables|MobSpawn|GetmaxBaseMobNumber) (Utilities|Array|Length (Variables|MobSpawn|GetlistMob))) (Math|Float|InRange(Float) (Math|Vector|Distance(Vector) (Transformation|GetActorLocation (Game|GetPlayerCharacter 0)) (Transformation|GetActorLocation (LocalVariables|GetSelectedTargetPoint))) (Variables|MobSpawn|GetminDistanceSpawn) (Variables|MobSpawn|GetmaxDistanceSpawn)))
            (bind _returnvalue_2 (Game|SpawnActorfromClass "/Game/Blueprints/NPC/AIMelee/BP_CharacterNpcMelee.BP_CharacterNpcMelee_C" (Math|Transform|MakeTransform (Math|Vector|MakeVector (.X (Math|Vector|BreakVector (Transformation|GetActorLocation (LocalVariables|GetSelectedTargetPoint)))) (.Y (Math|Vector|BreakVector (Transformation|GetActorLocation (LocalVariables|GetSelectedTargetPoint)))) (+ (.Z (Math|Vector|BreakVector (Transformation|GetActorLocation (LocalVariables|GetSelectedTargetPoint)))) (LocalVariables|GetHalfHeightMobMesh))) "0, 0, 0" "1.000000,1.000000,1.000000") "Undefined" "MultiplyWithRoot" 0 0))
            (Default|BecameAggro _returnvalue_2)
            (Utilities|Array|Add (Variables|MobSpawn|GetlistMob) _returnvalue_2)))))))

(fn CheckingWinCondition
  (if (and (Variables|EndingArena|GetisArenaTimerFinished) (== (Utilities|Array|Length (Variables|MobSpawn|GetlistMob)) 0))
    (Development|PrintString "Arena Finished")
    (Variables|EndingArena|SetArenaFinished true)
    (Default|CallArenaEndingEvent)
    (for _array_element (Variables|StartingArena|GetlistArenaBarrier)
      (Utilities|IsValid _array_element
        (:Is%20Valid
          (Default|DesactivateBarrier _array_element))))))