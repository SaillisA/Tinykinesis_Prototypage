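; BP_DamageExplosiveObject is a child destructible-object Blueprint that explodes and can kill enemies it affects.
; ExplosionEffect extends the parent with a radial force impulse and a world camera shake centred on the Tinykinesis player.
; EffectOfEnnemy casts the object's own owner to the NPC AI controller and removes its max HP.
; On death, it calls the hit enemy's Death with the impact location and fires the impulse again.
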(event EventBeginPlay
  (|CallParentFunction) ; This node is disabled and will not be called.\nDrag off pins to build functionality.
)

(event Collision|EventActorBeginOverlap
  (params (OtherActor :type Actor%20Object%20Reference))
  (|CallParentFunction OtherActor) ; This node is disabled and will not be called.\nDrag off pins to build functionality.
)

(event EventTick
  (params (DeltaSeconds :type Float%20%28single-precision%29))
  (|CallParentFunction DeltaSeconds) ; This node is disabled and will not be called.\nDrag off pins to build functionality.
)

(fn ConstructionScript
  (|CallParentFunction))

(fn ExplosionEffect
  (|CallParentFunction)
  (Class|RadialForceComponent|FireImpulse (Variables|Default|GetRadialForce))
  (bind _asbp_tinykinesis_player_character (Utilities|Casting|CastToBP_TinykinesisPlayerCharacter (Game|GetPlayerCharacter 0)))
  (Camera|PlayWorldCameraShake "/Game/Blueprints/Actors/BP_CameraShake.BP_CameraShake_C" (Transformation|GetActorLocation _asbp_tinykinesis_player_character) 0.0 5e+02))

(fn EffectOfEnnemy
  (params (EnnemyHit :type BP%20AI%20Character%20Blank%20Object%20Reference) (HitLocation :type Vector :default "0, 0, 0"))
  (|CallParentFunction EnnemyHit HitLocation)
  (bind _asbp_aic_npc_base (Utilities|Casting|CastToBP_AIC_NpcBase (Components|GetOwner)))
  (bind _isdead (Default|LooseHP (Variables|/Game/Blueprints/NPC/AIBase/BP_AIC_NpcBase.BP_AIC_NpcBase_C|GetHealthManager _asbp_aic_npc_base) (Variables|/Game/Blueprints/ActorComponents/BP_AC_Health.BP_AC_Health_C|GetmaxHP (Variables|/Game/Blueprints/NPC/AIBase/BP_AIC_NpcBase.BP_AIC_NpcBase_C|GetHealthManager _asbp_aic_npc_base))))
  (if _isdead
    (Default|Death EnnemyHit _asbp_aic_npc_base HitLocation 0.1 0.0)
    (Class|RadialForceComponent|FireImpulse (Variables|Default|GetRadialForce))))

(fn FractureMeshSpawn
  (|CallParentFunction))