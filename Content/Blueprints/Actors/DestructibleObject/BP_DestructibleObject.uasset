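; BP_DestructibleObject is a destructible world actor that loses health and destroys itself when depleted.
; When its projectile flag is on, mesh hits from BP_LightObject actors pass that object's damage value into TakeDamage.
; At zero health or below, Destruction kills every entry in MobTurretOn, calls the destruction effect, then destroys the actor.
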(event OnComponentHit(StaticMeshComponent)
  (params (HitComponent :type Primitive%20Component%20Object%20Reference) (OtherActor :type Actor%20Object%20Reference) (OtherComp :type Primitive%20Component%20Object%20Reference) (NormalImpulse :type Vector :default "0, 0, 0") (Hit :type Hit%20Result%20Structure%20%28by%20ref%29))
  (if (Variables|Default|GetCanBeDestoyByProjectile)
    (bind _asbp_light_object (Utilities|Casting|CastToBP_LightObject OtherActor))
    (CallFunction|TakeDamage (Variables|/Game/Blueprints/Actors/BP_LightObject.BP_LightObject_C|GetDammageLightObject _asbp_light_object))))

(event EventBeginPlay)

(event Collision|EventActorBeginOverlap
  (params (OtherActor :type Actor%20Object%20Reference)))

(event EventTick
  (params (DeltaSeconds :type Float%20%28single-precision%29)))

(fn ConstructionScript)

(fn TakeDamage
  (params (Damage :type Float%20%28double-precision%29))
  (bind _output_get (Variables|Default|SetHealth (- (Variables|Default|GetHealth) Damage)))
  (if (<= _output_get 0.0)
    (CallFunction|Destruction)))

(fn Destruction
  (for _array_element (Variables|Default|GetMobTurretOn)
    (Default|Death _array_element 0 "0, 0, 0" 0.0 0.0))
  (Default|CallOnDestructionEffect)
  (Actor|DestroyActor))