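; BP_Test is a test physics cube actor that exposes telekinesis-style events: levitate, grab, attract, throw and smash.
; Levitate raises it by timeline with gravity off, and Attract moves it to the player.
; Once grabbed, Propulse moves it to a locked target or launches it by impulse.
; Smash slams it down and flags it so Hit destroys the actor after a delay; a velocity-based throw reset is unwired.
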(event EventLevitate
  (bind _cube (Variables|Default|GetCube))
  (bind _returnvalue (Transformation|GetWorldLocation _cube))
  (bind (_x _y _z) (Math|Vector|BreakVector _returnvalue))
  (Class|PrimitiveComponent|SetAllPhysicsLinearVelocity (Variables|Default|GetCube) "0, 0, 0" false)
  (bind _levitation (Timeline|Levitation PlayFromStart)
    (:Update
      (Transformation|SetWorldLocation (Variables|Default|GetCube) (Math|Vector|MakeVector _x _y (+ _levitation (+ _z 1e+01))) true false)
      (Physics|SetEnableGravity (Variables|Default|GetCube) false))))

(event EventSmash
  (Physics|SetEnableGravity (Variables|Default|GetCube) true)
  (Physics|AddImpulse (Variables|Default|GetCube) "0.000000,0.000000,-2600.000000" "None" true)
  (Variables|Default|SetGettingSmashed true))

(event Collision|EventHit
  (params (MyComp :type Primitive%20Component%20Object%20Reference) (Other :type Actor%20Object%20Reference) (OtherComp :type Primitive%20Component%20Object%20Reference) (bSelfMoved :type Boolean) (HitLocation :type Vector :default "0, 0, 0") (HitNormal :type Vector :default "0, 0, 0") (NormalImpulse :type Vector :default "0, 0, 0") (Hit :type Hit%20Result%20Structure%20%28by%20ref%29))
  (if (Variables|Default|GetGettingSmashed)
    (Utilities|FlowControl|Delay 0.4)
    (Actor|DestroyActor)))

(event EventAttract
  (params (Player%20Location :type Vector :default "0, 0, 0"))
  (Components|MoveComponentTo (Variables|Default|GetCube) Player%20Location "0, 0, 0" false false 0.1 false))

(event EventPropulse
  (params (TargetLocation :type Vector :default "0, 0, 0") (PropulseLocation :type Vector :default "0, 0, 0") (TargetLocked? :type Boolean))
  (bind _cube (Variables|Default|GetCube))
  (if (Variables|Default|GetCanBeThrown)
    (if TargetLocked?
      (Components|MoveComponentTo _cube TargetLocation "0, 0, 0" false false 0.3 false)
      (Physics|SetEnableGravity (Variables|Default|GetCube) true)
      (else
        (Physics|SetPhysicsLinearVelocity _cube "0, 0, 0" false "None")
        (Physics|AddImpulse (Variables|Default|GetCube) (* PropulseLocation 3500) "None" true)
        (Physics|SetEnableGravity (Variables|Default|GetCube) true)))))

(event EventGrabObject
  (Variables|Default|SetCanBeThrown true)
  (Development|PrintString "Hello"))

(fn ConstructionScript)