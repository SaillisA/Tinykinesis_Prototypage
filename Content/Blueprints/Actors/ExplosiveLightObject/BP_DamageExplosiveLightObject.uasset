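; Damage variant of an explosive light object that kills enemy NPCs and emits a physical blast, built on parent-class logic.
; The construction script sizes the RadialForce component to ExplosionRadius.
; EffectOfEnnemy passes the NPC's MaxHP to its controller's HealthManager and, on a true result, triggers Death with the hit location.
; ExplosionEffect fires the radial impulse and plays a camera shake centered on the player rather than the blast.
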(event EventBeginPlay
  (|CallParentFunction) ; This node is disabled and will not be called.\nDrag off pins to build functionality.
)

(event Collision|EventActorBeginOverlap
  (params (OtherActor :type Actor%20Object%20Reference))
  (|CallParentFunction OtherActor) ; This node is disabled and will not be called.\nDrag off pins to build functionality.
)

(event EventTick
  (params (DeltaSeconds :type Float%20%28single-precision%29))
  (|CallParentFunction DeltaSeconds) ; This node is disabled and will not be called.\nDrag off pins to build functionality.
)

(fn ConstructionScript
  (|CallParentFunction)
  (Variables|/Script/Engine.RadialForceComponent|SetRadius (Variables|Default|GetRadialForce) (Variables|Default|GetExplosionRadius)))

(fn EffectOfEnnemy
  (params (EnnemyHit :type BP%20AI%20Character%20Blank%20Object%20Reference) (HitLocation :type Vector :default "0, 0, 0"))
  (bind _asaic_npc_base (Utilities|Casting|CastToAIC_NpcBase (Components|GetOwner EnnemyHit)))
  (bind _isdead (Default|ManageHP (Variables|/Game/Blueprints/NPC/AIBase/AIC_NpcBase.AIC_NpcBase_C|GetHealthManager _asaic_npc_base) (Variables|/Game/Blueprints/ActorComponents/BP_AC_HealthAI.BP_AC_HealthAI_C|GetmaxHP (Variables|/Game/Blueprints/NPC/AIBase/AIC_NpcBase.AIC_NpcBase_C|GetHealthManager _asaic_npc_base))))
  (if _isdead
    (Default|Death EnnemyHit _asaic_npc_base HitLocation 1.0 0.0)))

(fn ExplosionEffect
  (Class|RadialForceComponent|FireImpulse (Variables|Default|GetRadialForce))
  (bind _asbp_first_person_character (Utilities|Casting|CastToBP_FirstPersonCharacter (Game|GetPlayerCharacter 0)))
  (Camera|PlayWorldCameraShake "/Game/Blueprints/Actors/BP_CameraShake.BP_CameraShake_C" (Transformation|GetActorLocation _asbp_first_person_character) 0.0 5e+02))