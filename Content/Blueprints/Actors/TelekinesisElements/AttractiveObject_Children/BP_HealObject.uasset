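; BP_HealObject is a healing pickup, apparently a child of the telekinesis attractive object base.
; Overlapping its HitPlayerCollision passes the other actor to the inherited CollisionPickupObject logic.
; Its EffectOnPickup override calls the parent, plays the heal indicator animation and heals the player controller's health component by PowerAmount.
; The HealHP result then drives the HUD life bar update.
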(event OnComponentBeginOverlap(HitPlayerCollision)
  (params (OverlappedComponent :type Primitive%20Component%20Object%20Reference) (OtherActor :type Actor%20Object%20Reference) (OtherComp :type Primitive%20Component%20Object%20Reference) (OtherBodyIndex :type Integer) (bFromSweep :type Boolean) (SweepResult :type Hit%20Result%20Structure%20%28by%20ref%29))
  (CallFunction|CollisionPickupObject OtherActor))

(event EventBeginPlay
  (|CallParentFunction) ; This node is disabled and will not be called.\nDrag off pins to build functionality.
)

(event Collision|EventActorBeginOverlap
  (params (OtherActor :type Actor%20Object%20Reference))
  (|CallParentFunction OtherActor) ; This node is disabled and will not be called.\nDrag off pins to build functionality.
)

(event EventTick
  (params (DeltaSeconds :type Float%20%28single-precision%29))
  (|CallParentFunction DeltaSeconds) ; This node is disabled and will not be called.\nDrag off pins to build functionality.
)

(fn ConstructionScript
  (|CallParentFunction))

(fn EffectonPickup
  (bind _tinykinesisplayercontroller (CallFunction|GetTinykinesisPlayerController))
  (|CallParentFunction)
  (Default|LaunchAnimHealIndicator (Variables|/Game/Blueprints/Player/BP_TinykinesisPlayerController.BP_TinykinesisPlayerController_C|GetWBP_PickupIndicator _tinykinesisplayercontroller))
  (bind _actualhp (Default|HealHP (Variables|/Game/Blueprints/Player/BP_TinykinesisPlayerController.BP_TinykinesisPlayerController_C|GetBP_AC_Health _tinykinesisplayercontroller) (Variables|Default|GetPowerAmount)))
  (Default|UpdateHealthBarAnimRedBlink (Variables|/Game/Blueprints/WidgetBlueprints/HUD/WBP_PlayerHUD.WBP_PlayerHUD_C|GetWBP_PlayerLifeBar (Variables|/Game/Blueprints/Player/BP_TinykinesisPlayerController.BP_TinykinesisPlayerController_C|GetWBPPlayerHUD _tinykinesisplayercontroller)) _actualhp))