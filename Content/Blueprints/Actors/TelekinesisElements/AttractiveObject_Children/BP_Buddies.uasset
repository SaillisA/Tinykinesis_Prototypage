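; Collectible buddy NPC, a telekinesis-attractable object that counts toward the player's found buddies.
; A detection volume tracks the player and nearby mobs to pick its animation state, while an overlay outline material and Niagara effect highlight targeting.
; When grabbed it turns with the camera; on reaching the player, timelines scale and shake it before a poof and pickup.
; BPACStateGameplayElement handles activation and loading, and disables it in the save once collected.
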(event OnComponentBeginOverlap(DetectionPawn)
  (params (OverlappedComponent :type Primitive%20Component%20Object%20Reference) (OtherActor :type Actor%20Object%20Reference) (OtherComp :type Primitive%20Component%20Object%20Reference) (OtherBodyIndex :type Integer) (bFromSweep :type Boolean) (SweepResult :type Hit%20Result%20Structure%20%28by%20ref%29))
  (bind (_isplayernearby_ _ismobnearby_) (CallFunction|CheckPawnNearby OtherActor))
  (if _isplayernearby_
    (Variables|Default|SetPlayerNearby true)
    (CallFunction|SetCurrentAnim :!label _label)
    (elif _ismobnearby_
      (Math|Integer|IncrementInt (Variables|Default|GetNpcNearbyAmount)
        (:%20%20
          (goto _label))))))

(event OnComponentEndOverlap(DetectionPawn)
  (params (OverlappedComponent :type Primitive%20Component%20Object%20Reference) (OtherActor :type Actor%20Object%20Reference) (OtherComp :type Primitive%20Component%20Object%20Reference) (OtherBodyIndex :type Integer))
  (bind (_isplayernearby_ _ismobnearby_) (CallFunction|CheckPawnNearby OtherActor))
  (if _isplayernearby_
    (Variables|Default|SetPlayerNearby false)
    (CallFunction|SetCurrentAnim :!label _label)
    (elif _ismobnearby_
      (Math|Integer|DecrementInt (Variables|Default|GetNpcNearbyAmount)
        (:%20%20
          (goto _label))))))

(event OnComponentBeginOverlap(HitPlayerCollision)
  (params (OverlappedComponent :type Primitive%20Component%20Object%20Reference) (OtherActor :type Actor%20Object%20Reference) (OtherComp :type Primitive%20Component%20Object%20Reference) (OtherBodyIndex :type Integer) (bFromSweep :type Boolean) (SweepResult :type Hit%20Result%20Structure%20%28by%20ref%29))
  (bind _explodebuddy (Variables|Default|GetExplodeBuddy))
  (if (and (== OtherActor (CallFunction|GetTinykinesisPlayerCharacter)) (== (Variables|/Game/Blueprints/ActorComponents/PlayerAbilities/BP_AC_Telekinesis.BP_AC_Telekinesis_C|GetItemGrabbed (Variables|/Game/Blueprints/Player/BP_TinykinesisPlayerController.BP_TinykinesisPlayerController_C|GetBP_AC_Telekinesis (CallFunction|GetTinykinesisPlayerController))) self))
    (Variables|Default|SetIsExploding true)
    (Variables|Default|SetInititalRotation (Transformation|GetWorldRotation (Variables|Default|GetSkeletalMeshNpc)))
    (Components|Timeline|SetTimelineLength _explodebuddy 2.0)
    (Components|Timeline|PlayfromStart _explodebuddy)))

(event Custom|Update_ExplodeBuddy
  (bind _explodebuddy (Variables|Default|GetExplodeBuddy))
  (Transformation|SetRelativeScale3D (Variables|Default|GetSkeletalMeshNpc) (Math|Conversions|ToVector(Float) (CallFunction|TLCurve "/Game/Miscellaneous/Curves/C_ExploseBuddy.C_ExploseBuddy" _explodebuddy)))
  (Transformation|SetWorldRotation (Variables|Default|GetSkeletalMeshNpc) (Math|Rotator|MakeRotator 0.0 (.pitch (Math|Rotator|CombineRotators (Variables|Default|GetInititalRotation) (Math|Rotator|MakeRotator 0.0 (CallFunction|TLCurve "/Game/Miscellaneous/Curves/C_Shake.C_Shake" _explodebuddy) 0.0))) (+ (.yaw (Transformation|GetWorldRotation (Variables|/Script/Tinykinesis_Proto.Tinykinesis_ProtoCharacter|GetFirstPersonCameraComponent (CallFunction|GetTinykinesisPlayerCharacter)))) 1.1e+02)) false false))

(event Custom|Finished_ExplodeBuddy
  (bind _skeletalmeshnpc (Variables|Default|GetSkeletalMeshNpc))
  (Niagara|SpawnSystematLocation "/Game/VFX/Mobs/PoofEffect/NS_BuddyPoofExplosionDeath.NS_BuddyPoofExplosionDeath" (Transformation|GetWorldLocation _skeletalmeshnpc) (Transformation|GetWorldRotation _skeletalmeshnpc))
  (CallFunction|CollisionPickupObject (CallFunction|GetTinykinesisPlayerCharacter) (Variables|Default|GetSkeletalMeshNpc)))

(event Custom|LoadCollectibleNpc
  (bind _bp_ac_stategameplayelement (Variables|Default|GetBP_AC_StateGameplayElement))
  ;[0.298 1 0.5765] BeginPlay
  (Default|LoadElement _bp_ac_stategameplayelement (Variables|/Game/Blueprints/ActorComponents/BP_AC_StateGameplayElement.BP_AC_StateGameplayElement_C|GetIsActivated _bp_ac_stategameplayelement) self))

(event EventBeginPlay
  (bind _bp_ac_stategameplayelement (Variables|Default|GetBP_AC_StateGameplayElement))
  ;[0.298 1 0.5765] BeginPlay
  (EventDispatchers|BindEventtoBeginPlayActiveElement _bp_ac_stategameplayelement (EventDispatchers|CreateEvent :!event BeginPlayTelekinesisElement))
  (Default|LaunchBeginPlay _bp_ac_stategameplayelement))

(event EventFeedbacksDetectObject
  (Components|Activation|Activate (Variables|Default|GetNS_TelekinesisSelection) false)
  (CallFunction|SetMaterialInstanceBuddy (Variables|Default|GetColorMaterialInstance))
  (Default|CallFeedbacksEventDispatcher))

(event EventTick
  (params (DeltaSeconds :type Float%20%28single-precision%29))
  (bind _skeletalmeshnpc (Variables|Default|GetSkeletalMeshNpc))
  (if (Variables|Default|GetIsBeingGrabbed)
    ;[1 1 1] Attract in real time
    (CallFunction|GrabLight)
    (if (not (Variables|Default|GetIsExploding))
      (Utilities|IsValid _skeletalmeshnpc
        (:Is%20Valid
          ;[1 1 1] Rotate the projectile for flavor purpose
          (Transformation|SetWorldRotation _skeletalmeshnpc (Math|Rotator|MakeRotator 0.0 0.0 (+ (.yaw (Transformation|GetWorldRotation (Variables|/Script/Tinykinesis_Proto.Tinykinesis_ProtoCharacter|GetFirstPersonCameraComponent (CallFunction|GetTinykinesisPlayerCharacter)))) 1.1e+02)) false false))))))

(event EventDeleteFeedbacksDetectObject
  (Components|Activation|Deactivate (Variables|Default|GetNS_TelekinesisSelection))
  (CallFunction|SetMaterialInstanceBuddy)
  (Default|CallDeleteFeedbacksEventDispatcher))

(event EventGetRepulsedWave
  (params (ForceRepulse :type Float%20%28double-precision%29) (HitLocation :type Vector :default "0, 0, 0"))
  ;[1 1 1] Override events, because it's a character
)

(event EventGetHitTelekinesisElement
  (params (CanDamage :type Boolean) (DamageObject :type Float%20%28double-precision%29))
  (CallFunction|SetBuddyAnimationState "NewEnumerator4")
  (Utilities|FlowControl|Delay 0.2)
  (CallFunction|SetCurrentAnim))

(event EventSetActive
  (params (IsActive :type Boolean))
  (bind _bp_ac_stategameplayelement (Variables|Default|GetBP_AC_StateGameplayElement))
  ;[0.298 1 0.5765] BeginPlay
  (EventDispatchers|BindEventtoSetActiveElementEventDispatcher _bp_ac_stategameplayelement (EventDispatchers|CreateEvent :!event Custom|LoadCollectibleNpc))
  (EventDispatchers|BindEventtoBeginPlayActiveElement _bp_ac_stategameplayelement (EventDispatchers|CreateEvent :!event BeginPlayTelekinesisElement))
  (Default|SetActiveElement (Variables|Default|GetBP_AC_StateGameplayElement) IsActive))

(event EventGrabLight
  (bind _rotatebuddy (Variables|Default|GetRotateBuddy))
  (|CallParentFunction)
  (CallFunction|SetBuddyAnimationState "NewEnumerator1")
  (Components|Timeline|SetTimelineLength _rotatebuddy 0.5)
  (Components|Timeline|PlayfromStart _rotatebuddy))

(fn ConstructionScript
  (|CallParentFunction)
  (CallFunction|SetBuddyMaterial))

(fn CheckPawnNearby
  (params (ActorCollision :type Object%20Object%20Reference))
  (if (Utilities|DoesObjectImplementInterface ActorCollision "/Game/Blueprints/Interfaces/BPI_Target.BPI_Target_C")
    (return false true)
    (elif (== ActorCollision (CallFunction|GetTinykinesisPlayerCharacter))
      (return true false))))

(fn SetCurrentAnim
  (if (< (Variables|Default|GetNpcNearbyAmount) 1)
    (if (Variables|Default|GetPlayerNearby)
      (CallFunction|SetBuddyAnimationState "NewEnumerator2")
      (else
        (CallFunction|SetBuddyAnimationState "NewEnumerator1")))
    (else
      (CallFunction|SetBuddyAnimationState "NewEnumerator0"))))

(fn EffectonPickup
  (|CallParentFunction)
  (Default|DisableinSave (Variables|Default|GetBP_AC_StateGameplayElement))
  (Default|IncrementBuddiesFounded (CallFunction|GetTinykinesisPlayerController)))

(fn SetBuddyAnimationState
  (params (AnimationBuddy :type E_Buddies_AnimationStates%20Enum :default "NewEnumerator1"))
  (bind _asabp_buddies (Utilities|Casting|CastToABP_Buddies (Components|SkeletalMesh|GetAnimInstance (Variables|Default|GetSkeletalMeshNpc))))
  (Variables|/Game/Characters/Buddies/Animations/ABP_Buddies.ABP_Buddies_C|SetAnimationBuddy _asabp_buddies AnimationBuddy))

(fn SetMaterialInstanceBuddy
  (params (Value :type Linear%20Color%20Structure))
  (Rendering|Material|SetVectorParameterValue (Variables|Default|GetMaterialInstanceBuddy) "Color" Value :!class /Script/Engine.MaterialInstanceDynamic))

(fn SetBuddyMaterial
  (Rendering|Material|SetMaterial (Variables|Default|GetSkeletalMeshNpc) 0 (Variables|/Game/Blueprints/Actors/TelekinesisElements/DataAssets/PDA_TelekinesisElement.PDA_TelekinesisElement_C|GetMaterialInstance (Variables|Default|GetDataAsset)))
  (bind _returnvalue (Rendering|Material|CreateDynamicMaterialInstance (Variables|Default|GetSkeletalMeshNpc) 1 "/Game/Materials/MI_OutlineTarget_BeforeGrab.MI_OutlineTarget_BeforeGrab" "None" :!class /Script/Engine.PrimitiveComponent))
  (bind _output_get (Variables|Default|SetMaterialInstanceBuddy _returnvalue))
  (Rendering|Material|SetOverlayMaterial (Variables|Default|GetSkeletalMeshNpc) _output_get :!class /Script/Engine.MeshComponent)
  (CallFunction|DeleteFeedbacksDetectObject))