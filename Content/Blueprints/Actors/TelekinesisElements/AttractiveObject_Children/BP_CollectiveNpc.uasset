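; BP_CollectiveNpc is a collectible NPC character built as an AttractiveObject child, which can be grabbed, hit by telekinesis and picked up on player contact.
; A detection volume tracks player presence and counts nearby BPI_Target mobs to choose its animation state, with mobs taking priority.
; Grab and hit events override that state, the hit one briefly.
; BPACStateGameplayElement handles activation and loading, and disables the NPC in the save on pickup.
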(event OnComponentBeginOverlap(DetectionPawn)
  (params (OverlappedComponent :type Primitive%20Component%20Object%20Reference) (OtherActor :type Actor%20Object%20Reference) (OtherComp :type Primitive%20Component%20Object%20Reference) (OtherBodyIndex :type Integer) (bFromSweep :type Boolean) (SweepResult :type Hit%20Result%20Structure%20%28by%20ref%29))
  (bind (_isplayernearby_ _ismobnearby_) (CallFunction|CheckPawnNearby OtherActor))
  (if _isplayernearby_
    (Variables|Default|SetPlayerNearby true)
    (CallFunction|SetCurrentAnim :!label _label)
    (elif _ismobnearby_
      (Math|Integer|IncrementInt (Variables|Default|GetNpcNearbyAmount)
        (:%20%20
          (goto _label))))))

(event OnComponentEndOverlap(DetectionPawn)
  (params (OverlappedComponent :type Primitive%20Component%20Object%20Reference) (OtherActor :type Actor%20Object%20Reference) (OtherComp :type Primitive%20Component%20Object%20Reference) (OtherBodyIndex :type Integer))
  (bind (_isplayernearby_ _ismobnearby_) (CallFunction|CheckPawnNearby OtherActor))
  (if _isplayernearby_
    (Variables|Default|SetPlayerNearby false)
    (CallFunction|SetCurrentAnim :!label _label)
    (elif _ismobnearby_
      (Math|Integer|DecrementInt (Variables|Default|GetNpcNearbyAmount)
        (:%20%20
          (goto _label))))))

(event OnComponentBeginOverlap(HitPlayerCollision)
  (params (OverlappedComponent :type Primitive%20Component%20Object%20Reference) (OtherActor :type Actor%20Object%20Reference) (OtherComp :type Primitive%20Component%20Object%20Reference) (OtherBodyIndex :type Integer) (bFromSweep :type Boolean) (SweepResult :type Hit%20Result%20Structure%20%28by%20ref%29))
  (if (== OtherActor (CallFunction|GetTinykinesisPlayerCharacter))
    (CallFunction|CollisionPickupObject OtherActor)))

(event Custom|LoadCollectibleNpc
  (bind _bp_ac_stategameplayelement (Variables|Default|GetBP_AC_StateGameplayElement))
  ;[0.298 1 0.5765] BeginPlay
  (Default|LoadElement _bp_ac_stategameplayelement (Variables|/Game/Blueprints/ActorComponents/BP_AC_StateGameplayElement.BP_AC_StateGameplayElement_C|GetIsActivated _bp_ac_stategameplayelement) self))

(event EventBeginPlay
  (bind _bp_ac_stategameplayelement (Variables|Default|GetBP_AC_StateGameplayElement))
  ;[0.298 1 0.5765] BeginPlay
  (EventDispatchers|BindEventtoBeginPlayActiveElement _bp_ac_stategameplayelement (EventDispatchers|CreateEvent :!event BeginPlayTelekinesisElement))
  (Default|LaunchBeginPlay _bp_ac_stategameplayelement))

(event EventTick
  (params (DeltaSeconds :type Float%20%28single-precision%29))
  (|CallParentFunction DeltaSeconds) ; This node is disabled and will not be called.\nDrag off pins to build functionality.
)

(event EventGrabLight
  (|CallParentFunction)
  (Variables|Default|SetAnimationState "NewEnumerator3"))

(event EventGetRepulsedWave
  (params (ForceRepulse :type Float%20%28double-precision%29) (HitLocation :type Vector :default "0, 0, 0"))
  ;[1 1 1] Override events, because it's a character
)

(event EventGetHitTelekinesisElement
  (params (CanDamage :type Boolean) (DamageObject :type Float%20%28double-precision%29))
  (Variables|Default|SetAnimationState "NewEnumerator4")
  (Utilities|FlowControl|Delay 0.2)
  (Variables|Default|SetAnimationState "NewEnumerator1"))

(event Collision|EventActorBeginOverlap
  (params (OtherActor :type Actor%20Object%20Reference)))

(event EventSetActive
  (params (IsActive :type Boolean))
  (bind _bp_ac_stategameplayelement (Variables|Default|GetBP_AC_StateGameplayElement))
  ;[0.298 1 0.5765] BeginPlay
  (EventDispatchers|BindEventtoSetActiveElementEventDispatcher _bp_ac_stategameplayelement (EventDispatchers|CreateEvent :!event Custom|LoadCollectibleNpc))
  (EventDispatchers|BindEventtoBeginPlayActiveElement _bp_ac_stategameplayelement (EventDispatchers|CreateEvent :!event BeginPlayTelekinesisElement))
  (Default|SetActiveElement (Variables|Default|GetBP_AC_StateGameplayElement) IsActive))

(fn ConstructionScript
  (|CallParentFunction)
  (Utilities|FlowControl|Sequence
    (:then_0
      (if (Utilities|Enum|Equal(Enum) (Variables|/Game/Blueprints/Actors/TelekinesisElements/DataAssets/PDA_TelekinesisElement.PDA_TelekinesisElement_C|GetName (Variables|Default|GetDataAsset)) "TheRightName")
        (Components|SkeletalMesh|SetSkeletalMeshAsset (Variables|Default|GetSkeletalMeshNpc) 0)))))

(fn CheckPawnNearby
  (params (ActorCollision :type Object%20Object%20Reference))
  (if (Utilities|DoesObjectImplementInterface ActorCollision "/Game/Blueprints/Interfaces/BPI_Target.BPI_Target_C")
    (return false true)
    (elif (== ActorCollision (CallFunction|GetTinykinesisPlayerCharacter))
      (return true false))))

(fn SetCurrentAnim
  (if (< (Variables|Default|GetNpcNearbyAmount) 1)
    (if (Variables|Default|GetPlayerNearby)
      (Variables|Default|SetAnimationState "NewEnumerator2")
      (else
        (Variables|Default|SetAnimationState "NewEnumerator1")))
    (else
      (Variables|Default|SetAnimationState "NewEnumerator0"))))

(fn EffectonPickup
  (|CallParentFunction)
  (Default|DisableinSave (Variables|Default|GetBP_AC_StateGameplayElement)))