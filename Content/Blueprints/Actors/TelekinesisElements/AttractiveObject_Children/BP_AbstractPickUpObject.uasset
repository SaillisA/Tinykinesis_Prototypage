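; Abstract base for telekinesis-attractable pickups, a child of the attractive object class that disables the inherited charge, release, hit and damage-range events because it is not a projectile.
; When the player overlaps its hit collision, it runs an empty EffectOnPickup hook, clears telekinesis and animation state if currently grabbed, stops its attraction audio and destroys itself.
; EffectOnGrab sets the hit sphere to a dedicated grab radius.
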(event OnComponentBeginOverlap(HitPlayerCollision)
  (params (OverlappedComponent :type Primitive%20Component%20Object%20Reference) (OtherActor :type Actor%20Object%20Reference) (OtherComp :type Primitive%20Component%20Object%20Reference) (OtherBodyIndex :type Integer) (bFromSweep :type Boolean) (SweepResult :type Hit%20Result%20Structure%20%28by%20ref%29))
  ;[1 0.2696 0.3095] Collisions
  (if (== OtherActor (CallFunction|GetTinykinesisPlayerCharacter))
    (CallFunction|EffectonPickup)
    (Utilities|FlowControl|Sequence
      (:then_0
        (if (== (Variables|/Game/Blueprints/ActorComponents/PlayerAbilities/BP_AC_Telekinesis.BP_AC_Telekinesis_C|GetItemGrabbed (Variables|/Game/Blueprints/Player/BP_TinykinesisPlayerController.BP_TinykinesisPlayerController_C|GetBP_AC_Telekinesis (CallFunction|GetTinykinesisPlayerController))) self)
          (Default|ClearParameters (Variables|/Game/Blueprints/Player/BP_TinykinesisPlayerController.BP_TinykinesisPlayerController_C|GetBP_AC_Telekinesis (CallFunction|GetTinykinesisPlayerController)))
          (Default|ObjectAnimation (CallFunction|GetTinykinesisPlayerCharacter) "NewEnumerator3")
          (Default|SetPlayerAnimTelekinesisState (CallFunction|GetTinykinesisPlayerCharacter) "NewEnumerator6")))
      (:then_1
        (Class|FMODBlueprintStatics|EventInstanceStop (Variables|/Game/Blueprints/ActorComponents/BP_AC_AttractionElement.BP_AC_AttractionElement_C|GetAudioInstance (Variables|Default|GetBP_AC_AttractionElement)) false)
        (Actor|DestroyActor)))))

(event OnComponentBeginOverlap(DamageRangeCollision)
  (params (OverlappedComponent :type Primitive%20Component%20Object%20Reference) (OtherActor :type Actor%20Object%20Reference) (OtherComp :type Primitive%20Component%20Object%20Reference) (OtherBodyIndex :type Integer) (bFromSweep :type Boolean) (SweepResult :type Hit%20Result%20Structure%20%28by%20ref%29))
  ;[1 1 1] Override all events, because it's not a projectile
)

(event EventBeginPlay
  (|CallParentFunction))

(event EventTick
  (params (DeltaSeconds :type Float%20%28single-precision%29))
  (|CallParentFunction DeltaSeconds))

(event EventReleaseObject
  ;[1 1 1] Override all events, because it's not a projectile
)

(event EventChargeObject
  ;[1 1 1] Override all events, because it's not a projectile
)

(event Collision|EventHit
  (params (MyComp :type Primitive%20Component%20Object%20Reference) (Other :type Actor%20Object%20Reference) (OtherComp :type Primitive%20Component%20Object%20Reference) (bSelfMoved :type Boolean) (HitLocation :type Vector :default "0, 0, 0") (HitNormal :type Vector :default "0, 0, 0") (NormalImpulse :type Vector :default "0, 0, 0") (Hit :type Hit%20Result%20Structure%20%28by%20ref%29))
  ;[1 1 1] Override all events, because it's not a projectile
)

(fn ConstructionScript
  (|CallParentFunction))

(fn EffectonPickup)

(fn EffectonGrab
  (Utilities|IsValid (Variables|Default|GetHitPlayerCollision)
    (:Is%20Valid
      (Components|Sphere|SetSphereRadius (Variables|Default|GetHitPlayerCollision) (Variables|Default|GetSphereRangeOnGrab) true))))