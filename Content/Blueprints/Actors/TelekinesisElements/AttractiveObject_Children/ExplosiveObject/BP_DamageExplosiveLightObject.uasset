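; A light explosive telekinesis object that deals lethal damage to melee NPCs it affects.
; Construction sizes the radial force to the explosion radius and sets a fixed knockback force.
; The enemy effect removes the NPC's full max HP through the HealthManager of its melee AI controller.
; The explosion effect fires the radial impulse and plays a camera shake centered on the player rather than the blast.
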(event EventBeginPlay
  (|CallParentFunction) ; This node is disabled and will not be called.\nDrag off pins to build functionality.
)

(event Collision|EventActorBeginOverlap
  (params (OtherActor :type Actor%20Object%20Reference))
  (|CallParentFunction OtherActor) ; This node is disabled and will not be called.\nDrag off pins to build functionality.
)

(event EventTick
  (params (DeltaSeconds :type Float%20%28single-precision%29))
  (|CallParentFunction DeltaSeconds) ; This node is disabled and will not be called.\nDrag off pins to build functionality.
)

(fn ConstructionScript
  (|CallParentFunction)
  (Variables|/Script/Engine.RadialForceComponent|SetRadius (Variables|Default|GetRadialForce) (Variables|Default|GetExplosionRadius))
  (Variables|Default|SetCurrentForceKnockback "12000.000000,12000.000000,15000.000000"))

(fn EffectonEnnemy
  (params (EnnemyHit :type BP%20AI%20Character%20Blank%20Object%20Reference) (HitLocation :type Vector :default "0, 0, 0"))
  (bind _asbp_aic_npc_melee (Utilities|Casting|CastToBP_AIC_NpcMelee (Components|GetOwner EnnemyHit)))
  (bind _isdead (Default|LooseHP (Variables|/Game/Blueprints/NPC/AIDefault/BP_AIC_NpcMelee.BP_AIC_NpcMelee_C|GetHealthManager _asbp_aic_npc_melee) (Variables|/Game/Blueprints/ActorComponents/BP_AC_Health.BP_AC_Health_C|GetmaxHP (Variables|/Game/Blueprints/NPC/AIDefault/BP_AIC_NpcMelee.BP_AIC_NpcMelee_C|GetHealthManager _asbp_aic_npc_melee))))
  (if _isdead
    _))

(fn ExplosionSpecialEffect
  (Class|RadialForceComponent|FireImpulse (Variables|Default|GetRadialForce))
  (bind _asbp_tinykinesis_player_character (Utilities|Casting|CastToBP_TinykinesisPlayerCharacter (Game|GetPlayerCharacter 0)))
  (Camera|PlayWorldCameraShake "/Game/Blueprints/Actors/CameraManager/BP_CameraShake.BP_CameraShake_C" (Transformation|GetActorLocation _asbp_tinykinesis_player_character) 0.0 5e+02))