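; Bait variant of the explosive telekinesis light object that lures AI characters.
; When an AI character enters its damage range collision, it calls GetBaited on that character with the hit position and prints a debug string.
; Its explosion feedback consists only of a camera shake centered on the player character.
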(event OnComponentBeginOverlap(DamageRangeCollision)
  (params (OverlappedComponent :type Primitive%20Component%20Object%20Reference) (OtherActor :type Actor%20Object%20Reference) (OtherComp :type Primitive%20Component%20Object%20Reference) (OtherBodyIndex :type Integer) (bFromSweep :type Boolean) (SweepResult :type Hit%20Result%20Structure%20%28by%20ref%29))
  (bind _asbp_aicharacter_blank (Utilities|Casting|CastToBP_AICharacterBlank OtherActor))
  (Default|GetBaited _asbp_aicharacter_blank 0 (Variables|Default|GetVectorHit))
  (Development|PrintString "BAIT"))

(event EventBeginPlay
  (|CallParentFunction) ; This node is disabled and will not be called.\nDrag off pins to build functionality.
)

(event Collision|EventActorBeginOverlap
  (params (OtherActor :type Actor%20Object%20Reference))
  (|CallParentFunction OtherActor) ; This node is disabled and will not be called.\nDrag off pins to build functionality.
)

(event EventTick
  (params (DeltaSeconds :type Float%20%28single-precision%29))
  (|CallParentFunction DeltaSeconds) ; This node is disabled and will not be called.\nDrag off pins to build functionality.
)

(fn ConstructionScript)

(fn ExplosionFeedbacks
  ;[1 1 1] Juste ça à avoir
  (Camera|PlayWorldCameraShake "/Game/Blueprints/Actors/CameraManager/BP_CameraShake.BP_CameraShake_C" (Transformation|GetActorLocation (CallFunction|GetTinykinesisPlayerCharacter)) 0.0 5e+02))