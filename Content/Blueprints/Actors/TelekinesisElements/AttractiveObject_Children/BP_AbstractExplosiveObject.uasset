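; Base Blueprint for explosive telekinesis objects, extending the attractive object parent.
; Hitting or being hit, via bound dispatchers, spawns a scaled Niagara impact and calls ExplosionFeedbacks, empty here.
; Poison and bait types then set IsDestroyed, so Tick skips parent logic and counts down CurrentDelayReinitialize before destroying the actor.
; A sphere previews ExplosionRadius from the construction script and is removed at BeginPlay.
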(event Custom|Hit_ExplosiveElement
  (params (HitActor :type Actor%20Object%20Reference))
  (bind _dataasset (Variables|Default|GetDataAsset))
  (bind _mesh (Variables|Character|GetMesh))
  (bind _returnvalue (Transformation|GetWorldTransform _mesh))
  (bind _objecttype (Variables|/Game/Blueprints/Actors/TelekinesisElements/DataAssets/PDA_TelekinesisElement.PDA_TelekinesisElement_C|GetObjectType _dataasset))
  ;[1 1 1] Hit_Explosive
  ;;[1 0.2706 0.3098] Collisions
  (bind _returnvalue_2 (Niagara|SpawnSystematLocation (Variables|Default|GetFXatImpact) (.location _returnvalue) (.rotation _returnvalue) (.scale _returnvalue)))
  (Niagara|SetNiagaraVariable(Float) _returnvalue_2 "ScaleMultiplier" 2.0)
  (CallFunction|ExplosionFeedbacks)
  (if (or (== _objecttype "PoisonObject") (== _objecttype "BaitObject"))
    (Variables|Default|SetIsDestroyed true)))

(event Custom|GetHit_ExplosiveElement
  (bind _dataasset (Variables|Default|GetDataAsset))
  (bind _mesh (Variables|Character|GetMesh))
  (bind _returnvalue (Transformation|GetWorldTransform _mesh))
  (bind _objecttype (Variables|/Game/Blueprints/Actors/TelekinesisElements/DataAssets/PDA_TelekinesisElement.PDA_TelekinesisElement_C|GetObjectType _dataasset))
  ;[1 1 1] Hit_Explosive
  ;;[1 0.2706 0.3098] Collisions
  (bind _returnvalue_2 (Niagara|SpawnSystematLocation (Variables|Default|GetFXatImpact) (.location _returnvalue) (.rotation _returnvalue) (.scale _returnvalue)))
  (Niagara|SetNiagaraVariable(Float) _returnvalue_2 "ScaleMultiplier" 2.0)
  (CallFunction|ExplosionFeedbacks)
  (if (or (== _objecttype "PoisonObject") (== _objecttype "BaitObject"))
    (Variables|Default|SetIsDestroyed true)))

(event EventBeginPlay
  (|CallParentFunction)
  (EventDispatchers|BindEventtoHitEventDispatcher (EventDispatchers|CreateEvent :!event Custom|Hit_ExplosiveElement))
  (EventDispatchers|BindEventtoGetHitEventDispatcher (EventDispatchers|CreateEvent :!event Custom|GetHit_ExplosiveElement))
  (Components|DestroyComponent (Variables|Default|GetExplosionRadius_Visual)))

(event EventTick
  (params (DeltaSeconds :type Float%20%28single-precision%29))
  (if (Variables|Default|GetIsDestroyed)
    (bind _output_get (Variables|Default|SetCurrentDelayReinitialize (- (Variables|Default|GetCurrentDelayReinitialize) (Utilities|Time|GetWorldDeltaSeconds))))
    (if (<= _output_get 0.0)
      (Actor|DestroyActor))
    (else
      (|CallParentFunction 0.0))))

(fn ConstructionScript
  (|CallParentFunction)
  (Components|Sphere|SetSphereRadius (Variables|Default|GetExplosionRadius_Visual) (Variables|Default|GetExplosionRadius) false))

(fn ExplosionFeedbacks)