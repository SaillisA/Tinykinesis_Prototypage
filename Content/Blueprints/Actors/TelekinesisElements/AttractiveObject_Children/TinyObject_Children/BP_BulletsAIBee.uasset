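; Bullet fired by an AI bee, built as a tiny telekinesis object that can be grabbed.
; It starts flagged as a mob projectile and destroys itself if not grabbed within a short delay after spawn.
; The first light grab clears that flag and marks it as grabbed, cancelling the timed death.
; Until grabbed it ignores hits on its owning bee, while other hits go to the parent logic.
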(event EventBeginPlay
  ;[0.298 1 0.5765] Begin Play
  (|CallParentFunction)
  (EventDispatchers|UnbindallEventsfromGrabEventDispatcher)
  (EventDispatchers|BindEventtoGrabEventDispatcher (EventDispatchers|CreateEvent :!event GrabLight))
  (Variables|Default|SetIsMobProjectile true)
  (Utilities|FlowControl|Delay 1e+01)
  (if (not (Variables|Default|GetHasBeenGrabbed))
    (CallFunction|DeathTelekinesisElement)))

(event EventGrabLight
  (Utilities|FlowControl|Sequence
    (:then_0
      (Utilities|FlowControl|DoOnce false
        (:Completed
          (Variables|Default|SetHasBeenGrabbed true)
          (Variables|Default|SetIsMobProjectile false))))
    (:then_1
      (|CallParentFunction))))

(event Collision|EventHit
  (params (MyComp :type Primitive%20Component%20Object%20Reference) (Other :type Actor%20Object%20Reference) (OtherComp :type Primitive%20Component%20Object%20Reference) (bSelfMoved :type Boolean) (HitLocation :type Vector :default "0, 0, 0") (HitNormal :type Vector :default "0, 0, 0") (NormalImpulse :type Vector :default "0, 0, 0") (Hit :type Hit%20Result%20Structure%20%28by%20ref%29))
  ;[1 0.2706 0.3098] Hit NCP
  (if (Variables|Default|GetHasBeenGrabbed)
    (|CallParentFunction MyComp Other OtherComp bSelfMoved HitLocation HitNormal NormalImpulse Hit :!label _label)
    (elif (!= Other (Variables|Default|GetBeeOwner))
      (goto _label))))

(fn ConstructionScript)