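; BP_BulletsAIDistance is a tiny telekinesis object that acts as a ranged AI bullet, damaging the player unless grabbed.
; It rebinds the grab dispatcher on spawn and self-destroys after ten seconds if never grabbed.
; Ungrabbed hits damage and knock back the player character on contact and launch destruction on any impact.
; The first grab sets new damage and knockback values and hands later hits to the parent's logic.
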(event EventBeginPlay
  ;[0.298 1 0.5765] Begin Play
  (|CallParentFunction)
  (EventDispatchers|UnbindallEventsfromGrabEventDispatcher)
  (EventDispatchers|BindEventtoGrabEventDispatcher (EventDispatchers|CreateEvent :!event GrabLight))
  (Utilities|FlowControl|Delay 1e+01)
  (if (not (Variables|Default|GetHasBeenGrabbed))
    (Actor|DestroyActor)))

(event EventGrabLight
  (Utilities|FlowControl|DoOnce false
    (:Completed
      (Variables|Default|SetHasBeenGrabbed true)
      (Variables|Default|SetCurrentDamageObject 1e+02)
      (Variables|Default|SetCurrentForceKnockback "5000.000000,5000.000000,5000.000000"))))

(event EventHit
  (params (MyComp :type Primitive%20Component%20Object%20Reference) (Other :type Actor%20Object%20Reference) (OtherComp :type Primitive%20Component%20Object%20Reference) (bSelfMoved :type Boolean) (HitLocation :type Vector :default "0, 0, 0") (HitNormal :type Vector :default "0, 0, 0") (NormalImpulse :type Vector :default "0, 0, 0") (Hit :type Hit%20Result%20Structure%20%28by%20ref%29))
  ;[1 0.2706 0.3098] Hit NCP
  (if (Variables|Default|GetHasBeenGrabbed)
    (|CallParentFunction MyComp Other OtherComp bSelfMoved HitLocation HitNormal NormalImpulse Hit)
    (else
      (bind _asbp_tinykinesis_player_character (Utilities|Casting|CastToBP_TinykinesisPlayerCharacter Other)
        (:then
          (Default|EventGetHit _asbp_tinykinesis_player_character (Transformation|GetActorLocation) (Variables|Default|GetCurrentForceKnockback) (Variables|Default|GetCurrentDamageObject)))
        (:CastFailed
          _))
      (Default|LaunchDestruction (Variables|Default|GetBP_AC_DestructionElement) (Transformation|GetRelativeTransform (Variables|Character|GetMesh)) 0.0 self))))

(fn ConstructionScript)