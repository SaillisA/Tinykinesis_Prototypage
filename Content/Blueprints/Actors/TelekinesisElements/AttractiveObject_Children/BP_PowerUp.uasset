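; Collectible power-up, a child actor in the telekinesis elements, that grants double jump, dash, repulse, freeze time or the final area key.
; PowerUpType selects the mesh on BeginPlay (key or upgrade ticket) and the effect on pickup, which calls the matching player controller component or sets HasFoundKey.
; Player overlap with HitPlayer applies the effect, stops audio, disables the element in the save, triggers a level manager save and destroys the actor.
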(event OnComponentBeginOverlap(HitPlayer)
  (params (OverlappedComponent :type Primitive%20Component%20Object%20Reference) (OtherActor :type Actor%20Object%20Reference) (OtherComp :type Primitive%20Component%20Object%20Reference) (OtherBodyIndex :type Integer) (bFromSweep :type Boolean) (SweepResult :type Hit%20Result%20Structure%20%28by%20ref%29))
  (if (== OtherActor (CallFunction|GetTinykinesisPlayerCharacter))
    (CallFunction|EffectonPickup)
    (Class|FMODBlueprintStatics|EventInstanceStop (Variables|Default|GetAudioInstance) false)
    (Default|DisableinSave (Variables|Default|GetBP_AC_StateGameplayElement))
    (Utilities|FlowControl|Sequence
      (:then_0
        (bind _returnvalue (Actor|GetActorOfClass "/Game/Blueprints/SaveSystem/BP_AbstractLevelManager.BP_AbstractLevelManager_C"))
        (Utilities|IsValid _returnvalue
          (:Is%20Valid
            (Default|TriggerSaveGame _returnvalue (Transformation|GetActorTransform (CallFunction|GetTinykinesisPlayerController))))))
      (:then_1
        (Actor|DestroyActor)))))

(event EventBeginPlay
  (CallFunction|SetMesh))

(event Collision|EventActorBeginOverlap
  (params (OtherActor :type Actor%20Object%20Reference))
  (|CallParentFunction OtherActor) ; This node is disabled and will not be called.\nDrag off pins to build functionality.
)

(event EventTick
  (params (DeltaSeconds :type Float%20%28single-precision%29))
  (|CallParentFunction DeltaSeconds) ; This node is disabled and will not be called.\nDrag off pins to build functionality.
)

(fn ConstructionScript
  (|CallParentFunction))

(fn EffectonPickup
  (bind _tinykinesisplayercontroller (CallFunction|GetTinykinesisPlayerController))
  (switch Utilities|FlowControl|Switch|SwitchonE_PowerUps (Variables|Default|GetPowerUpType)
    (:NewEnumerator0
      (Default|PowerUpDoubleJump (Variables|/Game/Blueprints/Player/BP_TinykinesisPlayerController.BP_TinykinesisPlayerController_C|GetBP_AC_Jump _tinykinesisplayercontroller)))
    (:NewEnumerator1
      (Default|PowerUpDash (Variables|/Game/Blueprints/Player/BP_TinykinesisPlayerController.BP_TinykinesisPlayerController_C|GetBP_AC_Dash _tinykinesisplayercontroller)))
    (:NewEnumerator2
      (Default|PowerUpRepulse (Variables|/Game/Blueprints/Player/BP_TinykinesisPlayerController.BP_TinykinesisPlayerController_C|GetBP_AC_Repulse _tinykinesisplayercontroller)))
    (:NewEnumerator3
      (Default|PowerUpFreezeTime (Variables|/Game/Blueprints/Player/BP_TinykinesisPlayerController.BP_TinykinesisPlayerController_C|GetBP_AC_FreezeTime _tinykinesisplayercontroller)))
    (:NewEnumerator4
      (Variables|/Game/Blueprints/Player/BP_TinykinesisPlayerController.BP_TinykinesisPlayerController_C|SetHasFoundKey _tinykinesisplayercontroller true))))

(fn SetMesh
  (switch Utilities|FlowControl|Switch|SwitchonE_PowerUps (Variables|Default|GetPowerUpType)
    (:NewEnumerator0
      (Components|StaticMesh|SetStaticMesh (Variables|Default|GetStaticMesh) "/Game/StaticMeshes/SM_TicketUpgrade_001.SM_TicketUpgrade_001"))
    (:NewEnumerator1
      (Components|StaticMesh|SetStaticMesh (Variables|Default|GetStaticMesh) "/Game/StaticMeshes/SM_TicketUpgrade_001.SM_TicketUpgrade_001"))
    (:NewEnumerator2
      (Components|StaticMesh|SetStaticMesh (Variables|Default|GetStaticMesh) "/Game/StaticMeshes/SM_TicketUpgrade_001.SM_TicketUpgrade_001"))
    (:NewEnumerator3
      (Components|StaticMesh|SetStaticMesh (Variables|Default|GetStaticMesh) "/Game/StaticMeshes/SM_TicketUpgrade_001.SM_TicketUpgrade_001"))
    (:NewEnumerator4
      (Components|StaticMesh|SetStaticMesh (Variables|Default|GetStaticMesh) "/Game/StaticMeshes/Props/SM_Key_001.SM_Key_001"))))