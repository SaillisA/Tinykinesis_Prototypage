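; Abstract base for telekinesis pickup objects that take effect when they reach the Tinykinesis player character.
; Grabbing the object marks it as throwable and sets its player collision sphere to a grab-specific radius.
; When that sphere overlaps the player, it calls an empty pickup-effect function, a hook for children to override, then destroys the actor.
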(event OnComponentBeginOverlap(HitPlayerCollision)
  (params (OverlappedComponent :type Primitive%20Component%20Object%20Reference) (OtherActor :type Actor%20Object%20Reference) (OtherComp :type Primitive%20Component%20Object%20Reference) (OtherBodyIndex :type Integer) (bFromSweep :type Boolean) (SweepResult :type Hit%20Result%20Structure%20%28by%20ref%29))
  (if (== OtherActor (CallFunction|GetTinykinesisPlayerCharacter))
    (CallFunction|EffectonPickup)
    (Actor|DestroyActor)))

(event EventBeginPlay
  (|CallParentFunction) ; This node is disabled and will not be called.\nDrag off pins to build functionality.
)

(event Collision|EventActorBeginOverlap
  (params (OtherActor :type Actor%20Object%20Reference)))

(event EventTick
  (params (DeltaSeconds :type Float%20%28single-precision%29)))

(event EventGrabObject
  (Variables|Default|SetCanBeThrown true)
  (CallFunction|EffectonGrab))

(fn ConstructionScript
  (|CallParentFunction))

(fn EffectonGrab
  (Components|Sphere|SetSphereRadius (Variables|Default|GetHitPlayerCollision) (Variables|Default|GetRangeOnGrab) true))

(fn EffectonPickup)