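; BP_PickupObject_HealItem is a telekinesis pickup object that heals the player when picked up.
; It overrides Effect on Pickup to add a WBP_HealIndicator widget to the viewport, then calls HealHP with HealAmount on the BPACHealth component of the Tinykinesis player controller.
; All other behavior comes from the parent, as its own event nodes are disabled and construction only calls the parent script.
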(event EventBeginPlay
  (|CallParentFunction) ; This node is disabled and will not be called.\nDrag off pins to build functionality.
)

(event Collision|EventActorBeginOverlap
  (params (OtherActor :type Actor%20Object%20Reference))
  (|CallParentFunction OtherActor) ; This node is disabled and will not be called.\nDrag off pins to build functionality.
)

(event EventTick
  (params (DeltaSeconds :type Float%20%28single-precision%29))
  (|CallParentFunction DeltaSeconds) ; This node is disabled and will not be called.\nDrag off pins to build functionality.
)

(fn ConstructionScript
  (|CallParentFunction))

(fn EffectonPickup
  (bind _returnvalue (UserInterface|CreateWidget "/Game/Blueprints/WidgetBlueprints/HUD/WBP_HealIndicator.WBP_HealIndicator_C"))
  (UserInterface|Viewport|AddtoViewport _returnvalue 0)
  (Default|HealHP (Variables|/Game/Blueprints/Player/BP_TinykinesisPlayerController.BP_TinykinesisPlayerController_C|GetBP_AC_Health (CallFunction|GetTinykinesisPlayerController)) (Variables|Default|GetHealAmount)))