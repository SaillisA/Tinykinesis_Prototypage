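; Stun variant of the explosive light object, a telekinesis element that stuns melee enemies it affects.
; It overrides EffectOfEnnemy to cast the hit enemy's owner to the melee NPC AI controller and call its stun event.
; Enemies without that controller type get no effect from the override, which ignores the hit location and does not call the parent version.
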(event EventBeginPlay
  (|CallParentFunction) ; This node is disabled and will not be called.\nDrag off pins to build functionality.
)

(event Collision|EventActorBeginOverlap
  (params (OtherActor :type Actor%20Object%20Reference))
  (|CallParentFunction OtherActor) ; This node is disabled and will not be called.\nDrag off pins to build functionality.
)

(event EventTick
  (params (DeltaSeconds :type Float%20%28single-precision%29))
  (|CallParentFunction DeltaSeconds) ; This node is disabled and will not be called.\nDrag off pins to build functionality.
)

(fn ConstructionScript
  (|CallParentFunction))

(fn EffectOfEnnemy
  (params (EnnemyHit :type BP%20AI%20Character%20Blank%20Object%20Reference) (HitLocation :type Vector :default "0, 0, 0"))
  (bind _asbp_aic_npc_melee (Utilities|Casting|CastToBP_AIC_NpcMelee (Components|GetOwner EnnemyHit)))
  (Default|EventStun _asbp_aic_npc_melee))