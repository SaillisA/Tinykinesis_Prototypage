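; BP_TinyObject is a small telekinesis object that can be grabbed, charged, dropped or propelled.
; It binds the parent's grab, cancel, charge, release and feedback dispatchers on BeginPlay, delegating movement and per-tick updates to BPACAttractionElement.
; A charge timeline raises release speed, knockback and tattoo emissive, then shakes the camera and pulses the tattoos on completion.
; Cancel and release stop the charge; both target feedback handlers are empty.
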(event Custom|Grab_Tiny
  ;[0.1041 0.6523 1] Grab
  (Default|AttractObject (Variables|Default|GetBP_AC_AttractionElement) (Variables|Character|GetMesh) (Variables|Default|GetSpeedGrab)))

(event Custom|CancelGrab_Tiny
  ;[0.5208 0.814 1] Cancel Grab
  (Default|DropObject (Variables|Default|GetBP_AC_AttractionElement) (Variables|Character|GetMesh))
  ;[0.3251 0.199 1] Charge
  (bind (_direction _newspeedrelease _newknockbackforce _emissiveparameter) (Timeline|Charging_Tiny Stop)
    (:Update
      (CallFunction|UpdateChargeTelekinesis 0.0 _newspeedrelease _newknockbackforce _emissiveparameter))
    (:Finished
      (Camera|PlayWorldCameraShake "/Game/Blueprints/Actors/CameraManager/BP_AttractCompleteCameraShake.BP_AttractCompleteCameraShake_C" (Transformation|GetActorLocation (CallFunction|GetTinykinesisPlayerCharacter)) 0.0 5e+02)
      (CallFunction|EmissiveTatoosChanges 6e+02 0.2)
      (Utilities|FlowControl|Delay 0.21)
      (CallFunction|EmissiveTatoosChanges 75.0 0.2))))

(event Custom|Charge_Tiny
  ;[0.3251 0.199 1] Charge
  (bind (_direction _newspeedrelease _newknockbackforce _emissiveparameter) (Timeline|Charging_Tiny PlayFromStart)
    (:Update
      (CallFunction|UpdateChargeTelekinesis 0.0 _newspeedrelease _newknockbackforce _emissiveparameter))
    (:Finished
      (Camera|PlayWorldCameraShake "/Game/Blueprints/Actors/CameraManager/BP_AttractCompleteCameraShake.BP_AttractCompleteCameraShake_C" (Transformation|GetActorLocation (CallFunction|GetTinykinesisPlayerCharacter)) 0.0 5e+02)
      (CallFunction|EmissiveTatoosChanges 6e+02 0.2)
      (Utilities|FlowControl|Delay 0.21)
      (CallFunction|EmissiveTatoosChanges 75.0 0.2))))

(event Custom|Feedbacks_Tiny
  ;[1 0.8515 0] Feedback for Target
)

(event Custom|DeleteFeedbacks_Tiny
  ;[1 0.8515 0] Feedback for Target
)

(event Custom|Release_Tiny
  ;[1 0.1667 0.6787] Release
  (Default|PropulseObject (Variables|Default|GetBP_AC_AttractionElement) (Variables|Character|GetMesh) (Variables|Default|GetSpeedRelease))
  ;[0.3251 0.199 1] Charge
  (bind (_direction _newspeedrelease _newknockbackforce _emissiveparameter) (Timeline|Charging_Tiny Stop)
    (:Update
      (CallFunction|UpdateChargeTelekinesis 0.0 _newspeedrelease _newknockbackforce _emissiveparameter))
    (:Finished
      (Camera|PlayWorldCameraShake "/Game/Blueprints/Actors/CameraManager/BP_AttractCompleteCameraShake.BP_AttractCompleteCameraShake_C" (Transformation|GetActorLocation (CallFunction|GetTinykinesisPlayerCharacter)) 0.0 5e+02)
      (CallFunction|EmissiveTatoosChanges 6e+02 0.2)
      (Utilities|FlowControl|Delay 0.21)
      (CallFunction|EmissiveTatoosChanges 75.0 0.2))))

(event EventBeginPlay
  ;[0.298 1 0.5765] BeginPlay
  (|CallParentFunction)
  (EventDispatchers|BindEventtoGrabEventDispatcher (EventDispatchers|CreateEvent :!event Custom|Grab_Tiny))
  (EventDispatchers|BindEventtoCancelEventDispatcher (EventDispatchers|CreateEvent :!event Custom|CancelGrab_Tiny))
  (EventDispatchers|AssignChargeEventDispatcher (EventDispatchers|CreateEvent :!event Custom|Charge_Tiny))
  (EventDispatchers|BindEventtoReleaseEventDispatcher (EventDispatchers|CreateEvent :!event Custom|Release_Tiny))
  (EventDispatchers|AssignFeedbacksEventDispatcher (EventDispatchers|CreateEvent :!event Custom|Feedbacks_Tiny))
  (EventDispatchers|AssignDeleteFeedbacksEventDispatcher (EventDispatchers|CreateEvent :!event Custom|DeleteFeedbacks_Tiny)))

(event Collision|EventActorBeginOverlap
  (params (OtherActor :type Actor%20Object%20Reference)))

(event EventTick
  (params (DeltaSeconds :type Float%20%28single-precision%29))
  ;[0.7412 1 0.3412] TICK
  (|CallParentFunction 0.0)
  (Default|TickAttractiveElement (Variables|Default|GetBP_AC_AttractionElement) (Variables|Character|GetMesh) (Variables|Default|GetSpeedGrab) (Variables|Default|GetSpeedRelease) (Variables|Default|GetIsBeingGrabbed) (Variables|Default|GetIsBeingReleased) (Variables|Default|GetCurrentRotation)))

(fn ConstructionScript
  (|CallParentFunction))