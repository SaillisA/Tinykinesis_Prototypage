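; Light telekinesis object that the player can grab, charge, launch or drop, with mesh and material taken from a data asset.
; It binds handlers to inherited dispatchers and delegates attract, drop, propulse and per-tick movement to BPACAttractionElement.
; A ChargingPropulse timeline scales damage radius and release speed, then shakes the camera when finished.
; The damage sphere overlaps only after a hit; impact and feedback hooks are empty.
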(event Custom|Grab_Light
  ;[0.1041 0.6523 1] Grab
  (Default|AttractObject (Variables|Default|GetBP_AC_AttractionElement) (Variables|Character|GetMesh) (Variables|Default|GetSpeedRelease)))

(event Custom|CancelGrab_Light
  (bind _damagerangecollision (Variables|Default|GetDamageRangeCollision))
  ;[0.5208 0.814 1] Cancel Grab
  (Default|DropObject (Variables|Default|GetBP_AC_AttractionElement) (Variables|Character|GetMesh))
  (Components|Sphere|SetSphereRadius _damagerangecollision (Variables|Default|GetRadiusMinDamageRange) true)
  (Collision|SetCollisionResponsetoAllChannels _damagerangecollision "ECR_Ignore")
  ;[0.3251 0.199 1] Charge
  (bind (_direction _newsphereradius _newspeedrelease) (Timeline|ChargingPropulse Stop)
    (:Update
      (CallFunction|UpdateChargeTelekinesis _newsphereradius _newspeedrelease "0, 0, 0"))
    (:Finished
      (Camera|PlayWorldCameraShake "/Game/Blueprints/Actors/BlueprintClasses/BP_AttractCompleteCameraShake.BP_AttractCompleteCameraShake_C" (Transformation|GetActorLocation (CallFunction|GetTinykinesisPlayerCharacter)) 0.0 5e+02))))

(event Custom|Charge_Light
  ;[0.3251 0.199 1] Charge
  (bind (_direction _newsphereradius _newspeedrelease) (Timeline|ChargingPropulse PlayFromStart)
    (:Update
      (CallFunction|UpdateChargeTelekinesis _newsphereradius _newspeedrelease "0, 0, 0"))
    (:Finished
      (Camera|PlayWorldCameraShake "/Game/Blueprints/Actors/BlueprintClasses/BP_AttractCompleteCameraShake.BP_AttractCompleteCameraShake_C" (Transformation|GetActorLocation (CallFunction|GetTinykinesisPlayerCharacter)) 0.0 5e+02))))

(event Custom|Hit_Light
  (params (HitActor :type Actor%20Object%20Reference))
  ;[1 0.2696 0.3095] Collisions
  ;;[1 1 1] Hit Object
  (Collision|SetCollisionResponsetoAllChannels (Variables|Default|GetDamageRangeCollision) "ECR_Overlap")
  (CallFunction|ImpactEffect))

(event Custom|Feedbacks_Light
  ;[1 0.851 0] Feedback for Target
)

(event Custom|DeleteFeedbacks_Light
  ;[1 0.851 0] Feedback for Target
)

(event Custom|Release_Light
  ;[1 0.1667 0.6787] Release
  (Default|PropulseObject (Variables|Default|GetBP_AC_AttractionElement) (Variables|Character|GetMesh) (Variables|Default|GetSpeedRelease))
  ;[0.3251 0.199 1] Charge
  (bind (_direction _newsphereradius _newspeedrelease) (Timeline|ChargingPropulse Stop)
    (:Update
      (CallFunction|UpdateChargeTelekinesis _newsphereradius _newspeedrelease "0, 0, 0"))
    (:Finished
      (Camera|PlayWorldCameraShake "/Game/Blueprints/Actors/BlueprintClasses/BP_AttractCompleteCameraShake.BP_AttractCompleteCameraShake_C" (Transformation|GetActorLocation (CallFunction|GetTinykinesisPlayerCharacter)) 0.0 5e+02))))

(event EventBeginPlay
  (bind _damagerangecollision (Variables|Default|GetDamageRangeCollision))
  ;[0.298 1 0.5765] BeginPlay
  (|CallParentFunction)
  (Components|Sphere|SetSphereRadius _damagerangecollision (Variables|Default|GetRadiusMinDamageRange) true)
  (Collision|SetCollisionResponsetoAllChannels _damagerangecollision "ECR_Ignore")
  (EventDispatchers|BindEventtoGrabEventDispatcher (EventDispatchers|CreateEvent :!event Custom|Grab_Light))
  (EventDispatchers|BindEventtoCancelEventDispatcher (EventDispatchers|CreateEvent :!event Custom|CancelGrab_Light))
  (EventDispatchers|AssignChargeEventDispatcher (EventDispatchers|CreateEvent :!event Custom|Charge_Light))
  (EventDispatchers|BindEventtoReleaseEventDispatcher (EventDispatchers|CreateEvent :!event Custom|Release_Light))
  (EventDispatchers|BindEventtoHitEventDispatcher (EventDispatchers|CreateEvent :!event Custom|Hit_Light))
  (EventDispatchers|AssignFeedbacksEventDispatcher (EventDispatchers|CreateEvent :!event Custom|Feedbacks_Light))
  (EventDispatchers|AssignDeleteFeedbacksEventDispatcher (EventDispatchers|CreateEvent :!event Custom|DeleteFeedbacks_Light)))

(event EventTick
  (params (DeltaSeconds :type Float%20%28single-precision%29))
  ;[0.7412 1 0.3412] TICK
  (|CallParentFunction 0.0)
  (Default|TickAttractiveElement (Variables|Default|GetBP_AC_AttractionElement) (Variables|Character|GetMesh) 0.0 (Variables|Default|GetSpeedRelease) (Variables|Default|GetIsBeingGrabbed) (Variables|Default|GetIsBeingReleased) (Variables|Default|GetCurrentRotation)))

(fn ConstructionScript
  (bind _dataasset (Variables|Default|GetDataAsset))
  (|CallParentFunction)
  (Components|StaticMesh|SetStaticMesh (Variables|Character|GetMesh) (Variables|/Game/Blueprints/Actors/TelekinesisElements/Test_DataAssets/PDA_LightObject.PDA_LightObject_C|GetMesh _dataasset))
  (Rendering|Material|SetMaterial (Variables|Character|GetMesh) 0 (Variables|/Game/Blueprints/Actors/TelekinesisElements/Test_DataAssets/PDA_LightObject.PDA_LightObject_C|GetMaterial _dataasset)))

(fn DeathbyNPC
  (Actor|DestroyActor)
  (return))

(fn ImpactEffect)