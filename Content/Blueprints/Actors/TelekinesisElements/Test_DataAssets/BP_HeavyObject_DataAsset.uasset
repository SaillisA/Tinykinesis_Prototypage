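; Heavy telekinetic object actor that extends a parent class by binding its grab, charge, cancel, release and hit dispatchers.
; Grab levitates the mesh via timeline, while Tick eases its rotation.
; The charge timeline lifts it further, scaling damage radius, release speed and knockback, then signals completion with camera shake and tattoo glow.
; Release fires mesh and radial impulses; hit shakes the camera and switches the damage sphere to overlap.
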(event Custom|Grab_Heavy
  (bind _tinykinesisplayercharacter (CallFunction|GetTinykinesisPlayerCharacter))
  ;[0.1041 0.6523 1] Grab
  (Utilities|FlowControl|DoOnce false
    (:Completed
      (Class|PrimitiveComponent|SetAllPhysicsLinearVelocity (Variables|Character|GetMesh) "0, 0, 0" false)
      (Default|Animation _tinykinesisplayercharacter "NewEnumerator1")
      (Default|ObjectAnimation _tinykinesisplayercharacter "NewEnumerator1")
      (CallFunction|RotationEvent)
      (bind _levitationheight (Timeline|TimelineLevitation PlayFromStart)
        (:Update
          (CallFunction|LevitateObject (Variables|Character|GetMesh) _levitationheight))))))

(event Custom|Hit_Heavy
  (params (HitActor :type Actor%20Object%20Reference))
  ;[1 0.2696 0.3095] Collisions
  ;;[1 1 1] Hit Object
  (Camera|PlayWorldCameraShake "/Game/Blueprints/Actors/CameraManager/BP_CameraShake.BP_CameraShake_C" (Transformation|GetActorLocation (Game|GetPlayerCharacter 0)) 0.0 5e+02)
  (Collision|SetCollisionResponsetoAllChannels (Variables|Default|GetDamageRangeCollision) "ECR_Overlap"))

(event Custom|CancelGrab_Heavy
  (bind _tinykinesisplayercharacter (CallFunction|GetTinykinesisPlayerCharacter))
  (bind _damagerangecollision (Variables|Default|GetDamageRangeCollision))
  ;[0.5208 0.814 1] Cancel Grab
  (Components|Sphere|SetSphereRadius _damagerangecollision (Variables|Default|GetRadiusMinDamageRange) true)
  (Collision|SetCollisionResponsetoAllChannels _damagerangecollision "ECR_Ignore")
  (Utilities|FlowControl|Sequence
    (:then_0
      ;[0.1041 0.6523 1] Grab
      (Utilities|FlowControl|DoOnce false) ; enters at Reset
    )
    (:then_1
      ;[0.3251 0.199 1] Charge
      (bind (_direction _newsphereradius _newspeedrelease _levitationspeed _forceknockback) (Timeline|ChargingSmash Stop)
        (:Update
          (CallFunction|LevitateObject (Variables|Character|GetMesh) _levitationspeed)
          (CallFunction|UpdateChargeTelekinesis _newsphereradius _newspeedrelease _forceknockback 0.0))
        (:Finished
          (Camera|PlayWorldCameraShake "/Game/Blueprints/Actors/CameraManager/BP_AttractCompleteCameraShake.BP_AttractCompleteCameraShake_C" (Transformation|GetActorLocation (CallFunction|GetTinykinesisPlayerCharacter)) 0.0 5e+02)
          (CallFunction|EmissiveTatoosChanges 6e+02 0.2)
          (Utilities|FlowControl|Delay 0.21)
          (CallFunction|EmissiveTatoosChanges 75.0 0.2))))))

(event Custom|Release_Heavy
  ;[1 0.1667 0.6787] Release
  (Physics|AddImpulse (Variables|Character|GetMesh) (Math|Vector|MakeVector 0.0 0.0 (Variables|Default|GetSpeedRelease)) "None" true)
  (Class|RadialForceComponent|FireImpulse (Variables|Default|GetRadialForce))
  (Default|Animation (CallFunction|GetTinykinesisPlayerCharacter) "NewEnumerator2")
  ;[0.3251 0.199 1] Charge
  (bind (_direction _newsphereradius _newspeedrelease _levitationspeed _forceknockback) (Timeline|ChargingSmash Stop)
    (:Update
      (CallFunction|LevitateObject (Variables|Character|GetMesh) _levitationspeed)
      (CallFunction|UpdateChargeTelekinesis _newsphereradius _newspeedrelease _forceknockback 0.0))
    (:Finished
      (Camera|PlayWorldCameraShake "/Game/Blueprints/Actors/CameraManager/BP_AttractCompleteCameraShake.BP_AttractCompleteCameraShake_C" (Transformation|GetActorLocation (CallFunction|GetTinykinesisPlayerCharacter)) 0.0 5e+02)
      (CallFunction|EmissiveTatoosChanges 6e+02 0.2)
      (Utilities|FlowControl|Delay 0.21)
      (CallFunction|EmissiveTatoosChanges 75.0 0.2))))

(event Custom|Charge_Heavy
  ;[0.3251 0.199 1] Charge
  (bind (_direction _newsphereradius _newspeedrelease _levitationspeed _forceknockback) (Timeline|ChargingSmash PlayFromStart)
    (:Update
      (CallFunction|LevitateObject (Variables|Character|GetMesh) _levitationspeed)
      (CallFunction|UpdateChargeTelekinesis _newsphereradius _newspeedrelease _forceknockback 0.0))
    (:Finished
      (Camera|PlayWorldCameraShake "/Game/Blueprints/Actors/CameraManager/BP_AttractCompleteCameraShake.BP_AttractCompleteCameraShake_C" (Transformation|GetActorLocation (CallFunction|GetTinykinesisPlayerCharacter)) 0.0 5e+02)
      (CallFunction|EmissiveTatoosChanges 6e+02 0.2)
      (Utilities|FlowControl|Delay 0.21)
      (CallFunction|EmissiveTatoosChanges 75.0 0.2))))

(event Custom|Feedbacks_Heavy
  ;[1 0.8515 0] Feedback for Target
)

(event Custom|DeleteFeedbacks_Heavy
  ;[1 0.8515 0] Feedback for Target
)

(event EventBeginPlay
  (bind _damagerangecollision (Variables|Default|GetDamageRangeCollision))
  ;[0.298 1 0.5765] BeginPlay
  (|CallParentFunction)
  (Components|Sphere|SetSphereRadius _damagerangecollision (Variables|Default|GetRadiusMinDamageRange) true)
  (Collision|SetCollisionResponsetoAllChannels _damagerangecollision "ECR_Ignore")
  (EventDispatchers|BindEventtoGrabEventDispatcher (EventDispatchers|CreateEvent :!event Custom|Grab_Heavy))
  (EventDispatchers|BindEventtoCancelEventDispatcher (EventDispatchers|CreateEvent :!event Custom|CancelGrab_Heavy))
  (EventDispatchers|AssignChargeEventDispatcher (EventDispatchers|CreateEvent :!event Custom|Charge_Heavy))
  (EventDispatchers|BindEventtoReleaseEventDispatcher (EventDispatchers|CreateEvent :!event Custom|Release_Heavy))
  (EventDispatchers|BindEventtoHitEventDispatcher (EventDispatchers|CreateEvent :!event Custom|Hit_Heavy))
  (EventDispatchers|AssignFeedbacksEventDispatcher (EventDispatchers|CreateEvent :!event Custom|Feedbacks_Heavy))
  (EventDispatchers|AssignDeleteFeedbacksEventDispatcher (EventDispatchers|CreateEvent :!event Custom|DeleteFeedbacks_Heavy)))

(event EventTick
  (params (DeltaSeconds :type Float%20%28single-precision%29))
  ;[0.7412 1 0.3412] TICK (Rotation element)
  (|CallParentFunction 0.0)
  (if (Variables|Default|GetIsBeingGrabbed)
    (Transformation|SetRelativeRotation (Variables|Character|GetMesh) (Math|Rotator|Lerp(Rotator) (Variables|/Script/Engine.SceneComponent|GetRelativeRotation (Variables|Character|GetMesh)) (Variables|Default|GetCurrentRotation) (Utilities|Time|GetWorldDeltaSeconds) true) false false)))

(fn ConstructionScript
  (|CallParentFunction))

(fn LevitateObject
  (params (Mesh :type Static%20Mesh%20Component%20Object%20Reference) (NewHeight :type Float%20%28double-precision%29))
  (bind _returnvalue (Transformation|GetWorldLocation Mesh))
  (bind (_x _y _z) (Math|Vector|BreakVector _returnvalue))
  (Transformation|SetWorldLocation Mesh (Math|Vector|MakeVector _x _y (+ NewHeight _z)) true false))