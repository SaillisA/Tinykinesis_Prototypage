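; Base actor for objects the player can grab, charge and throw with telekinesis.
; Grab, cancel and release switch state flags, mesh physics and aim-assist collision, firing dispatchers alongside charge and translucent targeting feedback.
; A released impact sends damage and force to BPI_Target actors and launches the destruction component, while a charge-resized sphere also hits overlapping damageable targets.
; Grabbing picks random target rotations, but the lerp applying them is disconnected.
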(event OnComponentBeginOverlap(DamageRangeCollision)
  (params (OverlappedComponent :type Primitive%20Component%20Object%20Reference) (OtherActor :type Actor%20Object%20Reference) (OtherComp :type Primitive%20Component%20Object%20Reference) (OtherBodyIndex :type Integer) (bFromSweep :type Boolean) (SweepResult :type Hit%20Result%20Structure%20%28by%20ref%29))
  ;[1 0.2696 0.3095] Collisions
  ;;[1 1 1] Hit NCP
  (if (Utilities|DoesObjectImplementInterface OtherActor "/Game/Blueprints/Interfaces/BPI_Target.BPI_Target_C")
    (bind _cantakedamage (Class|BPITarget|GetCanTakeDamage(Message) OtherActor))
    (if _cantakedamage
      (Class|BPITarget|GetHit(Message) OtherActor self (Variables|StatusTelekinesis|GetIsBeingReleased) (Variables|Default|GetDamageObject) (Variables|Default|GetVectorHit) (Variables|Default|GetForceImpactXY) (Variables|Default|GetForceImpactZ)))))

(event EventBeginPlay
  (bind _mesh (Variables|Default|GetMesh))
  ;[0.298 1 0.5765] BeginPlay
  (Variables|Default|SetBaseMaterial (Rendering|Material|GetMaterial (Variables|Default|GetMesh) 0))
  (Components|Sphere|SetSphereRadius (Variables|SphereCollisions|GetAimAssistCollision) (Variables|SphereCollisions|GetRadiusAimAssist) true)
  (if (Variables|Default|GetBeginOnGround)
    (Physics|SetSimulatePhysics _mesh true)
    (else
      (Physics|SetSimulatePhysics _mesh false)))
  (Input|EnableInput (CallFunction|GetTinykinesisPlayerController)))

(event EventFeedbacksDetectObject
  ;[1 0.8515 0] Feedback for Target
  (Rendering|Material|SetMaterial (Variables|Default|GetMesh) 0 "/Game/Materials/M_Translucent.M_Translucent")
  (Default|CallFeedbacksEventDispatcher))

(event EventGrabObject
  ;[0.1041 0.6523 1] Grab
  (Utilities|FlowControl|Sequence
    (:then_0
      (Utilities|FlowControl|DoOnce false
        (:Completed
          (if (Variables|StatusTelekinesis|GetCanBeGrabbed)
            (Variables|StatusTelekinesis|SetIsBeingGrabbed true)
            (Variables|StatusTelekinesis|SetCanBeGrabbed true)
            (Variables|StatusTelekinesis|SetIsBeingReleased false)
            (Variables|StatusTelekinesis|SetCanBeReleased true)
            (CallFunction|DisableMeshPhysics "ECR_Ignore" false false)
            (Collision|SetCollisionResponsetoAllChannels (Variables|SphereCollisions|GetAimAssistCollision) "ECR_Ignore")
            (CallFunction|CreateNewRotator)))))
    (:then_1
      (if (Variables|Default|GetResetRotator)
        (Variables|Default|SetResetRotator false)
        (Utilities|FlowControl|Delay 2.5)
        (CallFunction|CreateNewRotator)
        (Variables|Default|SetResetRotator true)
        (Variables|Default|SetRotationLerp 0.0)))
    (:then_2
      (Default|CallGrabEventDispatcher))))

(event EventCancelGrabObject
  ;[0.5208 0.814 1] Cancel Grab
  (Default|ClearParameters (Variables|/Game/Blueprints/Player/BP_TinykinesisPlayerController.BP_TinykinesisPlayerController_C|GetBP_AC_Telekinesis (CallFunction|GetTinykinesisPlayerController)))
  (Variables|StatusTelekinesis|SetIsBeingGrabbed false)
  (Variables|StatusTelekinesis|SetCanBeGrabbed true)
  (Variables|StatusTelekinesis|SetIsBeingReleased false)
  (Variables|StatusTelekinesis|SetCanBeReleased false)
  (CallFunction|EnableMeshPhysics)
  (Collision|SetCollisionResponsetoAllChannels (Variables|SphereCollisions|GetAimAssistCollision) "ECR_Block")
  (Default|SetIddleAnimation (Variables|/Game/Blueprints/Player/BP_TinykinesisPlayerController.BP_TinykinesisPlayerController_C|GetBP_AC_Telekinesis (CallFunction|GetTinykinesisPlayerController)))
  (Default|CallCancelEventDispatcher)
  (Utilities|FlowControl|Sequence
    (:then_0
      ;[0.1041 0.6523 1] Grab
      (Utilities|FlowControl|DoOnce false) ; enters at Reset
    )
    (:then_1
      ;[0.3251 0.199 1] Charge
      (Utilities|FlowControl|DoOnce false) ; enters at Reset
    )))

(event EventReleaseObject
  ;[1 0.1667 0.6787] Release
  (if (Variables|StatusTelekinesis|GetIsBeingGrabbed)
    (Variables|StatusTelekinesis|SetIsBeingGrabbed false)
    (Variables|StatusTelekinesis|SetCanBeGrabbed false)
    (Variables|StatusTelekinesis|SetIsBeingReleased true)
    (Variables|StatusTelekinesis|SetCanBeReleased false)
    (CallFunction|EnableMeshPhysics)
    (Collision|SetCollisionEnabled (Variables|SphereCollisions|GetAimAssistCollision) "NoCollision")
    (Default|CallReleaseEventDispatcher)
    ;[0.3251 0.199 1] Charge
    (Utilities|FlowControl|DoOnce false) ; enters at Reset
  ))

(event EventChargeObject
  ;[0.3251 0.199 1] Charge
  (if (Variables|StatusTelekinesis|GetIsBeingGrabbed)
    (Utilities|FlowControl|DoOnce false
      (:Completed
        (Default|CallChargeEventDispatcher)))))

(event Collision|EventHit
  (params (MyComp :type Primitive%20Component%20Object%20Reference) (Other :type Actor%20Object%20Reference) (OtherComp :type Primitive%20Component%20Object%20Reference) (bSelfMoved :type Boolean) (HitLocation :type Vector :default "0, 0, 0") (HitNormal :type Vector :default "0, 0, 0") (NormalImpulse :type Vector :default "0, 0, 0") (Hit :type Hit%20Result%20Structure%20%28by%20ref%29))
  (bind _hitactor (Collision|BreakHitResult Hit))
  ;[1 0.2696 0.3095] Collisions
  ;;[1 1 1] Hit Object
  (if (Variables|StatusTelekinesis|GetIsBeingReleased)
    (if (!= _hitactor (CallFunction|GetTinykinesisPlayerCharacter))
      (Variables|Default|SetVectorHit HitLocation)
      (Default|CallHitEventDispatcher _hitactor)
      (Utilities|FlowControl|Sequence
        (:then_0
          (if (Utilities|DoesObjectImplementInterface _hitactor "/Game/Blueprints/Interfaces/BPI_Target.BPI_Target_C")
            (Class|BPITarget|GetHit(Message) _hitactor self (Variables|StatusTelekinesis|GetIsBeingReleased) (Variables|Default|GetDamageObject) (Variables|Default|GetVectorHit) (Variables|Default|GetForceImpactXY) (Variables|Default|GetForceImpactZ))))
        (:then_1
          (Variables|StatusTelekinesis|SetIsBeingGrabbed false)
          (Variables|StatusTelekinesis|SetCanBeGrabbed false)
          (Variables|StatusTelekinesis|SetIsBeingReleased false)
          (Variables|StatusTelekinesis|SetCanBeReleased false)
          (Default|LaunchDestruction (Variables|Fracturation|GetBP_AC_DestructionElement) (Transformation|GetRelativeTransform (Variables|Default|GetMesh)) self))))))

(event EventDeleteFeedbacksDetectObject
  ;[1 0.8515 0] Feedback for Target
  (Rendering|Material|SetMaterial (Variables|Default|GetMesh) 0 (Variables|Default|GetBaseMaterial))
  (Default|CallDeleteFeedbacksEventDispatcher))

(event EventTick
  (params (DeltaSeconds :type Float%20%28single-precision%29)))

(fn ConstructionScript)

(fn UpdateChargeTelekinesis
  (params (SphereRadius :type Float%20%28double-precision%29) (NewSpeedRelease :type Float%20%28double-precision%29) (NewForceImpactXY :type Float%20%28double-precision%29) (NewForceImpactZ :type Float%20%28double-precision%29))
  (Components|Sphere|SetSphereRadius (Variables|SphereCollisions|GetDamageRangeCollision) SphereRadius true)
  (Variables|Default|SetSpeedRelease NewSpeedRelease)
  (Variables|Default|SetForceImpactXY NewForceImpactXY)
  (Variables|Default|SetForceImpactZ NewForceImpactZ))

(fn EnableMeshPhysics
  (bind _mesh (Variables|Default|GetMesh))
  (Physics|SetSimulatePhysics _mesh true)
  (Physics|SetEnableGravity _mesh true)
  (Collision|SetCollisionEnabled _mesh "PhysicsOnly")
  (Collision|SetCollisionResponsetoChannel _mesh "ECC_WorldDynamic" "ECR_Block")
  (Collision|SetCollisionResponsetoChannel _mesh "ECC_Pawn" "ECR_Block")
  (Collision|SetCollisionResponsetoChannel _mesh "ECC_WorldStatic" "ECR_Block"))

(fn DisableMeshPhysics
  (params (NewResponse :type ECollisionResponse%20Enum :default "ECR_Ignore") (bSimulate :type Boolean) (bGravityEnabled :type Boolean))
  (bind _mesh (Variables|Default|GetMesh))
  (Physics|SetSimulatePhysics _mesh false)
  (Physics|SetEnableGravity _mesh false)
  (Collision|SetCollisionResponsetoChannel _mesh "ECC_WorldDynamic" "ECR_Ignore")
  (Collision|SetCollisionResponsetoChannel _mesh "ECC_PhysicsBody" "ECR_Ignore")
  (Collision|SetCollisionResponsetoChannel _mesh "ECC_Pawn" "ECR_Ignore")
  (Collision|SetCollisionResponsetoChannel _mesh "ECC_WorldStatic" "ECR_Ignore"))

(fn CreateNewRotator
  (bind _mesh (Variables|Default|GetMesh))
  (bind _relativerotation (Variables|/Script/Engine.SceneComponent|GetRelativeRotation _mesh))
  (Variables|Default|SetRotatorDestination (Math|Rotator|MakeRotator (Math|Random|RandomFloatinRange (- (.roll _relativerotation) 5e+01) (+ (.roll _relativerotation) 5e+01)) (Math|Random|RandomFloatinRange (- (.pitch _relativerotation) 5e+01) (+ (.pitch _relativerotation) 5e+01)) (Math|Random|RandomFloatinRange (- (.yaw _relativerotation) 5e+01) (+ (.yaw _relativerotation) 5e+01)))))

(fn TriggerGetHitDamage
  (params (HitActor :type Actor%20Object%20Reference))
  (Class|BPITarget|GetHit(Message) HitActor self (Variables|StatusTelekinesis|GetIsBeingReleased) (Variables|Default|GetDamageObject) (Variables|Default|GetVectorHit) (Variables|Default|GetForceImpactXY) (Variables|Default|GetForceImpactZ)))