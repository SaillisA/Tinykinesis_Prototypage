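; Telekinesis-grabbable object that is pulled to the player's hand and launched on release.
; Grab, cancel and release dispatchers are bound at BeginPlay; grab starts a distance-timed move to the right grab point.
; On arrival it plays audio, and while grabbed Tick lerps its rotation and, once arrived, its position.
; Release applies a velocity-change impulse along camera forward, or toward the aim trace's end if still in transit.
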(event Custom|Grab_Light
  (bind _mesh (Variables|Default|GetMesh))
  ;[0.1041 0.6523 1] Grab
  (Utilities|FlowControl|Sequence
    (:then_0
      ;;[1 1 1] Do Once
      (Utilities|FlowControl|DoOnce false
        (:Completed
          (Attraction|DoOnceAttract)
          (Components|MoveComponentTo (Variables|Default|GetMesh) (Transformation|GetWorldLocation (Variables|/Game/Blueprints/Player/BP_TinykinesisPlayerCharacter.BP_TinykinesisPlayerCharacter_C|GetGrabPointR (CallFunction|GetTinykinesisPlayerCharacter))) (Transformation|GetWorldRotation (Variables|/Script/Tinykinesis_Proto.Tinykinesis_ProtoCharacter|GetFirstPersonCameraComponent (CallFunction|GetTinykinesisPlayerCharacter))) false false (Variables|Attraction|GetDurationAbility) false)
          (Variables|Attraction|SetReachedPlayer true)
          (bind _returnvalue (Class|FMODBlueprintStatics|PlayEventatLocation (Variables|Default|GetAudioEvent) (Transformation|GetActorTransform (CallFunction|GetTinykinesisPlayerCharacter))))
          (Variables|Default|SetAudioInstance _returnvalue)
          (CallFunction|RotationEvent))))
    (:then_1
      (Variables|Attraction|SetTargetLocation (Transformation|GetWorldLocation (Variables|/Game/Blueprints/Player/BP_TinykinesisPlayerCharacter.BP_TinykinesisPlayerCharacter_C|GetGrabPointR (CallFunction|GetTinykinesisPlayerCharacter))))
      (if (Variables|Attraction|GetReachedPlayer)
        (Transformation|SetWorldLocation _mesh (Math|Vector|Lerp(Vector) (Transformation|GetWorldLocation _mesh) (Variables|Attraction|GetTargetLocation) (* (Utilities|Time|GetWorldDeltaSeconds) 8.0)) true false)))))

(event Custom|CancelGrab_Light
  ;[0.5208 0.814 1] Cancel Grab
  (Utilities|FlowControl|Sequence
    (:then_0
      ;[0.1041 0.6523 1] Grab
      ;;[1 1 1] Do Once
      (Utilities|FlowControl|DoOnce false) ; enters at Reset
    )
    (:then_1
      (Variables|Attraction|SetReachedPlayer false)
      (Class|FMODBlueprintStatics|EventInstanceStop (Variables|Default|GetAudioInstance) false))))

(event Custom|StopAttract
  ;[0.1041 0.6523 1] Grab
  ;;[1 1 1] Do Once
  (Components|MoveComponentTo (Variables|Default|GetMesh) (Transformation|GetWorldLocation (Variables|/Game/Blueprints/Player/BP_TinykinesisPlayerCharacter.BP_TinykinesisPlayerCharacter_C|GetGrabPointR (CallFunction|GetTinykinesisPlayerCharacter))) (Transformation|GetWorldRotation (Variables|/Script/Tinykinesis_Proto.Tinykinesis_ProtoCharacter|GetFirstPersonCameraComponent (CallFunction|GetTinykinesisPlayerCharacter))) false false (Variables|Attraction|GetDurationAbility) false) ; enters at Stop
)

(event Custom|Feedbacks_Light
  ;[1 0.851 0] Feedback for Target
)

(event Custom|DeleteFeedbacks_Light
  ;[1 0.851 0] Feedback for Target
)

(event Custom|Release_Light
  (bind _tinykinesisplayercontroller (CallFunction|GetTinykinesisPlayerController))
  (bind _bp_ac_telekinesis (Variables|/Game/Blueprints/Player/BP_TinykinesisPlayerController.BP_TinykinesisPlayerController_C|GetBP_AC_Telekinesis _tinykinesisplayercontroller))
  ;[1 0.1667 0.6787] Release
  (Default|ObjectAnimation (CallFunction|GetTinykinesisPlayerCharacter) "NewEnumerator0")
  (Class|FMODBlueprintStatics|EventInstanceStop (Variables|Default|GetAudioInstance) false)
  (Rendering|SetVisibility (Variables|/Game/Blueprints/Player/BP_TinykinesisPlayerCharacter.BP_TinykinesisPlayerCharacter_C|GetSparksHand (CallFunction|GetTinykinesisPlayerCharacter)) false false)
  (if (Variables|Attraction|GetReachedPlayer)
    (Default|BindandLaunchProjectionEventinTimeline (CallFunction|GetTinykinesisPlayerController) (EventDispatchers|CreateEvent :!event SetProjTowardsPlayer) 0.1)
    (Utilities|FlowControl|Delay 0.1)
    (Physics|AddImpulse (Variables|Default|GetMesh) (* (Math|Vector|GetForwardVector (Variables|/Script/Tinykinesis_Proto.Tinykinesis_ProtoCharacter|GetFirstPersonCameraComponent (CallFunction|GetTinykinesisPlayerCharacter))) (Variables|Default|GetCurrentReleaseForce)) "None" true)
    (else
      (CallFunction|StopAttract)
      (Variables|Attraction|SetReachedPlayer false)
      (bind (_start _end) (Default|GetAimCastDistance _bp_ac_telekinesis (Variables|/Game/Blueprints/ActorComponents/PlayerAbilities/BP_AC_Telekinesis.BP_AC_Telekinesis_C|GetRangeReleaseRaycast _bp_ac_telekinesis)))
      (bind _outhit (Collision|LineTraceByChannel _start _end "TraceTypeQuery1" false 0 "Persistent"))
      (Physics|AddImpulse (Variables|Default|GetMesh) (* (Math|Vector|GetForwardVector (Math|Rotator|FindLookatRotation (Transformation|GetWorldLocation (Variables|Character|GetMesh)) (.TraceEnd (Collision|BreakHitResult _outhit)))) (Variables|Default|GetCurrentReleaseForce)) "None" true))))

(event EventBeginPlay
  ;[0.298 1 0.5765] BeginPlay
  (|CallParentFunction)
  (Collision|SetCollisionResponsetoAllChannels (Variables|Default|GetDamageRangeCollision) "ECR_Ignore")
  (EventDispatchers|BindEventtoGrabEventDispatcher (EventDispatchers|CreateEvent :!event Custom|Grab_Light))
  (EventDispatchers|BindEventtoCancelEventDispatcher (EventDispatchers|CreateEvent :!event Custom|CancelGrab_Light))
  (EventDispatchers|BindEventtoReleaseEventDispatcher (EventDispatchers|CreateEvent :!event Custom|Release_Light))
  (EventDispatchers|AssignFeedbacksEventDispatcher (EventDispatchers|CreateEvent :!event Custom|Feedbacks_Light))
  (EventDispatchers|AssignDeleteFeedbacksEventDispatcher (EventDispatchers|CreateEvent :!event Custom|DeleteFeedbacks_Light))
  (Variables|Default|SetForceKnockbackMultiplier "1.000000,1.000000,1.000000"))

(event EventTick
  (params (DeltaSeconds :type Float%20%28single-precision%29))
  (bind _returnvalue (Utilities|Time|GetWorldDeltaSeconds))
  (bind _currentrotation (Variables|Default|GetCurrentRotation))
  (bind _mesh (Variables|Character|GetMesh))
  (bind _relativerotation (Variables|/Script/Engine.SceneComponent|GetRelativeRotation _mesh))
  (bind _returnvalue_2 (Math|Rotator|Lerp(Rotator) _relativerotation _currentrotation _returnvalue true))
  ;[0.7412 1 0.3412] TICK
  (|CallParentFunction 0.0)
  (if (Variables|Default|GetIsBeingGrabbed)
    ;;[1 1 1] Attract in real time
    (CallFunction|GrabLight)
    ;;[1 1 1] Rotate the projectile for flavor purpose
    (Transformation|SetRelativeRotation (Variables|Character|GetMesh) (Math|Rotator|MakeRotator (.roll _returnvalue_2) (.pitch _returnvalue_2) (.yaw (Transformation|GetWorldRotation (Variables|/Script/Tinykinesis_Proto.Tinykinesis_ProtoCharacter|GetFirstPersonCameraComponent (CallFunction|GetTinykinesisPlayerCharacter))))) false false)))

(fn ConstructionScript
  (|CallParentFunction))

(fn DoOnceAttract
  (Attraction|SetDurationAbility (Variables|Default|GetGrabSpeed) (Math|Vector|Distance(Vector) (Transformation|GetWorldLocation (Variables|Character|GetMesh)) (Transformation|GetWorldLocation (Variables|/Script/Tinykinesis_Proto.Tinykinesis_ProtoCharacter|GetFirstPersonCameraComponent (CallFunction|GetTinykinesisPlayerCharacter)))))
  (CallFunction|EmissiveTatoosChanges 1e+01 (Variables|Attraction|GetDurationAbility)))

(fn SetDurationAbility
  (params (Speed :type Float%20%28double-precision%29) (DistancePlayerTarget :type Float%20%28double-precision%29))
  (Variables|Attraction|SetDurationAbility (/ DistancePlayerTarget Speed)))

(fn DoOncePropulse)

(fn SetProjTowardsPlayer
  (params (Delta%20Time :type Float%20%28double-precision%29))
  (bind _tinykinesisplayercharacter (CallFunction|GetTinykinesisPlayerCharacter))
  (Transformation|SetWorldLocation (Variables|Default|GetMesh) (Math|Vector|Lerp(Vector) (Transformation|GetWorldLocation (Variables|/Game/Blueprints/Player/BP_TinykinesisPlayerCharacter.BP_TinykinesisPlayerCharacter_C|GetGrabPointR _tinykinesisplayercharacter)) (Transformation|GetWorldLocation (Variables|/Game/Blueprints/Player/BP_TinykinesisPlayerCharacter.BP_TinykinesisPlayerCharacter_C|GetGrabPointFront _tinykinesisplayercharacter)) Delta%20Time) false false))