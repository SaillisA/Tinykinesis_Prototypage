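; BP_LightObject is a light telekinesis object that the player can grab, charge, drop or propel.
; It binds inherited dispatchers to handlers that drive BPACAttractionElement, with a charge Timeline updating the damage sphere radius and shaking the camera on completion.
; Tick restores the base material whenever it is not the locked item, which the author flags as unoptimized.
; Impact and target-feedback handlers are empty, and DeathByNPC destroys the actor.
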(event Custom|Grab_Light
  ;[0.1041 0.6523 1] Grab
  (Default|AttractObject (Variables|Default|GetBP_AC_AttractionElement) 0 (Variables|Character|GetMesh) (Variables|Default|GetAimAssistCollision)))

(event Custom|CancelGrab_Light
  (bind _damagerangecollision (Variables|Default|GetDamageRangeCollision))
  ;[0.5208 0.814 1] Cancel Grab
  (Default|DropObject (Variables|Default|GetBP_AC_AttractionElement) (Variables|Character|GetMesh) (Variables|Default|GetAimAssistCollision))
  (Components|Sphere|SetSphereRadius _damagerangecollision (Variables|Default|GetRadiusMinDamageRange) true)
  (Collision|SetCollisionResponsetoAllChannels _damagerangecollision "ECR_Ignore")
  ;[0.3251 0.199 1] Charge
  (bind _size (Timeline|Timeline Stop)
    (:Update
      (CallFunction|UpdateChargeTelekinesis _size 0.0))
    (:Finished
      (Camera|PlayWorldCameraShake "/Game/Blueprints/Actors/BP_AttractCompleteCameraShake.BP_AttractCompleteCameraShake_C" (Transformation|GetActorLocation (CallFunction|GetTinykinesisPlayerCharacter)) 0.0 5e+02))))

(event Custom|Charge_Light
  ;[0.3251 0.199 1] Charge
  (bind _size (Timeline|Timeline PlayFromStart)
    (:Update
      (CallFunction|UpdateChargeTelekinesis _size 0.0))
    (:Finished
      (Camera|PlayWorldCameraShake "/Game/Blueprints/Actors/BP_AttractCompleteCameraShake.BP_AttractCompleteCameraShake_C" (Transformation|GetActorLocation (CallFunction|GetTinykinesisPlayerCharacter)) 0.0 5e+02))))

(event Custom|Release_Light
  ;[1 0.1667 0.6787] Release
  (Default|PropulseObject (Variables|Default|GetBP_AC_AttractionElement) (Variables|Character|GetMesh))
  ;[0.3251 0.199 1] Charge
  (bind _size (Timeline|Timeline Stop)
    (:Update
      (CallFunction|UpdateChargeTelekinesis _size 0.0))
    (:Finished
      (Camera|PlayWorldCameraShake "/Game/Blueprints/Actors/BP_AttractCompleteCameraShake.BP_AttractCompleteCameraShake_C" (Transformation|GetActorLocation (CallFunction|GetTinykinesisPlayerCharacter)) 0.0 5e+02))))

(event Custom|Hit_Light
  ;[1 0.2696 0.3095] Collisions
  ;;[1 1 1] Hit Object
  (CallFunction|ImpactEffect))

(event Custom|Feedbacks_Light
  ;[1 0.8515 0] Feedback for Target
)

(event Custom|DeleteFeedbacks_Light
  ;[1 0.8515 0] Feedback for Target
)

(event EventBeginPlay
  (bind _damagerangecollision (Variables|Default|GetDamageRangeCollision))
  ;[0.298 1 0.5765] BeginPlay
  (|CallParentFunction)
  (Components|Sphere|SetSphereRadius _damagerangecollision (Variables|Default|GetRadiusMinDamageRange) true)
  (Collision|SetCollisionResponsetoAllChannels _damagerangecollision "ECR_Ignore")
  (EventDispatchers|BindEventtoGrabEventDispatcher (delegate Custom|Grab_Light))
  (EventDispatchers|BindEventtoCancelEventDispatcher (delegate Custom|CancelGrab_Light))
  (EventDispatchers|AssignChargeEventDispatcher (delegate Custom|Charge_Light))
  (EventDispatchers|BindEventtoReleaseEventDispatcher (delegate Custom|Release_Light))
  (EventDispatchers|BindEventtoHitEventDispatcher (delegate Custom|Hit_Light))
  (EventDispatchers|AssignFeedbacksEventDispatcher (delegate Custom|Feedbacks_Light))
  (EventDispatchers|AssignDeleteFeedbacksEventDispatcher (delegate Custom|DeleteFeedbacks_Light)))

(event EventTick
  (params (DeltaSeconds :type Float%20%28single-precision%29))
  ;[0.7412 1 0.3412] TICK. Reset le material -> pas opti de faire ça en Tick. Ce serait cool de trouver une alternative
  (if (not (== (Variables|/Game/Blueprints/Player/BP_TinykinesisPlayerController.BP_TinykinesisPlayerController_C|GetLockedItem (CallFunction|GetTinykinesisPlayerController)) self))
    (Rendering|Material|SetMaterial (Variables|Character|GetMesh) 0 (Variables|Default|GetBaseMaterial))))

(fn ConstructionScript
  (|CallParentFunction))

(fn DeathbyNPC
  (Actor|DestroyActor)
  (return))

(fn ImpactEffect)