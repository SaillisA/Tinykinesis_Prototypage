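; A one-shot trigger area that introduces or unlocks a player ability, chosen by its PowerType: Movements, Jump or Telekinesis.
; When the player first overlaps the box, it disables itself in the save through BPACStateGameplayElement and fades in a colored tutorial popup with input icons.
; Jump and Telekinesis also set the unlock flag on their controller component and trigger a level manager save at the player's transform; Movements only shows the popup.
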(event OnComponentBeginOverlap(Box)
  (params (OverlappedComponent :type Primitive%20Component%20Object%20Reference) (OtherActor :type Actor%20Object%20Reference) (OtherComp :type Primitive%20Component%20Object%20Reference) (OtherBodyIndex :type Integer) (bFromSweep :type Boolean) (SweepResult :type Hit%20Result%20Structure%20%28by%20ref%29))
  (bind _tinykinesisplayercontroller (CallFunction|GetTinykinesisPlayerController))
  (bind _tinykinesisplayercontroller_2 (CallFunction|GetTinykinesisPlayerController))
  (bind _tinykinesisplayercontroller_3 (CallFunction|GetTinykinesisPlayerController))
  (bind _wbpplayerhud (Variables|/Game/Blueprints/Player/BP_TinykinesisPlayerController.BP_TinykinesisPlayerController_C|GetWBPPlayerHUD _tinykinesisplayercontroller_2))
  (bind _wbpplayerhud_2 (Variables|/Game/Blueprints/Player/BP_TinykinesisPlayerController.BP_TinykinesisPlayerController_C|GetWBPPlayerHUD _tinykinesisplayercontroller_3))
  (bind _wbpplayerhud_3 (Variables|/Game/Blueprints/Player/BP_TinykinesisPlayerController.BP_TinykinesisPlayerController_C|GetWBPPlayerHUD _tinykinesisplayercontroller))
  (bind _wbp_popuptuto (Variables|/Game/Blueprints/WidgetBlueprints/HUD/WBP_PlayerHUD.WBP_PlayerHUD_C|GetWBP_PopUpTuto _wbpplayerhud_3))
  (bind _wbp_popuptuto_2 (Variables|/Game/Blueprints/WidgetBlueprints/HUD/WBP_PlayerHUD.WBP_PlayerHUD_C|GetWBP_PopUpTuto _wbpplayerhud_2))
  (bind _wbp_popuptuto_3 (Variables|/Game/Blueprints/WidgetBlueprints/HUD/WBP_PlayerHUD.WBP_PlayerHUD_C|GetWBP_PopUpTuto _wbpplayerhud))
  (if (and (not (Variables|Default|GetHasOverlaped)) (== OtherActor (CallFunction|GetTinykinesisPlayerCharacter)))
    (Default|DisableinSave (Variables|Default|GetBP_AC_StateGameplayElement))
    (Variables|Default|SetHasOverlaped true)
    (switch Utilities|FlowControl|Switch|SwitchonE_StandardPowers (Variables|Default|GetPowerType)
      (:NewEnumerator0
        (Default|SetValue _wbp_popuptuto_3 "Move" (Utilities|Struct|MakeSlateColor "(R=1.000000,G=1.000000,B=1.000000,A=1.000000)") "/Game/UI/Sprites/InputsPlayer/T_IconInputSPACE_Sprite.T_IconInputSPACE_Sprite" "/Game/UI/Sprites/InputsPlayer/T_IconInputA_Sprite.T_IconInputA_Sprite")
        (Default|LaunchFadein _wbp_popuptuto_3 1.0))
      (:NewEnumerator1
        (Default|SetValue _wbp_popuptuto_2 "Jump" (Utilities|Struct|MakeSlateColor "(R=1.000000,G=0.226567,B=0.799607,A=1.000000)") "/Game/UI/Sprites/InputsPlayer/T_IconInputSPACE_Sprite.T_IconInputSPACE_Sprite" "/Game/UI/Sprites/InputsPlayer/T_IconInputA_Sprite.T_IconInputA_Sprite")
        (Default|LaunchFadein _wbp_popuptuto_2 1.0)
        (Variables|/Game/Blueprints/ActorComponents/PlayerAbilities/BP_AC_Jump.BP_AC_Jump_C|SetJumpUnlocked (Variables|/Game/Blueprints/Player/BP_TinykinesisPlayerController.BP_TinykinesisPlayerController_C|GetBP_AC_Jump _tinykinesisplayercontroller_3) true)
        (bind _returnvalue (Actor|GetActorOfClass "/Game/Blueprints/SaveSystem/BP_AbstractLevelManager.BP_AbstractLevelManager_C"))
        (Utilities|IsValid _returnvalue
          (:Is%20Valid
            (Default|TriggerSaveGame _returnvalue (Transformation|GetActorTransform (CallFunction|GetTinykinesisPlayerCharacter))))))
      (:NewEnumerator2
        (Default|SetValue _wbp_popuptuto "Use Tinykinesis" (Utilities|Struct|MakeSlateColor "(R=1.000000,G=0.768151,B=0.078187,A=1.000000)") "/Game/UI/Sprites/InputsPlayer/T_IconInputLightClick_Sprite.T_IconInputLightClick_Sprite" "/Game/UI/Sprites/InputsPlayer/T_IconInputRT_Sprite.T_IconInputRT_Sprite")
        (Default|LaunchFadein _wbp_popuptuto 1.0)
        (Variables|/Game/Blueprints/ActorComponents/PlayerAbilities/BP_AC_Telekinesis.BP_AC_Telekinesis_C|SetTelekinesisUnlocked (Variables|/Game/Blueprints/Player/BP_TinykinesisPlayerController.BP_TinykinesisPlayerController_C|GetBP_AC_Telekinesis _tinykinesisplayercontroller) true)
        (bind _returnvalue_2 (Actor|GetActorOfClass "/Game/Blueprints/SaveSystem/BP_AbstractLevelManager.BP_AbstractLevelManager_C"))
        (Utilities|IsValid _returnvalue_2
          (:Is%20Valid
            (Default|TriggerSaveGame _returnvalue_2 (Transformation|GetActorTransform (CallFunction|GetTinykinesisPlayerCharacter)))))))))

(event EventBeginPlay)

(event Collision|EventActorBeginOverlap
  (params (OtherActor :type Actor%20Object%20Reference)))

(event EventTick
  (params (DeltaSeconds :type Float%20%28single-precision%29)))

(fn ConstructionScript)