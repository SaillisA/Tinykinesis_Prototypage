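; BP_UnlockFinalDoor is a trigger actor that unlocks the final door once the player has found the key.
; When its sphere is overlapped, it checks a one-shot activation flag and the player controller's key flag.
; It then fires the unlock event dispatcher and plays the HUD key fade animation in reverse.
; The overlap does not check which actor entered the sphere.
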(event OnComponentBeginOverlap(Sphere)
  (params (OverlappedComponent :type Primitive%20Component%20Object%20Reference) (OtherActor :type Actor%20Object%20Reference) (OtherComp :type Primitive%20Component%20Object%20Reference) (OtherBodyIndex :type Integer) (bFromSweep :type Boolean) (SweepResult :type Hit%20Result%20Structure%20%28by%20ref%29))
  (if (and (not (Variables|Default|GetIsActivated)) (Variables|/Game/Blueprints/Player/BP_TinykinesisPlayerController.BP_TinykinesisPlayerController_C|GetHasFoundKey (CallFunction|GetTinykinesisPlayerController)))
    (Variables|Default|SetIsActivated true)
    (Default|CallUnlockFinalDoorEventDispatcher)
    (Default|LaunchAnimFadeKey (Variables|/Game/Blueprints/Player/BP_TinykinesisPlayerController.BP_TinykinesisPlayerController_C|GetWBPPlayerHUD (CallFunction|GetTinykinesisPlayerController)) "Reverse")))

(event EventBeginPlay)

(event Collision|EventActorBeginOverlap
  (params (OtherActor :type Actor%20Object%20Reference)))

(event EventTick
  (params (DeltaSeconds :type Float%20%28single-precision%29)))

(fn ConstructionScript)