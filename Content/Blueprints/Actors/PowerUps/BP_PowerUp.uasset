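; Pickup actor that grants the player a double jump, dash, repulse or freeze-time upgrade, or the final-area key.
; PowerUpType selects mesh and materials in SetMesh, and on player overlap picks the controller component to upgrade or sets the key flag and HUD.
; Overlap also stops audio, disables the element in save state via BPACStateGameplayElement, and triggers a level-manager save.
; Upgrades are destroyed immediately, while the key starts a scale-down timeline.
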(event OnComponentBeginOverlap(HitPlayer)
  (params (OverlappedComponent :type Primitive%20Component%20Object%20Reference) (OtherActor :type Actor%20Object%20Reference) (OtherComp :type Primitive%20Component%20Object%20Reference) (OtherBodyIndex :type Integer) (bFromSweep :type Boolean) (SweepResult :type Hit%20Result%20Structure%20%28by%20ref%29))
  (if (== OtherActor (CallFunction|GetTinykinesisPlayerCharacter))
    (CallFunction|EffectonPickup)
    (Class|FMODBlueprintStatics|EventInstanceStop (Variables|Default|GetAudioInstance) false)
    (Default|DisableinSave (Variables|Default|GetBP_AC_StateGameplayElement))
    (Utilities|FlowControl|Sequence
      (:then_0
        (bind _returnvalue (Actor|GetActorOfClass "/Game/Blueprints/SaveSystem/BP_AbstractLevelManager.BP_AbstractLevelManager_C"))
        (Utilities|IsValid _returnvalue
          (:Is%20Valid
            (Default|TriggerSaveGame _returnvalue (Transformation|GetActorTransform (CallFunction|GetTinykinesisPlayerCharacter))))))
      (:then_1
        (if (Utilities|Enum|NotEqual(Enum) (Variables|Default|GetPowerUpType) "NewEnumerator4")
          (Actor|DestroyActor))))))

(event Custom|BeginPlay_PowerUp
  ;[0.298 1 0.5765] BeginPlay
  (CallFunction|SetMesh))

(event Custom|LoadPowerUp
  (bind _bp_ac_stategameplayelement (Variables|Default|GetBP_AC_StateGameplayElement))
  ;[0.298 1 0.5765] BeginPlay
  (Default|LoadElement _bp_ac_stategameplayelement (Variables|/Game/Blueprints/ActorComponents/BP_AC_StateGameplayElement.BP_AC_StateGameplayElement_C|GetIsActivated _bp_ac_stategameplayelement) self))

(event EventBeginPlay
  ;[0.298 1 0.5765] BeginPlay
  (EventDispatchers|BindEventtoBeginPlayActiveElement (Variables|Default|GetBP_AC_StateGameplayElement) (EventDispatchers|CreateEvent :!event Custom|BeginPlay_PowerUp)))

(event Collision|EventActorBeginOverlap
  (params (OtherActor :type Actor%20Object%20Reference))
  (|CallParentFunction OtherActor) ; This node is disabled and will not be called.\nDrag off pins to build functionality.
)

(event EventTick
  (params (DeltaSeconds :type Float%20%28single-precision%29))
  (|CallParentFunction DeltaSeconds) ; This node is disabled and will not be called.\nDrag off pins to build functionality.
)

(event EventSetActive
  (params (IsActive :type Boolean))
  (bind _bp_ac_stategameplayelement (Variables|Default|GetBP_AC_StateGameplayElement))
  ;[0.298 1 0.5765] BeginPlay
  (EventDispatchers|BindEventtoSetActiveElementEventDispatcher _bp_ac_stategameplayelement (EventDispatchers|CreateEvent :!event Custom|LoadPowerUp))
  (EventDispatchers|BindEventtoBeginPlayActiveElement _bp_ac_stategameplayelement (EventDispatchers|CreateEvent :!event Custom|BeginPlay_PowerUp))
  (Default|SetActiveElement _bp_ac_stategameplayelement IsActive))

(fn ConstructionScript
  (|CallParentFunction)
  (CallFunction|SetMesh))

(fn EffectonPickup
  (bind _tinykinesisplayercontroller (CallFunction|GetTinykinesisPlayerController))
  (bind _scaledownkey (Variables|Default|GetScaleDownKey))
  (bind _wbpplayerhud (Variables|/Game/Blueprints/Player/BP_TinykinesisPlayerController.BP_TinykinesisPlayerController_C|GetWBPPlayerHUD _tinykinesisplayercontroller))
  (switch Utilities|FlowControl|Switch|SwitchonE_PowerUps (Variables|Default|GetPowerUpType)
    (:NewEnumerator0
      (Default|PowerUpDoubleJump (Variables|/Game/Blueprints/Player/BP_TinykinesisPlayerController.BP_TinykinesisPlayerController_C|GetBP_AC_Jump _tinykinesisplayercontroller)))
    (:NewEnumerator1
      (Default|PowerUpDash (Variables|/Game/Blueprints/Player/BP_TinykinesisPlayerController.BP_TinykinesisPlayerController_C|GetBP_AC_Dash _tinykinesisplayercontroller)))
    (:NewEnumerator2
      (Default|PowerUpRepulse (Variables|/Game/Blueprints/Player/BP_TinykinesisPlayerController.BP_TinykinesisPlayerController_C|GetBP_AC_Repulse _tinykinesisplayercontroller)))
    (:NewEnumerator3
      (Default|PowerUpFreezeTime (Variables|/Game/Blueprints/Player/BP_TinykinesisPlayerController.BP_TinykinesisPlayerController_C|GetBP_AC_FreezeTime _tinykinesisplayercontroller)))
    (:NewEnumerator4
      (if (not (Variables|/Game/Blueprints/Player/BP_TinykinesisPlayerController.BP_TinykinesisPlayerController_C|GetHasFoundKey _tinykinesisplayercontroller))
        (Variables|/Game/Blueprints/Player/BP_TinykinesisPlayerController.BP_TinykinesisPlayerController_C|SetHasFoundKey _tinykinesisplayercontroller true)
        (Components|Timeline|SetTimelineLength _scaledownkey 0.5)
        (Components|Timeline|PlayfromStart _scaledownkey)
        (Widget|SetVisibility (Variables|/Game/Blueprints/WidgetBlueprints/HUD/WBP_PlayerHUD.WBP_PlayerHUD_C|GetKey_Sprite _wbpplayerhud) "Visible")
        (Default|LaunchAnimFadeKey _wbpplayerhud "Forward")))))

(fn SetMesh
  (bind _staticmesh (Variables|Default|GetStaticMesh))
  (bind _staticmesh_2 (Variables|Default|GetStaticMesh))
  (bind _staticmesh_3 (Variables|Default|GetStaticMesh))
  (bind _staticmesh_4 (Variables|Default|GetStaticMesh))
  (bind _staticmesh_5 (Variables|Default|GetStaticMesh))
  (bind _returnvalue (Transformation|GetRelativeTransform _staticmesh))
  (switch Utilities|FlowControl|Switch|SwitchonE_PowerUps (Variables|Default|GetPowerUpType)
    (:NewEnumerator0
      (Components|StaticMesh|SetStaticMesh _staticmesh_3 "/Game/StaticMeshes/SM_TicketUpgrade_001.SM_TicketUpgrade_001")
      (Rendering|Material|SetMaterial _staticmesh_3 0 "/Game/Materials/MI_TicketUpgradeFairyJump_001.MI_TicketUpgradeFairyJump_001"))
    (:NewEnumerator1
      (Components|StaticMesh|SetStaticMesh _staticmesh_5 "/Game/StaticMeshes/SM_TicketUpgrade_001.SM_TicketUpgrade_001")
      (Rendering|Material|SetMaterial _staticmesh_5 0 "/Game/Materials/MI_TicketUpgrade_Dash_001.MI_TicketUpgrade_Dash_001"))
    (:NewEnumerator2
      (Components|StaticMesh|SetStaticMesh _staticmesh_2 "/Game/StaticMeshes/SM_TicketUpgrade_001.SM_TicketUpgrade_001")
      (Rendering|Material|SetMaterial _staticmesh_2 0 "/Game/Materials/MI_TicketUpgrade_Repulse_001.MI_TicketUpgrade_Repulse_001"))
    (:NewEnumerator3
      (Components|StaticMesh|SetStaticMesh _staticmesh_4 "/Game/StaticMeshes/SM_TicketUpgrade_001.SM_TicketUpgrade_001")
      (Rendering|Material|SetMaterial _staticmesh_4 0 "/Game/Materials/MI_TicketUpgrade_FreezeTime_001.MI_TicketUpgrade_FreezeTime_001"))
    (:NewEnumerator4
      (Components|StaticMesh|SetStaticMesh _staticmesh "/Game/StaticMeshes/Props/SM_Key_001.SM_Key_001")
      (Rendering|Material|SetMaterial _staticmesh 0 "/Game/Materials/MI_KeyBody_001.MI_KeyBody_001")
      (Rendering|Material|SetMaterial _staticmesh 1 "/Game/Materials/MI_KeyDeco_001.MI_KeyDeco_001")
      (Transformation|SetRelativeTransform _staticmesh (Math|Transform|MakeTransform (+ (.location _returnvalue) "") (Math|Rotator|CombineRotators (.rotation _returnvalue) "90.000000,0.000000,0.000000") "0.400000,0.400000,0.400000") false false)
      (Components|Sphere|SetSphereRadius (Variables|Default|GetHitPlayer) 4e+02 true))))