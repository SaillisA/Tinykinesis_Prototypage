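; Legacy telekinesis heavy object that the player levitates and slams down to damage melee NPCs and break apart.
; Grab disables physics and lifts it on a timeline; charging grows the damage sphere.
; Release fires downward and radial impulses, arming hits to trigger camera shake and the destruction component, and overlaps to deal max-HP damage.
; Tick cancels levitation when the player is hit, and otherwise restores physics and the untargeted material.
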(event OnComponentHit(Mesh)
  (params (HitComponent :type Primitive%20Component%20Object%20Reference) (OtherActor :type Actor%20Object%20Reference) (OtherComp :type Primitive%20Component%20Object%20Reference) (NormalImpulse :type Vector :default "0, 0, 0") (Hit :type Hit%20Result%20Structure%20%28by%20ref%29))
  ;[1 0.2696 0.3095] Collisions
  ;;[1 1 1] NPC chargent l'objet
  (Utilities|Casting|CastToBP_AICharacterBlank OtherActor))

(event OnComponentBeginOverlap(DamageRangeCollision)
  (params (OverlappedComponent :type Primitive%20Component%20Object%20Reference) (OtherActor :type Actor%20Object%20Reference) (OtherComp :type Primitive%20Component%20Object%20Reference) (OtherBodyIndex :type Integer) (bFromSweep :type Boolean) (SweepResult :type Hit%20Result%20Structure%20%28by%20ref%29))
  ;[1 0.2696 0.3095] Collisions
  ;;[1 1 1] Smash Kill NPC (Il faudrait checker le Got Hit à la place de tous ces nodes)
  (bind _asbp_aicharacter_blank (Utilities|Casting|CastToBP_AICharacterBlank OtherActor))
  (bind _asbp_aic_npc_melee (Utilities|Casting|CastToBP_AIC_NpcMelee (Components|GetOwner _asbp_aicharacter_blank)))
  (if (Variables|Default|GetGettingSmashed)
    (bind _isdead (Default|LooseHP (Variables|/Game/Blueprints/NPC/AIMelee/BP_AIC_NpcMelee.BP_AIC_NpcMelee_C|GetHealthManager _asbp_aic_npc_melee) (Variables|/Game/Blueprints/ActorComponents/BP_AC_Health.BP_AC_Health_C|GetmaxHP (Variables|/Game/Blueprints/NPC/AIMelee/BP_AIC_NpcMelee.BP_AIC_NpcMelee_C|GetHealthManager _asbp_aic_npc_melee))))
    (if _isdead
      _)))

(event EventBeginPlay
  (bind _damagerangecollision (Variables|Default|GetDamageRangeCollision))
  ;[0.298 1 0.5765] BeginPlay
  ;;[1 1 1] Quel intérêt quand on a déjà le Mesh ?
  (Variables|Default|SetUsableMesh (Actor|GetComponentbyClass "/Script/Engine.StaticMeshComponent"))
  (Components|Sphere|SetSphereRadius (Variables|Default|GetAimAssistCollision) (Variables|Default|GetRadiusAimAssist) true)
  (Components|Sphere|SetSphereRadius _damagerangecollision (Variables|Default|GetRadiusMinDamageRange) true)
  (Collision|SetCollisionResponsetoAllChannels _damagerangecollision "ECR_Ignore")
  ;;[0.3882 0.3804 1] Dans la classse parent
  (Variables|Default|SetBaseMaterial (Rendering|Material|GetMaterial (Variables|Default|GetMesh) 0)))

(event EventGrabObject
  (bind _usablemesh (Variables|Default|GetUsableMesh))
  (bind _usablemesh_2 (Variables|Default|GetUsableMesh))
  (bind _returnvalue (Transformation|GetWorldLocation _usablemesh))
  (bind (_x _y _z) (Math|Vector|BreakVector _returnvalue))
  ;[0.1041 0.6523 1] Grab
  (if (Variables|Default|GetCanBeGrabbed)
    (Utilities|FlowControl|DoOnce false
      (:Completed
        (Variables|Default|SetIsLevitating true)
        (Class|PrimitiveComponent|SetAllPhysicsLinearVelocity (Variables|Default|GetUsableMesh) "0, 0, 0" false)
        (Physics|SetSimulatePhysics _usablemesh_2 false)
        (Physics|SetEnableGravity _usablemesh_2 false)
        (Collision|SetCollisionResponsetoAllChannels (Variables|Default|GetMesh) "ECR_Ignore")
        (Collision|SetCollisionResponsetoAllChannels (Variables|Default|GetAimAssistCollision) "ECR_Ignore")
        (Default|Animation (CallFunction|GetTinykinesisPlayerCharacter) "NewEnumerator1")
        (bind _levitation (Timeline|Timeline PlayFromStart)
          (:Update
            (Transformation|SetWorldLocation (Variables|Default|GetUsableMesh) (Math|Vector|MakeVector _x _y (+ _levitation (+ _z 1e+01))) false false))
          (:Finished
            (if (Variables|Default|GetGettingSmashed)
              (CallFunction|ReleaseObject))))))))

(event EventCancelGrabObject
  (bind _usablemesh (Variables|Default|GetUsableMesh))
  (bind _usablemesh_2 (Variables|Default|GetUsableMesh))
  (bind _usablemesh_3 (Variables|Default|GetUsableMesh))
  (bind _damagerangecollision (Variables|Default|GetDamageRangeCollision))
  (bind _returnvalue (Transformation|GetWorldLocation _usablemesh_2))
  (bind (_x _y _z) (Math|Vector|BreakVector _returnvalue))
  ;[0.5208 0.814 1] Cancel Grab
  (Physics|SetSimulatePhysics _usablemesh true)
  (Physics|SetEnableGravity _usablemesh true)
  (Variables|Default|SetIsLevitating false)
  (Default|ClearParameters (Variables|/Game/Blueprints/Player/BP_TinykinesisPlayerController.BP_TinykinesisPlayerController_C|GetBP_AC_Telekinesis (CallFunction|GetTinykinesisPlayerController)))
  (Variables|Default|SetGettingSmashed false)
  (Variables|Default|SetCanBeGrabbed true)
  (Collision|SetCollisionResponsetoAllChannels (Variables|Default|GetMesh) "ECR_Block")
  (Collision|SetCollisionResponsetoAllChannels (Variables|Default|GetAimAssistCollision) "ECR_Block")
  (Default|SetIddleAnimation (Variables|/Game/Blueprints/Player/BP_TinykinesisPlayerController.BP_TinykinesisPlayerController_C|GetBP_AC_Telekinesis (CallFunction|GetTinykinesisPlayerController)))
  ;;[1 1 1] Garder dans le code Enfant
  (Components|Sphere|SetSphereRadius _damagerangecollision (Variables|Default|GetRadiusMinDamageRange) true)
  (Collision|SetCollisionResponsetoAllChannels _damagerangecollision "ECR_Ignore")
  ;[0.1041 0.6523 1] Grab
  (Utilities|FlowControl|DoOnce false) ; enters at Reset
)

(event EventReleaseObject
  ;[1 0.1667 0.6787] Release
  (if (Variables|Default|GetIsLevitating)
    (Physics|SetSimulatePhysics (Variables|Default|GetMesh) true)
    (Physics|SetEnableGravity (Variables|Default|GetMesh) true)
    (Physics|AddImpulse (Variables|Default|GetUsableMesh) "0.000000,0.000000,-2600.000000" "None" true)
    (Variables|Default|SetGettingSmashed true)
    (Class|RadialForceComponent|FireImpulse (Variables|Default|GetRadialForce))
    (Collision|SetCollisionResponsetoAllChannels (Variables|Default|GetMesh) "ECR_Block")
    (Collision|SetCollisionEnabled (Variables|Default|GetDamageRangeCollision) "QueryOnly")
    (Default|Animation (CallFunction|GetTinykinesisPlayerCharacter) "NewEnumerator2")
    ;[0.3251 0.199 1] Charge
    (Utilities|FlowControl|DoOnce false) ; enters at Reset
  ))

(event EventChargeObject
  ;[0.3251 0.199 1] Charge
  (Utilities|FlowControl|DoOnce false
    (:Completed
      (bind _size (Timeline|ChargingSmash PlayFromStart)
        (:Update
          (Components|Sphere|SetSphereRadius (Variables|Default|GetDamageRangeCollision) _size true))
        (:Finished
          (Camera|PlayWorldCameraShake "/Game/Blueprints/Actors/CameraManager/BP_AttractCompleteCameraShake.BP_AttractCompleteCameraShake_C" (Transformation|GetActorLocation (CallFunction|GetTinykinesisPlayerCharacter)) 0.0 5e+02))))))

(event Collision|EventHit
  (params (MyComp :type Primitive%20Component%20Object%20Reference) (Other :type Actor%20Object%20Reference) (OtherComp :type Primitive%20Component%20Object%20Reference) (bSelfMoved :type Boolean) (HitLocation :type Vector :default "0, 0, 0") (HitNormal :type Vector :default "0, 0, 0") (NormalImpulse :type Vector :default "0, 0, 0") (Hit :type Hit%20Result%20Structure%20%28by%20ref%29))
  ;[1 0.2696 0.3095] Collisions
  ;;[1 1 1] Hit Object
  (if (Variables|Default|GetGettingSmashed)
    (bind _asbp_tinykinesis_player_character (Utilities|Casting|CastToBP_TinykinesisPlayerCharacter (Game|GetPlayerCharacter 0)))
    ;;;[1 1 1] Garder dans le code enfant
    (Camera|PlayWorldCameraShake "/Game/Blueprints/Actors/CameraManager/BP_CameraShake.BP_CameraShake_C" (Transformation|GetActorLocation _asbp_tinykinesis_player_character) 0.0 5e+02)
    (Variables|Default|SetIsLevitating false)
    (Utilities|FlowControl|Delay 0.01)
    (Default|LaunchDestruction (Variables|Default|GetBP_AC_DestructionElement) (Transformation|GetRelativeTransform (Variables|Default|GetMesh)) self)))

(event EventTick
  (params (DeltaSeconds :type Float%20%28single-precision%29))
  ;[0.7412 1 0.3412] TICK. Reset le material & Cancel la lévitation si besoin -> pas opti de faire ça en Tick. Ce serait cool de trouver une alternative
  (if (Variables|Default|GetIsLevitating)
    (if (Variables|/Game/Blueprints/Player/BP_TinykinesisPlayerController.BP_TinykinesisPlayerController_C|GetGotHit (CallFunction|GetTinykinesisPlayerController))
      (CallFunction|CancelGrabObject))
    (else
      (Physics|SetEnableGravity (Variables|Default|GetUsableMesh) true)
      (Physics|SetSimulatePhysics (Variables|Default|GetUsableMesh) true)
      (if (not (== (Variables|/Game/Blueprints/ActorComponents/PlayerAbilities/BP_AC_Telekinesis.BP_AC_Telekinesis_C|GetLockedItem (Variables|/Game/Blueprints/Player/BP_TinykinesisPlayerController.BP_TinykinesisPlayerController_C|GetBP_AC_Telekinesis (CallFunction|GetTinykinesisPlayerController))) self))
        (Rendering|Material|SetMaterial (Variables|Default|GetMesh) 0 (Variables|Default|GetBaseMaterial))))))

(event EventDeleteFeedbacksDetectObject
  ;[1 0.8515 0] Feedback for Target
  ;;[1 1 1] Mis dans la classe parente
  (Rendering|Material|SetMaterial (Variables|Default|GetMesh) 0 (Variables|Default|GetBaseMaterial)))

(event EventFeedbacksDetectObject
  ;[1 0.8515 0] Feedback for Target
  ;;[1 1 1] Mis dans la classe parente
  (Rendering|Material|SetMaterial (Variables|Default|GetMesh) 0 "/Game/Materials/M_Translucent.M_Translucent"))

(fn ConstructionScript)

(fn DeathbyNPC
  (Actor|DestroyActor)
  (return))