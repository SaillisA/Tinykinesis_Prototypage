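; BP_ChargeTelekinesis is a camera modifier that, judging by its name, provides the telekinesis charge effect.
; It narrows the FOV from 90 to 85 while raising a post-process setting at full blend weight, leaving view location and rotation untouched.
; Both ramps use global game time modulo Duration, clamped at one second, so they repeat on the world clock rather than starting from activation.
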(fn BlueprintModifyPostProcess
  (params (DeltaTime :type Float%20%28single-precision%29))
  (return 1.0 (Utilities|Struct|MakePostProcessSettings (Math|Float|MapRangeClamped (Math|Float|%(Float) (Utilities|Time|GetGameTimeinSeconds) (Variables|Default|GetDuration)) 0.0 1.0 0.0 0.5))))

(fn BlueprintModifyCamera
  (params (DeltaTime :type Float%20%28single-precision%29) (ViewLocation :type Vector :default "0, 0, 0") (ViewRotation :type Rotator :default "0, 0, 0") (FOV :type Float%20%28single-precision%29))
  (return ViewLocation ViewRotation (Math|Float|MapRangeClamped (Math|Float|%(Float) (Utilities|Time|GetGameTimeinSeconds) (Variables|Default|GetDuration)) 0.0 1.0 9e+01 85.0)))