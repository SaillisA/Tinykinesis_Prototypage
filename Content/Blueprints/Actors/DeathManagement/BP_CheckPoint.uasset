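; Checkpoint actor that saves player and level progress the first time the player character overlaps its sphere.
; On that overlap, if a level manager exists, it sets the manager's spawn transform to its own, then synchronously saves data through the game instance, with player data saved first.
; A state gameplay-element component handles activation and begin-play; on load, a non-activated checkpoint is flagged as already saved.
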(event OnComponentBeginOverlap(Sphere)
  (params (OverlappedComponent :type Primitive%20Component%20Object%20Reference) (OtherActor :type Actor%20Object%20Reference) (OtherComp :type Primitive%20Component%20Object%20Reference) (OtherBodyIndex :type Integer) (bFromSweep :type Boolean) (SweepResult :type Hit%20Result%20Structure%20%28by%20ref%29))
  (if (not (Variables|Default|GetHasAlreadySave))
    (bind _returnvalue (Actor|GetActorOfClass "/Game/Blueprints/SaveSystem/BP_AbstractLevelManager.BP_AbstractLevelManager_C"))
    (Utilities|IsValid _returnvalue
      (:Is%20Valid
        (Utilities|Casting|CastToBP_TinykinesisPlayerCharacter OtherActor)
        (Variables|Default|SetHasAlreadySave true)
        (Development|PrintString "Checkpoint")
        (Utilities|FlowControl|Sequence
          (:then_0
            (Default|SavePlayerData (CallFunction|GetTinykinesisGameInstance) (Default|GetPlayerData (CallFunction|GetTinykinesisPlayerController)) false))
          (:then_1
            (bind _returnvalue_2 (Actor|GetActorOfClass "/Game/Blueprints/SaveSystem/BP_AbstractLevelManager.BP_AbstractLevelManager_C"))
            (Variables|/Game/Blueprints/SaveSystem/BP_AbstractLevelManager.BP_AbstractLevelManager_C|SetSpawnPlayerTransform _returnvalue_2 (Transformation|GetActorTransform))
            (Default|SaveLevelData (CallFunction|GetTinykinesisGameInstance) (Default|GetLevelData _returnvalue_2) false)))))))

(event Custom|BeginPlay_Checkpoint
  ;[0.298 1 0.5765] BeginPlay
)

(event Custom|LoadCheckpoint
  ;[0.298 1 0.5765] BeginPlay
  (Default|CallBeginPlayActiveElement (Variables|Default|GetBP_AC_StateGameplayElement))
  (if (not (Variables|/Game/Blueprints/ActorComponents/BP_AC_StateGameplayElement.BP_AC_StateGameplayElement_C|GetIsActivated (Variables|Default|GetBP_AC_StateGameplayElement)))
    (Variables|Default|SetHasAlreadySave true)))

(event EventBeginPlay
  (bind _bp_ac_stategameplayelement (Variables|Default|GetBP_AC_StateGameplayElement))
  ;[0.298 1 0.5765] BeginPlay
  (EventDispatchers|BindEventtoBeginPlayActiveElement _bp_ac_stategameplayelement (EventDispatchers|CreateEvent :!event Custom|BeginPlay_Checkpoint))
  (Default|LaunchBeginPlayifNoLevelManager _bp_ac_stategameplayelement))

(event Collision|EventActorBeginOverlap
  (params (OtherActor :type Actor%20Object%20Reference)))

(event EventTick
  (params (DeltaSeconds :type Float%20%28single-precision%29)))

(event EventSetActive
  (params (IsActive :type Boolean))
  (bind _bp_ac_stategameplayelement (Variables|Default|GetBP_AC_StateGameplayElement))
  ;[0.298 1 0.5765] BeginPlay
  (EventDispatchers|BindEventtoSetActiveElementEventDispatcher _bp_ac_stategameplayelement (EventDispatchers|CreateEvent :!event Custom|LoadCheckpoint))
  (EventDispatchers|BindEventtoBeginPlayActiveElement _bp_ac_stategameplayelement (EventDispatchers|CreateEvent :!event Custom|BeginPlay_Checkpoint))
  (Default|SetActiveElement _bp_ac_stategameplayelement IsActive))

(fn ConstructionScript)