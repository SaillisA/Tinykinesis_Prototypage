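; BP_LightObject_DistanceNpcBullets is a light-object child that acts, by its name, as the ranged NPC's bullet, setting its inherited damage value on BeginPlay.
; When the cube overlaps the Tinykinesis player, it prints a debug message, calls the player's bullet-hit event with the sweep location, then self-destroys after a short delay.
; A blocking hit destroys it immediately; the distance-NPC cast for other overlaps leads to no action.
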(event OnComponentBeginOverlap(Cube)
  (params (OverlappedComponent :type Primitive%20Component%20Object%20Reference) (OtherActor :type Actor%20Object%20Reference) (OtherComp :type Primitive%20Component%20Object%20Reference) (OtherBodyIndex :type Integer) (bFromSweep :type Boolean) (SweepResult :type Hit%20Result%20Structure%20%28by%20ref%29))
  (bind _asbp_first_person_character (Utilities|Casting|CastToBP_TinykinesisPlayerCharacter OtherActor)
    (:then
      (Development|PrintString "Youpi j'ai touché le joueur")
      (Default|EventGetHitbyBullets _asbp_first_person_character (.location SweepResult))
      (Utilities|FlowControl|Delay 0.2)
      (Actor|DestroyActor))
    (:CastFailed
      (Utilities|Casting|CastToBP_CharacterNpcDistance OtherActor))))

(event OnComponentHit(Cube)
  (params (HitComponent :type Primitive%20Component%20Object%20Reference) (OtherActor :type Actor%20Object%20Reference) (OtherComp :type Primitive%20Component%20Object%20Reference) (NormalImpulse :type Vector :default "0, 0, 0") (Hit :type Hit%20Result%20Structure%20%28by%20ref%29))
  (Actor|DestroyActor))

(event EventBeginPlay
  (|CallParentFunction)
  (Variables|Default|SetDammageLightObject 5e+01))

(event Collision|EventActorBeginOverlap
  (params (OtherActor :type Actor%20Object%20Reference)))

(event EventTick
  (params (DeltaSeconds :type Float%20%28single-precision%29)))

(fn ConstructionScript
  (|CallParentFunction))