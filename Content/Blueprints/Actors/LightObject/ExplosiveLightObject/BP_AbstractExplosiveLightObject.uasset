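; Abstract base for explosive light objects that affect AI characters within an explosion radius on impact.
; ImpactEffect sphere-traces at the Cube's location, passes each BP_AICharacterBlank hit to EffectOfEnnemy, spawns the impact FX, then calls ExplosionEffect.
; EffectOfEnnemy and ExplosionEffect are empty hooks, leaving the actual effects to child classes.
; The construction script sizes a preview sphere to ExplosionRadius, which BeginPlay destroys.
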(event EventBeginPlay
  (|CallParentFunction)
  (Components|DestroyComponent (Variables|Default|GetExplosionRadius_Visual)))

(event Collision|EventActorBeginOverlap
  (params (OtherActor :type Actor%20Object%20Reference)))

(event EventTick
  (params (DeltaSeconds :type Float%20%28single-precision%29)))

(fn ConstructionScript
  (|CallParentFunction)
  (Components|Sphere|SetSphereRadius (Variables|Default|GetExplosionRadius_Visual) (Variables|Default|GetExplosionRadius) false))

(fn EffectOfEnnemy
  (params (EnnemyHit :type BP%20AI%20Character%20Blank%20Object%20Reference) (HitLocation :type Vector)))

(fn ExplosionEffect)

(fn ImpactEffect
  (bind _cube (Variables|Default|GetCube))
  (bind _cube_2 (Variables|Default|GetCube))
  (bind _returnvalue (Transformation|GetWorldLocation _cube_2))
  (bind _returnvalue_2 (Transformation|GetWorldTransform _cube))
  (bind _outhits (Collision|MultiSphereTraceForObjects _returnvalue _returnvalue (Variables|Default|GetExplosionRadius) (Variables|Default|GetObject%20Types) false 0 "None"))
  (for _array_element _outhits
    (bind _asbp_aicharacter_blank (Utilities|Casting|CastToBP_AICharacterBlank (.HitActor (Collision|BreakHitResult _array_element))))
    (CallFunction|EffectOfEnnemy _asbp_aicharacter_blank (.Location (Collision|BreakHitResult _array_element))))
  (Niagara|SpawnSystematLocation (Variables|Default|GetFXatImpact) (.location _returnvalue_2) (.rotation _returnvalue_2) (.scale _returnvalue_2))
  (CallFunction|ExplosionEffect))