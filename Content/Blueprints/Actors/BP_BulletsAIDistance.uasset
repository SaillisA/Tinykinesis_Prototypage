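; Ranged-AI bullet that self-destructs after ten seconds and notifies the player on overlap; any overlap spawns its fractured version and destroys it.
; It also carries telekinesis throwable logic: Attract moves the mesh toward the player, and Propulse moves it to a locked target or launches it by impulse.
; Component hits pass damage and impact force to AI characters, and thrown bullets shatter.
; Smash and Levitate are empty, their logic disconnected.
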(event OnComponentHit(Cube)
  (params (HitComponent :type Primitive%20Component%20Object%20Reference) (OtherActor :type Actor%20Object%20Reference) (OtherComp :type Primitive%20Component%20Object%20Reference) (NormalImpulse :type Vector :default "0, 0, 0") (Hit :type Hit%20Result%20Structure%20%28by%20ref%29))
  ;[1 1 1] Hit NCP
  (bind _asbp_aicharacter_blank (Utilities|Casting|CastToBP_AICharacterBlank OtherActor))
  (Default|EventGetHit _asbp_aicharacter_blank 0 (Variables|Default|GetIsThrown) (Variables|Default|GetDammageLightObject) (Transformation|GetActorLocation (CallFunction|GetTinykinesisPlayerCharacter)) self (Variables|Default|GetForceImpact) (Variables|Default|GetForceImpulseZ)))

(event OnComponentBeginOverlap(Cube)
  (params (OverlappedComponent :type Primitive%20Component%20Object%20Reference) (OtherActor :type Actor%20Object%20Reference) (OtherComp :type Primitive%20Component%20Object%20Reference) (OtherBodyIndex :type Integer) (bFromSweep :type Boolean) (SweepResult :type Hit%20Result%20Structure%20%28by%20ref%29))
  ;[1 1 1] Hit Player
  (bind _asbp_tinykinesis_player_character (Utilities|Casting|CastToBP_TinykinesisPlayerCharacter OtherActor)
    (:then
      (Development|PrintString "Youpi j'ai touché le joueur")
      (Default|EventGetHitbyBullets _asbp_tinykinesis_player_character (Transformation|GetActorLocation))
      (Utilities|FlowControl|Delay 0.2)
      (Game|SpawnActorfromClass (Variables|Default|GetFracturedObject) (Transformation|GetRelativeTransform (Variables|Default|GetUsableMesh)) "Undefined" "MultiplyWithRoot" 0 0)
      (Actor|DestroyActor))
    (:CastFailed
      (Utilities|FlowControl|Delay 0.2)
      (Game|SpawnActorfromClass (Variables|Default|GetFracturedObject) (Transformation|GetRelativeTransform (Variables|Default|GetUsableMesh)) "Undefined" "MultiplyWithRoot" 0 0)
      ;[1 1 1] Propulse
      (Actor|DestroyActor))))

(event EventBeginPlay
  ;[1 1 1] Begin Play
  (Variables|Default|SetAttractSpeed 1.0)
  (Variables|Default|SetUsableMesh (Actor|GetComponentbyClass "/Script/Engine.StaticMeshComponent"))
  (Variables|Default|SetDammageLightObject 5e+01)
  (Utilities|FlowControl|Delay 1e+01)
  (Actor|DestroyActor))

(event EventSmash
  ;[1 0 0.0296] Poubelle
)

(event Collision|EventHit
  (params (MyComp :type Primitive%20Component%20Object%20Reference) (Other :type Actor%20Object%20Reference) (OtherComp :type Primitive%20Component%20Object%20Reference) (bSelfMoved :type Boolean) (HitLocation :type Vector :default "0, 0, 0") (HitNormal :type Vector :default "0, 0, 0") (NormalImpulse :type Vector :default "0, 0, 0") (Hit :type Hit%20Result%20Structure%20%28by%20ref%29))
  ;[1 1 1] Attract/Hit
  ;;[1 1 1] Hit
  (Utilities|FlowControl|Sequence
    (:then_0
      (if (Variables|Default|GetGettingSmashed)
        (Utilities|FlowControl|Delay 0.2)
        (Actor|DestroyActor)
        (Variables|Default|SetIsLevitating false)
        (Variables|Default|SetIsThrown false)))
    (:then_1
      (if (Variables|Default|GetIsThrown)
        (CallFunction|ImpactEffect)
        (Utilities|FlowControl|Delay 0.01)
        (Game|SpawnActorfromClass (Variables|Default|GetFracturedObject) (Transformation|GetRelativeTransform (Variables|Default|GetUsableMesh)) "Undefined" "MultiplyWithRoot" 0 0)
        (Actor|DestroyActor)
        (else
          ;;[1 1 1] Attract
          (Components|MoveComponentTo (Variables|Default|GetUsableMesh) (stale EventAttract Player%20Location%20R) "0, 0, 0" false false (* (Variables|Default|GetAttractSpeed) 0.1) false) ; enters at Stop
        )))))

(event EventAttract
  (params (Player%20Location%20R :type Vector :default "0, 0, 0") (Player%20Location%20Front :type Vector :default "0, 0, 0") (PlayerHit :type Boolean))
  ;[1 1 1] Attract/Hit
  ;;[1 1 1] Attract
  (if (and (Variables|Default|GetCanBeGrabbed) (not PlayerHit))
    (Variables|Default|SetIsThrown false)
    (Physics|SetSimulatePhysics (Variables|Default|GetUsableMesh) true)
    (if (not (Variables|Default|GetIsLevitating))
      (Variables|Default|SetCanBeThrown true)
      (Collision|SetCollisionResponsetoAllChannels (Variables|Default|GetUsableMesh) "ECR_Ignore")
      (Components|MoveComponentTo (Variables|Default|GetUsableMesh) Player%20Location%20R "0, 0, 0" false false (* (Variables|Default|GetAttractSpeed) 0.1) false))
    (else
      (Collision|SetCollisionResponsetoAllChannels (Variables|Default|GetUsableMesh) "ECR_Block")
      (Variables|Default|SetCanBeThrown false))))

(event EventPropulse
  (params (TargetLocation :type Vector :default "0, 0, 0") (PropulseLocation :type Vector :default "0, 0, 0") (TargetLocked? :type Boolean))
  (bind _usablemesh (Variables|Default|GetUsableMesh))
  ;[1 1 1] Propulse
  (Variables|Default|SetLocationBeforeThrown PropulseLocation)
  (if (Variables|Default|GetCanBeThrown)
    (if TargetLocked?
      (Collision|SetCollisionResponsetoAllChannels (Variables|Default|GetUsableMesh) "ECR_Block")
      (Variables|Default|SetIsThrown true)
      (Components|MoveComponentTo _usablemesh (+ TargetLocation 25.0) "0, 0, 0" false false 0.15 false)
      (Physics|SetEnableGravity (Variables|Default|GetUsableMesh) true)
      (Variables|Default|SetCanBeGrabbed false)
      (Variables|Default|SetCanBeThrown false)
      (else
        (Collision|SetCollisionResponsetoAllChannels (Variables|Default|GetUsableMesh) "ECR_Block")
        (Physics|SetPhysicsLinearVelocity _usablemesh "0, 0, 0" false "None")
        (Physics|AddImpulse (Variables|Default|GetUsableMesh) (* PropulseLocation 5500) "None" true)
        (Physics|SetEnableGravity (Variables|Default|GetUsableMesh) true)
        (Variables|Default|SetCanBeGrabbed false)
        (Variables|Default|SetCanBeThrown false)
        (Variables|Default|SetIsThrown true)))))

(event EventLevitate
  ;[1 0 0.0296] Poubelle
)

(event EventGrabObject
  ;[1 1 1] Grab Object
  (Variables|Default|SetCanBeThrown true))

(fn ConstructionScript)

(fn DeathbyNPC
  (Actor|DestroyActor)
  (return))

(fn ImpactEffect)