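; BP_SwitchLevel is a trigger volume that moves the Tinykinesis player to another level.
; On player overlap it disables input, shows the death black screen and has the level manager save the game with the new level's respawn transform.
; After a short delay it stops the exploration ambience audio and opens the target level.
; The player's velocity is stored, but the node that would reapply it is disconnected.
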(event OnComponentBeginOverlap(TriggerZone)
  (params (OverlappedComponent :type Primitive%20Component%20Object%20Reference) (OtherActor :type Actor%20Object%20Reference) (OtherComp :type Primitive%20Component%20Object%20Reference) (OtherBodyIndex :type Integer) (bFromSweep :type Boolean) (SweepResult :type Hit%20Result%20Structure%20%28by%20ref%29))
  (bind _tinykinesisplayercontroller (CallFunction|GetTinykinesisPlayerController))
  (bind _tinykinesisplayercharacter (CallFunction|GetTinykinesisPlayerCharacter))
  (if (== OtherActor _tinykinesisplayercharacter)
    (Variables|Default|SetCurrentPlayerVelocity (Transformation|GetVelocity _tinykinesisplayercharacter))
    (Input|DisableInput _tinykinesisplayercharacter _tinykinesisplayercontroller)
    (Default|DeathBlackScreen (Variables|/Game/Blueprints/Player/BP_TinykinesisPlayerController.BP_TinykinesisPlayerController_C|GetWBPBlackScreen _tinykinesisplayercontroller))
    (Utilities|FlowControl|Sequence
      (:then_0
        (bind _returnvalue (Actor|GetActorOfClass "/Game/Blueprints/SaveSystem/BP_AbstractLevelManager.BP_AbstractLevelManager_C"))
        (Utilities|IsValid _returnvalue
          (:Is%20Valid
            (Default|TriggerSaveGame _returnvalue (Variables|Default|GetNewLevelTransformRespawn)))))
      (:then_1
        (Utilities|FlowControl|Delay 1.0)
        (Class|FMODBlueprintStatics|EventInstanceStop (Variables|/Game/Blueprints/ActorComponents/PlayerAbilities/BP_AC_AmbianceMusic.BP_AC_AmbianceMusic_C|GetExplorationAudioInst (Variables|/Game/Blueprints/Player/BP_TinykinesisPlayerController.BP_TinykinesisPlayerController_C|GetBP_AC_AmbianceMusic (CallFunction|GetTinykinesisPlayerController))) false)
        (Game|OpenLevel(byObjectReference) (Variables|Default|GetLevelName))))))

(event EventBeginPlay)

(event Collision|EventActorBeginOverlap
  (params (OtherActor :type Actor%20Object%20Reference)))

(event EventTick
  (params (DeltaSeconds :type Float%20%28single-precision%29)))

(fn ConstructionScript)