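; Game instance for Tinykinesis that owns the save game object and handles the player's respawn transform.
; On Init it loads the save from its named slot, or creates a fresh save object if none exists.
; Helper functions copy RespawnTransform between the player controller and the in-memory save data, without writing to disk.
; ClearSaveData deletes the slot but leaves the loaded object untouched.
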(event EventInit
  (bind _returnvalue (SaveGame|DoesSaveGameExist (Variables|Default|GetSaveSlotName)))
  (if _returnvalue
    (bind _returnvalue_2 (SaveGame|LoadGamefromSlot (Variables|Default|GetSaveSlotName)))
    (bind _asbp_save_game_tinykinesis (Utilities|Casting|CastToBP_SaveGameTinykinesis _returnvalue_2))
    (Variables|Default|SetSaveGameData _asbp_save_game_tinykinesis)
    (else
      (bind _returnvalue_3 (SaveGame|CreateSaveGameObject "/Game/Blueprints/SaveSystem/BP_SaveGameTinykinesis.BP_SaveGameTinykinesis_C"))
      (Variables|Default|SetSaveGameData _returnvalue_3))))

(fn SavePlayerData
  (bind _output_get (LocalVariables|SetPlayerRef (CallFunction|GetTinykinesisPlayerController)))
  (Variables|/Game/Blueprints/SaveSystem/BP_SaveGameTinykinesis.BP_SaveGameTinykinesis_C|SetRespawnTransform (Variables|Default|GetSaveGameData) (Variables|/Game/Blueprints/Player/BP_TinykinesisPlayerController.BP_TinykinesisPlayerController_C|GetRespawnTransform _output_get)))

(fn GetPlayerData
  (bind _output_get (LocalVariables|SetPlayerRef (CallFunction|GetTinykinesisPlayerController)))
  (Variables|/Game/Blueprints/Player/BP_TinykinesisPlayerController.BP_TinykinesisPlayerController_C|SetRespawnTransform _output_get (Variables|/Game/Blueprints/SaveSystem/BP_SaveGameTinykinesis.BP_SaveGameTinykinesis_C|GetRespawnTransform (Variables|Default|GetSaveGameData))))

(fn ClearSaveData
  (SaveGame|DeleteGameinSlot (Variables|Default|GetSaveSlotName)))