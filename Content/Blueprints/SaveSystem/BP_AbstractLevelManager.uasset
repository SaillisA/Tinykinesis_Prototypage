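; Base level manager that saves and restores a level's gameplay element active states and player spawn transform.
; On BeginPlay in BuildMod, it loads the level's save from the game instance or writes a fresh one, then messages each element its state.
; Element states are saved by map key index rather than actor reference.
; TriggerSaveGame updates respawn transforms and synchronously saves player and level data.
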(event EventBeginPlay
  (if (Variables|/Game/Blueprints/Player/BP_TinykinesisPlayerController.BP_TinykinesisPlayerController_C|GetBuildMod (CallFunction|GetTinykinesisPlayerController))
    (Utilities|IsValid (Variables|/Game/Blueprints/SaveSystem/BP_GameInstanceTinykinesis.BP_GameInstanceTinykinesis_C|GetSavedGameData (CallFunction|GetTinykinesisGameInstance))
      (:Is%20Valid
        (Variables|Default|SetCurrentGameplayElements (Variables|Default|GetInitialGameplayElements))
        (bind (_saveexist _levelsavecopy) (Default|GetSaveLevel (CallFunction|GetTinykinesisGameInstance) (Variables|Default|GetNameLevel)))
        (if (and _saveexist (not (Variables|Default|GetAlwaysClearDataWhenLaunching)))
          (CallFunction|LoadLevelData _levelsavecopy)
          (else
            (Variables|Default|SetAlwaysClearDataWhenLaunching false)
            (Default|SaveLevelData (CallFunction|GetTinykinesisGameInstance) (CallFunction|GetLevelData) false)))
        (CallFunction|SetActiveAllGameplayElements)
        (Utilities|FlowControl|Delay 1.0)
        (Variables|Default|SetHasLaunchedLevel true)))))

(event Collision|EventActorBeginOverlap
  (params (OtherActor :type Actor%20Object%20Reference)))

(event EventTick
  (params (DeltaSeconds :type Float%20%28single-precision%29)))

(fn ConstructionScript)

(fn GetLevelData
  (bind _currentgameplayelements (Variables|Default|GetCurrentGameplayElements))
  (bind _keys (Utilities|Map|Keys _currentgameplayelements))
  (for (_array_element _array_index) _keys
    (if (.ReturnValue (Utilities|Map|Find _currentgameplayelements _array_element))
      (Utilities|Map|Add (LocalVariables|GetLevelDataCurrentGameplayElementIndexes) _array_index (.Value (Utilities|Map|Find _currentgameplayelements _array_element)))))
  (return (Utilities|Struct|MakeSLevel_Data (Variables|Default|GetNameLevel) (LocalVariables|GetLevelDataCurrentGameplayElementIndexes) (Variables|Default|GetSpawnPlayerTransform))))

(fn LoadLevelData
  (params (LevelSave :type S%20Level%20Data%20Structure))
  (bind _currentgameplayelements (Variables|Default|GetCurrentGameplayElements))
  (Utilities|FlowControl|Sequence
    (:then_0
      (bind _keys (Utilities|Map|Keys _currentgameplayelements))
      (for (_array_element _array_index) _keys
        (if (.ReturnValue (Utilities|Map|Find (.currentgameplayelements LevelSave) _array_index))
          (Utilities|Map|Add _currentgameplayelements _array_element (.Value (Utilities|Map|Find (.currentgameplayelements LevelSave) _array_index)))
          (Development|PrintString (Utilities|String|ToString(Boolean) (.Value (Utilities|Map|Find (.currentgameplayelements LevelSave) _array_index)))))))
    (:then_1
      (bind _output_get (Variables|Default|SetSpawnPlayerTransform (.spawnplayertransform LevelSave)))
      (if (not (== _output_get (Math|Transform|MakeTransform "0, 0, 0")))
        (Transformation|SetActorTransform (CallFunction|GetTinykinesisPlayerCharacter) _output_get)))))

(fn SetBoolActive
  (params (Actor :type Actor%20Object%20Reference))
  (Utilities|Map|Add (Variables|Default|GetCurrentGameplayElements) Actor false))

(fn SetActiveAllGameplayElements
  (bind _keys (Utilities|Map|Keys (Variables|Default|GetCurrentGameplayElements)))
  (for _array_element _keys
    (if (.ReturnValue (Utilities|Map|Find (Variables|Default|GetCurrentGameplayElements) _array_element))
      (Class|BPIGameplayElement|SetActive(Message) _array_element (.Value (Utilities|Map|Find (Variables|Default|GetCurrentGameplayElements) _array_element))))))

(fn TriggerSaveGame
  (params (TransformRespawn :type Transform))
  (bind (_location _rotation) (Math|Transform|BreakTransform TransformRespawn))
  (Variables|/Game/Blueprints/Player/BP_TinykinesisPlayerController.BP_TinykinesisPlayerController_C|SetFall_RespawnTransform (CallFunction|GetTinykinesisPlayerController) (Math|Transform|MakeTransform _location _rotation "1.000000,1.000000,1.000000"))
  (Utilities|FlowControl|Sequence
    (:then_0
      (Default|SavePlayerData (CallFunction|GetTinykinesisGameInstance) (Default|GetPlayerData (CallFunction|GetTinykinesisPlayerController)) false))
    (:then_1
      (bind _returnvalue (Actor|GetActorOfClass "BP_AbstractLevelManager_C"))
      (Variables|BP_AbstractLevelManager_C|SetSpawnPlayerTransform _returnvalue TransformRespawn)
      (Default|SaveLevelData (CallFunction|GetTinykinesisGameInstance) (CallFunction|GetLevelData _returnvalue) false))))